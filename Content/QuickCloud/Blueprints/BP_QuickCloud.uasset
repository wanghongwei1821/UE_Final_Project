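; BP_QuickCloud is a volumetric cloud actor that renders a Sparse Volume Texture through a dynamic instance of M_QuicklyCloud.
; One shared function runs from the Construction Script on QuickCloudConstruction and from BeginPlay on QuickCloudRender.
; It pushes scattering, density, extinction, self-shadow and optional sun/sky light-mixing settings into the material.
; It also issues console commands for path tracer support, Lumen indirect lighting and visible distance, so those settings are global.
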(event EventBeginPlay
  (BasicFunctions|ScriptFunction false))

(event Collision|EventActorBeginOverlap
  (params (OtherActor :type Actor%20Object%20Reference)))

(event EventTick
  (params (DeltaSeconds :type Float%20%28single-precision%29)))

(fn ConstructionScript
  (BasicFunctions|ScriptFunction true))

(fn ScriptFunction
  (params (Is_Construction :type Boolean))
  (bind _cvar_lumen_indirectlighting_support (Variables|GlobalCvar|GetCvar_Lumen_IndirectLighting_Support))
  (bind _cvar_path_tracer_support (Variables|GlobalCvar|GetCvar_Path_Tracer_Support))
  (Utilities|FlowControl|Sequence
    (:then_0
      (if Is_Construction
        (bind _returnvalue (Rendering|Material|CreateDynamicMaterialInstance (Variables|Default|GetQuickCloud_Construction) 0 "/Game/QuickCloud/Materials/M_QuicklyCloud.M_QuicklyCloud" "None" :!class /Script/Engine.PrimitiveComponent))
        (Variables|GlobalBasicSettings|SetVDB_Clouds_Material_Instance _returnvalue)
        (else
          (bind _returnvalue_2 (Rendering|Material|CreateDynamicMaterialInstance (Variables|Default|GetQuickCloud_Render) 0 "/Game/QuickCloud/Materials/M_QuicklyCloud.M_QuicklyCloud" "None" :!class /Script/Engine.PrimitiveComponent))
          (Variables|GlobalBasicSettings|SetVDB_Clouds_Material_Instance _returnvalue_2))))
    (:then_1
      (Class|MaterialInstanceDynamic|SetSparseVolumeTextureParameterValue (Variables|GlobalBasicSettings|GetVDB_Clouds_Material_Instance) "Input SVT" (Variables|BasicControls|GetSparse_Volume_Texture))
      (Rendering|Material|SetVectorParameterValue (Variables|GlobalBasicSettings|GetVDB_Clouds_Material_Instance) "Scattering Color" (Variables|BasicControls|GetScattering_Color) :!class /Script/Engine.MaterialInstanceDynamic)
      (Rendering|Material|SetScalarParameterValue (Variables|GlobalBasicSettings|GetVDB_Clouds_Material_Instance) "Scattering Intensity" (Variables|BasicControls|GetScattering_Intensity) :!class /Script/Engine.MaterialInstanceDynamic)
      (Rendering|Material|SetScalarParameterValue (Variables|GlobalBasicSettings|GetVDB_Clouds_Material_Instance) "Density" (Variables|BasicControls|GetDensity) :!class /Script/Engine.MaterialInstanceDynamic)
      (Rendering|Material|SetScalarParameterValue (Variables|GlobalBasicSettings|GetVDB_Clouds_Material_Instance) "Thick" (/ (Variables|BasicControls|GetExtinction) 1e+01) :!class /Script/Engine.MaterialInstanceDynamic))
    (:then_2
      (if (Variables|AmbientLightMixing|GetUse_Ambient_Light_Mixing)
        (Rendering|Material|SetScalarParameterValue (Variables|GlobalBasicSettings|GetVDB_Clouds_Material_Instance) "Sun Intensity" (/ (Variables|AmbientLightMixing|GetLight_Intensity_Multiplier) 1e+01) :!class /Script/Engine.MaterialInstanceDynamic)
        (Rendering|Material|SetScalarParameterValue (Variables|GlobalBasicSettings|GetVDB_Clouds_Material_Instance) "Sun Contribution" (Variables|AmbientLightMixing|GetLight_Color_Saturation) :!class /Script/Engine.MaterialInstanceDynamic)
        (Rendering|Material|SetVectorParameterValue (Variables|GlobalBasicSettings|GetVDB_Clouds_Material_Instance) "Sun Color" (Variables|AmbientLightMixing|GetLight_Color_Multiplier) :!class /Script/Engine.MaterialInstanceDynamic)
        (Rendering|Material|SetScalarParameterValue (Variables|GlobalBasicSettings|GetVDB_Clouds_Material_Instance) "sky Light Leaking" (Variables|AmbientLightMixing|GetSky_Light_Leaking) :!class /Script/Engine.MaterialInstanceDynamic)
        (Rendering|Material|SetVectorParameterValue (Variables|GlobalBasicSettings|GetVDB_Clouds_Material_Instance) "Sky Light Color" (Variables|AmbientLightMixing|GetSky_Light_Color_Multiplier) :!class /Script/Engine.MaterialInstanceDynamic)
        (Rendering|Material|SetScalarParameterValue (Variables|GlobalBasicSettings|GetVDB_Clouds_Material_Instance) "Sky Light Saturation" (Variables|AmbientLightMixing|GetSky_Light_Saturation) :!class /Script/Engine.MaterialInstanceDynamic)))
    (:then_3
      (Rendering|Material|SetVectorParameterValue (Variables|GlobalBasicSettings|GetVDB_Clouds_Material_Instance) "Self Shadow Color" (Variables|BasicControls|GetDetail_Shadow_Color) :!class /Script/Engine.MaterialInstanceDynamic)
      (Rendering|Material|SetScalarParameterValue (Variables|GlobalBasicSettings|GetVDB_Clouds_Material_Instance) "Self Shadow Intensity" (Variables|BasicControls|GetDetail_Shadow) :!class /Script/Engine.MaterialInstanceDynamic))
    (:then_4
      (if (Variables|GlobalRenderingSettings|GetPath_Tracer_Support)
        (bind _return_value (BasicFunctions|CvarAppend _cvar_path_tracer_support "1"))
        (Development|ExecuteConsoleCommand _return_value 0)
        (else
          (bind _return_value_2 (BasicFunctions|CvarAppend _cvar_path_tracer_support "0"))
          (Development|ExecuteConsoleCommand _return_value_2 0))))
    (:then_5
      (if (Variables|GlobalRenderingSettings|GetLumen_IndirectLighting_Support)
        (bind _return_value_3 (BasicFunctions|CvarAppend _cvar_lumen_indirectlighting_support "1"))
        (Development|ExecuteConsoleCommand _return_value_3 0)
        (else
          (bind _return_value_4 (BasicFunctions|CvarAppend _cvar_lumen_indirectlighting_support "0"))
          (Development|ExecuteConsoleCommand _return_value_4 0))))
    (:then_6
      (bind _return_value_5 (BasicFunctions|CvarAppend (Variables|GlobalCvar|GetCvar_Visible_Distance) (Utilities|String|ToString(Float) (Variables|GlobalRenderingSettings|GetVisible_Distance))))
      (Development|ExecuteConsoleCommand _return_value_5 0))))

(fn CvarAppend
  (params (Cvar%20Body :type String) (Cvar%20Value :type String))
  (return (Utilities|String|Append Cvar%20Body " " Cvar%20Value)))