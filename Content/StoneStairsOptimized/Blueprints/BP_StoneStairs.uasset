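; Stone stairs actor that procedurally assembles its stones in the Construction Script from transforms stored in a data table.
; Each row passes a despawner filter, then its ID and the undamaged/extra stone options route it to lazily created hierarchical instanced mesh components.
; A seeded stream randomizes rotation and single-axis displacement, with preset flips and an optional editor-previewed box modulating displacement.
; An optional invisible mesh adds extra collision.
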(fn ConstructionScript
  (bind _extrastones (Variables|Default|GetExtraStones))
  (bind _undamaged_stones (Variables|Default|GetUndamaged%20Stones))
  (bind _extrastones_2 (Variables|Default|GetExtraStones))
  (bind _undamaged_stones_2 (Variables|Default|GetUndamaged%20Stones))
  (bind _displacement_randomize (Variables|Default|GetDisplacement%20Randomize))
  (bind _displacement_randomize_2 (Variables|Default|GetDisplacement%20Randomize))
  (bind _boxcontrolleddisplacement (Variables|Default|GetBoxControlledDisplacement))
  (bind _reorientstones (Variables|Default|GetReorientStones))
  (bind _extrastones_3 (Variables|Default|GetExtraStones))
  (bind _undamaged_stones_3 (Variables|Default|GetUndamaged%20Stones))
  (bind _defaultsceneroot (Variables|Default|GetDefaultSceneRoot))
  (bind _object_dat (Variables|Default|GetObject%20DAT))
  (bind _displacement (Variables|Default|GetDisplacement))
  (bind _returnvalue (Transformation|GetWorldRotation _defaultsceneroot))
  (bind _returnvalue_2 (* _displacement -1.0))
  (bind _returnvalue_3 (Math|Random|RandomFloatinRangefromStream _returnvalue_2 _displacement _displacement_randomize_2))
  (Development|SetHiddeninGame (Variables|Default|GetThumbFix) false false)
  (if (Variables|Default|GetExtraCollision)
    (bind _returnvalue_4 (AddComponent|AddStaticMeshComponent false))
    (Components|StaticMesh|SetStaticMesh _returnvalue_4 (Variables|Default|GetExtraCollisionMesh))
    (Rendering|SetVisibility _returnvalue_4 false false))
  (Rendering|Debug|FlushPersistentDebugLines)
  (if (Variables|Default|GetBoxControlledDisplacement)
    (Utilities|IsValid (Game|GetGameState)
      (:Is%20Not%20Valid
        (Rendering|Debug|DrawDebugBox (Math|Transform|TransformLocation (Math|Transform|MakeTransform (Transformation|GetWorldLocation _defaultsceneroot) _returnvalue) (Variables|Default|GetBox%20Origin%20[XYZ])) (Variables|Default|GetBox%20Extent%20[XYZ]) "(R=1.000000,G=0.000000,B=0.000000,A=1.000000)" (Math|Rotator|CombineRotators (Variables|Default|GetBox%20Rotation%20[XYZ]) _returnvalue) 3.0 3.0))))
  (Variables|Default|SetScale (Variables|Default|GetScale))
  (Utilities|FlowControl|Sequence
    (:then_0
      (if (== _reorientstones 0)
        (Variables|Default|SetShuffle "0, 0, 0")
        (elif (== _reorientstones 1)
          (Variables|Default|SetShuffle "0, 0,180.000000")
          (elif (== _reorientstones 2)
            (Variables|Default|SetShuffle "0,180.000000,0.000000")
            (elif (== _reorientstones 3)
              (Variables|Default|SetShuffle "180.000000,0.000000,0.000000")
              (elif (== _reorientstones 4)
                (Variables|Default|SetShuffle "180.000000,0.000000,180.000000")
                (elif (== _reorientstones 5)
                  (Variables|Default|SetShuffle "180.000000,180.000000,0.000000")
                  (elif (== _reorientstones 6)
                    (Variables|Default|SetShuffle "0.000000,180.000000,180.000000")
                    (elif (== _reorientstones 7)
                      (Variables|Default|SetShuffle "180.000000,180.000000,180.000000"))))))))))
    (:then_1
      (bind _outrownames (DataTable|GetDataTableRowNames _object_dat))
      (for _array_element _outrownames
        (bind _returnvalue_5 (Utilities|GetDataTableRow _object_dat _array_element)
          (:then
            (|DespawnerGraph (Math|Vector|MakeVector (.T_X (Utilities|Struct|BreakF_CSVdata _returnvalue_5)) (.T_Y (Utilities|Struct|BreakF_CSVdata _returnvalue_5)) (.T_Z (Utilities|Struct|BreakF_CSVdata _returnvalue_5)))
              (:Output
                (switch int (.ID (Utilities|Struct|BreakF_CSVdata _returnvalue_5))
                  (:1
                    (Utilities|FlowControl|Sequence :!label _label
                      (:then_0
                        (Utilities|FlowControl|DoOnce false
                          (:Completed
                            (bind _returnvalue_6 (AddComponent|AddHierarchicalInstancedStaticMeshComponent false))
                            (bind _output_get (Variables|Default|Set01 _returnvalue_6))
                            (Rendering|Material|SetMaterial _output_get 0 (Variables|Default|GetStone%20Material)))))
                      (:then_1
                        (Components|InstancedStaticMesh|AddInstance (Variables|Default|Get01) (Math|Transform|MakeTransform (Math|Transform|TransformLocation (Math|Transform|MakeTransform (Math|Vector|MakeVector (.T_X (Utilities|Struct|BreakF_CSVdata _returnvalue_5)) (.T_Y (Utilities|Struct|BreakF_CSVdata _returnvalue_5)) (.T_Z (Utilities|Struct|BreakF_CSVdata _returnvalue_5))) (Math|Rotator|Lerp(Rotator) (Math|Rotator|CombineRotators (Math|Rotator|MakeRotator (.X (Math|Vector|BreakVector (+ (Math|Vector|MakeVector (Math|Random|RandomFloatinRangefromStream (* (.X (Math|Vector|BreakVector (* (Variables|Default|GetRandom%20Rotation%20[XYZ]) (Math|Conversions|ToFloat(Boolean) (!= (- (Math|Conversions|ToInteger(Boolean) (Variables|Default|GetRotation%20clamped%20to%20Displacement)) 1) (.AXIS (Utilities|Struct|BreakF_CSVdata _returnvalue_5))))))) -1.0) (.X (Math|Vector|BreakVector (* (Variables|Default|GetRandom%20Rotation%20[XYZ]) (Math|Conversions|ToFloat(Boolean) (!= (- (Math|Conversions|ToInteger(Boolean) (Variables|Default|GetRotation%20clamped%20to%20Displacement)) 1) (.AXIS (Utilities|Struct|BreakF_CSVdata _returnvalue_5))))))) _displacement_randomize) (Math|Random|RandomFloatinRangefromStream (* (.Y (Math|Vector|BreakVector (* (Variables|Default|GetRandom%20Rotation%20[XYZ]) (Math|Conversions|ToFloat(Boolean) (!= (- (Math|Conversions|ToInteger(Boolean) (Variables|Default|GetRotation%20clamped%20to%20Displacement)) 1) (.AXIS (Utilities|Struct|BreakF_CSVdata _returnvalue_5))))))) -1.0) (.Y (Math|Vector|BreakVector (* (Variables|Default|GetRandom%20Rotation%20[XYZ]) (Math|Conversions|ToFloat(Boolean) (!= (- (Math|Conversions|ToInteger(Boolean) (Variables|Default|GetRotation%20clamped%20to%20Displacement)) 1) (.AXIS (Utilities|Struct|BreakF_CSVdata _returnvalue_5))))))) _displacement_randomize) (Math|Random|RandomFloatinRangefromStream (* (.Z (Math|Vector|BreakVector (* (Variables|Default|GetRandom%20Rotation%20[XYZ]) (Math|Conversions|ToFloat(Boolean) (!= (- (Math|Conversions|ToInteger(Boolean) (Variables|Default|GetRotation%20clamped%20to%20Displacement)) 1) (.AXIS (Utilities|Struct|BreakF_CSVdata _returnvalue_5))))))) -1.0) (.Z (Math|Vector|BreakVector (* (Variables|Default|GetRandom%20Rotation%20[XYZ]) (Math|Conversions|ToFloat(Boolean) (!= (- (Math|Conversions|ToInteger(Boolean) (Variables|Default|GetRotation%20clamped%20to%20Displacement)) 1) (.AXIS (Utilities|Struct|BreakF_CSVdata _returnvalue_5))))))) _displacement_randomize)) (Variables|Default|GetShuffle)))) (.Y (Math|Vector|BreakVector (+ (Math|Vector|MakeVector (Math|Random|RandomFloatinRangefromStream (* (.X (Math|Vector|BreakVector (* (Variables|Default|GetRandom%20Rotation%20[XYZ]) (Math|Conversions|ToFloat(Boolean) (!= (- (Math|Conversions|ToInteger(Boolean) (Variables|Default|GetRotation%20clamped%20to%20Displacement)) 1) (.AXIS (Utilities|Struct|BreakF_CSVdata _returnvalue_5))))))) -1.0) (.X (Math|Vector|BreakVector (* (Variables|Default|GetRandom%20Rotation%20[XYZ]) (Math|Conversions|ToFloat(Boolean) (!= (- (Math|Conversions|ToInteger(Boolean) (Variables|Default|GetRotation%20clamped%20to%20Displacement)) 1) (.AXIS (Utilities|Struct|BreakF_CSVdata _returnvalue_5))))))) _displacement_randomize) (Math|Random|RandomFloatinRangefromStream (* (.Y (Math|Vector|BreakVector (* (Variables|Default|GetRandom%20Rotation%20[XYZ]) (Math|Conversions|ToFloat(Boolean) (!= (- (Math|Conversions|ToInteger(Boolean) (Variables|Default|GetRotation%20clamped%20to%20Displacement)) 1) (.AXIS (Utilities|Struct|BreakF_CSVdata _returnvalue_5))))))) -1.0) (.Y (Math|Vector|BreakVector (* (Variables|Default|GetRandom%20Rotation%20[XYZ]) (Math|Conversions|ToFloat(Boolean) (!= (- (Math|Conversions|ToInteger(Boolean) (Variables|Default|GetRotation%20clamped%20to%20Displacement)) 1) (.AXIS (Utilities|Struct|BreakF_CSVdata _returnvalue_5))))))) _displacement_randomize) (Math|Random|RandomFloatinRangefromStream (* (.Z (Math|Vector|BreakVector (* (Variables|Default|GetRandom%20Rotation%20[XYZ]) (Math|Conversions|ToFloat(Boolean) (!= (- (Math|Conversions|ToInteger(Boolean) (Variables|Default|GetRotation%20clamped%20to%20Displacement)) 1) (.AXIS (Utilities|Struct|BreakF_CSVdata _returnvalue_5))))))) -1.0) (.Z (Math|Vector|BreakVector (* (Variables|Default|GetRandom%20Rotation%20[XYZ]) (Math|Conversions|ToFloat(Boolean) (!= (- (Math|Conversions|ToInteger(Boolean) (Variables|Default|GetRotation%20clamped%20to%20Displacement)) 1) (.AXIS (Utilities|Struct|BreakF_CSVdata _returnvalue_5))))))) _displacement_randomize)) (Variables|Default|GetShuffle)))) (.Z (Math|Vector|BreakVector (+ (Math|Vector|MakeVector (Math|Random|RandomFloatinRangefromStream (* (.X (Math|Vector|BreakVector (* (Variables|Default|GetRandom%20Rotation%20[XYZ]) (Math|Conversions|ToFloat(Boolean) (!= (- (Math|Conversions|ToInteger(Boolean) (Variables|Default|GetRotation%20clamped%20to%20Displacement)) 1) (.AXIS (Utilities|Struct|BreakF_CSVdata _returnvalue_5))))))) -1.0) (.X (Math|Vector|BreakVector (* (Variables|Default|GetRandom%20Rotation%20[XYZ]) (Math|Conversions|ToFloat(Boolean) (!= (- (Math|Conversions|ToInteger(Boolean) (Variables|Default|GetRotation%20clamped%20to%20Displacement)) 1) (.AXIS (Utilities|Struct|BreakF_CSVdata _returnvalue_5))))))) _displacement_randomize) (Math|Random|RandomFloatinRangefromStream (* (.Y (Math|Vector|BreakVector (* (Variables|Default|GetRandom%20Rotation%20[XYZ]) (Math|Conversions|ToFloat(Boolean) (!= (- (Math|Conversions|ToInteger(Boolean) (Variables|Default|GetRotation%20clamped%20to%20Displacement)) 1) (.AXIS (Utilities|Struct|BreakF_CSVdata _returnvalue_5))))))) -1.0) (.Y (Math|Vector|BreakVector (* (Variables|Default|GetRandom%20Rotation%20[XYZ]) (Math|Conversions|ToFloat(Boolean) (!= (- (Math|Conversions|ToInteger(Boolean) (Variables|Default|GetRotation%20clamped%20to%20Displacement)) 1) (.AXIS (Utilities|Struct|BreakF_CSVdata _returnvalue_5))))))) _displacement_randomize) (Math|Random|RandomFloatinRangefromStream (* (.Z (Math|Vector|BreakVector (* (Variables|Default|GetRandom%20Rotation%20[XYZ]) (Math|Conversions|ToFloat(Boolean) (!= (- (Math|Conversions|ToInteger(Boolean) (Variables|Default|GetRotation%20clamped%20to%20Displacement)) 1) (.AXIS (Utilities|Struct|BreakF_CSVdata _returnvalue_5))))))) -1.0) (.Z (Math|Vector|BreakVector (* (Variables|Default|GetRandom%20Rotation%20[XYZ]) (Math|Conversions|ToFloat(Boolean) (!= (- (Math|Conversions|ToInteger(Boolean) (Variables|Default|GetRotation%20clamped%20to%20Displacement)) 1) (.AXIS (Utilities|Struct|BreakF_CSVdata _returnvalue_5))))))) _displacement_randomize)) (Variables|Default|GetShuffle))))) (Math|Rotator|MakeRotator (.R_X (Utilities|Struct|BreakF_CSVdata _returnvalue_5)) (.R_Y (Utilities|Struct|BreakF_CSVdata _returnvalue_5)) (.R_Z (Utilities|Struct|BreakF_CSVdata _returnvalue_5)))) (Math|Rotator|MakeRotator (.X (Math|Vector|BreakVector (+ (+ (Math|Vector|MakeVector (Math|Random|RandomFloatinRangefromStream (* (.X (Math|Vector|BreakVector (* (Variables|Default|GetRandom%20Rotation%20[XYZ]) (Math|Conversions|ToFloat(Boolean) (!= (- (Math|Conversions|ToInteger(Boolean) (Variables|Default|GetRotation%20clamped%20to%20Displacement)) 1) (.AXIS (Utilities|Struct|BreakF_CSVdata _returnvalue_5))))))) -1.0) (.X (Math|Vector|BreakVector (* (Variables|Default|GetRandom%20Rotation%20[XYZ]) (Math|Conversions|ToFloat(Boolean) (!= (- (Math|Conversions|ToInteger(Boolean) (Variables|Default|GetRotation%20clamped%20to%20Displacement)) 1) (.AXIS (Utilities|Struct|BreakF_CSVdata _returnvalue_5))))))) _displacement_randomize) (Math|Random|RandomFloatinRangefromStream (* (.Y (Math|Vector|BreakVector (* (Variables|Default|GetRandom%20Rotation%20[XYZ]) (Math|Conversions|ToFloat(Boolean) (!= (- (Math|Conversions|ToInteger(Boolean) (Variables|Default|GetRotation%20clamped%20to%20Displacement)) 1) (.AXIS (Utilities|Struct|BreakF_CSVdata _returnvalue_5))))))) -1.0) (.Y (Math|Vector|BreakVector (* (Variables|Default|GetRandom%20Rotation%20[XYZ]) (Math|Conversions|ToFloat(Boolean) (!= (- (Math|Conversions|ToInteger(Boolean) (Variables|Default|GetRotation%20clamped%20to%20Displacement)) 1) (.AXIS (Utilities|Struct|BreakF_CSVdata _returnvalue_5))))))) _displacement_randomize) (Math|Random|RandomFloatinRangefromStream (* (.Z (Math|Vector|BreakVector (* (Variables|Default|GetRandom%20Rotation%20[XYZ]) (Math|Conversions|ToFloat(Boolean) (!= (- (Math|Conversions|ToInteger(Boolean) (Variables|Default|GetRotation%20clamped%20to%20Displacement)) 1) (.AXIS (Utilities|Struct|BreakF_CSVdata _returnvalue_5))))))) -1.0) (.Z (Math|Vector|BreakVector (* (Variables|Default|GetRandom%20Rotation%20[XYZ]) (Math|Conversions|ToFloat(Boolean) (!= (- (Math|Conversions|ToInteger(Boolean) (Variables|Default|GetRotation%20clamped%20to%20Displacement)) 1) (.AXIS (Utilities|Struct|BreakF_CSVdata _returnvalue_5))))))) _displacement_randomize)) (Variables|Default|GetShuffle)) (Math|Vector|MakeVector (.R_X (Utilities|Struct|BreakF_CSVdata _returnvalue_5)) (.R_Y (Utilities|Struct|BreakF_CSVdata _returnvalue_5)) (.R_Z (Utilities|Struct|BreakF_CSVdata _returnvalue_5)))))) (.Y (Math|Vector|BreakVector (+ (+ (Math|Vector|MakeVector (Math|Random|RandomFloatinRangefromStream (* (.X (Math|Vector|BreakVector (* (Variables|Default|GetRandom%20Rotation%20[XYZ]) (Math|Conversions|ToFloat(Boolean) (!= (- (Math|Conversions|ToInteger(Boolean) (Variables|Default|GetRotation%20clamped%20to%20Displacement)) 1) (.AXIS (Utilities|Struct|BreakF_CSVdata _returnvalue_5))))))) -1.0) (.X (Math|Vector|BreakVector (* (Variables|Default|GetRandom%20Rotation%20[XYZ]) (Math|Conversions|ToFloat(Boolean) (!= (- (Math|Conversions|ToInteger(Boolean) (Variables|Default|GetRotation%20clamped%20to%20Displacement)) 1) (.AXIS (Utilities|Struct|BreakF_CSVdata _returnvalue_5))))))) _displacement_randomize) (Math|Random|RandomFloatinRangefromStream (* (.Y (Math|Vector|BreakVector (* (Variables|Default|GetRandom%20Rotation%20[XYZ]) (Math|Conversions|ToFloat(Boolean) (!= (- (Math|Conversions|ToInteger(Boolean) (Variables|Default|GetRotation%20clamped%20to%20Displacement)) 1) (.AXIS (Utilities|Struct|BreakF_CSVdata _returnvalue_5))))))) -1.0) (.Y (Math|Vector|BreakVector (* (Variables|Default|GetRandom%20Rotation%20[XYZ]) (Math|Conversions|ToFloat(Boolean) (!= (- (Math|Conversions|ToInteger(Boolean) (Variables|Default|GetRotation%20clamped%20to%20Displacement)) 1) (.AXIS (Utilities|Struct|BreakF_CSVdata _returnvalue_5))))))) _displacement_randomize) (Math|Random|RandomFloatinRangefromStream (* (.Z (Math|Vector|BreakVector (* (Variables|Default|GetRandom%20Rotation%20[XYZ]) (Math|Conversions|ToFloat(Boolean) (!= (- (Math|Conversions|ToInteger(Boolean) (Variables|Default|GetRotation%20clamped%20to%20Displacement)) 1) (.AXIS (Utilities|Struct|BreakF_CSVdata _returnvalue_5))))))) -1.0) (.Z (Math|Vector|BreakVector (* (Variables|Default|GetRandom%20Rotation%20[XYZ]) (Math|Conversions|ToFloat(Boolean) (!= (- (Math|Conversions|ToInteger(Boolean) (Variables|Default|GetRotation%20clamped%20to%20Displacement)) 1) (.AXIS (Utilities|Struct|BreakF_CSVdata _returnvalue_5))))))) _displacement_randomize)) (Variables|Default|GetShuffle)) (Math|Vector|MakeVector (.R_X (Utilities|Struct|BreakF_CSVdata _returnvalue_5)) (.R_Y (Utilities|Struct|BreakF_CSVdata _returnvalue_5)) (.R_Z (Utilities|Struct|BreakF_CSVdata _returnvalue_5)))))) (.Z (Math|Vector|BreakVector (+ (+ (Math|Vector|MakeVector (Math|Random|RandomFloatinRangefromStream (* (.X (Math|Vector|BreakVector (* (Variables|Default|GetRandom%20Rotation%20[XYZ]) (Math|Conversions|ToFloat(Boolean) (!= (- (Math|Conversions|ToInteger(Boolean) (Variables|Default|GetRotation%20clamped%20to%20Displacement)) 1) (.AXIS (Utilities|Struct|BreakF_CSVdata _returnvalue_5))))))) -1.0) (.X (Math|Vector|BreakVector (* (Variables|Default|GetRandom%20Rotation%20[XYZ]) (Math|Conversions|ToFloat(Boolean) (!= (- (Math|Conversions|ToInteger(Boolean) (Variables|Default|GetRotation%20clamped%20to%20Displacement)) 1) (.AXIS (Utilities|Struct|BreakF_CSVdata _returnvalue_5))))))) _displacement_randomize) (Math|Random|RandomFloatinRangefromStream (* (.Y (Math|Vector|BreakVector (* (Variables|Default|GetRandom%20Rotation%20[XYZ]) (Math|Conversions|ToFloat(Boolean) (!= (- (Math|Conversions|ToInteger(Boolean) (Variables|Default|GetRotation%20clamped%20to%20Displacement)) 1) (.AXIS (Utilities|Struct|BreakF_CSVdata _returnvalue_5))))))) -1.0) (.Y (Math|Vector|BreakVector (* (Variables|Default|GetRandom%20Rotation%20[XYZ]) (Math|Conversions|ToFloat(Boolean) (!= (- (Math|Conversions|ToInteger(Boolean) (Variables|Default|GetRotation%20clamped%20to%20Displacement)) 1) (.AXIS (Utilities|Struct|BreakF_CSVdata _returnvalue_5))))))) _displacement_randomize) (Math|Random|RandomFloatinRangefromStream (* (.Z (Math|Vector|BreakVector (* (Variables|Default|GetRandom%20Rotation%20[XYZ]) (Math|Conversions|ToFloat(Boolean) (!= (- (Math|Conversions|ToInteger(Boolean) (Variables|Default|GetRotation%20clamped%20to%20Displacement)) 1) (.AXIS (Utilities|Struct|BreakF_CSVdata _returnvalue_5))))))) -1.0) (.Z (Math|Vector|BreakVector (* (Variables|Default|GetRandom%20Rotation%20[XYZ]) (Math|Conversions|ToFloat(Boolean) (!= (- (Math|Conversions|ToInteger(Boolean) (Variables|Default|GetRotation%20clamped%20to%20Displacement)) 1) (.AXIS (Utilities|Struct|BreakF_CSVdata _returnvalue_5))))))) _displacement_randomize)) (Variables|Default|GetShuffle)) (Math|Vector|MakeVector (.R_X (Utilities|Struct|BreakF_CSVdata _returnvalue_5)) (.R_Y (Utilities|Struct|BreakF_CSVdata _returnvalue_5)) (.R_Z (Utilities|Struct|BreakF_CSVdata _returnvalue_5))))))) (Math|Conversions|ToFloat(Boolean) (Variables|Default|GetRandom%20Rotation%20LOCAL/GLOBAL))) (* (Math|Vector|MakeVector (.S_X (Utilities|Struct|BreakF_CSVdata _returnvalue_5)) (.S_Y (Utilities|Struct|BreakF_CSVdata _returnvalue_5)) (.S_Z (Utilities|Struct|BreakF_CSVdata _returnvalue_5))) (Variables|Default|GetScale))) (* (Math|Vector|MakeVector (* (Math|Conversions|ToFloat(Boolean) (== (.AXIS (Utilities|Struct|BreakF_CSVdata _returnvalue_5)) 1)) _returnvalue_3) (* (Math|Conversions|ToFloat(Boolean) (== (.AXIS (Utilities|Struct|BreakF_CSVdata _returnvalue_5)) 2)) _returnvalue_3) (* (Math|Conversions|ToFloat(Boolean) (== (.AXIS (Utilities|Struct|BreakF_CSVdata _returnvalue_5)) 3)) _returnvalue_3)) (Math|Float|Clamp(Float) (+ (Math|Conversions|ToFloat(Boolean) (and (not (Class|KismetMathLibrary|IsPointinBoxwithTransform (Math|Vector|MakeVector (.T_X (Utilities|Struct|BreakF_CSVdata _returnvalue_5)) (.T_Y (Utilities|Struct|BreakF_CSVdata _returnvalue_5)) (.T_Z (Utilities|Struct|BreakF_CSVdata _returnvalue_5))) (Math|Transform|MakeTransform (Variables|Default|GetBox%20Origin%20[XYZ]) (Variables|Default|GetBox%20Rotation%20[XYZ])) (Variables|Default|GetBox%20Extent%20[XYZ]))) _boxcontrolleddisplacement)) (Variables|Default|GetBox%20Intensity)) (Math|Conversions|ToFloat(Boolean) (not _boxcontrolleddisplacement))))) (Math|Rotator|Lerp(Rotator) (Math|Rotator|CombineRotators (Math|Rotator|MakeRotator (.X (Math|Vector|BreakVector (+ (Math|Vector|MakeVector (Math|Random|RandomFloatinRangefromStream (* (.X (Math|Vector|BreakVector (* (Variables|Default|GetRandom%20Rotation%20[XYZ]) (Math|Conversions|ToFloat(Boolean) (!= (- (Math|Conversions|ToInteger(Boolean) (Variables|Default|GetRotation%20clamped%20to%20Displacement)) 1) (.AXIS (Utilities|Struct|BreakF_CSVdata _returnvalue_5))))))) -1.0) (.X (Math|Vector|BreakVector (* (Variables|Default|GetRandom%20Rotation%20[XYZ]) (Math|Conversions|ToFloat(Boolean) (!= (- (Math|Conversions|ToInteger(Boolean) (Variables|Default|GetRotation%20clamped%20to%20Displacement)) 1) (.AXIS (Utilities|Struct|BreakF_CSVdata _returnvalue_5))))))) _displacement_randomize) (Math|Random|RandomFloatinRangefromStream (* (.Y (Math|Vector|BreakVector (* (Variables|Default|GetRandom%20Rotation%20[XYZ]) (Math|Conversions|ToFloat(Boolean) (!= (- (Math|Conversions|ToInteger(Boolean) (Variables|Default|GetRotation%20clamped%20to%20Displacement)) 1) (.AXIS (Utilities|Struct|BreakF_CSVdata _returnvalue_5))))))) -1.0) (.Y (Math|Vector|BreakVector (* (Variables|Default|GetRandom%20Rotation%20[XYZ]) (Math|Conversions|ToFloat(Boolean) (!= (- (Math|Conversions|ToInteger(Boolean) (Variables|Default|GetRotation%20clamped%20to%20Displacement)) 1) (.AXIS (Utilities|Struct|BreakF_CSVdata _returnvalue_5))))))) _displacement_randomize) (Math|Random|RandomFloatinRangefromStream (* (.Z (Math|Vector|BreakVector (* (Variables|Default|GetRandom%20Rotation%20[XYZ]) (Math|Conversions|ToFloat(Boolean) (!= (- (Math|Conversions|ToInteger(Boolean) (Variables|Default|GetRotation%20clamped%20to%20Displacement)) 1) (.AXIS (Utilities|Struct|BreakF_CSVdata _returnvalue_5))))))) -1.0) (.Z (Math|Vector|BreakVector (* (Variables|Default|GetRandom%20Rotation%20[XYZ]) (Math|Conversions|ToFloat(Boolean) (!= (- (Math|Conversions|ToInteger(Boolean) (Variables|Default|GetRotation%20clamped%20to%20Displacement)) 1) (.AXIS (Utilities|Struct|BreakF_CSVdata _returnvalue_5))))))) _displacement_randomize)) (Variables|Default|GetShuffle)))) (.Y (Math|Vector|BreakVector (+ (Math|Vector|MakeVector (Math|Random|RandomFloatinRangefromStream (* (.X (Math|Vector|BreakVector (* (Variables|Default|GetRandom%20Rotation%20[XYZ]) (Math|Conversions|ToFloat(Boolean) (!= (- (Math|Conversions|ToInteger(Boolean) (Variables|Default|GetRotation%20clamped%20to%20Displacement)) 1) (.AXIS (Utilities|Struct|BreakF_CSVdata _returnvalue_5))))))) -1.0) (.X (Math|Vector|BreakVector (* (Variables|Default|GetRandom%20Rotation%20[XYZ]) (Math|Conversions|ToFloat(Boolean) (!= (- (Math|Conversions|ToInteger(Boolean) (Variables|Default|GetRotation%20clamped%20to%20Displacement)) 1) (.AXIS (Utilities|Struct|BreakF_CSVdata _returnvalue_5))))))) _displacement_randomize) (Math|Random|RandomFloatinRangefromStream (* (.Y (Math|Vector|BreakVector (* (Variables|Default|GetRandom%20Rotation%20[XYZ]) (Math|Conversions|ToFloat(Boolean) (!= (- (Math|Conversions|ToInteger(Boolean) (Variables|Default|GetRotation%20clamped%20to%20Displacement)) 1) (.AXIS (Utilities|Struct|BreakF_CSVdata _returnvalue_5))))))) -1.0) (.Y (Math|Vector|BreakVector (* (Variables|Default|GetRandom%20Rotation%20[XYZ]) (Math|Conversions|ToFloat(Boolean) (!= (- (Math|Conversions|ToInteger(Boolean) (Variables|Default|GetRotation%20clamped%20to%20Displacement)) 1) (.AXIS (Utilities|Struct|BreakF_CSVdata _returnvalue_5))))))) _displacement_randomize) (Math|Random|RandomFloatinRangefromStream (* (.Z (Math|Vector|BreakVector (* (Variables|Default|GetRandom%20Rotation%20[XYZ]) (Math|Conversions|ToFloat(Boolean) (!= (- (Math|Conversions|ToInteger(Boolean) (Variables|Default|GetRotation%20clamped%20to%20Displacement)) 1) (.AXIS (Utilities|Struct|BreakF_CSVdata _returnvalue_5))))))) -1.0) (.Z (Math|Vector|BreakVector (* (Variables|Default|GetRandom%20Rotation%20[XYZ]) (Math|Conversions|ToFloat(Boolean) (!= (- (Math|Conversions|ToInteger(Boolean) (Variables|Default|GetRotation%20clamped%20to%20Displacement)) 1) (.AXIS (Utilities|Struct|BreakF_CSVdata _returnvalue_5))))))) _displacement_randomize)) (Variables|Default|GetShuffle)))) (.Z (Math|Vector|BreakVector (+ (Math|Vector|MakeVector (Math|Random|RandomFloatinRangefromStream (* (.X (Math|Vector|BreakVector (* (Variables|Default|GetRandom%20Rotation%20[XYZ]) (Math|Conversions|ToFloat(Boolean) (!= (- (Math|Conversions|ToInteger(Boolean) (Variables|Default|GetRotation%20clamped%20to%20Displacement)) 1) (.AXIS (Utilities|Struct|BreakF_CSVdata _returnvalue_5))))))) -1.0) (.X (Math|Vector|BreakVector (* (Variables|Default|GetRandom%20Rotation%20[XYZ]) (Math|Conversions|ToFloat(Boolean) (!= (- (Math|Conversions|ToInteger(Boolean) (Variables|Default|GetRotation%20clamped%20to%20Displacement)) 1) (.AXIS (Utilities|Struct|BreakF_CSVdata _returnvalue_5))))))) _displacement_randomize) (Math|Random|RandomFloatinRangefromStream (* (.Y (Math|Vector|BreakVector (* (Variables|Default|GetRandom%20Rotation%20[XYZ]) (Math|Conversions|ToFloat(Boolean) (!= (- (Math|Conversions|ToInteger(Boolean) (Variables|Default|GetRotation%20clamped%20to%20Displacement)) 1) (.AXIS (Utilities|Struct|BreakF_CSVdata _returnvalue_5))))))) -1.0) (.Y (Math|Vector|BreakVector (* (Variables|Default|GetRandom%20Rotation%20[XYZ]) (Math|Conversions|ToFloat(Boolean) (!= (- (Math|Conversions|ToInteger(Boolean) (Variables|Default|GetRotation%20clamped%20to%20Displacement)) 1) (.AXIS (Utilities|Struct|BreakF_CSVdata _returnvalue_5))))))) _displacement_randomize) (Math|Random|RandomFloatinRangefromStream (* (.Z (Math|Vector|BreakVector (* (Variables|Default|GetRandom%20Rotation%20[XYZ]) (Math|Conversions|ToFloat(Boolean) (!= (- (Math|Conversions|ToInteger(Boolean) (Variables|Default|GetRotation%20clamped%20to%20Displacement)) 1) (.AXIS (Utilities|Struct|BreakF_CSVdata _returnvalue_5))))))) -1.0) (.Z (Math|Vector|BreakVector (* (Variables|Default|GetRandom%20Rotation%20[XYZ]) (Math|Conversions|ToFloat(Boolean) (!= (- (Math|Conversions|ToInteger(Boolean) (Variables|Default|GetRotation%20clamped%20to%20Displacement)) 1) (.AXIS (Utilities|Struct|BreakF_CSVdata _returnvalue_5))))))) _displacement_randomize)) (Variables|Default|GetShuffle))))) (Math|Rotator|MakeRotator (.R_X (Utilities|Struct|BreakF_CSVdata _returnvalue_5)) (.R_Y (Utilities|Struct|BreakF_CSVdata _returnvalue_5)) (.R_Z (Utilities|Struct|BreakF_CSVdata _returnvalue_5)))) (Math|Rotator|MakeRotator (.X (Math|Vector|BreakVector (+ (+ (Math|Vector|MakeVector (Math|Random|RandomFloatinRangefromStream (* (.X (Math|Vector|BreakVector (* (Variables|Default|GetRandom%20Rotation%20[XYZ]) (Math|Conversions|ToFloat(Boolean) (!= (- (Math|Conversions|ToInteger(Boolean) (Variables|Default|GetRotation%20clamped%20to%20Displacement)) 1) (.AXIS (Utilities|Struct|BreakF_CSVdata _returnvalue_5))))))) -1.0) (.X (Math|Vector|BreakVector (* (Variables|Default|GetRandom%20Rotation%20[XYZ]) (Math|Conversions|ToFloat(Boolean) (!= (- (Math|Conversions|ToInteger(Boolean) (Variables|Default|GetRotation%20clamped%20to%20Displacement)) 1) (.AXIS (Utilities|Struct|BreakF_CSVdata _returnvalue_5))))))) _displacement_randomize) (Math|Random|RandomFloatinRangefromStream (* (.Y (Math|Vector|BreakVector (* (Variables|Default|GetRandom%20Rotation%20[XYZ]) (Math|Conversions|ToFloat(Boolean) (!= (- (Math|Conversions|ToInteger(Boolean) (Variables|Default|GetRotation%20clamped%20to%20Displacement)) 1) (.AXIS (Utilities|Struct|BreakF_CSVdata _returnvalue_5))))))) -1.0) (.Y (Math|Vector|BreakVector (* (Variables|Default|GetRandom%20Rotation%20[XYZ]) (Math|Conversions|ToFloat(Boolean) (!= (- (Math|Conversions|ToInteger(Boolean) (Variables|Default|GetRotation%20clamped%20to%20Displacement)) 1) (.AXIS (Utilities|Struct|BreakF_CSVdata _returnvalue_5))))))) _displacement_randomize) (Math|Random|RandomFloatinRangefromStream (* (.Z (Math|Vector|BreakVector (* (Variables|Default|GetRandom%20Rotation%20[XYZ]) (Math|Conversions|ToFloat(Boolean) (!= (- (Math|Conversions|ToInteger(Boolean) (Variables|Default|GetRotation%20clamped%20to%20Displacement)) 1) (.AXIS (Utilities|Struct|BreakF_CSVdata _returnvalue_5))))))) -1.0) (.Z (Math|Vector|BreakVector (* (Variables|Default|GetRandom%20Rotation%20[XYZ]) (Math|Conversions|ToFloat(Boolean) (!= (- (Math|Conversions|ToInteger(Boolean) (Variables|Default|GetRotation%20clamped%20to%20Displacement)) 1) (.AXIS (Utilities|Struct|BreakF_CSVdata _returnvalue_5))))))) _displacement_randomize)) (Variables|Default|GetShuffle)) (Math|Vector|MakeVector (.R_X (Utilities|Struct|BreakF_CSVdata _returnvalue_5)) (.R_Y (Utilities|Struct|BreakF_CSVdata _returnvalue_5)) (.R_Z (Utilities|Struct|BreakF_CSVdata _returnvalue_5)))))) (.Y (Math|Vector|BreakVector (+ (+ (Math|Vector|MakeVector (Math|Random|RandomFloatinRangefromStream (* (.X (Math|Vector|BreakVector (* (Variables|Default|GetRandom%20Rotation%20[XYZ]) (Math|Conversions|ToFloat(Boolean) (!= (- (Math|Conversions|ToInteger(Boolean) (Variables|Default|GetRotation%20clamped%20to%20Displacement)) 1) (.AXIS (Utilities|Struct|BreakF_CSVdata _returnvalue_5))))))) -1.0) (.X (Math|Vector|BreakVector (* (Variables|Default|GetRandom%20Rotation%20[XYZ]) (Math|Conversions|ToFloat(Boolean) (!= (- (Math|Conversions|ToInteger(Boolean) (Variables|Default|GetRotation%20clamped%20to%20Displacement)) 1) (.AXIS (Utilities|Struct|BreakF_CSVdata _returnvalue_5))))))) _displacement_randomize) (Math|Random|RandomFloatinRangefromStream (* (.Y (Math|Vector|BreakVector (* (Variables|Default|GetRandom%20Rotation%20[XYZ]) (Math|Conversions|ToFloat(Boolean) (!= (- (Math|Conversions|ToInteger(Boolean) (Variables|Default|GetRotation%20clamped%20to%20Displacement)) 1) (.AXIS (Utilities|Struct|BreakF_CSVdata _returnvalue_5))))))) -1.0) (.Y (Math|Vector|BreakVector (* (Variables|Default|GetRandom%20Rotation%20[XYZ]) (Math|Conversions|ToFloat(Boolean) (!= (- (Math|Conversions|ToInteger(Boolean) (Variables|Default|GetRotation%20clamped%20to%20Displacement)) 1) (.AXIS (Utilities|Struct|BreakF_CSVdata _returnvalue_5))))))) _displacement_randomize) (Math|Random|RandomFloatinRangefromStream (* (.Z (Math|Vector|BreakVector (* (Variables|Default|GetRandom%20Rotation%20[XYZ]) (Math|Conversions|ToFloat(Boolean) (!= (- (Math|Conversions|ToInteger(Boolean) (Variables|Default|GetRotation%20clamped%20to%20Displacement)) 1) (.AXIS (Utilities|Struct|BreakF_CSVdata _returnvalue_5))))))) -1.0) (.Z (Math|Vector|BreakVector (* (Variables|Default|GetRandom%20Rotation%20[XYZ]) (Math|Conversions|ToFloat(Boolean) (!= (- (Math|Conversions|ToInteger(Boolean) (Variables|Default|GetRotation%20clamped%20to%20Displacement)) 1) (.AXIS (Utilities|Struct|BreakF_CSVdata _returnvalue_5))))))) _displacement_randomize)) (Variables|Default|GetShuffle)) (Math|Vector|MakeVector (.R_X (Utilities|Struct|BreakF_CSVdata _returnvalue_5)) (.R_Y (Utilities|Struct|BreakF_CSVdata _returnvalue_5)) (.R_Z (Utilities|Struct|BreakF_CSVdata _returnvalue_5)))))) (.Z (Math|Vector|BreakVector (+ (+ (Math|Vector|MakeVector (Math|Random|RandomFloatinRangefromStream (* (.X (Math|Vector|BreakVector (* (Variables|Default|GetRandom%20Rotation%20[XYZ]) (Math|Conversions|ToFloat(Boolean) (!= (- (Math|Conversions|ToInteger(Boolean) (Variables|Default|GetRotation%20clamped%20to%20Displacement)) 1) (.AXIS (Utilities|Struct|BreakF_CSVdata _returnvalue_5))))))) -1.0) (.X (Math|Vector|BreakVector (* (Variables|Default|GetRandom%20Rotation%20[XYZ]) (Math|Conversions|ToFloat(Boolean) (!= (- (Math|Conversions|ToInteger(Boolean) (Variables|Default|GetRotation%20clamped%20to%20Displacement)) 1) (.AXIS (Utilities|Struct|BreakF_CSVdata _returnvalue_5))))))) _displacement_randomize) (Math|Random|RandomFloatinRangefromStream (* (.Y (Math|Vector|BreakVector (* (Variables|Default|GetRandom%20Rotation%20[XYZ]) (Math|Conversions|ToFloat(Boolean) (!= (- (Math|Conversions|ToInteger(Boolean) (Variables|Default|GetRotation%20clamped%20to%20Displacement)) 1) (.AXIS (Utilities|Struct|BreakF_CSVdata _returnvalue_5))))))) -1.0) (.Y (Math|Vector|BreakVector (* (Variables|Default|GetRandom%20Rotation%20[XYZ]) (Math|Conversions|ToFloat(Boolean) (!= (- (Math|Conversions|ToInteger(Boolean) (Variables|Default|GetRotation%20clamped%20to%20Displacement)) 1) (.AXIS (Utilities|Struct|BreakF_CSVdata _returnvalue_5))))))) _displacement_randomize) (Math|Random|RandomFloatinRangefromStream (* (.Z (Math|Vector|BreakVector (* (Variables|Default|GetRandom%20Rotation%20[XYZ]) (Math|Conversions|ToFloat(Boolean) (!= (- (Math|Conversions|ToInteger(Boolean) (Variables|Default|GetRotation%20clamped%20to%20Displacement)) 1) (.AXIS (Utilities|Struct|BreakF_CSVdata _returnvalue_5))))))) -1.0) (.Z (Math|Vector|BreakVector (* (Variables|Default|GetRandom%20Rotation%20[XYZ]) (Math|Conversions|ToFloat(Boolean) (!= (- (Math|Conversions|ToInteger(Boolean) (Variables|Default|GetRotation%20clamped%20to%20Displacement)) 1) (.AXIS (Utilities|Struct|BreakF_CSVdata _returnvalue_5))))))) _displacement_randomize)) (Variables|Default|GetShuffle)) (Math|Vector|MakeVector (.R_X (Utilities|Struct|BreakF_CSVdata _returnvalue_5)) (.R_Y (Utilities|Struct|BreakF_CSVdata _returnvalue_5)) (.R_Z (Utilities|Struct|BreakF_CSVdata _returnvalue_5))))))) (Math|Conversions|ToFloat(Boolean) (Variables|Default|GetRandom%20Rotation%20LOCAL/GLOBAL))) (* (Math|Vector|MakeVector (.S_X (Utilities|Struct|BreakF_CSVdata _returnvalue_5)) (.S_Y (Utilities|Struct|BreakF_CSVdata _returnvalue_5)) (.S_Z (Utilities|Struct|BreakF_CSVdata _returnvalue_5))) (Variables|Default|GetScale))) false))))
                  (:2
                    (if _undamaged_stones
                      (goto _label)
                      (elif _extrastones
                        (Utilities|FlowControl|MultiGate false true (Variables|Default|GetShuffleExtraStones) :!label _label_2
                          (:Out%200
                            (Utilities|FlowControl|Sequence :!label _label_3
                              (:then_0
                                (Utilities|FlowControl|DoOnce false
                                  (:Completed
                                    (bind _returnvalue_7 (AddComponent|AddHierarchicalInstancedStaticMeshComponent false))
                                    (bind _output_get_2 (Variables|Default|Set04 _returnvalue_7))
                                    (Rendering|Material|SetMaterial _output_get_2 0 (Variables|Default|GetStone%20Material)))))
                              (:then_1
                                (Components|InstancedStaticMesh|AddInstance (Variables|Default|Get04) (Math|Transform|MakeTransform (Math|Transform|TransformLocation (Math|Transform|MakeTransform (Math|Vector|MakeVector (.T_X (Utilities|Struct|BreakF_CSVdata _returnvalue_5)) (.T_Y (Utilities|Struct|BreakF_CSVdata _returnvalue_5)) (.T_Z (Utilities|Struct|BreakF_CSVdata _returnvalue_5))) (Math|Rotator|Lerp(Rotator) (Math|Rotator|CombineRotators (Math|Rotator|MakeRotator (.X (Math|Vector|BreakVector (+ (Math|Vector|MakeVector (Math|Random|RandomFloatinRangefromStream (* (.X (Math|Vector|BreakVector (* (Variables|Default|GetRandom%20Rotation%20[XYZ]) (Math|Conversions|ToFloat(Boolean) (!= (- (Math|Conversions|ToInteger(Boolean) (Variables|Default|GetRotation%20clamped%20to%20Displacement)) 1) (.AXIS (Utilities|Struct|BreakF_CSVdata _returnvalue_5))))))) -1.0) (.X (Math|Vector|BreakVector (* (Variables|Default|GetRandom%20Rotation%20[XYZ]) (Math|Conversions|ToFloat(Boolean) (!= (- (Math|Conversions|ToInteger(Boolean) (Variables|Default|GetRotation%20clamped%20to%20Displacement)) 1) (.AXIS (Utilities|Struct|BreakF_CSVdata _returnvalue_5))))))) _displacement_randomize) (Math|Random|RandomFloatinRangefromStream (* (.Y (Math|Vector|BreakVector (* (Variables|Default|GetRandom%20Rotation%20[XYZ]) (Math|Conversions|ToFloat(Boolean) (!= (- (Math|Conversions|ToInteger(Boolean) (Variables|Default|GetRotation%20clamped%20to%20Displacement)) 1) (.AXIS (Utilities|Struct|BreakF_CSVdata _returnvalue_5))))))) -1.0) (.Y (Math|Vector|BreakVector (* (Variables|Default|GetRandom%20Rotation%20[XYZ]) (Math|Conversions|ToFloat(Boolean) (!= (- (Math|Conversions|ToInteger(Boolean) (Variables|Default|GetRotation%20clamped%20to%20Displacement)) 1) (.AXIS (Utilities|Struct|BreakF_CSVdata _returnvalue_5))))))) _displacement_randomize) (Math|Random|RandomFloatinRangefromStream (* (.Z (Math|Vector|BreakVector (* (Variables|Default|GetRandom%20Rotation%20[XYZ]) (Math|Conversions|ToFloat(Boolean) (!= (- (Math|Conversions|ToInteger(Boolean) (Variables|Default|GetRotation%20clamped%20to%20Displacement)) 1) (.AXIS (Utilities|Struct|BreakF_CSVdata _returnvalue_5))))))) -1.0) (.Z (Math|Vector|BreakVector (* (Variables|Default|GetRandom%20Rotation%20[XYZ]) (Math|Conversions|ToFloat(Boolean) (!= (- (Math|Conversions|ToInteger(Boolean) (Variables|Default|GetRotation%20clamped%20to%20Displacement)) 1) (.AXIS (Utilities|Struct|BreakF_CSVdata _returnvalue_5))))))) _displacement_randomize)) (Variables|Default|GetShuffle)))) (.Y (Math|Vector|BreakVector (+ (Math|Vector|MakeVector (Math|Random|RandomFloatinRangefromStream (* (.X (Math|Vector|BreakVector (* (Variables|Default|GetRandom%20Rotation%20[XYZ]) (Math|Conversions|ToFloat(Boolean) (!= (- (Math|Conversions|ToInteger(Boolean) (Variables|Default|GetRotation%20clamped%20to%20Displacement)) 1) (.AXIS (Utilities|Struct|BreakF_CSVdata _returnvalue_5))))))) -1.0) (.X (Math|Vector|BreakVector (* (Variables|Default|GetRandom%20Rotation%20[XYZ]) (Math|Conversions|ToFloat(Boolean) (!= (- (Math|Conversions|ToInteger(Boolean) (Variables|Default|GetRotation%20clamped%20to%20Displacement)) 1) (.AXIS (Utilities|Struct|BreakF_CSVdata _returnvalue_5))))))) _displacement_randomize) (Math|Random|RandomFloatinRangefromStream (* (.Y (Math|Vector|BreakVector (* (Variables|Default|GetRandom%20Rotation%20[XYZ]) (Math|Conversions|ToFloat(Boolean) (!= (- (Math|Conversions|ToInteger(Boolean) (Variables|Default|GetRotation%20clamped%20to%20Displacement)) 1) (.AXIS (Utilities|Struct|BreakF_CSVdata _returnvalue_5))))))) -1.0) (.Y (Math|Vector|BreakVector (* (Variables|Default|GetRandom%20Rotation%20[XYZ]) (Math|Conversions|ToFloat(Boolean) (!= (- (Math|Conversions|ToInteger(Boolean) (Variables|Default|GetRotation%20clamped%20to%20Displacement)) 1) (.AXIS (Utilities|Struct|BreakF_CSVdata _returnvalue_5))))))) _displacement_randomize) (Math|Random|RandomFloatinRangefromStream (* (.Z (Math|Vector|BreakVector (* (Variables|Default|GetRandom%20Rotation%20[XYZ]) (Math|Conversions|ToFloat(Boolean) (!= (- (Math|Conversions|ToInteger(Boolean) (Variables|Default|GetRotation%20clamped%20to%20Displacement)) 1) (.AXIS (Utilities|Struct|BreakF_CSVdata _returnvalue_5))))))) -1.0) (.Z (Math|Vector|BreakVector (* (Variables|Default|GetRandom%20Rotation%20[XYZ]) (Math|Conversions|ToFloat(Boolean) (!= (- (Math|Conversions|ToInteger(Boolean) (Variables|Default|GetRotation%20clamped%20to%20Displacement)) 1) (.AXIS (Utilities|Struct|BreakF_CSVdata _returnvalue_5))))))) _displacement_randomize)) (Variables|Default|GetShuffle)))) (.Z (Math|Vector|BreakVector (+ (Math|Vector|MakeVector (Math|Random|RandomFloatinRangefromStream (* (.X (Math|Vector|BreakVector (* (Variables|Default|GetRandom%20Rotation%20[XYZ]) (Math|Conversions|ToFloat(Boolean) (!= (- (Math|Conversions|ToInteger(Boolean) (Variables|Default|GetRotation%20clamped%20to%20Displacement)) 1) (.AXIS (Utilities|Struct|BreakF_CSVdata _returnvalue_5))))))) -1.0) (.X (Math|Vector|BreakVector (* (Variables|Default|GetRandom%20Rotation%20[XYZ]) (Math|Conversions|ToFloat(Boolean) (!= (- (Math|Conversions|ToInteger(Boolean) (Variables|Default|GetRotation%20clamped%20to%20Displacement)) 1) (.AXIS (Utilities|Struct|BreakF_CSVdata _returnvalue_5))))))) _displacement_randomize) (Math|Random|RandomFloatinRangefromStream (* (.Y (Math|Vector|BreakVector (* (Variables|Default|GetRandom%20Rotation%20[XYZ]) (Math|Conversions|ToFloat(Boolean) (!= (- (Math|Conversions|ToInteger(Boolean) (Variables|Default|GetRotation%20clamped%20to%20Displacement)) 1) (.AXIS (Utilities|Struct|BreakF_CSVdata _returnvalue_5))))))) -1.0) (.Y (Math|Vector|BreakVector (* (Variables|Default|GetRandom%20Rotation%20[XYZ]) (Math|Conversions|ToFloat(Boolean) (!= (- (Math|Conversions|ToInteger(Boolean) (Variables|Default|GetRotation%20clamped%20to%20Displacement)) 1) (.AXIS (Utilities|Struct|BreakF_CSVdata _returnvalue_5))))))) _displacement_randomize) (Math|Random|RandomFloatinRangefromStream (* (.Z (Math|Vector|BreakVector (* (Variables|Default|GetRandom%20Rotation%20[XYZ]) (Math|Conversions|ToFloat(Boolean) (!= (- (Math|Conversions|ToInteger(Boolean) (Variables|Default|GetRotation%20clamped%20to%20Displacement)) 1) (.AXIS (Utilities|Struct|BreakF_CSVdata _returnvalue_5))))))) -1.0) (.Z (Math|Vector|BreakVector (* (Variables|Default|GetRandom%20Rotation%20[XYZ]) (Math|Conversions|ToFloat(Boolean) (!= (- (Math|Conversions|ToInteger(Boolean) (Variables|Default|GetRotation%20clamped%20to%20Displacement)) 1) (.AXIS (Utilities|Struct|BreakF_CSVdata _returnvalue_5))))))) _displacement_randomize)) (Variables|Default|GetShuffle))))) (Math|Rotator|MakeRotator (.R_X (Utilities|Struct|BreakF_CSVdata _returnvalue_5)) (.R_Y (Utilities|Struct|BreakF_CSVdata _returnvalue_5)) (.R_Z (Utilities|Struct|BreakF_CSVdata _returnvalue_5)))) (Math|Rotator|MakeRotator (.X (Math|Vector|BreakVector (+ (+ (Math|Vector|MakeVector (Math|Random|RandomFloatinRangefromStream (* (.X (Math|Vector|BreakVector (* (Variables|Default|GetRandom%20Rotation%20[XYZ]) (Math|Conversions|ToFloat(Boolean) (!= (- (Math|Conversions|ToInteger(Boolean) (Variables|Default|GetRotation%20clamped%20to%20Displacement)) 1) (.AXIS (Utilities|Struct|BreakF_CSVdata _returnvalue_5))))))) -1.0) (.X (Math|Vector|BreakVector (* (Variables|Default|GetRandom%20Rotation%20[XYZ]) (Math|Conversions|ToFloat(Boolean) (!= (- (Math|Conversions|ToInteger(Boolean) (Variables|Default|GetRotation%20clamped%20to%20Displacement)) 1) (.AXIS (Utilities|Struct|BreakF_CSVdata _returnvalue_5))))))) _displacement_randomize) (Math|Random|RandomFloatinRangefromStream (* (.Y (Math|Vector|BreakVector (* (Variables|Default|GetRandom%20Rotation%20[XYZ]) (Math|Conversions|ToFloat(Boolean) (!= (- (Math|Conversions|ToInteger(Boolean) (Variables|Default|GetRotation%20clamped%20to%20Displacement)) 1) (.AXIS (Utilities|Struct|BreakF_CSVdata _returnvalue_5))))))) -1.0) (.Y (Math|Vector|BreakVector (* (Variables|Default|GetRandom%20Rotation%20[XYZ]) (Math|Conversions|ToFloat(Boolean) (!= (- (Math|Conversions|ToInteger(Boolean) (Variables|Default|GetRotation%20clamped%20to%20Displacement)) 1) (.AXIS (Utilities|Struct|BreakF_CSVdata _returnvalue_5))))))) _displacement_randomize) (Math|Random|RandomFloatinRangefromStream (* (.Z (Math|Vector|BreakVector (* (Variables|Default|GetRandom%20Rotation%20[XYZ]) (Math|Conversions|ToFloat(Boolean) (!= (- (Math|Conversions|ToInteger(Boolean) (Variables|Default|GetRotation%20clamped%20to%20Displacement)) 1) (.AXIS (Utilities|Struct|BreakF_CSVdata _returnvalue_5))))))) -1.0) (.Z (Math|Vector|BreakVector (* (Variables|Default|GetRandom%20Rotation%20[XYZ]) (Math|Conversions|ToFloat(Boolean) (!= (- (Math|Conversions|ToInteger(Boolean) (Variables|Default|GetRotation%20clamped%20to%20Displacement)) 1) (.AXIS (Utilities|Struct|BreakF_CSVdata _returnvalue_5))))))) _displacement_randomize)) (Variables|Default|GetShuffle)) (Math|Vector|MakeVector (.R_X (Utilities|Struct|BreakF_CSVdata _returnvalue_5)) (.R_Y (Utilities|Struct|BreakF_CSVdata _returnvalue_5)) (.R_Z (Utilities|Struct|BreakF_CSVdata _returnvalue_5)))))) (.Y (Math|Vector|BreakVector (+ (+ (Math|Vector|MakeVector (Math|Random|RandomFloatinRangefromStream (* (.X (Math|Vector|BreakVector (* (Variables|Default|GetRandom%20Rotation%20[XYZ]) (Math|Conversions|ToFloat(Boolean) (!= (- (Math|Conversions|ToInteger(Boolean) (Variables|Default|GetRotation%20clamped%20to%20Displacement)) 1) (.AXIS (Utilities|Struct|BreakF_CSVdata _returnvalue_5))))))) -1.0) (.X (Math|Vector|BreakVector (* (Variables|Default|GetRandom%20Rotation%20[XYZ]) (Math|Conversions|ToFloat(Boolean) (!= (- (Math|Conversions|ToInteger(Boolean) (Variables|Default|GetRotation%20clamped%20to%20Displacement)) 1) (.AXIS (Utilities|Struct|BreakF_CSVdata _returnvalue_5))))))) _displacement_randomize) (Math|Random|RandomFloatinRangefromStream (* (.Y (Math|Vector|BreakVector (* (Variables|Default|GetRandom%20Rotation%20[XYZ]) (Math|Conversions|ToFloat(Boolean) (!= (- (Math|Conversions|ToInteger(Boolean) (Variables|Default|GetRotation%20clamped%20to%20Displacement)) 1) (.AXIS (Utilities|Struct|BreakF_CSVdata _returnvalue_5))))))) -1.0) (.Y (Math|Vector|BreakVector (* (Variables|Default|GetRandom%20Rotation%20[XYZ]) (Math|Conversions|ToFloat(Boolean) (!= (- (Math|Conversions|ToInteger(Boolean) (Variables|Default|GetRotation%20clamped%20to%20Displacement)) 1) (.AXIS (Utilities|Struct|BreakF_CSVdata _returnvalue_5))))))) _displacement_randomize) (Math|Random|RandomFloatinRangefromStream (* (.Z (Math|Vector|BreakVector (* (Variables|Default|GetRandom%20Rotation%20[XYZ]) (Math|Conversions|ToFloat(Boolean) (!= (- (Math|Conversions|ToInteger(Boolean) (Variables|Default|GetRotation%20clamped%20to%20Displacement)) 1) (.AXIS (Utilities|Struct|BreakF_CSVdata _returnvalue_5))))))) -1.0) (.Z (Math|Vector|BreakVector (* (Variables|Default|GetRandom%20Rotation%20[XYZ]) (Math|Conversions|ToFloat(Boolean) (!= (- (Math|Conversions|ToInteger(Boolean) (Variables|Default|GetRotation%20clamped%20to%20Displacement)) 1) (.AXIS (Utilities|Struct|BreakF_CSVdata _returnvalue_5))))))) _displacement_randomize)) (Variables|Default|GetShuffle)) (Math|Vector|MakeVector (.R_X (Utilities|Struct|BreakF_CSVdata _returnvalue_5)) (.R_Y (Utilities|Struct|BreakF_CSVdata _returnvalue_5)) (.R_Z (Utilities|Struct|BreakF_CSVdata _returnvalue_5)))))) (.Z (Math|Vector|BreakVector (+ (+ (Math|Vector|MakeVector (Math|Random|RandomFloatinRangefromStream (* (.X (Math|Vector|BreakVector (* (Variables|Default|GetRandom%20Rotation%20[XYZ]) (Math|Conversions|ToFloat(Boolean) (!= (- (Math|Conversions|ToInteger(Boolean) (Variables|Default|GetRotation%20clamped%20to%20Displacement)) 1) (.AXIS (Utilities|Struct|BreakF_CSVdata _returnvalue_5))))))) -1.0) (.X (Math|Vector|BreakVector (* (Variables|Default|GetRandom%20Rotation%20[XYZ]) (Math|Conversions|ToFloat(Boolean) (!= (- (Math|Conversions|ToInteger(Boolean) (Variables|Default|GetRotation%20clamped%20to%20Displacement)) 1) (.AXIS (Utilities|Struct|BreakF_CSVdata _returnvalue_5))))))) _displacement_randomize) (Math|Random|RandomFloatinRangefromStream (* (.Y (Math|Vector|BreakVector (* (Variables|Default|GetRandom%20Rotation%20[XYZ]) (Math|Conversions|ToFloat(Boolean) (!= (- (Math|Conversions|ToInteger(Boolean) (Variables|Default|GetRotation%20clamped%20to%20Displacement)) 1) (.AXIS (Utilities|Struct|BreakF_CSVdata _returnvalue_5))))))) -1.0) (.Y (Math|Vector|BreakVector (* (Variables|Default|GetRandom%20Rotation%20[XYZ]) (Math|Conversions|ToFloat(Boolean) (!= (- (Math|Conversions|ToInteger(Boolean) (Variables|Default|GetRotation%20clamped%20to%20Displacement)) 1) (.AXIS (Utilities|Struct|BreakF_CSVdata _returnvalue_5))))))) _displacement_randomize) (Math|Random|RandomFloatinRangefromStream (* (.Z (Math|Vector|BreakVector (* (Variables|Default|GetRandom%20Rotation%20[XYZ]) (Math|Conversions|ToFloat(Boolean) (!= (- (Math|Conversions|ToInteger(Boolean) (Variables|Default|GetRotation%20clamped%20to%20Displacement)) 1) (.AXIS (Utilities|Struct|BreakF_CSVdata _returnvalue_5))))))) -1.0) (.Z (Math|Vector|BreakVector (* (Variables|Default|GetRandom%20Rotation%20[XYZ]) (Math|Conversions|ToFloat(Boolean) (!= (- (Math|Conversions|ToInteger(Boolean) (Variables|Default|GetRotation%20clamped%20to%20Displacement)) 1) (.AXIS (Utilities|Struct|BreakF_CSVdata _returnvalue_5))))))) _displacement_randomize)) (Variables|Default|GetShuffle)) (Math|Vector|MakeVector (.R_X (Utilities|Struct|BreakF_CSVdata _returnvalue_5)) (.R_Y (Utilities|Struct|BreakF_CSVdata _returnvalue_5)) (.R_Z (Utilities|Struct|BreakF_CSVdata _returnvalue_5))))))) (Math|Conversions|ToFloat(Boolean) (Variables|Default|GetRandom%20Rotation%20LOCAL/GLOBAL))) (* (Math|Vector|MakeVector (.S_X (Utilities|Struct|BreakF_CSVdata _returnvalue_5)) (.S_Y (Utilities|Struct|BreakF_CSVdata _returnvalue_5)) (.S_Z (Utilities|Struct|BreakF_CSVdata _returnvalue_5))) (Variables|Default|GetScale))) (* (Math|Vector|MakeVector (* (Math|Conversions|ToFloat(Boolean) (== (.AXIS (Utilities|Struct|BreakF_CSVdata _returnvalue_5)) 1)) _returnvalue_3) (* (Math|Conversions|ToFloat(Boolean) (== (.AXIS (Utilities|Struct|BreakF_CSVdata _returnvalue_5)) 2)) _returnvalue_3) (* (Math|Conversions|ToFloat(Boolean) (== (.AXIS (Utilities|Struct|BreakF_CSVdata _returnvalue_5)) 3)) _returnvalue_3)) (Math|Float|Clamp(Float) (+ (Math|Conversions|ToFloat(Boolean) (and (not (Class|KismetMathLibrary|IsPointinBoxwithTransform (Math|Vector|MakeVector (.T_X (Utilities|Struct|BreakF_CSVdata _returnvalue_5)) (.T_Y (Utilities|Struct|BreakF_CSVdata _returnvalue_5)) (.T_Z (Utilities|Struct|BreakF_CSVdata _returnvalue_5))) (Math|Transform|MakeTransform (Variables|Default|GetBox%20Origin%20[XYZ]) (Variables|Default|GetBox%20Rotation%20[XYZ])) (Variables|Default|GetBox%20Extent%20[XYZ]))) _boxcontrolleddisplacement)) (Variables|Default|GetBox%20Intensity)) (Math|Conversions|ToFloat(Boolean) (not _boxcontrolleddisplacement))))) (Math|Rotator|Lerp(Rotator) (Math|Rotator|CombineRotators (Math|Rotator|MakeRotator (.X (Math|Vector|BreakVector (+ (Math|Vector|MakeVector (Math|Random|RandomFloatinRangefromStream (* (.X (Math|Vector|BreakVector (* (Variables|Default|GetRandom%20Rotation%20[XYZ]) (Math|Conversions|ToFloat(Boolean) (!= (- (Math|Conversions|ToInteger(Boolean) (Variables|Default|GetRotation%20clamped%20to%20Displacement)) 1) (.AXIS (Utilities|Struct|BreakF_CSVdata _returnvalue_5))))))) -1.0) (.X (Math|Vector|BreakVector (* (Variables|Default|GetRandom%20Rotation%20[XYZ]) (Math|Conversions|ToFloat(Boolean) (!= (- (Math|Conversions|ToInteger(Boolean) (Variables|Default|GetRotation%20clamped%20to%20Displacement)) 1) (.AXIS (Utilities|Struct|BreakF_CSVdata _returnvalue_5))))))) _displacement_randomize) (Math|Random|RandomFloatinRangefromStream (* (.Y (Math|Vector|BreakVector (* (Variables|Default|GetRandom%20Rotation%20[XYZ]) (Math|Conversions|ToFloat(Boolean) (!= (- (Math|Conversions|ToInteger(Boolean) (Variables|Default|GetRotation%20clamped%20to%20Displacement)) 1) (.AXIS (Utilities|Struct|BreakF_CSVdata _returnvalue_5))))))) -1.0) (.Y (Math|Vector|BreakVector (* (Variables|Default|GetRandom%20Rotation%20[XYZ]) (Math|Conversions|ToFloat(Boolean) (!= (- (Math|Conversions|ToInteger(Boolean) (Variables|Default|GetRotation%20clamped%20to%20Displacement)) 1) (.AXIS (Utilities|Struct|BreakF_CSVdata _returnvalue_5))))))) _displacement_randomize) (Math|Random|RandomFloatinRangefromStream (* (.Z (Math|Vector|BreakVector (* (Variables|Default|GetRandom%20Rotation%20[XYZ]) (Math|Conversions|ToFloat(Boolean) (!= (- (Math|Conversions|ToInteger(Boolean) (Variables|Default|GetRotation%20clamped%20to%20Displacement)) 1) (.AXIS (Utilities|Struct|BreakF_CSVdata _returnvalue_5))))))) -1.0) (.Z (Math|Vector|BreakVector (* (Variables|Default|GetRandom%20Rotation%20[XYZ]) (Math|Conversions|ToFloat(Boolean) (!= (- (Math|Conversions|ToInteger(Boolean) (Variables|Default|GetRotation%20clamped%20to%20Displacement)) 1) (.AXIS (Utilities|Struct|BreakF_CSVdata _returnvalue_5))))))) _displacement_randomize)) (Variables|Default|GetShuffle)))) (.Y (Math|Vector|BreakVector (+ (Math|Vector|MakeVector (Math|Random|RandomFloatinRangefromStream (* (.X (Math|Vector|BreakVector (* (Variables|Default|GetRandom%20Rotation%20[XYZ]) (Math|Conversions|ToFloat(Boolean) (!= (- (Math|Conversions|ToInteger(Boolean) (Variables|Default|GetRotation%20clamped%20to%20Displacement)) 1) (.AXIS (Utilities|Struct|BreakF_CSVdata _returnvalue_5))))))) -1.0) (.X (Math|Vector|BreakVector (* (Variables|Default|GetRandom%20Rotation%20[XYZ]) (Math|Conversions|ToFloat(Boolean) (!= (- (Math|Conversions|ToInteger(Boolean) (Variables|Default|GetRotation%20clamped%20to%20Displacement)) 1) (.AXIS (Utilities|Struct|BreakF_CSVdata _returnvalue_5))))))) _displacement_randomize) (Math|Random|RandomFloatinRangefromStream (* (.Y (Math|Vector|BreakVector (* (Variables|Default|GetRandom%20Rotation%20[XYZ]) (Math|Conversions|ToFloat(Boolean) (!= (- (Math|Conversions|ToInteger(Boolean) (Variables|Default|GetRotation%20clamped%20to%20Displacement)) 1) (.AXIS (Utilities|Struct|BreakF_CSVdata _returnvalue_5))))))) -1.0) (.Y (Math|Vector|BreakVector (* (Variables|Default|GetRandom%20Rotation%20[XYZ]) (Math|Conversions|ToFloat(Boolean) (!= (- (Math|Conversions|ToInteger(Boolean) (Variables|Default|GetRotation%20clamped%20to%20Displacement)) 1) (.AXIS (Utilities|Struct|BreakF_CSVdata _returnvalue_5))))))) _displacement_randomize) (Math|Random|RandomFloatinRangefromStream (* (.Z (Math|Vector|BreakVector (* (Variables|Default|GetRandom%20Rotation%20[XYZ]) (Math|Conversions|ToFloat(Boolean) (!= (- (Math|Conversions|ToInteger(Boolean) (Variables|Default|GetRotation%20clamped%20to%20Displacement)) 1) (.AXIS (Utilities|Struct|BreakF_CSVdata _returnvalue_5))))))) -1.0) (.Z (Math|Vector|BreakVector (* (Variables|Default|GetRandom%20Rotation%20[XYZ]) (Math|Conversions|ToFloat(Boolean) (!= (- (Math|Conversions|ToInteger(Boolean) (Variables|Default|GetRotation%20clamped%20to%20Displacement)) 1) (.AXIS (Utilities|Struct|BreakF_CSVdata _returnvalue_5))))))) _displacement_randomize)) (Variables|Default|GetShuffle)))) (.Z (Math|Vector|BreakVector (+ (Math|Vector|MakeVector (Math|Random|RandomFloatinRangefromStream (* (.X (Math|Vector|BreakVector (* (Variables|Default|GetRandom%20Rotation%20[XYZ]) (Math|Conversions|ToFloat(Boolean) (!= (- (Math|Conversions|ToInteger(Boolean) (Variables|Default|GetRotation%20clamped%20to%20Displacement)) 1) (.AXIS (Utilities|Struct|BreakF_CSVdata _returnvalue_5))))))) -1.0) (.X (Math|Vector|BreakVector (* (Variables|Default|GetRandom%20Rotation%20[XYZ]) (Math|Conversions|ToFloat(Boolean) (!= (- (Math|Conversions|ToInteger(Boolean) (Variables|Default|GetRotation%20clamped%20to%20Displacement)) 1) (.AXIS (Utilities|Struct|BreakF_CSVdata _returnvalue_5))))))) _displacement_randomize) (Math|Random|RandomFloatinRangefromStream (* (.Y (Math|Vector|BreakVector (* (Variables|Default|GetRandom%20Rotation%20[XYZ]) (Math|Conversions|ToFloat(Boolean) (!= (- (Math|Conversions|ToInteger(Boolean) (Variables|Default|GetRotation%20clamped%20to%20Displacement)) 1) (.AXIS (Utilities|Struct|BreakF_CSVdata _returnvalue_5))))))) -1.0) (.Y (Math|Vector|BreakVector (* (Variables|Default|GetRandom%20Rotation%20[XYZ]) (Math|Conversions|ToFloat(Boolean) (!= (- (Math|Conversions|ToInteger(Boolean) (Variables|Default|GetRotation%20clamped%20to%20Displacement)) 1) (.AXIS (Utilities|Struct|BreakF_CSVdata _returnvalue_5))))))) _displacement_randomize) (Math|Random|RandomFloatinRangefromStream (* (.Z (Math|Vector|BreakVector (* (Variables|Default|GetRandom%20Rotation%20[XYZ]) (Math|Conversions|ToFloat(Boolean) (!= (- (Math|Conversions|ToInteger(Boolean) (Variables|Default|GetRotation%20clamped%20to%20Displacement)) 1) (.AXIS (Utilities|Struct|BreakF_CSVdata _returnvalue_5))))))) -1.0) (.Z (Math|Vector|BreakVector (* (Variables|Default|GetRandom%20Rotation%20[XYZ]) (Math|Conversions|ToFloat(Boolean) (!= (- (Math|Conversions|ToInteger(Boolean) (Variables|Default|GetRotation%20clamped%20to%20Displacement)) 1) (.AXIS (Utilities|Struct|BreakF_CSVdata _returnvalue_5))))))) _displacement_randomize)) (Variables|Default|GetShuffle))))) (Math|Rotator|MakeRotator (.R_X (Utilities|Struct|BreakF_CSVdata _returnvalue_5)) (.R_Y (Utilities|Struct|BreakF_CSVdata _returnvalue_5)) (.R_Z (Utilities|Struct|BreakF_CSVdata _returnvalue_5)))) (Math|Rotator|MakeRotator (.X (Math|Vector|BreakVector (+ (+ (Math|Vector|MakeVector (Math|Random|RandomFloatinRangefromStream (* (.X (Math|Vector|BreakVector (* (Variables|Default|GetRandom%20Rotation%20[XYZ]) (Math|Conversions|ToFloat(Boolean) (!= (- (Math|Conversions|ToInteger(Boolean) (Variables|Default|GetRotation%20clamped%20to%20Displacement)) 1) (.AXIS (Utilities|Struct|BreakF_CSVdata _returnvalue_5))))))) -1.0) (.X (Math|Vector|BreakVector (* (Variables|Default|GetRandom%20Rotation%20[XYZ]) (Math|Conversions|ToFloat(Boolean) (!= (- (Math|Conversions|ToInteger(Boolean) (Variables|Default|GetRotation%20clamped%20to%20Displacement)) 1) (.AXIS (Utilities|Struct|BreakF_CSVdata _returnvalue_5))))))) _displacement_randomize) (Math|Random|RandomFloatinRangefromStream (* (.Y (Math|Vector|BreakVector (* (Variables|Default|GetRandom%20Rotation%20[XYZ]) (Math|Conversions|ToFloat(Boolean) (!= (- (Math|Conversions|ToInteger(Boolean) (Variables|Default|GetRotation%20clamped%20to%20Displacement)) 1) (.AXIS (Utilities|Struct|BreakF_CSVdata _returnvalue_5))))))) -1.0) (.Y (Math|Vector|BreakVector (* (Variables|Default|GetRandom%20Rotation%20[XYZ]) (Math|Conversions|ToFloat(Boolean) (!= (- (Math|Conversions|ToInteger(Boolean) (Variables|Default|GetRotation%20clamped%20to%20Displacement)) 1) (.AXIS (Utilities|Struct|BreakF_CSVdata _returnvalue_5))))))) _displacement_randomize) (Math|Random|RandomFloatinRangefromStream (* (.Z (Math|Vector|BreakVector (* (Variables|Default|GetRandom%20Rotation%20[XYZ]) (Math|Conversions|ToFloat(Boolean) (!= (- (Math|Conversions|ToInteger(Boolean) (Variables|Default|GetRotation%20clamped%20to%20Displacement)) 1) (.AXIS (Utilities|Struct|BreakF_CSVdata _returnvalue_5))))))) -1.0) (.Z (Math|Vector|BreakVector (* (Variables|Default|GetRandom%20Rotation%20[XYZ]) (Math|Conversions|ToFloat(Boolean) (!= (- (Math|Conversions|ToInteger(Boolean) (Variables|Default|GetRotation%20clamped%20to%20Displacement)) 1) (.AXIS (Utilities|Struct|BreakF_CSVdata _returnvalue_5))))))) _displacement_randomize)) (Variables|Default|GetShuffle)) (Math|Vector|MakeVector (.R_X (Utilities|Struct|BreakF_CSVdata _returnvalue_5)) (.R_Y (Utilities|Struct|BreakF_CSVdata _returnvalue_5)) (.R_Z (Utilities|Struct|BreakF_CSVdata _returnvalue_5)))))) (.Y (Math|Vector|BreakVector (+ (+ (Math|Vector|MakeVector (Math|Random|RandomFloatinRangefromStream (* (.X (Math|Vector|BreakVector (* (Variables|Default|GetRandom%20Rotation%20[XYZ]) (Math|Conversions|ToFloat(Boolean) (!= (- (Math|Conversions|ToInteger(Boolean) (Variables|Default|GetRotation%20clamped%20to%20Displacement)) 1) (.AXIS (Utilities|Struct|BreakF_CSVdata _returnvalue_5))))))) -1.0) (.X (Math|Vector|BreakVector (* (Variables|Default|GetRandom%20Rotation%20[XYZ]) (Math|Conversions|ToFloat(Boolean) (!= (- (Math|Conversions|ToInteger(Boolean) (Variables|Default|GetRotation%20clamped%20to%20Displacement)) 1) (.AXIS (Utilities|Struct|BreakF_CSVdata _returnvalue_5))))))) _displacement_randomize) (Math|Random|RandomFloatinRangefromStream (* (.Y (Math|Vector|BreakVector (* (Variables|Default|GetRandom%20Rotation%20[XYZ]) (Math|Conversions|ToFloat(Boolean) (!= (- (Math|Conversions|ToInteger(Boolean) (Variables|Default|GetRotation%20clamped%20to%20Displacement)) 1) (.AXIS (Utilities|Struct|BreakF_CSVdata _returnvalue_5))))))) -1.0) (.Y (Math|Vector|BreakVector (* (Variables|Default|GetRandom%20Rotation%20[XYZ]) (Math|Conversions|ToFloat(Boolean) (!= (- (Math|Conversions|ToInteger(Boolean) (Variables|Default|GetRotation%20clamped%20to%20Displacement)) 1) (.AXIS (Utilities|Struct|BreakF_CSVdata _returnvalue_5))))))) _displacement_randomize) (Math|Random|RandomFloatinRangefromStream (* (.Z (Math|Vector|BreakVector (* (Variables|Default|GetRandom%20Rotation%20[XYZ]) (Math|Conversions|ToFloat(Boolean) (!= (- (Math|Conversions|ToInteger(Boolean) (Variables|Default|GetRotation%20clamped%20to%20Displacement)) 1) (.AXIS (Utilities|Struct|BreakF_CSVdata _returnvalue_5))))))) -1.0) (.Z (Math|Vector|BreakVector (* (Variables|Default|GetRandom%20Rotation%20[XYZ]) (Math|Conversions|ToFloat(Boolean) (!= (- (Math|Conversions|ToInteger(Boolean) (Variables|Default|GetRotation%20clamped%20to%20Displacement)) 1) (.AXIS (Utilities|Struct|BreakF_CSVdata _returnvalue_5))))))) _displacement_randomize)) (Variables|Default|GetShuffle)) (Math|Vector|MakeVector (.R_X (Utilities|Struct|BreakF_CSVdata _returnvalue_5)) (.R_Y (Utilities|Struct|BreakF_CSVdata _returnvalue_5)) (.R_Z (Utilities|Struct|BreakF_CSVdata _returnvalue_5)))))) (.Z (Math|Vector|BreakVector (+ (+ (Math|Vector|MakeVector (Math|Random|RandomFloatinRangefromStream (* (.X (Math|Vector|BreakVector (* (Variables|Default|GetRandom%20Rotation%20[XYZ]) (Math|Conversions|ToFloat(Boolean) (!= (- (Math|Conversions|ToInteger(Boolean) (Variables|Default|GetRotation%20clamped%20to%20Displacement)) 1) (.AXIS (Utilities|Struct|BreakF_CSVdata _returnvalue_5))))))) -1.0) (.X (Math|Vector|BreakVector (* (Variables|Default|GetRandom%20Rotation%20[XYZ]) (Math|Conversions|ToFloat(Boolean) (!= (- (Math|Conversions|ToInteger(Boolean) (Variables|Default|GetRotation%20clamped%20to%20Displacement)) 1) (.AXIS (Utilities|Struct|BreakF_CSVdata _returnvalue_5))))))) _displacement_randomize) (Math|Random|RandomFloatinRangefromStream (* (.Y (Math|Vector|BreakVector (* (Variables|Default|GetRandom%20Rotation%20[XYZ]) (Math|Conversions|ToFloat(Boolean) (!= (- (Math|Conversions|ToInteger(Boolean) (Variables|Default|GetRotation%20clamped%20to%20Displacement)) 1) (.AXIS (Utilities|Struct|BreakF_CSVdata _returnvalue_5))))))) -1.0) (.Y (Math|Vector|BreakVector (* (Variables|Default|GetRandom%20Rotation%20[XYZ]) (Math|Conversions|ToFloat(Boolean) (!= (- (Math|Conversions|ToInteger(Boolean) (Variables|Default|GetRotation%20clamped%20to%20Displacement)) 1) (.AXIS (Utilities|Struct|BreakF_CSVdata _returnvalue_5))))))) _displacement_randomize) (Math|Random|RandomFloatinRangefromStream (* (.Z (Math|Vector|BreakVector (* (Variables|Default|GetRandom%20Rotation%20[XYZ]) (Math|Conversions|ToFloat(Boolean) (!= (- (Math|Conversions|ToInteger(Boolean) (Variables|Default|GetRotation%20clamped%20to%20Displacement)) 1) (.AXIS (Utilities|Struct|BreakF_CSVdata _returnvalue_5))))))) -1.0) (.Z (Math|Vector|BreakVector (* (Variables|Default|GetRandom%20Rotation%20[XYZ]) (Math|Conversions|ToFloat(Boolean) (!= (- (Math|Conversions|ToInteger(Boolean) (Variables|Default|GetRotation%20clamped%20to%20Displacement)) 1) (.AXIS (Utilities|Struct|BreakF_CSVdata _returnvalue_5))))))) _displacement_randomize)) (Variables|Default|GetShuffle)) (Math|Vector|MakeVector (.R_X (Utilities|Struct|BreakF_CSVdata _returnvalue_5)) (.R_Y (Utilities|Struct|BreakF_CSVdata _returnvalue_5)) (.R_Z (Utilities|Struct|BreakF_CSVdata _returnvalue_5))))))) (Math|Conversions|ToFloat(Boolean) (Variables|Default|GetRandom%20Rotation%20LOCAL/GLOBAL))) (* (Math|Vector|MakeVector (.S_X (Utilities|Struct|BreakF_CSVdata _returnvalue_5)) (.S_Y (Utilities|Struct|BreakF_CSVdata _returnvalue_5)) (.S_Z (Utilities|Struct|BreakF_CSVdata _returnvalue_5))) (Variables|Default|GetScale))) false))))
                          (:Out%201
                            (Utilities|FlowControl|Sequence :!label _label_4
                              (:then_0
                                (Utilities|FlowControl|DoOnce false
                                  (:Completed
                                    (bind _returnvalue_8 (AddComponent|AddHierarchicalInstancedStaticMeshComponent false))
                                    (bind _output_get_3 (Variables|Default|Set02 _returnvalue_8))
                                    (Rendering|Material|SetMaterial _output_get_3 0 (Variables|Default|GetStone%20Material)))))
                              (:then_1
                                (Components|InstancedStaticMesh|AddInstance (Variables|Default|Get02) (Math|Transform|MakeTransform (Math|Transform|TransformLocation (Math|Transform|MakeTransform (Math|Vector|MakeVector (.T_X (Utilities|Struct|BreakF_CSVdata _returnvalue_5)) (.T_Y (Utilities|Struct|BreakF_CSVdata _returnvalue_5)) (.T_Z (Utilities|Struct|BreakF_CSVdata _returnvalue_5))) (Math|Rotator|Lerp(Rotator) (Math|Rotator|CombineRotators (Math|Rotator|MakeRotator (.X (Math|Vector|BreakVector (+ (Math|Vector|MakeVector (Math|Random|RandomFloatinRangefromStream (* (.X (Math|Vector|BreakVector (* (Variables|Default|GetRandom%20Rotation%20[XYZ]) (Math|Conversions|ToFloat(Boolean) (!= (- (Math|Conversions|ToInteger(Boolean) (Variables|Default|GetRotation%20clamped%20to%20Displacement)) 1) (.AXIS (Utilities|Struct|BreakF_CSVdata _returnvalue_5))))))) -1.0) (.X (Math|Vector|BreakVector (* (Variables|Default|GetRandom%20Rotation%20[XYZ]) (Math|Conversions|ToFloat(Boolean) (!= (- (Math|Conversions|ToInteger(Boolean) (Variables|Default|GetRotation%20clamped%20to%20Displacement)) 1) (.AXIS (Utilities|Struct|BreakF_CSVdata _returnvalue_5))))))) _displacement_randomize) (Math|Random|RandomFloatinRangefromStream (* (.Y (Math|Vector|BreakVector (* (Variables|Default|GetRandom%20Rotation%20[XYZ]) (Math|Conversions|ToFloat(Boolean) (!= (- (Math|Conversions|ToInteger(Boolean) (Variables|Default|GetRotation%20clamped%20to%20Displacement)) 1) (.AXIS (Utilities|Struct|BreakF_CSVdata _returnvalue_5))))))) -1.0) (.Y (Math|Vector|BreakVector (* (Variables|Default|GetRandom%20Rotation%20[XYZ]) (Math|Conversions|ToFloat(Boolean) (!= (- (Math|Conversions|ToInteger(Boolean) (Variables|Default|GetRotation%20clamped%20to%20Displacement)) 1) (.AXIS (Utilities|Struct|BreakF_CSVdata _returnvalue_5))))))) _displacement_randomize) (Math|Random|RandomFloatinRangefromStream (* (.Z (Math|Vector|BreakVector (* (Variables|Default|GetRandom%20Rotation%20[XYZ]) (Math|Conversions|ToFloat(Boolean) (!= (- (Math|Conversions|ToInteger(Boolean) (Variables|Default|GetRotation%20clamped%20to%20Displacement)) 1) (.AXIS (Utilities|Struct|BreakF_CSVdata _returnvalue_5))))))) -1.0) (.Z (Math|Vector|BreakVector (* (Variables|Default|GetRandom%20Rotation%20[XYZ]) (Math|Conversions|ToFloat(Boolean) (!= (- (Math|Conversions|ToInteger(Boolean) (Variables|Default|GetRotation%20clamped%20to%20Displacement)) 1) (.AXIS (Utilities|Struct|BreakF_CSVdata _returnvalue_5))))))) _displacement_randomize)) (Variables|Default|GetShuffle)))) (.Y (Math|Vector|BreakVector (+ (Math|Vector|MakeVector (Math|Random|RandomFloatinRangefromStream (* (.X (Math|Vector|BreakVector (* (Variables|Default|GetRandom%20Rotation%20[XYZ]) (Math|Conversions|ToFloat(Boolean) (!= (- (Math|Conversions|ToInteger(Boolean) (Variables|Default|GetRotation%20clamped%20to%20Displacement)) 1) (.AXIS (Utilities|Struct|BreakF_CSVdata _returnvalue_5))))))) -1.0) (.X (Math|Vector|BreakVector (* (Variables|Default|GetRandom%20Rotation%20[XYZ]) (Math|Conversions|ToFloat(Boolean) (!= (- (Math|Conversions|ToInteger(Boolean) (Variables|Default|GetRotation%20clamped%20to%20Displacement)) 1) (.AXIS (Utilities|Struct|BreakF_CSVdata _returnvalue_5))))))) _displacement_randomize) (Math|Random|RandomFloatinRangefromStream (* (.Y (Math|Vector|BreakVector (* (Variables|Default|GetRandom%20Rotation%20[XYZ]) (Math|Conversions|ToFloat(Boolean) (!= (- (Math|Conversions|ToInteger(Boolean) (Variables|Default|GetRotation%20clamped%20to%20Displacement)) 1) (.AXIS (Utilities|Struct|BreakF_CSVdata _returnvalue_5))))))) -1.0) (.Y (Math|Vector|BreakVector (* (Variables|Default|GetRandom%20Rotation%20[XYZ]) (Math|Conversions|ToFloat(Boolean) (!= (- (Math|Conversions|ToInteger(Boolean) (Variables|Default|GetRotation%20clamped%20to%20Displacement)) 1) (.AXIS (Utilities|Struct|BreakF_CSVdata _returnvalue_5))))))) _displacement_randomize) (Math|Random|RandomFloatinRangefromStream (* (.Z (Math|Vector|BreakVector (* (Variables|Default|GetRandom%20Rotation%20[XYZ]) (Math|Conversions|ToFloat(Boolean) (!= (- (Math|Conversions|ToInteger(Boolean) (Variables|Default|GetRotation%20clamped%20to%20Displacement)) 1) (.AXIS (Utilities|Struct|BreakF_CSVdata _returnvalue_5))))))) -1.0) (.Z (Math|Vector|BreakVector (* (Variables|Default|GetRandom%20Rotation%20[XYZ]) (Math|Conversions|ToFloat(Boolean) (!= (- (Math|Conversions|ToInteger(Boolean) (Variables|Default|GetRotation%20clamped%20to%20Displacement)) 1) (.AXIS (Utilities|Struct|BreakF_CSVdata _returnvalue_5))))))) _displacement_randomize)) (Variables|Default|GetShuffle)))) (.Z (Math|Vector|BreakVector (+ (Math|Vector|MakeVector (Math|Random|RandomFloatinRangefromStream (* (.X (Math|Vector|BreakVector (* (Variables|Default|GetRandom%20Rotation%20[XYZ]) (Math|Conversions|ToFloat(Boolean) (!= (- (Math|Conversions|ToInteger(Boolean) (Variables|Default|GetRotation%20clamped%20to%20Displacement)) 1) (.AXIS (Utilities|Struct|BreakF_CSVdata _returnvalue_5))))))) -1.0) (.X (Math|Vector|BreakVector (* (Variables|Default|GetRandom%20Rotation%20[XYZ]) (Math|Conversions|ToFloat(Boolean) (!= (- (Math|Conversions|ToInteger(Boolean) (Variables|Default|GetRotation%20clamped%20to%20Displacement)) 1) (.AXIS (Utilities|Struct|BreakF_CSVdata _returnvalue_5))))))) _displacement_randomize) (Math|Random|RandomFloatinRangefromStream (* (.Y (Math|Vector|BreakVector (* (Variables|Default|GetRandom%20Rotation%20[XYZ]) (Math|Conversions|ToFloat(Boolean) (!= (- (Math|Conversions|ToInteger(Boolean) (Variables|Default|GetRotation%20clamped%20to%20Displacement)) 1) (.AXIS (Utilities|Struct|BreakF_CSVdata _returnvalue_5))))))) -1.0) (.Y (Math|Vector|BreakVector (* (Variables|Default|GetRandom%20Rotation%20[XYZ]) (Math|Conversions|ToFloat(Boolean) (!= (- (Math|Conversions|ToInteger(Boolean) (Variables|Default|GetRotation%20clamped%20to%20Displacement)) 1) (.AXIS (Utilities|Struct|BreakF_CSVdata _returnvalue_5))))))) _displacement_randomize) (Math|Random|RandomFloatinRangefromStream (* (.Z (Math|Vector|BreakVector (* (Variables|Default|GetRandom%20Rotation%20[XYZ]) (Math|Conversions|ToFloat(Boolean) (!= (- (Math|Conversions|ToInteger(Boolean) (Variables|Default|GetRotation%20clamped%20to%20Displacement)) 1) (.AXIS (Utilities|Struct|BreakF_CSVdata _returnvalue_5))))))) -1.0) (.Z (Math|Vector|BreakVector (* (Variables|Default|GetRandom%20Rotation%20[XYZ]) (Math|Conversions|ToFloat(Boolean) (!= (- (Math|Conversions|ToInteger(Boolean) (Variables|Default|GetRotation%20clamped%20to%20Displacement)) 1) (.AXIS (Utilities|Struct|BreakF_CSVdata _returnvalue_5))))))) _displacement_randomize)) (Variables|Default|GetShuffle))))) (Math|Rotator|MakeRotator (.R_X (Utilities|Struct|BreakF_CSVdata _returnvalue_5)) (.R_Y (Utilities|Struct|BreakF_CSVdata _returnvalue_5)) (.R_Z (Utilities|Struct|BreakF_CSVdata _returnvalue_5)))) (Math|Rotator|MakeRotator (.X (Math|Vector|BreakVector (+ (+ (Math|Vector|MakeVector (Math|Random|RandomFloatinRangefromStream (* (.X (Math|Vector|BreakVector (* (Variables|Default|GetRandom%20Rotation%20[XYZ]) (Math|Conversions|ToFloat(Boolean) (!= (- (Math|Conversions|ToInteger(Boolean) (Variables|Default|GetRotation%20clamped%20to%20Displacement)) 1) (.AXIS (Utilities|Struct|BreakF_CSVdata _returnvalue_5))))))) -1.0) (.X (Math|Vector|BreakVector (* (Variables|Default|GetRandom%20Rotation%20[XYZ]) (Math|Conversions|ToFloat(Boolean) (!= (- (Math|Conversions|ToInteger(Boolean) (Variables|Default|GetRotation%20clamped%20to%20Displacement)) 1) (.AXIS (Utilities|Struct|BreakF_CSVdata _returnvalue_5))))))) _displacement_randomize) (Math|Random|RandomFloatinRangefromStream (* (.Y (Math|Vector|BreakVector (* (Variables|Default|GetRandom%20Rotation%20[XYZ]) (Math|Conversions|ToFloat(Boolean) (!= (- (Math|Conversions|ToInteger(Boolean) (Variables|Default|GetRotation%20clamped%20to%20Displacement)) 1) (.AXIS (Utilities|Struct|BreakF_CSVdata _returnvalue_5))))))) -1.0) (.Y (Math|Vector|BreakVector (* (Variables|Default|GetRandom%20Rotation%20[XYZ]) (Math|Conversions|ToFloat(Boolean) (!= (- (Math|Conversions|ToInteger(Boolean) (Variables|Default|GetRotation%20clamped%20to%20Displacement)) 1) (.AXIS (Utilities|Struct|BreakF_CSVdata _returnvalue_5))))))) _displacement_randomize) (Math|Random|RandomFloatinRangefromStream (* (.Z (Math|Vector|BreakVector (* (Variables|Default|GetRandom%20Rotation%20[XYZ]) (Math|Conversions|ToFloat(Boolean) (!= (- (Math|Conversions|ToInteger(Boolean) (Variables|Default|GetRotation%20clamped%20to%20Displacement)) 1) (.AXIS (Utilities|Struct|BreakF_CSVdata _returnvalue_5))))))) -1.0) (.Z (Math|Vector|BreakVector (* (Variables|Default|GetRandom%20Rotation%20[XYZ]) (Math|Conversions|ToFloat(Boolean) (!= (- (Math|Conversions|ToInteger(Boolean) (Variables|Default|GetRotation%20clamped%20to%20Displacement)) 1) (.AXIS (Utilities|Struct|BreakF_CSVdata _returnvalue_5))))))) _displacement_randomize)) (Variables|Default|GetShuffle)) (Math|Vector|MakeVector (.R_X (Utilities|Struct|BreakF_CSVdata _returnvalue_5)) (.R_Y (Utilities|Struct|BreakF_CSVdata _returnvalue_5)) (.R_Z (Utilities|Struct|BreakF_CSVdata _returnvalue_5)))))) (.Y (Math|Vector|BreakVector (+ (+ (Math|Vector|MakeVector (Math|Random|RandomFloatinRangefromStream (* (.X (Math|Vector|BreakVector (* (Variables|Default|GetRandom%20Rotation%20[XYZ]) (Math|Conversions|ToFloat(Boolean) (!= (- (Math|Conversions|ToInteger(Boolean) (Variables|Default|GetRotation%20clamped%20to%20Displacement)) 1) (.AXIS (Utilities|Struct|BreakF_CSVdata _returnvalue_5))))))) -1.0) (.X (Math|Vector|BreakVector (* (Variables|Default|GetRandom%20Rotation%20[XYZ]) (Math|Conversions|ToFloat(Boolean) (!= (- (Math|Conversions|ToInteger(Boolean) (Variables|Default|GetRotation%20clamped%20to%20Displacement)) 1) (.AXIS (Utilities|Struct|BreakF_CSVdata _returnvalue_5))))))) _displacement_randomize) (Math|Random|RandomFloatinRangefromStream (* (.Y (Math|Vector|BreakVector (* (Variables|Default|GetRandom%20Rotation%20[XYZ]) (Math|Conversions|ToFloat(Boolean) (!= (- (Math|Conversions|ToInteger(Boolean) (Variables|Default|GetRotation%20clamped%20to%20Displacement)) 1) (.AXIS (Utilities|Struct|BreakF_CSVdata _returnvalue_5))))))) -1.0) (.Y (Math|Vector|BreakVector (* (Variables|Default|GetRandom%20Rotation%20[XYZ]) (Math|Conversions|ToFloat(Boolean) (!= (- (Math|Conversions|ToInteger(Boolean) (Variables|Default|GetRotation%20clamped%20to%20Displacement)) 1) (.AXIS (Utilities|Struct|BreakF_CSVdata _returnvalue_5))))))) _displacement_randomize) (Math|Random|RandomFloatinRangefromStream (* (.Z (Math|Vector|BreakVector (* (Variables|Default|GetRandom%20Rotation%20[XYZ]) (Math|Conversions|ToFloat(Boolean) (!= (- (Math|Conversions|ToInteger(Boolean) (Variables|Default|GetRotation%20clamped%20to%20Displacement)) 1) (.AXIS (Utilities|Struct|BreakF_CSVdata _returnvalue_5))))))) -1.0) (.Z (Math|Vector|BreakVector (* (Variables|Default|GetRandom%20Rotation%20[XYZ]) (Math|Conversions|ToFloat(Boolean) (!= (- (Math|Conversions|ToInteger(Boolean) (Variables|Default|GetRotation%20clamped%20to%20Displacement)) 1) (.AXIS (Utilities|Struct|BreakF_CSVdata _returnvalue_5))))))) _displacement_randomize)) (Variables|Default|GetShuffle)) (Math|Vector|MakeVector (.R_X (Utilities|Struct|BreakF_CSVdata _returnvalue_5)) (.R_Y (Utilities|Struct|BreakF_CSVdata _returnvalue_5)) (.R_Z (Utilities|Struct|BreakF_CSVdata _returnvalue_5)))))) (.Z (Math|Vector|BreakVector (+ (+ (Math|Vector|MakeVector (Math|Random|RandomFloatinRangefromStream (* (.X (Math|Vector|BreakVector (* (Variables|Default|GetRandom%20Rotation%20[XYZ]) (Math|Conversions|ToFloat(Boolean) (!= (- (Math|Conversions|ToInteger(Boolean) (Variables|Default|GetRotation%20clamped%20to%20Displacement)) 1) (.AXIS (Utilities|Struct|BreakF_CSVdata _returnvalue_5))))))) -1.0) (.X (Math|Vector|BreakVector (* (Variables|Default|GetRandom%20Rotation%20[XYZ]) (Math|Conversions|ToFloat(Boolean) (!= (- (Math|Conversions|ToInteger(Boolean) (Variables|Default|GetRotation%20clamped%20to%20Displacement)) 1) (.AXIS (Utilities|Struct|BreakF_CSVdata _returnvalue_5))))))) _displacement_randomize) (Math|Random|RandomFloatinRangefromStream (* (.Y (Math|Vector|BreakVector (* (Variables|Default|GetRandom%20Rotation%20[XYZ]) (Math|Conversions|ToFloat(Boolean) (!= (- (Math|Conversions|ToInteger(Boolean) (Variables|Default|GetRotation%20clamped%20to%20Displacement)) 1) (.AXIS (Utilities|Struct|BreakF_CSVdata _returnvalue_5))))))) -1.0) (.Y (Math|Vector|BreakVector (* (Variables|Default|GetRandom%20Rotation%20[XYZ]) (Math|Conversions|ToFloat(Boolean) (!= (- (Math|Conversions|ToInteger(Boolean) (Variables|Default|GetRotation%20clamped%20to%20Displacement)) 1) (.AXIS (Utilities|Struct|BreakF_CSVdata _returnvalue_5))))))) _displacement_randomize) (Math|Random|RandomFloatinRangefromStream (* (.Z (Math|Vector|BreakVector (* (Variables|Default|GetRandom%20Rotation%20[XYZ]) (Math|Conversions|ToFloat(Boolean) (!= (- (Math|Conversions|ToInteger(Boolean) (Variables|Default|GetRotation%20clamped%20to%20Displacement)) 1) (.AXIS (Utilities|Struct|BreakF_CSVdata _returnvalue_5))))))) -1.0) (.Z (Math|Vector|BreakVector (* (Variables|Default|GetRandom%20Rotation%20[XYZ]) (Math|Conversions|ToFloat(Boolean) (!= (- (Math|Conversions|ToInteger(Boolean) (Variables|Default|GetRotation%20clamped%20to%20Displacement)) 1) (.AXIS (Utilities|Struct|BreakF_CSVdata _returnvalue_5))))))) _displacement_randomize)) (Variables|Default|GetShuffle)) (Math|Vector|MakeVector (.R_X (Utilities|Struct|BreakF_CSVdata _returnvalue_5)) (.R_Y (Utilities|Struct|BreakF_CSVdata _returnvalue_5)) (.R_Z (Utilities|Struct|BreakF_CSVdata _returnvalue_5))))))) (Math|Conversions|ToFloat(Boolean) (Variables|Default|GetRandom%20Rotation%20LOCAL/GLOBAL))) (* (Math|Vector|MakeVector (.S_X (Utilities|Struct|BreakF_CSVdata _returnvalue_5)) (.S_Y (Utilities|Struct|BreakF_CSVdata _returnvalue_5)) (.S_Z (Utilities|Struct|BreakF_CSVdata _returnvalue_5))) (Variables|Default|GetScale))) (* (Math|Vector|MakeVector (* (Math|Conversions|ToFloat(Boolean) (== (.AXIS (Utilities|Struct|BreakF_CSVdata _returnvalue_5)) 1)) _returnvalue_3) (* (Math|Conversions|ToFloat(Boolean) (== (.AXIS (Utilities|Struct|BreakF_CSVdata _returnvalue_5)) 2)) _returnvalue_3) (* (Math|Conversions|ToFloat(Boolean) (== (.AXIS (Utilities|Struct|BreakF_CSVdata _returnvalue_5)) 3)) _returnvalue_3)) (Math|Float|Clamp(Float) (+ (Math|Conversions|ToFloat(Boolean) (and (not (Class|KismetMathLibrary|IsPointinBoxwithTransform (Math|Vector|MakeVector (.T_X (Utilities|Struct|BreakF_CSVdata _returnvalue_5)) (.T_Y (Utilities|Struct|BreakF_CSVdata _returnvalue_5)) (.T_Z (Utilities|Struct|BreakF_CSVdata _returnvalue_5))) (Math|Transform|MakeTransform (Variables|Default|GetBox%20Origin%20[XYZ]) (Variables|Default|GetBox%20Rotation%20[XYZ])) (Variables|Default|GetBox%20Extent%20[XYZ]))) _boxcontrolleddisplacement)) (Variables|Default|GetBox%20Intensity)) (Math|Conversions|ToFloat(Boolean) (not _boxcontrolleddisplacement))))) (Math|Rotator|Lerp(Rotator) (Math|Rotator|CombineRotators (Math|Rotator|MakeRotator (.X (Math|Vector|BreakVector (+ (Math|Vector|MakeVector (Math|Random|RandomFloatinRangefromStream (* (.X (Math|Vector|BreakVector (* (Variables|Default|GetRandom%20Rotation%20[XYZ]) (Math|Conversions|ToFloat(Boolean) (!= (- (Math|Conversions|ToInteger(Boolean) (Variables|Default|GetRotation%20clamped%20to%20Displacement)) 1) (.AXIS (Utilities|Struct|BreakF_CSVdata _returnvalue_5))))))) -1.0) (.X (Math|Vector|BreakVector (* (Variables|Default|GetRandom%20Rotation%20[XYZ]) (Math|Conversions|ToFloat(Boolean) (!= (- (Math|Conversions|ToInteger(Boolean) (Variables|Default|GetRotation%20clamped%20to%20Displacement)) 1) (.AXIS (Utilities|Struct|BreakF_CSVdata _returnvalue_5))))))) _displacement_randomize) (Math|Random|RandomFloatinRangefromStream (* (.Y (Math|Vector|BreakVector (* (Variables|Default|GetRandom%20Rotation%20[XYZ]) (Math|Conversions|ToFloat(Boolean) (!= (- (Math|Conversions|ToInteger(Boolean) (Variables|Default|GetRotation%20clamped%20to%20Displacement)) 1) (.AXIS (Utilities|Struct|BreakF_CSVdata _returnvalue_5))))))) -1.0) (.Y (Math|Vector|BreakVector (* (Variables|Default|GetRandom%20Rotation%20[XYZ]) (Math|Conversions|ToFloat(Boolean) (!= (- (Math|Conversions|ToInteger(Boolean) (Variables|Default|GetRotation%20clamped%20to%20Displacement)) 1) (.AXIS (Utilities|Struct|BreakF_CSVdata _returnvalue_5))))))) _displacement_randomize) (Math|Random|RandomFloatinRangefromStream (* (.Z (Math|Vector|BreakVector (* (Variables|Default|GetRandom%20Rotation%20[XYZ]) (Math|Conversions|ToFloat(Boolean) (!= (- (Math|Conversions|ToInteger(Boolean) (Variables|Default|GetRotation%20clamped%20to%20Displacement)) 1) (.AXIS (Utilities|Struct|BreakF_CSVdata _returnvalue_5))))))) -1.0) (.Z (Math|Vector|BreakVector (* (Variables|Default|GetRandom%20Rotation%20[XYZ]) (Math|Conversions|ToFloat(Boolean) (!= (- (Math|Conversions|ToInteger(Boolean) (Variables|Default|GetRotation%20clamped%20to%20Displacement)) 1) (.AXIS (Utilities|Struct|BreakF_CSVdata _returnvalue_5))))))) _displacement_randomize)) (Variables|Default|GetShuffle)))) (.Y (Math|Vector|BreakVector (+ (Math|Vector|MakeVector (Math|Random|RandomFloatinRangefromStream (* (.X (Math|Vector|BreakVector (* (Variables|Default|GetRandom%20Rotation%20[XYZ]) (Math|Conversions|ToFloat(Boolean) (!= (- (Math|Conversions|ToInteger(Boolean) (Variables|Default|GetRotation%20clamped%20to%20Displacement)) 1) (.AXIS (Utilities|Struct|BreakF_CSVdata _returnvalue_5))))))) -1.0) (.X (Math|Vector|BreakVector (* (Variables|Default|GetRandom%20Rotation%20[XYZ]) (Math|Conversions|ToFloat(Boolean) (!= (- (Math|Conversions|ToInteger(Boolean) (Variables|Default|GetRotation%20clamped%20to%20Displacement)) 1) (.AXIS (Utilities|Struct|BreakF_CSVdata _returnvalue_5))))))) _displacement_randomize) (Math|Random|RandomFloatinRangefromStream (* (.Y (Math|Vector|BreakVector (* (Variables|Default|GetRandom%20Rotation%20[XYZ]) (Math|Conversions|ToFloat(Boolean) (!= (- (Math|Conversions|ToInteger(Boolean) (Variables|Default|GetRotation%20clamped%20to%20Displacement)) 1) (.AXIS (Utilities|Struct|BreakF_CSVdata _returnvalue_5))))))) -1.0) (.Y (Math|Vector|BreakVector (* (Variables|Default|GetRandom%20Rotation%20[XYZ]) (Math|Conversions|ToFloat(Boolean) (!= (- (Math|Conversions|ToInteger(Boolean) (Variables|Default|GetRotation%20clamped%20to%20Displacement)) 1) (.AXIS (Utilities|Struct|BreakF_CSVdata _returnvalue_5))))))) _displacement_randomize) (Math|Random|RandomFloatinRangefromStream (* (.Z (Math|Vector|BreakVector (* (Variables|Default|GetRandom%20Rotation%20[XYZ]) (Math|Conversions|ToFloat(Boolean) (!= (- (Math|Conversions|ToInteger(Boolean) (Variables|Default|GetRotation%20clamped%20to%20Displacement)) 1) (.AXIS (Utilities|Struct|BreakF_CSVdata _returnvalue_5))))))) -1.0) (.Z (Math|Vector|BreakVector (* (Variables|Default|GetRandom%20Rotation%20[XYZ]) (Math|Conversions|ToFloat(Boolean) (!= (- (Math|Conversions|ToInteger(Boolean) (Variables|Default|GetRotation%20clamped%20to%20Displacement)) 1) (.AXIS (Utilities|Struct|BreakF_CSVdata _returnvalue_5))))))) _displacement_randomize)) (Variables|Default|GetShuffle)))) (.Z (Math|Vector|BreakVector (+ (Math|Vector|MakeVector (Math|Random|RandomFloatinRangefromStream (* (.X (Math|Vector|BreakVector (* (Variables|Default|GetRandom%20Rotation%20[XYZ]) (Math|Conversions|ToFloat(Boolean) (!= (- (Math|Conversions|ToInteger(Boolean) (Variables|Default|GetRotation%20clamped%20to%20Displacement)) 1) (.AXIS (Utilities|Struct|BreakF_CSVdata _returnvalue_5))))))) -1.0) (.X (Math|Vector|BreakVector (* (Variables|Default|GetRandom%20Rotation%20[XYZ]) (Math|Conversions|ToFloat(Boolean) (!= (- (Math|Conversions|ToInteger(Boolean) (Variables|Default|GetRotation%20clamped%20to%20Displacement)) 1) (.AXIS (Utilities|Struct|BreakF_CSVdata _returnvalue_5))))))) _displacement_randomize) (Math|Random|RandomFloatinRangefromStream (* (.Y (Math|Vector|BreakVector (* (Variables|Default|GetRandom%20Rotation%20[XYZ]) (Math|Conversions|ToFloat(Boolean) (!= (- (Math|Conversions|ToInteger(Boolean) (Variables|Default|GetRotation%20clamped%20to%20Displacement)) 1) (.AXIS (Utilities|Struct|BreakF_CSVdata _returnvalue_5))))))) -1.0) (.Y (Math|Vector|BreakVector (* (Variables|Default|GetRandom%20Rotation%20[XYZ]) (Math|Conversions|ToFloat(Boolean) (!= (- (Math|Conversions|ToInteger(Boolean) (Variables|Default|GetRotation%20clamped%20to%20Displacement)) 1) (.AXIS (Utilities|Struct|BreakF_CSVdata _returnvalue_5))))))) _displacement_randomize) (Math|Random|RandomFloatinRangefromStream (* (.Z (Math|Vector|BreakVector (* (Variables|Default|GetRandom%20Rotation%20[XYZ]) (Math|Conversions|ToFloat(Boolean) (!= (- (Math|Conversions|ToInteger(Boolean) (Variables|Default|GetRotation%20clamped%20to%20Displacement)) 1) (.AXIS (Utilities|Struct|BreakF_CSVdata _returnvalue_5))))))) -1.0) (.Z (Math|Vector|BreakVector (* (Variables|Default|GetRandom%20Rotation%20[XYZ]) (Math|Conversions|ToFloat(Boolean) (!= (- (Math|Conversions|ToInteger(Boolean) (Variables|Default|GetRotation%20clamped%20to%20Displacement)) 1) (.AXIS (Utilities|Struct|BreakF_CSVdata _returnvalue_5))))))) _displacement_randomize)) (Variables|Default|GetShuffle))))) (Math|Rotator|MakeRotator (.R_X (Utilities|Struct|BreakF_CSVdata _returnvalue_5)) (.R_Y (Utilities|Struct|BreakF_CSVdata _returnvalue_5)) (.R_Z (Utilities|Struct|BreakF_CSVdata _returnvalue_5)))) (Math|Rotator|MakeRotator (.X (Math|Vector|BreakVector (+ (+ (Math|Vector|MakeVector (Math|Random|RandomFloatinRangefromStream (* (.X (Math|Vector|BreakVector (* (Variables|Default|GetRandom%20Rotation%20[XYZ]) (Math|Conversions|ToFloat(Boolean) (!= (- (Math|Conversions|ToInteger(Boolean) (Variables|Default|GetRotation%20clamped%20to%20Displacement)) 1) (.AXIS (Utilities|Struct|BreakF_CSVdata _returnvalue_5))))))) -1.0) (.X (Math|Vector|BreakVector (* (Variables|Default|GetRandom%20Rotation%20[XYZ]) (Math|Conversions|ToFloat(Boolean) (!= (- (Math|Conversions|ToInteger(Boolean) (Variables|Default|GetRotation%20clamped%20to%20Displacement)) 1) (.AXIS (Utilities|Struct|BreakF_CSVdata _returnvalue_5))))))) _displacement_randomize) (Math|Random|RandomFloatinRangefromStream (* (.Y (Math|Vector|BreakVector (* (Variables|Default|GetRandom%20Rotation%20[XYZ]) (Math|Conversions|ToFloat(Boolean) (!= (- (Math|Conversions|ToInteger(Boolean) (Variables|Default|GetRotation%20clamped%20to%20Displacement)) 1) (.AXIS (Utilities|Struct|BreakF_CSVdata _returnvalue_5))))))) -1.0) (.Y (Math|Vector|BreakVector (* (Variables|Default|GetRandom%20Rotation%20[XYZ]) (Math|Conversions|ToFloat(Boolean) (!= (- (Math|Conversions|ToInteger(Boolean) (Variables|Default|GetRotation%20clamped%20to%20Displacement)) 1) (.AXIS (Utilities|Struct|BreakF_CSVdata _returnvalue_5))))))) _displacement_randomize) (Math|Random|RandomFloatinRangefromStream (* (.Z (Math|Vector|BreakVector (* (Variables|Default|GetRandom%20Rotation%20[XYZ]) (Math|Conversions|ToFloat(Boolean) (!= (- (Math|Conversions|ToInteger(Boolean) (Variables|Default|GetRotation%20clamped%20to%20Displacement)) 1) (.AXIS (Utilities|Struct|BreakF_CSVdata _returnvalue_5))))))) -1.0) (.Z (Math|Vector|BreakVector (* (Variables|Default|GetRandom%20Rotation%20[XYZ]) (Math|Conversions|ToFloat(Boolean) (!= (- (Math|Conversions|ToInteger(Boolean) (Variables|Default|GetRotation%20clamped%20to%20Displacement)) 1) (.AXIS (Utilities|Struct|BreakF_CSVdata _returnvalue_5))))))) _displacement_randomize)) (Variables|Default|GetShuffle)) (Math|Vector|MakeVector (.R_X (Utilities|Struct|BreakF_CSVdata _returnvalue_5)) (.R_Y (Utilities|Struct|BreakF_CSVdata _returnvalue_5)) (.R_Z (Utilities|Struct|BreakF_CSVdata _returnvalue_5)))))) (.Y (Math|Vector|BreakVector (+ (+ (Math|Vector|MakeVector (Math|Random|RandomFloatinRangefromStream (* (.X (Math|Vector|BreakVector (* (Variables|Default|GetRandom%20Rotation%20[XYZ]) (Math|Conversions|ToFloat(Boolean) (!= (- (Math|Conversions|ToInteger(Boolean) (Variables|Default|GetRotation%20clamped%20to%20Displacement)) 1) (.AXIS (Utilities|Struct|BreakF_CSVdata _returnvalue_5))))))) -1.0) (.X (Math|Vector|BreakVector (* (Variables|Default|GetRandom%20Rotation%20[XYZ]) (Math|Conversions|ToFloat(Boolean) (!= (- (Math|Conversions|ToInteger(Boolean) (Variables|Default|GetRotation%20clamped%20to%20Displacement)) 1) (.AXIS (Utilities|Struct|BreakF_CSVdata _returnvalue_5))))))) _displacement_randomize) (Math|Random|RandomFloatinRangefromStream (* (.Y (Math|Vector|BreakVector (* (Variables|Default|GetRandom%20Rotation%20[XYZ]) (Math|Conversions|ToFloat(Boolean) (!= (- (Math|Conversions|ToInteger(Boolean) (Variables|Default|GetRotation%20clamped%20to%20Displacement)) 1) (.AXIS (Utilities|Struct|BreakF_CSVdata _returnvalue_5))))))) -1.0) (.Y (Math|Vector|BreakVector (* (Variables|Default|GetRandom%20Rotation%20[XYZ]) (Math|Conversions|ToFloat(Boolean) (!= (- (Math|Conversions|ToInteger(Boolean) (Variables|Default|GetRotation%20clamped%20to%20Displacement)) 1) (.AXIS (Utilities|Struct|BreakF_CSVdata _returnvalue_5))))))) _displacement_randomize) (Math|Random|RandomFloatinRangefromStream (* (.Z (Math|Vector|BreakVector (* (Variables|Default|GetRandom%20Rotation%20[XYZ]) (Math|Conversions|ToFloat(Boolean) (!= (- (Math|Conversions|ToInteger(Boolean) (Variables|Default|GetRotation%20clamped%20to%20Displacement)) 1) (.AXIS (Utilities|Struct|BreakF_CSVdata _returnvalue_5))))))) -1.0) (.Z (Math|Vector|BreakVector (* (Variables|Default|GetRandom%20Rotation%20[XYZ]) (Math|Conversions|ToFloat(Boolean) (!= (- (Math|Conversions|ToInteger(Boolean) (Variables|Default|GetRotation%20clamped%20to%20Displacement)) 1) (.AXIS (Utilities|Struct|BreakF_CSVdata _returnvalue_5))))))) _displacement_randomize)) (Variables|Default|GetShuffle)) (Math|Vector|MakeVector (.R_X (Utilities|Struct|BreakF_CSVdata _returnvalue_5)) (.R_Y (Utilities|Struct|BreakF_CSVdata _returnvalue_5)) (.R_Z (Utilities|Struct|BreakF_CSVdata _returnvalue_5)))))) (.Z (Math|Vector|BreakVector (+ (+ (Math|Vector|MakeVector (Math|Random|RandomFloatinRangefromStream (* (.X (Math|Vector|BreakVector (* (Variables|Default|GetRandom%20Rotation%20[XYZ]) (Math|Conversions|ToFloat(Boolean) (!= (- (Math|Conversions|ToInteger(Boolean) (Variables|Default|GetRotation%20clamped%20to%20Displacement)) 1) (.AXIS (Utilities|Struct|BreakF_CSVdata _returnvalue_5))))))) -1.0) (.X (Math|Vector|BreakVector (* (Variables|Default|GetRandom%20Rotation%20[XYZ]) (Math|Conversions|ToFloat(Boolean) (!= (- (Math|Conversions|ToInteger(Boolean) (Variables|Default|GetRotation%20clamped%20to%20Displacement)) 1) (.AXIS (Utilities|Struct|BreakF_CSVdata _returnvalue_5))))))) _displacement_randomize) (Math|Random|RandomFloatinRangefromStream (* (.Y (Math|Vector|BreakVector (* (Variables|Default|GetRandom%20Rotation%20[XYZ]) (Math|Conversions|ToFloat(Boolean) (!= (- (Math|Conversions|ToInteger(Boolean) (Variables|Default|GetRotation%20clamped%20to%20Displacement)) 1) (.AXIS (Utilities|Struct|BreakF_CSVdata _returnvalue_5))))))) -1.0) (.Y (Math|Vector|BreakVector (* (Variables|Default|GetRandom%20Rotation%20[XYZ]) (Math|Conversions|ToFloat(Boolean) (!= (- (Math|Conversions|ToInteger(Boolean) (Variables|Default|GetRotation%20clamped%20to%20Displacement)) 1) (.AXIS (Utilities|Struct|BreakF_CSVdata _returnvalue_5))))))) _displacement_randomize) (Math|Random|RandomFloatinRangefromStream (* (.Z (Math|Vector|BreakVector (* (Variables|Default|GetRandom%20Rotation%20[XYZ]) (Math|Conversions|ToFloat(Boolean) (!= (- (Math|Conversions|ToInteger(Boolean) (Variables|Default|GetRotation%20clamped%20to%20Displacement)) 1) (.AXIS (Utilities|Struct|BreakF_CSVdata _returnvalue_5))))))) -1.0) (.Z (Math|Vector|BreakVector (* (Variables|Default|GetRandom%20Rotation%20[XYZ]) (Math|Conversions|ToFloat(Boolean) (!= (- (Math|Conversions|ToInteger(Boolean) (Variables|Default|GetRotation%20clamped%20to%20Displacement)) 1) (.AXIS (Utilities|Struct|BreakF_CSVdata _returnvalue_5))))))) _displacement_randomize)) (Variables|Default|GetShuffle)) (Math|Vector|MakeVector (.R_X (Utilities|Struct|BreakF_CSVdata _returnvalue_5)) (.R_Y (Utilities|Struct|BreakF_CSVdata _returnvalue_5)) (.R_Z (Utilities|Struct|BreakF_CSVdata _returnvalue_5))))))) (Math|Conversions|ToFloat(Boolean) (Variables|Default|GetRandom%20Rotation%20LOCAL/GLOBAL))) (* (Math|Vector|MakeVector (.S_X (Utilities|Struct|BreakF_CSVdata _returnvalue_5)) (.S_Y (Utilities|Struct|BreakF_CSVdata _returnvalue_5)) (.S_Z (Utilities|Struct|BreakF_CSVdata _returnvalue_5))) (Variables|Default|GetScale))) false))))
                          (:Out%202
                            (Utilities|FlowControl|Sequence :!label _label_5
                              (:then_0
                                (Utilities|FlowControl|DoOnce false
                                  (:Completed
                                    (bind _returnvalue_9 (AddComponent|AddHierarchicalInstancedStaticMeshComponent false))
                                    (bind _output_get_4 (Variables|Default|Set03 _returnvalue_9))
                                    (Rendering|Material|SetMaterial _output_get_4 0 (Variables|Default|GetStone%20Material)))))
                              (:then_1
                                (Components|InstancedStaticMesh|AddInstance (Variables|Default|Get03) (Math|Transform|MakeTransform (Math|Transform|TransformLocation (Math|Transform|MakeTransform (Math|Vector|MakeVector (.T_X (Utilities|Struct|BreakF_CSVdata _returnvalue_5)) (.T_Y (Utilities|Struct|BreakF_CSVdata _returnvalue_5)) (.T_Z (Utilities|Struct|BreakF_CSVdata _returnvalue_5))) (Math|Rotator|Lerp(Rotator) (Math|Rotator|CombineRotators (Math|Rotator|MakeRotator (.X (Math|Vector|BreakVector (+ (Math|Vector|MakeVector (Math|Random|RandomFloatinRangefromStream (* (.X (Math|Vector|BreakVector (* (Variables|Default|GetRandom%20Rotation%20[XYZ]) (Math|Conversions|ToFloat(Boolean) (!= (- (Math|Conversions|ToInteger(Boolean) (Variables|Default|GetRotation%20clamped%20to%20Displacement)) 1) (.AXIS (Utilities|Struct|BreakF_CSVdata _returnvalue_5))))))) -1.0) (.X (Math|Vector|BreakVector (* (Variables|Default|GetRandom%20Rotation%20[XYZ]) (Math|Conversions|ToFloat(Boolean) (!= (- (Math|Conversions|ToInteger(Boolean) (Variables|Default|GetRotation%20clamped%20to%20Displacement)) 1) (.AXIS (Utilities|Struct|BreakF_CSVdata _returnvalue_5))))))) _displacement_randomize) (Math|Random|RandomFloatinRangefromStream (* (.Y (Math|Vector|BreakVector (* (Variables|Default|GetRandom%20Rotation%20[XYZ]) (Math|Conversions|ToFloat(Boolean) (!= (- (Math|Conversions|ToInteger(Boolean) (Variables|Default|GetRotation%20clamped%20to%20Displacement)) 1) (.AXIS (Utilities|Struct|BreakF_CSVdata _returnvalue_5))))))) -1.0) (.Y (Math|Vector|BreakVector (* (Variables|Default|GetRandom%20Rotation%20[XYZ]) (Math|Conversions|ToFloat(Boolean) (!= (- (Math|Conversions|ToInteger(Boolean) (Variables|Default|GetRotation%20clamped%20to%20Displacement)) 1) (.AXIS (Utilities|Struct|BreakF_CSVdata _returnvalue_5))))))) _displacement_randomize) (Math|Random|RandomFloatinRangefromStream (* (.Z (Math|Vector|BreakVector (* (Variables|Default|GetRandom%20Rotation%20[XYZ]) (Math|Conversions|ToFloat(Boolean) (!= (- (Math|Conversions|ToInteger(Boolean) (Variables|Default|GetRotation%20clamped%20to%20Displacement)) 1) (.AXIS (Utilities|Struct|BreakF_CSVdata _returnvalue_5))))))) -1.0) (.Z (Math|Vector|BreakVector (* (Variables|Default|GetRandom%20Rotation%20[XYZ]) (Math|Conversions|ToFloat(Boolean) (!= (- (Math|Conversions|ToInteger(Boolean) (Variables|Default|GetRotation%20clamped%20to%20Displacement)) 1) (.AXIS (Utilities|Struct|BreakF_CSVdata _returnvalue_5))))))) _displacement_randomize)) (Variables|Default|GetShuffle)))) (.Y (Math|Vector|BreakVector (+ (Math|Vector|MakeVector (Math|Random|RandomFloatinRangefromStream (* (.X (Math|Vector|BreakVector (* (Variables|Default|GetRandom%20Rotation%20[XYZ]) (Math|Conversions|ToFloat(Boolean) (!= (- (Math|Conversions|ToInteger(Boolean) (Variables|Default|GetRotation%20clamped%20to%20Displacement)) 1) (.AXIS (Utilities|Struct|BreakF_CSVdata _returnvalue_5))))))) -1.0) (.X (Math|Vector|BreakVector (* (Variables|Default|GetRandom%20Rotation%20[XYZ]) (Math|Conversions|ToFloat(Boolean) (!= (- (Math|Conversions|ToInteger(Boolean) (Variables|Default|GetRotation%20clamped%20to%20Displacement)) 1) (.AXIS (Utilities|Struct|BreakF_CSVdata _returnvalue_5))))))) _displacement_randomize) (Math|Random|RandomFloatinRangefromStream (* (.Y (Math|Vector|BreakVector (* (Variables|Default|GetRandom%20Rotation%20[XYZ]) (Math|Conversions|ToFloat(Boolean) (!= (- (Math|Conversions|ToInteger(Boolean) (Variables|Default|GetRotation%20clamped%20to%20Displacement)) 1) (.AXIS (Utilities|Struct|BreakF_CSVdata _returnvalue_5))))))) -1.0) (.Y (Math|Vector|BreakVector (* (Variables|Default|GetRandom%20Rotation%20[XYZ]) (Math|Conversions|ToFloat(Boolean) (!= (- (Math|Conversions|ToInteger(Boolean) (Variables|Default|GetRotation%20clamped%20to%20Displacement)) 1) (.AXIS (Utilities|Struct|BreakF_CSVdata _returnvalue_5))))))) _displacement_randomize) (Math|Random|RandomFloatinRangefromStream (* (.Z (Math|Vector|BreakVector (* (Variables|Default|GetRandom%20Rotation%20[XYZ]) (Math|Conversions|ToFloat(Boolean) (!= (- (Math|Conversions|ToInteger(Boolean) (Variables|Default|GetRotation%20clamped%20to%20Displacement)) 1) (.AXIS (Utilities|Struct|BreakF_CSVdata _returnvalue_5))))))) -1.0) (.Z (Math|Vector|BreakVector (* (Variables|Default|GetRandom%20Rotation%20[XYZ]) (Math|Conversions|ToFloat(Boolean) (!= (- (Math|Conversions|ToInteger(Boolean) (Variables|Default|GetRotation%20clamped%20to%20Displacement)) 1) (.AXIS (Utilities|Struct|BreakF_CSVdata _returnvalue_5))))))) _displacement_randomize)) (Variables|Default|GetShuffle)))) (.Z (Math|Vector|BreakVector (+ (Math|Vector|MakeVector (Math|Random|RandomFloatinRangefromStream (* (.X (Math|Vector|BreakVector (* (Variables|Default|GetRandom%20Rotation%20[XYZ]) (Math|Conversions|ToFloat(Boolean) (!= (- (Math|Conversions|ToInteger(Boolean) (Variables|Default|GetRotation%20clamped%20to%20Displacement)) 1) (.AXIS (Utilities|Struct|BreakF_CSVdata _returnvalue_5))))))) -1.0) (.X (Math|Vector|BreakVector (* (Variables|Default|GetRandom%20Rotation%20[XYZ]) (Math|Conversions|ToFloat(Boolean) (!= (- (Math|Conversions|ToInteger(Boolean) (Variables|Default|GetRotation%20clamped%20to%20Displacement)) 1) (.AXIS (Utilities|Struct|BreakF_CSVdata _returnvalue_5))))))) _displacement_randomize) (Math|Random|RandomFloatinRangefromStream (* (.Y (Math|Vector|BreakVector (* (Variables|Default|GetRandom%20Rotation%20[XYZ]) (Math|Conversions|ToFloat(Boolean) (!= (- (Math|Conversions|ToInteger(Boolean) (Variables|Default|GetRotation%20clamped%20to%20Displacement)) 1) (.AXIS (Utilities|Struct|BreakF_CSVdata _returnvalue_5))))))) -1.0) (.Y (Math|Vector|BreakVector (* (Variables|Default|GetRandom%20Rotation%20[XYZ]) (Math|Conversions|ToFloat(Boolean) (!= (- (Math|Conversions|ToInteger(Boolean) (Variables|Default|GetRotation%20clamped%20to%20Displacement)) 1) (.AXIS (Utilities|Struct|BreakF_CSVdata _returnvalue_5))))))) _displacement_randomize) (Math|Random|RandomFloatinRangefromStream (* (.Z (Math|Vector|BreakVector (* (Variables|Default|GetRandom%20Rotation%20[XYZ]) (Math|Conversions|ToFloat(Boolean) (!= (- (Math|Conversions|ToInteger(Boolean) (Variables|Default|GetRotation%20clamped%20to%20Displacement)) 1) (.AXIS (Utilities|Struct|BreakF_CSVdata _returnvalue_5))))))) -1.0) (.Z (Math|Vector|BreakVector (* (Variables|Default|GetRandom%20Rotation%20[XYZ]) (Math|Conversions|ToFloat(Boolean) (!= (- (Math|Conversions|ToInteger(Boolean) (Variables|Default|GetRotation%20clamped%20to%20Displacement)) 1) (.AXIS (Utilities|Struct|BreakF_CSVdata _returnvalue_5))))))) _displacement_randomize)) (Variables|Default|GetShuffle))))) (Math|Rotator|MakeRotator (.R_X (Utilities|Struct|BreakF_CSVdata _returnvalue_5)) (.R_Y (Utilities|Struct|BreakF_CSVdata _returnvalue_5)) (.R_Z (Utilities|Struct|BreakF_CSVdata _returnvalue_5)))) (Math|Rotator|MakeRotator (.X (Math|Vector|BreakVector (+ (+ (Math|Vector|MakeVector (Math|Random|RandomFloatinRangefromStream (* (.X (Math|Vector|BreakVector (* (Variables|Default|GetRandom%20Rotation%20[XYZ]) (Math|Conversions|ToFloat(Boolean) (!= (- (Math|Conversions|ToInteger(Boolean) (Variables|Default|GetRotation%20clamped%20to%20Displacement)) 1) (.AXIS (Utilities|Struct|BreakF_CSVdata _returnvalue_5))))))) -1.0) (.X (Math|Vector|BreakVector (* (Variables|Default|GetRandom%20Rotation%20[XYZ]) (Math|Conversions|ToFloat(Boolean) (!= (- (Math|Conversions|ToInteger(Boolean) (Variables|Default|GetRotation%20clamped%20to%20Displacement)) 1) (.AXIS (Utilities|Struct|BreakF_CSVdata _returnvalue_5))))))) _displacement_randomize) (Math|Random|RandomFloatinRangefromStream (* (.Y (Math|Vector|BreakVector (* (Variables|Default|GetRandom%20Rotation%20[XYZ]) (Math|Conversions|ToFloat(Boolean) (!= (- (Math|Conversions|ToInteger(Boolean) (Variables|Default|GetRotation%20clamped%20to%20Displacement)) 1) (.AXIS (Utilities|Struct|BreakF_CSVdata _returnvalue_5))))))) -1.0) (.Y (Math|Vector|BreakVector (* (Variables|Default|GetRandom%20Rotation%20[XYZ]) (Math|Conversions|ToFloat(Boolean) (!= (- (Math|Conversions|ToInteger(Boolean) (Variables|Default|GetRotation%20clamped%20to%20Displacement)) 1) (.AXIS (Utilities|Struct|BreakF_CSVdata _returnvalue_5))))))) _displacement_randomize) (Math|Random|RandomFloatinRangefromStream (* (.Z (Math|Vector|BreakVector (* (Variables|Default|GetRandom%20Rotation%20[XYZ]) (Math|Conversions|ToFloat(Boolean) (!= (- (Math|Conversions|ToInteger(Boolean) (Variables|Default|GetRotation%20clamped%20to%20Displacement)) 1) (.AXIS (Utilities|Struct|BreakF_CSVdata _returnvalue_5))))))) -1.0) (.Z (Math|Vector|BreakVector (* (Variables|Default|GetRandom%20Rotation%20[XYZ]) (Math|Conversions|ToFloat(Boolean) (!= (- (Math|Conversions|ToInteger(Boolean) (Variables|Default|GetRotation%20clamped%20to%20Displacement)) 1) (.AXIS (Utilities|Struct|BreakF_CSVdata _returnvalue_5))))))) _displacement_randomize)) (Variables|Default|GetShuffle)) (Math|Vector|MakeVector (.R_X (Utilities|Struct|BreakF_CSVdata _returnvalue_5)) (.R_Y (Utilities|Struct|BreakF_CSVdata _returnvalue_5)) (.R_Z (Utilities|Struct|BreakF_CSVdata _returnvalue_5)))))) (.Y (Math|Vector|BreakVector (+ (+ (Math|Vector|MakeVector (Math|Random|RandomFloatinRangefromStream (* (.X (Math|Vector|BreakVector (* (Variables|Default|GetRandom%20Rotation%20[XYZ]) (Math|Conversions|ToFloat(Boolean) (!= (- (Math|Conversions|ToInteger(Boolean) (Variables|Default|GetRotation%20clamped%20to%20Displacement)) 1) (.AXIS (Utilities|Struct|BreakF_CSVdata _returnvalue_5))))))) -1.0) (.X (Math|Vector|BreakVector (* (Variables|Default|GetRandom%20Rotation%20[XYZ]) (Math|Conversions|ToFloat(Boolean) (!= (- (Math|Conversions|ToInteger(Boolean) (Variables|Default|GetRotation%20clamped%20to%20Displacement)) 1) (.AXIS (Utilities|Struct|BreakF_CSVdata _returnvalue_5))))))) _displacement_randomize) (Math|Random|RandomFloatinRangefromStream (* (.Y (Math|Vector|BreakVector (* (Variables|Default|GetRandom%20Rotation%20[XYZ]) (Math|Conversions|ToFloat(Boolean) (!= (- (Math|Conversions|ToInteger(Boolean) (Variables|Default|GetRotation%20clamped%20to%20Displacement)) 1) (.AXIS (Utilities|Struct|BreakF_CSVdata _returnvalue_5))))))) -1.0) (.Y (Math|Vector|BreakVector (* (Variables|Default|GetRandom%20Rotation%20[XYZ]) (Math|Conversions|ToFloat(Boolean) (!= (- (Math|Conversions|ToInteger(Boolean) (Variables|Default|GetRotation%20clamped%20to%20Displacement)) 1) (.AXIS (Utilities|Struct|BreakF_CSVdata _returnvalue_5))))))) _displacement_randomize) (Math|Random|RandomFloatinRangefromStream (* (.Z (Math|Vector|BreakVector (* (Variables|Default|GetRandom%20Rotation%20[XYZ]) (Math|Conversions|ToFloat(Boolean) (!= (- (Math|Conversions|ToInteger(Boolean) (Variables|Default|GetRotation%20clamped%20to%20Displacement)) 1) (.AXIS (Utilities|Struct|BreakF_CSVdata _returnvalue_5))))))) -1.0) (.Z (Math|Vector|BreakVector (* (Variables|Default|GetRandom%20Rotation%20[XYZ]) (Math|Conversions|ToFloat(Boolean) (!= (- (Math|Conversions|ToInteger(Boolean) (Variables|Default|GetRotation%20clamped%20to%20Displacement)) 1) (.AXIS (Utilities|Struct|BreakF_CSVdata _returnvalue_5))))))) _displacement_randomize)) (Variables|Default|GetShuffle)) (Math|Vector|MakeVector (.R_X (Utilities|Struct|BreakF_CSVdata _returnvalue_5)) (.R_Y (Utilities|Struct|BreakF_CSVdata _returnvalue_5)) (.R_Z (Utilities|Struct|BreakF_CSVdata _returnvalue_5)))))) (.Z (Math|Vector|BreakVector (+ (+ (Math|Vector|MakeVector (Math|Random|RandomFloatinRangefromStream (* (.X (Math|Vector|BreakVector (* (Variables|Default|GetRandom%20Rotation%20[XYZ]) (Math|Conversions|ToFloat(Boolean) (!= (- (Math|Conversions|ToInteger(Boolean) (Variables|Default|GetRotation%20clamped%20to%20Displacement)) 1) (.AXIS (Utilities|Struct|BreakF_CSVdata _returnvalue_5))))))) -1.0) (.X (Math|Vector|BreakVector (* (Variables|Default|GetRandom%20Rotation%20[XYZ]) (Math|Conversions|ToFloat(Boolean) (!= (- (Math|Conversions|ToInteger(Boolean) (Variables|Default|GetRotation%20clamped%20to%20Displacement)) 1) (.AXIS (Utilities|Struct|BreakF_CSVdata _returnvalue_5))))))) _displacement_randomize) (Math|Random|RandomFloatinRangefromStream (* (.Y (Math|Vector|BreakVector (* (Variables|Default|GetRandom%20Rotation%20[XYZ]) (Math|Conversions|ToFloat(Boolean) (!= (- (Math|Conversions|ToInteger(Boolean) (Variables|Default|GetRotation%20clamped%20to%20Displacement)) 1) (.AXIS (Utilities|Struct|BreakF_CSVdata _returnvalue_5))))))) -1.0) (.Y (Math|Vector|BreakVector (* (Variables|Default|GetRandom%20Rotation%20[XYZ]) (Math|Conversions|ToFloat(Boolean) (!= (- (Math|Conversions|ToInteger(Boolean) (Variables|Default|GetRotation%20clamped%20to%20Displacement)) 1) (.AXIS (Utilities|Struct|BreakF_CSVdata _returnvalue_5))))))) _displacement_randomize) (Math|Random|RandomFloatinRangefromStream (* (.Z (Math|Vector|BreakVector (* (Variables|Default|GetRandom%20Rotation%20[XYZ]) (Math|Conversions|ToFloat(Boolean) (!= (- (Math|Conversions|ToInteger(Boolean) (Variables|Default|GetRotation%20clamped%20to%20Displacement)) 1) (.AXIS (Utilities|Struct|BreakF_CSVdata _returnvalue_5))))))) -1.0) (.Z (Math|Vector|BreakVector (* (Variables|Default|GetRandom%20Rotation%20[XYZ]) (Math|Conversions|ToFloat(Boolean) (!= (- (Math|Conversions|ToInteger(Boolean) (Variables|Default|GetRotation%20clamped%20to%20Displacement)) 1) (.AXIS (Utilities|Struct|BreakF_CSVdata _returnvalue_5))))))) _displacement_randomize)) (Variables|Default|GetShuffle)) (Math|Vector|MakeVector (.R_X (Utilities|Struct|BreakF_CSVdata _returnvalue_5)) (.R_Y (Utilities|Struct|BreakF_CSVdata _returnvalue_5)) (.R_Z (Utilities|Struct|BreakF_CSVdata _returnvalue_5))))))) (Math|Conversions|ToFloat(Boolean) (Variables|Default|GetRandom%20Rotation%20LOCAL/GLOBAL))) (* (Math|Vector|MakeVector (.S_X (Utilities|Struct|BreakF_CSVdata _returnvalue_5)) (.S_Y (Utilities|Struct|BreakF_CSVdata _returnvalue_5)) (.S_Z (Utilities|Struct|BreakF_CSVdata _returnvalue_5))) (Variables|Default|GetScale))) (* (Math|Vector|MakeVector (* (Math|Conversions|ToFloat(Boolean) (== (.AXIS (Utilities|Struct|BreakF_CSVdata _returnvalue_5)) 1)) _returnvalue_3) (* (Math|Conversions|ToFloat(Boolean) (== (.AXIS (Utilities|Struct|BreakF_CSVdata _returnvalue_5)) 2)) _returnvalue_3) (* (Math|Conversions|ToFloat(Boolean) (== (.AXIS (Utilities|Struct|BreakF_CSVdata _returnvalue_5)) 3)) _returnvalue_3)) (Math|Float|Clamp(Float) (+ (Math|Conversions|ToFloat(Boolean) (and (not (Class|KismetMathLibrary|IsPointinBoxwithTransform (Math|Vector|MakeVector (.T_X (Utilities|Struct|BreakF_CSVdata _returnvalue_5)) (.T_Y (Utilities|Struct|BreakF_CSVdata _returnvalue_5)) (.T_Z (Utilities|Struct|BreakF_CSVdata _returnvalue_5))) (Math|Transform|MakeTransform (Variables|Default|GetBox%20Origin%20[XYZ]) (Variables|Default|GetBox%20Rotation%20[XYZ])) (Variables|Default|GetBox%20Extent%20[XYZ]))) _boxcontrolleddisplacement)) (Variables|Default|GetBox%20Intensity)) (Math|Conversions|ToFloat(Boolean) (not _boxcontrolleddisplacement))))) (Math|Rotator|Lerp(Rotator) (Math|Rotator|CombineRotators (Math|Rotator|MakeRotator (.X (Math|Vector|BreakVector (+ (Math|Vector|MakeVector (Math|Random|RandomFloatinRangefromStream (* (.X (Math|Vector|BreakVector (* (Variables|Default|GetRandom%20Rotation%20[XYZ]) (Math|Conversions|ToFloat(Boolean) (!= (- (Math|Conversions|ToInteger(Boolean) (Variables|Default|GetRotation%20clamped%20to%20Displacement)) 1) (.AXIS (Utilities|Struct|BreakF_CSVdata _returnvalue_5))))))) -1.0) (.X (Math|Vector|BreakVector (* (Variables|Default|GetRandom%20Rotation%20[XYZ]) (Math|Conversions|ToFloat(Boolean) (!= (- (Math|Conversions|ToInteger(Boolean) (Variables|Default|GetRotation%20clamped%20to%20Displacement)) 1) (.AXIS (Utilities|Struct|BreakF_CSVdata _returnvalue_5))))))) _displacement_randomize) (Math|Random|RandomFloatinRangefromStream (* (.Y (Math|Vector|BreakVector (* (Variables|Default|GetRandom%20Rotation%20[XYZ]) (Math|Conversions|ToFloat(Boolean) (!= (- (Math|Conversions|ToInteger(Boolean) (Variables|Default|GetRotation%20clamped%20to%20Displacement)) 1) (.AXIS (Utilities|Struct|BreakF_CSVdata _returnvalue_5))))))) -1.0) (.Y (Math|Vector|BreakVector (* (Variables|Default|GetRandom%20Rotation%20[XYZ]) (Math|Conversions|ToFloat(Boolean) (!= (- (Math|Conversions|ToInteger(Boolean) (Variables|Default|GetRotation%20clamped%20to%20Displacement)) 1) (.AXIS (Utilities|Struct|BreakF_CSVdata _returnvalue_5))))))) _displacement_randomize) (Math|Random|RandomFloatinRangefromStream (* (.Z (Math|Vector|BreakVector (* (Variables|Default|GetRandom%20Rotation%20[XYZ]) (Math|Conversions|ToFloat(Boolean) (!= (- (Math|Conversions|ToInteger(Boolean) (Variables|Default|GetRotation%20clamped%20to%20Displacement)) 1) (.AXIS (Utilities|Struct|BreakF_CSVdata _returnvalue_5))))))) -1.0) (.Z (Math|Vector|BreakVector (* (Variables|Default|GetRandom%20Rotation%20[XYZ]) (Math|Conversions|ToFloat(Boolean) (!= (- (Math|Conversions|ToInteger(Boolean) (Variables|Default|GetRotation%20clamped%20to%20Displacement)) 1) (.AXIS (Utilities|Struct|BreakF_CSVdata _returnvalue_5))))))) _displacement_randomize)) (Variables|Default|GetShuffle)))) (.Y (Math|Vector|BreakVector (+ (Math|Vector|MakeVector (Math|Random|RandomFloatinRangefromStream (* (.X (Math|Vector|BreakVector (* (Variables|Default|GetRandom%20Rotation%20[XYZ]) (Math|Conversions|ToFloat(Boolean) (!= (- (Math|Conversions|ToInteger(Boolean) (Variables|Default|GetRotation%20clamped%20to%20Displacement)) 1) (.AXIS (Utilities|Struct|BreakF_CSVdata _returnvalue_5))))))) -1.0) (.X (Math|Vector|BreakVector (* (Variables|Default|GetRandom%20Rotation%20[XYZ]) (Math|Conversions|ToFloat(Boolean) (!= (- (Math|Conversions|ToInteger(Boolean) (Variables|Default|GetRotation%20clamped%20to%20Displacement)) 1) (.AXIS (Utilities|Struct|BreakF_CSVdata _returnvalue_5))))))) _displacement_randomize) (Math|Random|RandomFloatinRangefromStream (* (.Y (Math|Vector|BreakVector (* (Variables|Default|GetRandom%20Rotation%20[XYZ]) (Math|Conversions|ToFloat(Boolean) (!= (- (Math|Conversions|ToInteger(Boolean) (Variables|Default|GetRotation%20clamped%20to%20Displacement)) 1) (.AXIS (Utilities|Struct|BreakF_CSVdata _returnvalue_5))))))) -1.0) (.Y (Math|Vector|BreakVector (* (Variables|Default|GetRandom%20Rotation%20[XYZ]) (Math|Conversions|ToFloat(Boolean) (!= (- (Math|Conversions|ToInteger(Boolean) (Variables|Default|GetRotation%20clamped%20to%20Displacement)) 1) (.AXIS (Utilities|Struct|BreakF_CSVdata _returnvalue_5))))))) _displacement_randomize) (Math|Random|RandomFloatinRangefromStream (* (.Z (Math|Vector|BreakVector (* (Variables|Default|GetRandom%20Rotation%20[XYZ]) (Math|Conversions|ToFloat(Boolean) (!= (- (Math|Conversions|ToInteger(Boolean) (Variables|Default|GetRotation%20clamped%20to%20Displacement)) 1) (.AXIS (Utilities|Struct|BreakF_CSVdata _returnvalue_5))))))) -1.0) (.Z (Math|Vector|BreakVector (* (Variables|Default|GetRandom%20Rotation%20[XYZ]) (Math|Conversions|ToFloat(Boolean) (!= (- (Math|Conversions|ToInteger(Boolean) (Variables|Default|GetRotation%20clamped%20to%20Displacement)) 1) (.AXIS (Utilities|Struct|BreakF_CSVdata _returnvalue_5))))))) _displacement_randomize)) (Variables|Default|GetShuffle)))) (.Z (Math|Vector|BreakVector (+ (Math|Vector|MakeVector (Math|Random|RandomFloatinRangefromStream (* (.X (Math|Vector|BreakVector (* (Variables|Default|GetRandom%20Rotation%20[XYZ]) (Math|Conversions|ToFloat(Boolean) (!= (- (Math|Conversions|ToInteger(Boolean) (Variables|Default|GetRotation%20clamped%20to%20Displacement)) 1) (.AXIS (Utilities|Struct|BreakF_CSVdata _returnvalue_5))))))) -1.0) (.X (Math|Vector|BreakVector (* (Variables|Default|GetRandom%20Rotation%20[XYZ]) (Math|Conversions|ToFloat(Boolean) (!= (- (Math|Conversions|ToInteger(Boolean) (Variables|Default|GetRotation%20clamped%20to%20Displacement)) 1) (.AXIS (Utilities|Struct|BreakF_CSVdata _returnvalue_5))))))) _displacement_randomize) (Math|Random|RandomFloatinRangefromStream (* (.Y (Math|Vector|BreakVector (* (Variables|Default|GetRandom%20Rotation%20[XYZ]) (Math|Conversions|ToFloat(Boolean) (!= (- (Math|Conversions|ToInteger(Boolean) (Variables|Default|GetRotation%20clamped%20to%20Displacement)) 1) (.AXIS (Utilities|Struct|BreakF_CSVdata _returnvalue_5))))))) -1.0) (.Y (Math|Vector|BreakVector (* (Variables|Default|GetRandom%20Rotation%20[XYZ]) (Math|Conversions|ToFloat(Boolean) (!= (- (Math|Conversions|ToInteger(Boolean) (Variables|Default|GetRotation%20clamped%20to%20Displacement)) 1) (.AXIS (Utilities|Struct|BreakF_CSVdata _returnvalue_5))))))) _displacement_randomize) (Math|Random|RandomFloatinRangefromStream (* (.Z (Math|Vector|BreakVector (* (Variables|Default|GetRandom%20Rotation%20[XYZ]) (Math|Conversions|ToFloat(Boolean) (!= (- (Math|Conversions|ToInteger(Boolean) (Variables|Default|GetRotation%20clamped%20to%20Displacement)) 1) (.AXIS (Utilities|Struct|BreakF_CSVdata _returnvalue_5))))))) -1.0) (.Z (Math|Vector|BreakVector (* (Variables|Default|GetRandom%20Rotation%20[XYZ]) (Math|Conversions|ToFloat(Boolean) (!= (- (Math|Conversions|ToInteger(Boolean) (Variables|Default|GetRotation%20clamped%20to%20Displacement)) 1) (.AXIS (Utilities|Struct|BreakF_CSVdata _returnvalue_5))))))) _displacement_randomize)) (Variables|Default|GetShuffle))))) (Math|Rotator|MakeRotator (.R_X (Utilities|Struct|BreakF_CSVdata _returnvalue_5)) (.R_Y (Utilities|Struct|BreakF_CSVdata _returnvalue_5)) (.R_Z (Utilities|Struct|BreakF_CSVdata _returnvalue_5)))) (Math|Rotator|MakeRotator (.X (Math|Vector|BreakVector (+ (+ (Math|Vector|MakeVector (Math|Random|RandomFloatinRangefromStream (* (.X (Math|Vector|BreakVector (* (Variables|Default|GetRandom%20Rotation%20[XYZ]) (Math|Conversions|ToFloat(Boolean) (!= (- (Math|Conversions|ToInteger(Boolean) (Variables|Default|GetRotation%20clamped%20to%20Displacement)) 1) (.AXIS (Utilities|Struct|BreakF_CSVdata _returnvalue_5))))))) -1.0) (.X (Math|Vector|BreakVector (* (Variables|Default|GetRandom%20Rotation%20[XYZ]) (Math|Conversions|ToFloat(Boolean) (!= (- (Math|Conversions|ToInteger(Boolean) (Variables|Default|GetRotation%20clamped%20to%20Displacement)) 1) (.AXIS (Utilities|Struct|BreakF_CSVdata _returnvalue_5))))))) _displacement_randomize) (Math|Random|RandomFloatinRangefromStream (* (.Y (Math|Vector|BreakVector (* (Variables|Default|GetRandom%20Rotation%20[XYZ]) (Math|Conversions|ToFloat(Boolean) (!= (- (Math|Conversions|ToInteger(Boolean) (Variables|Default|GetRotation%20clamped%20to%20Displacement)) 1) (.AXIS (Utilities|Struct|BreakF_CSVdata _returnvalue_5))))))) -1.0) (.Y (Math|Vector|BreakVector (* (Variables|Default|GetRandom%20Rotation%20[XYZ]) (Math|Conversions|ToFloat(Boolean) (!= (- (Math|Conversions|ToInteger(Boolean) (Variables|Default|GetRotation%20clamped%20to%20Displacement)) 1) (.AXIS (Utilities|Struct|BreakF_CSVdata _returnvalue_5))))))) _displacement_randomize) (Math|Random|RandomFloatinRangefromStream (* (.Z (Math|Vector|BreakVector (* (Variables|Default|GetRandom%20Rotation%20[XYZ]) (Math|Conversions|ToFloat(Boolean) (!= (- (Math|Conversions|ToInteger(Boolean) (Variables|Default|GetRotation%20clamped%20to%20Displacement)) 1) (.AXIS (Utilities|Struct|BreakF_CSVdata _returnvalue_5))))))) -1.0) (.Z (Math|Vector|BreakVector (* (Variables|Default|GetRandom%20Rotation%20[XYZ]) (Math|Conversions|ToFloat(Boolean) (!= (- (Math|Conversions|ToInteger(Boolean) (Variables|Default|GetRotation%20clamped%20to%20Displacement)) 1) (.AXIS (Utilities|Struct|BreakF_CSVdata _returnvalue_5))))))) _displacement_randomize)) (Variables|Default|GetShuffle)) (Math|Vector|MakeVector (.R_X (Utilities|Struct|BreakF_CSVdata _returnvalue_5)) (.R_Y (Utilities|Struct|BreakF_CSVdata _returnvalue_5)) (.R_Z (Utilities|Struct|BreakF_CSVdata _returnvalue_5)))))) (.Y (Math|Vector|BreakVector (+ (+ (Math|Vector|MakeVector (Math|Random|RandomFloatinRangefromStream (* (.X (Math|Vector|BreakVector (* (Variables|Default|GetRandom%20Rotation%20[XYZ]) (Math|Conversions|ToFloat(Boolean) (!= (- (Math|Conversions|ToInteger(Boolean) (Variables|Default|GetRotation%20clamped%20to%20Displacement)) 1) (.AXIS (Utilities|Struct|BreakF_CSVdata _returnvalue_5))))))) -1.0) (.X (Math|Vector|BreakVector (* (Variables|Default|GetRandom%20Rotation%20[XYZ]) (Math|Conversions|ToFloat(Boolean) (!= (- (Math|Conversions|ToInteger(Boolean) (Variables|Default|GetRotation%20clamped%20to%20Displacement)) 1) (.AXIS (Utilities|Struct|BreakF_CSVdata _returnvalue_5))))))) _displacement_randomize) (Math|Random|RandomFloatinRangefromStream (* (.Y (Math|Vector|BreakVector (* (Variables|Default|GetRandom%20Rotation%20[XYZ]) (Math|Conversions|ToFloat(Boolean) (!= (- (Math|Conversions|ToInteger(Boolean) (Variables|Default|GetRotation%20clamped%20to%20Displacement)) 1) (.AXIS (Utilities|Struct|BreakF_CSVdata _returnvalue_5))))))) -1.0) (.Y (Math|Vector|BreakVector (* (Variables|Default|GetRandom%20Rotation%20[XYZ]) (Math|Conversions|ToFloat(Boolean) (!= (- (Math|Conversions|ToInteger(Boolean) (Variables|Default|GetRotation%20clamped%20to%20Displacement)) 1) (.AXIS (Utilities|Struct|BreakF_CSVdata _returnvalue_5))))))) _displacement_randomize) (Math|Random|RandomFloatinRangefromStream (* (.Z (Math|Vector|BreakVector (* (Variables|Default|GetRandom%20Rotation%20[XYZ]) (Math|Conversions|ToFloat(Boolean) (!= (- (Math|Conversions|ToInteger(Boolean) (Variables|Default|GetRotation%20clamped%20to%20Displacement)) 1) (.AXIS (Utilities|Struct|BreakF_CSVdata _returnvalue_5))))))) -1.0) (.Z (Math|Vector|BreakVector (* (Variables|Default|GetRandom%20Rotation%20[XYZ]) (Math|Conversions|ToFloat(Boolean) (!= (- (Math|Conversions|ToInteger(Boolean) (Variables|Default|GetRotation%20clamped%20to%20Displacement)) 1) (.AXIS (Utilities|Struct|BreakF_CSVdata _returnvalue_5))))))) _displacement_randomize)) (Variables|Default|GetShuffle)) (Math|Vector|MakeVector (.R_X (Utilities|Struct|BreakF_CSVdata _returnvalue_5)) (.R_Y (Utilities|Struct|BreakF_CSVdata _returnvalue_5)) (.R_Z (Utilities|Struct|BreakF_CSVdata _returnvalue_5)))))) (.Z (Math|Vector|BreakVector (+ (+ (Math|Vector|MakeVector (Math|Random|RandomFloatinRangefromStream (* (.X (Math|Vector|BreakVector (* (Variables|Default|GetRandom%20Rotation%20[XYZ]) (Math|Conversions|ToFloat(Boolean) (!= (- (Math|Conversions|ToInteger(Boolean) (Variables|Default|GetRotation%20clamped%20to%20Displacement)) 1) (.AXIS (Utilities|Struct|BreakF_CSVdata _returnvalue_5))))))) -1.0) (.X (Math|Vector|BreakVector (* (Variables|Default|GetRandom%20Rotation%20[XYZ]) (Math|Conversions|ToFloat(Boolean) (!= (- (Math|Conversions|ToInteger(Boolean) (Variables|Default|GetRotation%20clamped%20to%20Displacement)) 1) (.AXIS (Utilities|Struct|BreakF_CSVdata _returnvalue_5))))))) _displacement_randomize) (Math|Random|RandomFloatinRangefromStream (* (.Y (Math|Vector|BreakVector (* (Variables|Default|GetRandom%20Rotation%20[XYZ]) (Math|Conversions|ToFloat(Boolean) (!= (- (Math|Conversions|ToInteger(Boolean) (Variables|Default|GetRotation%20clamped%20to%20Displacement)) 1) (.AXIS (Utilities|Struct|BreakF_CSVdata _returnvalue_5))))))) -1.0) (.Y (Math|Vector|BreakVector (* (Variables|Default|GetRandom%20Rotation%20[XYZ]) (Math|Conversions|ToFloat(Boolean) (!= (- (Math|Conversions|ToInteger(Boolean) (Variables|Default|GetRotation%20clamped%20to%20Displacement)) 1) (.AXIS (Utilities|Struct|BreakF_CSVdata _returnvalue_5))))))) _displacement_randomize) (Math|Random|RandomFloatinRangefromStream (* (.Z (Math|Vector|BreakVector (* (Variables|Default|GetRandom%20Rotation%20[XYZ]) (Math|Conversions|ToFloat(Boolean) (!= (- (Math|Conversions|ToInteger(Boolean) (Variables|Default|GetRotation%20clamped%20to%20Displacement)) 1) (.AXIS (Utilities|Struct|BreakF_CSVdata _returnvalue_5))))))) -1.0) (.Z (Math|Vector|BreakVector (* (Variables|Default|GetRandom%20Rotation%20[XYZ]) (Math|Conversions|ToFloat(Boolean) (!= (- (Math|Conversions|ToInteger(Boolean) (Variables|Default|GetRotation%20clamped%20to%20Displacement)) 1) (.AXIS (Utilities|Struct|BreakF_CSVdata _returnvalue_5))))))) _displacement_randomize)) (Variables|Default|GetShuffle)) (Math|Vector|MakeVector (.R_X (Utilities|Struct|BreakF_CSVdata _returnvalue_5)) (.R_Y (Utilities|Struct|BreakF_CSVdata _returnvalue_5)) (.R_Z (Utilities|Struct|BreakF_CSVdata _returnvalue_5))))))) (Math|Conversions|ToFloat(Boolean) (Variables|Default|GetRandom%20Rotation%20LOCAL/GLOBAL))) (* (Math|Vector|MakeVector (.S_X (Utilities|Struct|BreakF_CSVdata _returnvalue_5)) (.S_Y (Utilities|Struct|BreakF_CSVdata _returnvalue_5)) (.S_Z (Utilities|Struct|BreakF_CSVdata _returnvalue_5))) (Variables|Default|GetScale))) false))))
                          (:Out%203
                            (Utilities|FlowControl|Sequence :!label _label_6
                              (:then_0
                                (Utilities|FlowControl|DoOnce false
                                  (:Completed
                                    (bind _returnvalue_10 (AddComponent|AddHierarchicalInstancedStaticMeshComponent false))
                                    (bind _output_get_5 (Variables|Default|Set05 _returnvalue_10))
                                    (Rendering|Material|SetMaterial _output_get_5 0 (Variables|Default|GetStone%20Material)))))
                              (:then_1
                                (Components|InstancedStaticMesh|AddInstance (Variables|Default|Get05) (Math|Transform|MakeTransform (Math|Transform|TransformLocation (Math|Transform|MakeTransform (Math|Vector|MakeVector (.T_X (Utilities|Struct|BreakF_CSVdata _returnvalue_5)) (.T_Y (Utilities|Struct|BreakF_CSVdata _returnvalue_5)) (.T_Z (Utilities|Struct|BreakF_CSVdata _returnvalue_5))) (Math|Rotator|Lerp(Rotator) (Math|Rotator|CombineRotators (Math|Rotator|MakeRotator (.X (Math|Vector|BreakVector (+ (Math|Vector|MakeVector (Math|Random|RandomFloatinRangefromStream (* (.X (Math|Vector|BreakVector (* (Variables|Default|GetRandom%20Rotation%20[XYZ]) (Math|Conversions|ToFloat(Boolean) (!= (- (Math|Conversions|ToInteger(Boolean) (Variables|Default|GetRotation%20clamped%20to%20Displacement)) 1) (.AXIS (Utilities|Struct|BreakF_CSVdata _returnvalue_5))))))) -1.0) (.X (Math|Vector|BreakVector (* (Variables|Default|GetRandom%20Rotation%20[XYZ]) (Math|Conversions|ToFloat(Boolean) (!= (- (Math|Conversions|ToInteger(Boolean) (Variables|Default|GetRotation%20clamped%20to%20Displacement)) 1) (.AXIS (Utilities|Struct|BreakF_CSVdata _returnvalue_5))))))) _displacement_randomize) (Math|Random|RandomFloatinRangefromStream (* (.Y (Math|Vector|BreakVector (* (Variables|Default|GetRandom%20Rotation%20[XYZ]) (Math|Conversions|ToFloat(Boolean) (!= (- (Math|Conversions|ToInteger(Boolean) (Variables|Default|GetRotation%20clamped%20to%20Displacement)) 1) (.AXIS (Utilities|Struct|BreakF_CSVdata _returnvalue_5))))))) -1.0) (.Y (Math|Vector|BreakVector (* (Variables|Default|GetRandom%20Rotation%20[XYZ]) (Math|Conversions|ToFloat(Boolean) (!= (- (Math|Conversions|ToInteger(Boolean) (Variables|Default|GetRotation%20clamped%20to%20Displacement)) 1) (.AXIS (Utilities|Struct|BreakF_CSVdata _returnvalue_5))))))) _displacement_randomize) (Math|Random|RandomFloatinRangefromStream (* (.Z (Math|Vector|BreakVector (* (Variables|Default|GetRandom%20Rotation%20[XYZ]) (Math|Conversions|ToFloat(Boolean) (!= (- (Math|Conversions|ToInteger(Boolean) (Variables|Default|GetRotation%20clamped%20to%20Displacement)) 1) (.AXIS (Utilities|Struct|BreakF_CSVdata _returnvalue_5))))))) -1.0) (.Z (Math|Vector|BreakVector (* (Variables|Default|GetRandom%20Rotation%20[XYZ]) (Math|Conversions|ToFloat(Boolean) (!= (- (Math|Conversions|ToInteger(Boolean) (Variables|Default|GetRotation%20clamped%20to%20Displacement)) 1) (.AXIS (Utilities|Struct|BreakF_CSVdata _returnvalue_5))))))) _displacement_randomize)) (Variables|Default|GetShuffle)))) (.Y (Math|Vector|BreakVector (+ (Math|Vector|MakeVector (Math|Random|RandomFloatinRangefromStream (* (.X (Math|Vector|BreakVector (* (Variables|Default|GetRandom%20Rotation%20[XYZ]) (Math|Conversions|ToFloat(Boolean) (!= (- (Math|Conversions|ToInteger(Boolean) (Variables|Default|GetRotation%20clamped%20to%20Displacement)) 1) (.AXIS (Utilities|Struct|BreakF_CSVdata _returnvalue_5))))))) -1.0) (.X (Math|Vector|BreakVector (* (Variables|Default|GetRandom%20Rotation%20[XYZ]) (Math|Conversions|ToFloat(Boolean) (!= (- (Math|Conversions|ToInteger(Boolean) (Variables|Default|GetRotation%20clamped%20to%20Displacement)) 1) (.AXIS (Utilities|Struct|BreakF_CSVdata _returnvalue_5))))))) _displacement_randomize) (Math|Random|RandomFloatinRangefromStream (* (.Y (Math|Vector|BreakVector (* (Variables|Default|GetRandom%20Rotation%20[XYZ]) (Math|Conversions|ToFloat(Boolean) (!= (- (Math|Conversions|ToInteger(Boolean) (Variables|Default|GetRotation%20clamped%20to%20Displacement)) 1) (.AXIS (Utilities|Struct|BreakF_CSVdata _returnvalue_5))))))) -1.0) (.Y (Math|Vector|BreakVector (* (Variables|Default|GetRandom%20Rotation%20[XYZ]) (Math|Conversions|ToFloat(Boolean) (!= (- (Math|Conversions|ToInteger(Boolean) (Variables|Default|GetRotation%20clamped%20to%20Displacement)) 1) (.AXIS (Utilities|Struct|BreakF_CSVdata _returnvalue_5))))))) _displacement_randomize) (Math|Random|RandomFloatinRangefromStream (* (.Z (Math|Vector|BreakVector (* (Variables|Default|GetRandom%20Rotation%20[XYZ]) (Math|Conversions|ToFloat(Boolean) (!= (- (Math|Conversions|ToInteger(Boolean) (Variables|Default|GetRotation%20clamped%20to%20Displacement)) 1) (.AXIS (Utilities|Struct|BreakF_CSVdata _returnvalue_5))))))) -1.0) (.Z (Math|Vector|BreakVector (* (Variables|Default|GetRandom%20Rotation%20[XYZ]) (Math|Conversions|ToFloat(Boolean) (!= (- (Math|Conversions|ToInteger(Boolean) (Variables|Default|GetRotation%20clamped%20to%20Displacement)) 1) (.AXIS (Utilities|Struct|BreakF_CSVdata _returnvalue_5))))))) _displacement_randomize)) (Variables|Default|GetShuffle)))) (.Z (Math|Vector|BreakVector (+ (Math|Vector|MakeVector (Math|Random|RandomFloatinRangefromStream (* (.X (Math|Vector|BreakVector (* (Variables|Default|GetRandom%20Rotation%20[XYZ]) (Math|Conversions|ToFloat(Boolean) (!= (- (Math|Conversions|ToInteger(Boolean) (Variables|Default|GetRotation%20clamped%20to%20Displacement)) 1) (.AXIS (Utilities|Struct|BreakF_CSVdata _returnvalue_5))))))) -1.0) (.X (Math|Vector|BreakVector (* (Variables|Default|GetRandom%20Rotation%20[XYZ]) (Math|Conversions|ToFloat(Boolean) (!= (- (Math|Conversions|ToInteger(Boolean) (Variables|Default|GetRotation%20clamped%20to%20Displacement)) 1) (.AXIS (Utilities|Struct|BreakF_CSVdata _returnvalue_5))))))) _displacement_randomize) (Math|Random|RandomFloatinRangefromStream (* (.Y (Math|Vector|BreakVector (* (Variables|Default|GetRandom%20Rotation%20[XYZ]) (Math|Conversions|ToFloat(Boolean) (!= (- (Math|Conversions|ToInteger(Boolean) (Variables|Default|GetRotation%20clamped%20to%20Displacement)) 1) (.AXIS (Utilities|Struct|BreakF_CSVdata _returnvalue_5))))))) -1.0) (.Y (Math|Vector|BreakVector (* (Variables|Default|GetRandom%20Rotation%20[XYZ]) (Math|Conversions|ToFloat(Boolean) (!= (- (Math|Conversions|ToInteger(Boolean) (Variables|Default|GetRotation%20clamped%20to%20Displacement)) 1) (.AXIS (Utilities|Struct|BreakF_CSVdata _returnvalue_5))))))) _displacement_randomize) (Math|Random|RandomFloatinRangefromStream (* (.Z (Math|Vector|BreakVector (* (Variables|Default|GetRandom%20Rotation%20[XYZ]) (Math|Conversions|ToFloat(Boolean) (!= (- (Math|Conversions|ToInteger(Boolean) (Variables|Default|GetRotation%20clamped%20to%20Displacement)) 1) (.AXIS (Utilities|Struct|BreakF_CSVdata _returnvalue_5))))))) -1.0) (.Z (Math|Vector|BreakVector (* (Variables|Default|GetRandom%20Rotation%20[XYZ]) (Math|Conversions|ToFloat(Boolean) (!= (- (Math|Conversions|ToInteger(Boolean) (Variables|Default|GetRotation%20clamped%20to%20Displacement)) 1) (.AXIS (Utilities|Struct|BreakF_CSVdata _returnvalue_5))))))) _displacement_randomize)) (Variables|Default|GetShuffle))))) (Math|Rotator|MakeRotator (.R_X (Utilities|Struct|BreakF_CSVdata _returnvalue_5)) (.R_Y (Utilities|Struct|BreakF_CSVdata _returnvalue_5)) (.R_Z (Utilities|Struct|BreakF_CSVdata _returnvalue_5)))) (Math|Rotator|MakeRotator (.X (Math|Vector|BreakVector (+ (+ (Math|Vector|MakeVector (Math|Random|RandomFloatinRangefromStream (* (.X (Math|Vector|BreakVector (* (Variables|Default|GetRandom%20Rotation%20[XYZ]) (Math|Conversions|ToFloat(Boolean) (!= (- (Math|Conversions|ToInteger(Boolean) (Variables|Default|GetRotation%20clamped%20to%20Displacement)) 1) (.AXIS (Utilities|Struct|BreakF_CSVdata _returnvalue_5))))))) -1.0) (.X (Math|Vector|BreakVector (* (Variables|Default|GetRandom%20Rotation%20[XYZ]) (Math|Conversions|ToFloat(Boolean) (!= (- (Math|Conversions|ToInteger(Boolean) (Variables|Default|GetRotation%20clamped%20to%20Displacement)) 1) (.AXIS (Utilities|Struct|BreakF_CSVdata _returnvalue_5))))))) _displacement_randomize) (Math|Random|RandomFloatinRangefromStream (* (.Y (Math|Vector|BreakVector (* (Variables|Default|GetRandom%20Rotation%20[XYZ]) (Math|Conversions|ToFloat(Boolean) (!= (- (Math|Conversions|ToInteger(Boolean) (Variables|Default|GetRotation%20clamped%20to%20Displacement)) 1) (.AXIS (Utilities|Struct|BreakF_CSVdata _returnvalue_5))))))) -1.0) (.Y (Math|Vector|BreakVector (* (Variables|Default|GetRandom%20Rotation%20[XYZ]) (Math|Conversions|ToFloat(Boolean) (!= (- (Math|Conversions|ToInteger(Boolean) (Variables|Default|GetRotation%20clamped%20to%20Displacement)) 1) (.AXIS (Utilities|Struct|BreakF_CSVdata _returnvalue_5))))))) _displacement_randomize) (Math|Random|RandomFloatinRangefromStream (* (.Z (Math|Vector|BreakVector (* (Variables|Default|GetRandom%20Rotation%20[XYZ]) (Math|Conversions|ToFloat(Boolean) (!= (- (Math|Conversions|ToInteger(Boolean) (Variables|Default|GetRotation%20clamped%20to%20Displacement)) 1) (.AXIS (Utilities|Struct|BreakF_CSVdata _returnvalue_5))))))) -1.0) (.Z (Math|Vector|BreakVector (* (Variables|Default|GetRandom%20Rotation%20[XYZ]) (Math|Conversions|ToFloat(Boolean) (!= (- (Math|Conversions|ToInteger(Boolean) (Variables|Default|GetRotation%20clamped%20to%20Displacement)) 1) (.AXIS (Utilities|Struct|BreakF_CSVdata _returnvalue_5))))))) _displacement_randomize)) (Variables|Default|GetShuffle)) (Math|Vector|MakeVector (.R_X (Utilities|Struct|BreakF_CSVdata _returnvalue_5)) (.R_Y (Utilities|Struct|BreakF_CSVdata _returnvalue_5)) (.R_Z (Utilities|Struct|BreakF_CSVdata _returnvalue_5)))))) (.Y (Math|Vector|BreakVector (+ (+ (Math|Vector|MakeVector (Math|Random|RandomFloatinRangefromStream (* (.X (Math|Vector|BreakVector (* (Variables|Default|GetRandom%20Rotation%20[XYZ]) (Math|Conversions|ToFloat(Boolean) (!= (- (Math|Conversions|ToInteger(Boolean) (Variables|Default|GetRotation%20clamped%20to%20Displacement)) 1) (.AXIS (Utilities|Struct|BreakF_CSVdata _returnvalue_5))))))) -1.0) (.X (Math|Vector|BreakVector (* (Variables|Default|GetRandom%20Rotation%20[XYZ]) (Math|Conversions|ToFloat(Boolean) (!= (- (Math|Conversions|ToInteger(Boolean) (Variables|Default|GetRotation%20clamped%20to%20Displacement)) 1) (.AXIS (Utilities|Struct|BreakF_CSVdata _returnvalue_5))))))) _displacement_randomize) (Math|Random|RandomFloatinRangefromStream (* (.Y (Math|Vector|BreakVector (* (Variables|Default|GetRandom%20Rotation%20[XYZ]) (Math|Conversions|ToFloat(Boolean) (!= (- (Math|Conversions|ToInteger(Boolean) (Variables|Default|GetRotation%20clamped%20to%20Displacement)) 1) (.AXIS (Utilities|Struct|BreakF_CSVdata _returnvalue_5))))))) -1.0) (.Y (Math|Vector|BreakVector (* (Variables|Default|GetRandom%20Rotation%20[XYZ]) (Math|Conversions|ToFloat(Boolean) (!= (- (Math|Conversions|ToInteger(Boolean) (Variables|Default|GetRotation%20clamped%20to%20Displacement)) 1) (.AXIS (Utilities|Struct|BreakF_CSVdata _returnvalue_5))))))) _displacement_randomize) (Math|Random|RandomFloatinRangefromStream (* (.Z (Math|Vector|BreakVector (* (Variables|Default|GetRandom%20Rotation%20[XYZ]) (Math|Conversions|ToFloat(Boolean) (!= (- (Math|Conversions|ToInteger(Boolean) (Variables|Default|GetRotation%20clamped%20to%20Displacement)) 1) (.AXIS (Utilities|Struct|BreakF_CSVdata _returnvalue_5))))))) -1.0) (.Z (Math|Vector|BreakVector (* (Variables|Default|GetRandom%20Rotation%20[XYZ]) (Math|Conversions|ToFloat(Boolean) (!= (- (Math|Conversions|ToInteger(Boolean) (Variables|Default|GetRotation%20clamped%20to%20Displacement)) 1) (.AXIS (Utilities|Struct|BreakF_CSVdata _returnvalue_5))))))) _displacement_randomize)) (Variables|Default|GetShuffle)) (Math|Vector|MakeVector (.R_X (Utilities|Struct|BreakF_CSVdata _returnvalue_5)) (.R_Y (Utilities|Struct|BreakF_CSVdata _returnvalue_5)) (.R_Z (Utilities|Struct|BreakF_CSVdata _returnvalue_5)))))) (.Z (Math|Vector|BreakVector (+ (+ (Math|Vector|MakeVector (Math|Random|RandomFloatinRangefromStream (* (.X (Math|Vector|BreakVector (* (Variables|Default|GetRandom%20Rotation%20[XYZ]) (Math|Conversions|ToFloat(Boolean) (!= (- (Math|Conversions|ToInteger(Boolean) (Variables|Default|GetRotation%20clamped%20to%20Displacement)) 1) (.AXIS (Utilities|Struct|BreakF_CSVdata _returnvalue_5))))))) -1.0) (.X (Math|Vector|BreakVector (* (Variables|Default|GetRandom%20Rotation%20[XYZ]) (Math|Conversions|ToFloat(Boolean) (!= (- (Math|Conversions|ToInteger(Boolean) (Variables|Default|GetRotation%20clamped%20to%20Displacement)) 1) (.AXIS (Utilities|Struct|BreakF_CSVdata _returnvalue_5))))))) _displacement_randomize) (Math|Random|RandomFloatinRangefromStream (* (.Y (Math|Vector|BreakVector (* (Variables|Default|GetRandom%20Rotation%20[XYZ]) (Math|Conversions|ToFloat(Boolean) (!= (- (Math|Conversions|ToInteger(Boolean) (Variables|Default|GetRotation%20clamped%20to%20Displacement)) 1) (.AXIS (Utilities|Struct|BreakF_CSVdata _returnvalue_5))))))) -1.0) (.Y (Math|Vector|BreakVector (* (Variables|Default|GetRandom%20Rotation%20[XYZ]) (Math|Conversions|ToFloat(Boolean) (!= (- (Math|Conversions|ToInteger(Boolean) (Variables|Default|GetRotation%20clamped%20to%20Displacement)) 1) (.AXIS (Utilities|Struct|BreakF_CSVdata _returnvalue_5))))))) _displacement_randomize) (Math|Random|RandomFloatinRangefromStream (* (.Z (Math|Vector|BreakVector (* (Variables|Default|GetRandom%20Rotation%20[XYZ]) (Math|Conversions|ToFloat(Boolean) (!= (- (Math|Conversions|ToInteger(Boolean) (Variables|Default|GetRotation%20clamped%20to%20Displacement)) 1) (.AXIS (Utilities|Struct|BreakF_CSVdata _returnvalue_5))))))) -1.0) (.Z (Math|Vector|BreakVector (* (Variables|Default|GetRandom%20Rotation%20[XYZ]) (Math|Conversions|ToFloat(Boolean) (!= (- (Math|Conversions|ToInteger(Boolean) (Variables|Default|GetRotation%20clamped%20to%20Displacement)) 1) (.AXIS (Utilities|Struct|BreakF_CSVdata _returnvalue_5))))))) _displacement_randomize)) (Variables|Default|GetShuffle)) (Math|Vector|MakeVector (.R_X (Utilities|Struct|BreakF_CSVdata _returnvalue_5)) (.R_Y (Utilities|Struct|BreakF_CSVdata _returnvalue_5)) (.R_Z (Utilities|Struct|BreakF_CSVdata _returnvalue_5))))))) (Math|Conversions|ToFloat(Boolean) (Variables|Default|GetRandom%20Rotation%20LOCAL/GLOBAL))) (* (Math|Vector|MakeVector (.S_X (Utilities|Struct|BreakF_CSVdata _returnvalue_5)) (.S_Y (Utilities|Struct|BreakF_CSVdata _returnvalue_5)) (.S_Z (Utilities|Struct|BreakF_CSVdata _returnvalue_5))) (Variables|Default|GetScale))) (* (Math|Vector|MakeVector (* (Math|Conversions|ToFloat(Boolean) (== (.AXIS (Utilities|Struct|BreakF_CSVdata _returnvalue_5)) 1)) _returnvalue_3) (* (Math|Conversions|ToFloat(Boolean) (== (.AXIS (Utilities|Struct|BreakF_CSVdata _returnvalue_5)) 2)) _returnvalue_3) (* (Math|Conversions|ToFloat(Boolean) (== (.AXIS (Utilities|Struct|BreakF_CSVdata _returnvalue_5)) 3)) _returnvalue_3)) (Math|Float|Clamp(Float) (+ (Math|Conversions|ToFloat(Boolean) (and (not (Class|KismetMathLibrary|IsPointinBoxwithTransform (Math|Vector|MakeVector (.T_X (Utilities|Struct|BreakF_CSVdata _returnvalue_5)) (.T_Y (Utilities|Struct|BreakF_CSVdata _returnvalue_5)) (.T_Z (Utilities|Struct|BreakF_CSVdata _returnvalue_5))) (Math|Transform|MakeTransform (Variables|Default|GetBox%20Origin%20[XYZ]) (Variables|Default|GetBox%20Rotation%20[XYZ])) (Variables|Default|GetBox%20Extent%20[XYZ]))) _boxcontrolleddisplacement)) (Variables|Default|GetBox%20Intensity)) (Math|Conversions|ToFloat(Boolean) (not _boxcontrolleddisplacement))))) (Math|Rotator|Lerp(Rotator) (Math|Rotator|CombineRotators (Math|Rotator|MakeRotator (.X (Math|Vector|BreakVector (+ (Math|Vector|MakeVector (Math|Random|RandomFloatinRangefromStream (* (.X (Math|Vector|BreakVector (* (Variables|Default|GetRandom%20Rotation%20[XYZ]) (Math|Conversions|ToFloat(Boolean) (!= (- (Math|Conversions|ToInteger(Boolean) (Variables|Default|GetRotation%20clamped%20to%20Displacement)) 1) (.AXIS (Utilities|Struct|BreakF_CSVdata _returnvalue_5))))))) -1.0) (.X (Math|Vector|BreakVector (* (Variables|Default|GetRandom%20Rotation%20[XYZ]) (Math|Conversions|ToFloat(Boolean) (!= (- (Math|Conversions|ToInteger(Boolean) (Variables|Default|GetRotation%20clamped%20to%20Displacement)) 1) (.AXIS (Utilities|Struct|BreakF_CSVdata _returnvalue_5))))))) _displacement_randomize) (Math|Random|RandomFloatinRangefromStream (* (.Y (Math|Vector|BreakVector (* (Variables|Default|GetRandom%20Rotation%20[XYZ]) (Math|Conversions|ToFloat(Boolean) (!= (- (Math|Conversions|ToInteger(Boolean) (Variables|Default|GetRotation%20clamped%20to%20Displacement)) 1) (.AXIS (Utilities|Struct|BreakF_CSVdata _returnvalue_5))))))) -1.0) (.Y (Math|Vector|BreakVector (* (Variables|Default|GetRandom%20Rotation%20[XYZ]) (Math|Conversions|ToFloat(Boolean) (!= (- (Math|Conversions|ToInteger(Boolean) (Variables|Default|GetRotation%20clamped%20to%20Displacement)) 1) (.AXIS (Utilities|Struct|BreakF_CSVdata _returnvalue_5))))))) _displacement_randomize) (Math|Random|RandomFloatinRangefromStream (* (.Z (Math|Vector|BreakVector (* (Variables|Default|GetRandom%20Rotation%20[XYZ]) (Math|Conversions|ToFloat(Boolean) (!= (- (Math|Conversions|ToInteger(Boolean) (Variables|Default|GetRotation%20clamped%20to%20Displacement)) 1) (.AXIS (Utilities|Struct|BreakF_CSVdata _returnvalue_5))))))) -1.0) (.Z (Math|Vector|BreakVector (* (Variables|Default|GetRandom%20Rotation%20[XYZ]) (Math|Conversions|ToFloat(Boolean) (!= (- (Math|Conversions|ToInteger(Boolean) (Variables|Default|GetRotation%20clamped%20to%20Displacement)) 1) (.AXIS (Utilities|Struct|BreakF_CSVdata _returnvalue_5))))))) _displacement_randomize)) (Variables|Default|GetShuffle)))) (.Y (Math|Vector|BreakVector (+ (Math|Vector|MakeVector (Math|Random|RandomFloatinRangefromStream (* (.X (Math|Vector|BreakVector (* (Variables|Default|GetRandom%20Rotation%20[XYZ]) (Math|Conversions|ToFloat(Boolean) (!= (- (Math|Conversions|ToInteger(Boolean) (Variables|Default|GetRotation%20clamped%20to%20Displacement)) 1) (.AXIS (Utilities|Struct|BreakF_CSVdata _returnvalue_5))))))) -1.0) (.X (Math|Vector|BreakVector (* (Variables|Default|GetRandom%20Rotation%20[XYZ]) (Math|Conversions|ToFloat(Boolean) (!= (- (Math|Conversions|ToInteger(Boolean) (Variables|Default|GetRotation%20clamped%20to%20Displacement)) 1) (.AXIS (Utilities|Struct|BreakF_CSVdata _returnvalue_5))))))) _displacement_randomize) (Math|Random|RandomFloatinRangefromStream (* (.Y (Math|Vector|BreakVector (* (Variables|Default|GetRandom%20Rotation%20[XYZ]) (Math|Conversions|ToFloat(Boolean) (!= (- (Math|Conversions|ToInteger(Boolean) (Variables|Default|GetRotation%20clamped%20to%20Displacement)) 1) (.AXIS (Utilities|Struct|BreakF_CSVdata _returnvalue_5))))))) -1.0) (.Y (Math|Vector|BreakVector (* (Variables|Default|GetRandom%20Rotation%20[XYZ]) (Math|Conversions|ToFloat(Boolean) (!= (- (Math|Conversions|ToInteger(Boolean) (Variables|Default|GetRotation%20clamped%20to%20Displacement)) 1) (.AXIS (Utilities|Struct|BreakF_CSVdata _returnvalue_5))))))) _displacement_randomize) (Math|Random|RandomFloatinRangefromStream (* (.Z (Math|Vector|BreakVector (* (Variables|Default|GetRandom%20Rotation%20[XYZ]) (Math|Conversions|ToFloat(Boolean) (!= (- (Math|Conversions|ToInteger(Boolean) (Variables|Default|GetRotation%20clamped%20to%20Displacement)) 1) (.AXIS (Utilities|Struct|BreakF_CSVdata _returnvalue_5))))))) -1.0) (.Z (Math|Vector|BreakVector (* (Variables|Default|GetRandom%20Rotation%20[XYZ]) (Math|Conversions|ToFloat(Boolean) (!= (- (Math|Conversions|ToInteger(Boolean) (Variables|Default|GetRotation%20clamped%20to%20Displacement)) 1) (.AXIS (Utilities|Struct|BreakF_CSVdata _returnvalue_5))))))) _displacement_randomize)) (Variables|Default|GetShuffle)))) (.Z (Math|Vector|BreakVector (+ (Math|Vector|MakeVector (Math|Random|RandomFloatinRangefromStream (* (.X (Math|Vector|BreakVector (* (Variables|Default|GetRandom%20Rotation%20[XYZ]) (Math|Conversions|ToFloat(Boolean) (!= (- (Math|Conversions|ToInteger(Boolean) (Variables|Default|GetRotation%20clamped%20to%20Displacement)) 1) (.AXIS (Utilities|Struct|BreakF_CSVdata _returnvalue_5))))))) -1.0) (.X (Math|Vector|BreakVector (* (Variables|Default|GetRandom%20Rotation%20[XYZ]) (Math|Conversions|ToFloat(Boolean) (!= (- (Math|Conversions|ToInteger(Boolean) (Variables|Default|GetRotation%20clamped%20to%20Displacement)) 1) (.AXIS (Utilities|Struct|BreakF_CSVdata _returnvalue_5))))))) _displacement_randomize) (Math|Random|RandomFloatinRangefromStream (* (.Y (Math|Vector|BreakVector (* (Variables|Default|GetRandom%20Rotation%20[XYZ]) (Math|Conversions|ToFloat(Boolean) (!= (- (Math|Conversions|ToInteger(Boolean) (Variables|Default|GetRotation%20clamped%20to%20Displacement)) 1) (.AXIS (Utilities|Struct|BreakF_CSVdata _returnvalue_5))))))) -1.0) (.Y (Math|Vector|BreakVector (* (Variables|Default|GetRandom%20Rotation%20[XYZ]) (Math|Conversions|ToFloat(Boolean) (!= (- (Math|Conversions|ToInteger(Boolean) (Variables|Default|GetRotation%20clamped%20to%20Displacement)) 1) (.AXIS (Utilities|Struct|BreakF_CSVdata _returnvalue_5))))))) _displacement_randomize) (Math|Random|RandomFloatinRangefromStream (* (.Z (Math|Vector|BreakVector (* (Variables|Default|GetRandom%20Rotation%20[XYZ]) (Math|Conversions|ToFloat(Boolean) (!= (- (Math|Conversions|ToInteger(Boolean) (Variables|Default|GetRotation%20clamped%20to%20Displacement)) 1) (.AXIS (Utilities|Struct|BreakF_CSVdata _returnvalue_5))))))) -1.0) (.Z (Math|Vector|BreakVector (* (Variables|Default|GetRandom%20Rotation%20[XYZ]) (Math|Conversions|ToFloat(Boolean) (!= (- (Math|Conversions|ToInteger(Boolean) (Variables|Default|GetRotation%20clamped%20to%20Displacement)) 1) (.AXIS (Utilities|Struct|BreakF_CSVdata _returnvalue_5))))))) _displacement_randomize)) (Variables|Default|GetShuffle))))) (Math|Rotator|MakeRotator (.R_X (Utilities|Struct|BreakF_CSVdata _returnvalue_5)) (.R_Y (Utilities|Struct|BreakF_CSVdata _returnvalue_5)) (.R_Z (Utilities|Struct|BreakF_CSVdata _returnvalue_5)))) (Math|Rotator|MakeRotator (.X (Math|Vector|BreakVector (+ (+ (Math|Vector|MakeVector (Math|Random|RandomFloatinRangefromStream (* (.X (Math|Vector|BreakVector (* (Variables|Default|GetRandom%20Rotation%20[XYZ]) (Math|Conversions|ToFloat(Boolean) (!= (- (Math|Conversions|ToInteger(Boolean) (Variables|Default|GetRotation%20clamped%20to%20Displacement)) 1) (.AXIS (Utilities|Struct|BreakF_CSVdata _returnvalue_5))))))) -1.0) (.X (Math|Vector|BreakVector (* (Variables|Default|GetRandom%20Rotation%20[XYZ]) (Math|Conversions|ToFloat(Boolean) (!= (- (Math|Conversions|ToInteger(Boolean) (Variables|Default|GetRotation%20clamped%20to%20Displacement)) 1) (.AXIS (Utilities|Struct|BreakF_CSVdata _returnvalue_5))))))) _displacement_randomize) (Math|Random|RandomFloatinRangefromStream (* (.Y (Math|Vector|BreakVector (* (Variables|Default|GetRandom%20Rotation%20[XYZ]) (Math|Conversions|ToFloat(Boolean) (!= (- (Math|Conversions|ToInteger(Boolean) (Variables|Default|GetRotation%20clamped%20to%20Displacement)) 1) (.AXIS (Utilities|Struct|BreakF_CSVdata _returnvalue_5))))))) -1.0) (.Y (Math|Vector|BreakVector (* (Variables|Default|GetRandom%20Rotation%20[XYZ]) (Math|Conversions|ToFloat(Boolean) (!= (- (Math|Conversions|ToInteger(Boolean) (Variables|Default|GetRotation%20clamped%20to%20Displacement)) 1) (.AXIS (Utilities|Struct|BreakF_CSVdata _returnvalue_5))))))) _displacement_randomize) (Math|Random|RandomFloatinRangefromStream (* (.Z (Math|Vector|BreakVector (* (Variables|Default|GetRandom%20Rotation%20[XYZ]) (Math|Conversions|ToFloat(Boolean) (!= (- (Math|Conversions|ToInteger(Boolean) (Variables|Default|GetRotation%20clamped%20to%20Displacement)) 1) (.AXIS (Utilities|Struct|BreakF_CSVdata _returnvalue_5))))))) -1.0) (.Z (Math|Vector|BreakVector (* (Variables|Default|GetRandom%20Rotation%20[XYZ]) (Math|Conversions|ToFloat(Boolean) (!= (- (Math|Conversions|ToInteger(Boolean) (Variables|Default|GetRotation%20clamped%20to%20Displacement)) 1) (.AXIS (Utilities|Struct|BreakF_CSVdata _returnvalue_5))))))) _displacement_randomize)) (Variables|Default|GetShuffle)) (Math|Vector|MakeVector (.R_X (Utilities|Struct|BreakF_CSVdata _returnvalue_5)) (.R_Y (Utilities|Struct|BreakF_CSVdata _returnvalue_5)) (.R_Z (Utilities|Struct|BreakF_CSVdata _returnvalue_5)))))) (.Y (Math|Vector|BreakVector (+ (+ (Math|Vector|MakeVector (Math|Random|RandomFloatinRangefromStream (* (.X (Math|Vector|BreakVector (* (Variables|Default|GetRandom%20Rotation%20[XYZ]) (Math|Conversions|ToFloat(Boolean) (!= (- (Math|Conversions|ToInteger(Boolean) (Variables|Default|GetRotation%20clamped%20to%20Displacement)) 1) (.AXIS (Utilities|Struct|BreakF_CSVdata _returnvalue_5))))))) -1.0) (.X (Math|Vector|BreakVector (* (Variables|Default|GetRandom%20Rotation%20[XYZ]) (Math|Conversions|ToFloat(Boolean) (!= (- (Math|Conversions|ToInteger(Boolean) (Variables|Default|GetRotation%20clamped%20to%20Displacement)) 1) (.AXIS (Utilities|Struct|BreakF_CSVdata _returnvalue_5))))))) _displacement_randomize) (Math|Random|RandomFloatinRangefromStream (* (.Y (Math|Vector|BreakVector (* (Variables|Default|GetRandom%20Rotation%20[XYZ]) (Math|Conversions|ToFloat(Boolean) (!= (- (Math|Conversions|ToInteger(Boolean) (Variables|Default|GetRotation%20clamped%20to%20Displacement)) 1) (.AXIS (Utilities|Struct|BreakF_CSVdata _returnvalue_5))))))) -1.0) (.Y (Math|Vector|BreakVector (* (Variables|Default|GetRandom%20Rotation%20[XYZ]) (Math|Conversions|ToFloat(Boolean) (!= (- (Math|Conversions|ToInteger(Boolean) (Variables|Default|GetRotation%20clamped%20to%20Displacement)) 1) (.AXIS (Utilities|Struct|BreakF_CSVdata _returnvalue_5))))))) _displacement_randomize) (Math|Random|RandomFloatinRangefromStream (* (.Z (Math|Vector|BreakVector (* (Variables|Default|GetRandom%20Rotation%20[XYZ]) (Math|Conversions|ToFloat(Boolean) (!= (- (Math|Conversions|ToInteger(Boolean) (Variables|Default|GetRotation%20clamped%20to%20Displacement)) 1) (.AXIS (Utilities|Struct|BreakF_CSVdata _returnvalue_5))))))) -1.0) (.Z (Math|Vector|BreakVector (* (Variables|Default|GetRandom%20Rotation%20[XYZ]) (Math|Conversions|ToFloat(Boolean) (!= (- (Math|Conversions|ToInteger(Boolean) (Variables|Default|GetRotation%20clamped%20to%20Displacement)) 1) (.AXIS (Utilities|Struct|BreakF_CSVdata _returnvalue_5))))))) _displacement_randomize)) (Variables|Default|GetShuffle)) (Math|Vector|MakeVector (.R_X (Utilities|Struct|BreakF_CSVdata _returnvalue_5)) (.R_Y (Utilities|Struct|BreakF_CSVdata _returnvalue_5)) (.R_Z (Utilities|Struct|BreakF_CSVdata _returnvalue_5)))))) (.Z (Math|Vector|BreakVector (+ (+ (Math|Vector|MakeVector (Math|Random|RandomFloatinRangefromStream (* (.X (Math|Vector|BreakVector (* (Variables|Default|GetRandom%20Rotation%20[XYZ]) (Math|Conversions|ToFloat(Boolean) (!= (- (Math|Conversions|ToInteger(Boolean) (Variables|Default|GetRotation%20clamped%20to%20Displacement)) 1) (.AXIS (Utilities|Struct|BreakF_CSVdata _returnvalue_5))))))) -1.0) (.X (Math|Vector|BreakVector (* (Variables|Default|GetRandom%20Rotation%20[XYZ]) (Math|Conversions|ToFloat(Boolean) (!= (- (Math|Conversions|ToInteger(Boolean) (Variables|Default|GetRotation%20clamped%20to%20Displacement)) 1) (.AXIS (Utilities|Struct|BreakF_CSVdata _returnvalue_5))))))) _displacement_randomize) (Math|Random|RandomFloatinRangefromStream (* (.Y (Math|Vector|BreakVector (* (Variables|Default|GetRandom%20Rotation%20[XYZ]) (Math|Conversions|ToFloat(Boolean) (!= (- (Math|Conversions|ToInteger(Boolean) (Variables|Default|GetRotation%20clamped%20to%20Displacement)) 1) (.AXIS (Utilities|Struct|BreakF_CSVdata _returnvalue_5))))))) -1.0) (.Y (Math|Vector|BreakVector (* (Variables|Default|GetRandom%20Rotation%20[XYZ]) (Math|Conversions|ToFloat(Boolean) (!= (- (Math|Conversions|ToInteger(Boolean) (Variables|Default|GetRotation%20clamped%20to%20Displacement)) 1) (.AXIS (Utilities|Struct|BreakF_CSVdata _returnvalue_5))))))) _displacement_randomize) (Math|Random|RandomFloatinRangefromStream (* (.Z (Math|Vector|BreakVector (* (Variables|Default|GetRandom%20Rotation%20[XYZ]) (Math|Conversions|ToFloat(Boolean) (!= (- (Math|Conversions|ToInteger(Boolean) (Variables|Default|GetRotation%20clamped%20to%20Displacement)) 1) (.AXIS (Utilities|Struct|BreakF_CSVdata _returnvalue_5))))))) -1.0) (.Z (Math|Vector|BreakVector (* (Variables|Default|GetRandom%20Rotation%20[XYZ]) (Math|Conversions|ToFloat(Boolean) (!= (- (Math|Conversions|ToInteger(Boolean) (Variables|Default|GetRotation%20clamped%20to%20Displacement)) 1) (.AXIS (Utilities|Struct|BreakF_CSVdata _returnvalue_5))))))) _displacement_randomize)) (Variables|Default|GetShuffle)) (Math|Vector|MakeVector (.R_X (Utilities|Struct|BreakF_CSVdata _returnvalue_5)) (.R_Y (Utilities|Struct|BreakF_CSVdata _returnvalue_5)) (.R_Z (Utilities|Struct|BreakF_CSVdata _returnvalue_5))))))) (Math|Conversions|ToFloat(Boolean) (Variables|Default|GetRandom%20Rotation%20LOCAL/GLOBAL))) (* (Math|Vector|MakeVector (.S_X (Utilities|Struct|BreakF_CSVdata _returnvalue_5)) (.S_Y (Utilities|Struct|BreakF_CSVdata _returnvalue_5)) (.S_Z (Utilities|Struct|BreakF_CSVdata _returnvalue_5))) (Variables|Default|GetScale))) false)))))
                        (else
                          (goto _label_4)))))
                  (:3
                    (if _undamaged_stones
                      (goto _label)
                      (elif _extrastones
                        (goto _label_2)
                        (else
                          (goto _label_5)))))
                  (:4
                    (if _undamaged_stones
                      (goto _label)
                      (elif _extrastones
                        (goto _label_2)
                        (else
                          (goto _label_3)))))
                  (:5
                    (if _undamaged_stones
                      (goto _label)
                      (elif _extrastones
                        (goto _label_2)
                        (else
                          (goto _label_6)))))
                  (:6
                    (if _undamaged_stones
                      (goto _label)
                      (elif _extrastones
                        (goto _label_2)
                        (else
                          (Utilities|FlowControl|Sequence
                            (:then_0
                              (Utilities|FlowControl|DoOnce false
                                (:Completed
                                  (bind _returnvalue_11 (AddComponent|AddHierarchicalInstancedStaticMeshComponent false))
                                  (bind _output_get_6 (Variables|Default|Set06 _returnvalue_11))
                                  (Rendering|Material|SetMaterial _output_get_6 0 (Variables|Default|GetStone%20Material)))))
                            (:then_1
                              (Components|InstancedStaticMesh|AddInstance (Variables|Default|Get06) (Math|Transform|MakeTransform (Math|Transform|TransformLocation (Math|Transform|MakeTransform (Math|Vector|MakeVector (.T_X (Utilities|Struct|BreakF_CSVdata _returnvalue_5)) (.T_Y (Utilities|Struct|BreakF_CSVdata _returnvalue_5)) (.T_Z (Utilities|Struct|BreakF_CSVdata _returnvalue_5))) (Math|Rotator|Lerp(Rotator) (Math|Rotator|CombineRotators (Math|Rotator|MakeRotator (.X (Math|Vector|BreakVector (+ (Math|Vector|MakeVector (Math|Random|RandomFloatinRangefromStream (* (.X (Math|Vector|BreakVector (* (Variables|Default|GetRandom%20Rotation%20[XYZ]) (Math|Conversions|ToFloat(Boolean) (!= (- (Math|Conversions|ToInteger(Boolean) (Variables|Default|GetRotation%20clamped%20to%20Displacement)) 1) (.AXIS (Utilities|Struct|BreakF_CSVdata _returnvalue_5))))))) -1.0) (.X (Math|Vector|BreakVector (* (Variables|Default|GetRandom%20Rotation%20[XYZ]) (Math|Conversions|ToFloat(Boolean) (!= (- (Math|Conversions|ToInteger(Boolean) (Variables|Default|GetRotation%20clamped%20to%20Displacement)) 1) (.AXIS (Utilities|Struct|BreakF_CSVdata _returnvalue_5))))))) _displacement_randomize) (Math|Random|RandomFloatinRangefromStream (* (.Y (Math|Vector|BreakVector (* (Variables|Default|GetRandom%20Rotation%20[XYZ]) (Math|Conversions|ToFloat(Boolean) (!= (- (Math|Conversions|ToInteger(Boolean) (Variables|Default|GetRotation%20clamped%20to%20Displacement)) 1) (.AXIS (Utilities|Struct|BreakF_CSVdata _returnvalue_5))))))) -1.0) (.Y (Math|Vector|BreakVector (* (Variables|Default|GetRandom%20Rotation%20[XYZ]) (Math|Conversions|ToFloat(Boolean) (!= (- (Math|Conversions|ToInteger(Boolean) (Variables|Default|GetRotation%20clamped%20to%20Displacement)) 1) (.AXIS (Utilities|Struct|BreakF_CSVdata _returnvalue_5))))))) _displacement_randomize) (Math|Random|RandomFloatinRangefromStream (* (.Z (Math|Vector|BreakVector (* (Variables|Default|GetRandom%20Rotation%20[XYZ]) (Math|Conversions|ToFloat(Boolean) (!= (- (Math|Conversions|ToInteger(Boolean) (Variables|Default|GetRotation%20clamped%20to%20Displacement)) 1) (.AXIS (Utilities|Struct|BreakF_CSVdata _returnvalue_5))))))) -1.0) (.Z (Math|Vector|BreakVector (* (Variables|Default|GetRandom%20Rotation%20[XYZ]) (Math|Conversions|ToFloat(Boolean) (!= (- (Math|Conversions|ToInteger(Boolean) (Variables|Default|GetRotation%20clamped%20to%20Displacement)) 1) (.AXIS (Utilities|Struct|BreakF_CSVdata _returnvalue_5))))))) _displacement_randomize)) (Variables|Default|GetShuffle)))) (.Y (Math|Vector|BreakVector (+ (Math|Vector|MakeVector (Math|Random|RandomFloatinRangefromStream (* (.X (Math|Vector|BreakVector (* (Variables|Default|GetRandom%20Rotation%20[XYZ]) (Math|Conversions|ToFloat(Boolean) (!= (- (Math|Conversions|ToInteger(Boolean) (Variables|Default|GetRotation%20clamped%20to%20Displacement)) 1) (.AXIS (Utilities|Struct|BreakF_CSVdata _returnvalue_5))))))) -1.0) (.X (Math|Vector|BreakVector (* (Variables|Default|GetRandom%20Rotation%20[XYZ]) (Math|Conversions|ToFloat(Boolean) (!= (- (Math|Conversions|ToInteger(Boolean) (Variables|Default|GetRotation%20clamped%20to%20Displacement)) 1) (.AXIS (Utilities|Struct|BreakF_CSVdata _returnvalue_5))))))) _displacement_randomize) (Math|Random|RandomFloatinRangefromStream (* (.Y (Math|Vector|BreakVector (* (Variables|Default|GetRandom%20Rotation%20[XYZ]) (Math|Conversions|ToFloat(Boolean) (!= (- (Math|Conversions|ToInteger(Boolean) (Variables|Default|GetRotation%20clamped%20to%20Displacement)) 1) (.AXIS (Utilities|Struct|BreakF_CSVdata _returnvalue_5))))))) -1.0) (.Y (Math|Vector|BreakVector (* (Variables|Default|GetRandom%20Rotation%20[XYZ]) (Math|Conversions|ToFloat(Boolean) (!= (- (Math|Conversions|ToInteger(Boolean) (Variables|Default|GetRotation%20clamped%20to%20Displacement)) 1) (.AXIS (Utilities|Struct|BreakF_CSVdata _returnvalue_5))))))) _displacement_randomize) (Math|Random|RandomFloatinRangefromStream (* (.Z (Math|Vector|BreakVector (* (Variables|Default|GetRandom%20Rotation%20[XYZ]) (Math|Conversions|ToFloat(Boolean) (!= (- (Math|Conversions|ToInteger(Boolean) (Variables|Default|GetRotation%20clamped%20to%20Displacement)) 1) (.AXIS (Utilities|Struct|BreakF_CSVdata _returnvalue_5))))))) -1.0) (.Z (Math|Vector|BreakVector (* (Variables|Default|GetRandom%20Rotation%20[XYZ]) (Math|Conversions|ToFloat(Boolean) (!= (- (Math|Conversions|ToInteger(Boolean) (Variables|Default|GetRotation%20clamped%20to%20Displacement)) 1) (.AXIS (Utilities|Struct|BreakF_CSVdata _returnvalue_5))))))) _displacement_randomize)) (Variables|Default|GetShuffle)))) (.Z (Math|Vector|BreakVector (+ (Math|Vector|MakeVector (Math|Random|RandomFloatinRangefromStream (* (.X (Math|Vector|BreakVector (* (Variables|Default|GetRandom%20Rotation%20[XYZ]) (Math|Conversions|ToFloat(Boolean) (!= (- (Math|Conversions|ToInteger(Boolean) (Variables|Default|GetRotation%20clamped%20to%20Displacement)) 1) (.AXIS (Utilities|Struct|BreakF_CSVdata _returnvalue_5))))))) -1.0) (.X (Math|Vector|BreakVector (* (Variables|Default|GetRandom%20Rotation%20[XYZ]) (Math|Conversions|ToFloat(Boolean) (!= (- (Math|Conversions|ToInteger(Boolean) (Variables|Default|GetRotation%20clamped%20to%20Displacement)) 1) (.AXIS (Utilities|Struct|BreakF_CSVdata _returnvalue_5))))))) _displacement_randomize) (Math|Random|RandomFloatinRangefromStream (* (.Y (Math|Vector|BreakVector (* (Variables|Default|GetRandom%20Rotation%20[XYZ]) (Math|Conversions|ToFloat(Boolean) (!= (- (Math|Conversions|ToInteger(Boolean) (Variables|Default|GetRotation%20clamped%20to%20Displacement)) 1) (.AXIS (Utilities|Struct|BreakF_CSVdata _returnvalue_5))))))) -1.0) (.Y (Math|Vector|BreakVector (* (Variables|Default|GetRandom%20Rotation%20[XYZ]) (Math|Conversions|ToFloat(Boolean) (!= (- (Math|Conversions|ToInteger(Boolean) (Variables|Default|GetRotation%20clamped%20to%20Displacement)) 1) (.AXIS (Utilities|Struct|BreakF_CSVdata _returnvalue_5))))))) _displacement_randomize) (Math|Random|RandomFloatinRangefromStream (* (.Z (Math|Vector|BreakVector (* (Variables|Default|GetRandom%20Rotation%20[XYZ]) (Math|Conversions|ToFloat(Boolean) (!= (- (Math|Conversions|ToInteger(Boolean) (Variables|Default|GetRotation%20clamped%20to%20Displacement)) 1) (.AXIS (Utilities|Struct|BreakF_CSVdata _returnvalue_5))))))) -1.0) (.Z (Math|Vector|BreakVector (* (Variables|Default|GetRandom%20Rotation%20[XYZ]) (Math|Conversions|ToFloat(Boolean) (!= (- (Math|Conversions|ToInteger(Boolean) (Variables|Default|GetRotation%20clamped%20to%20Displacement)) 1) (.AXIS (Utilities|Struct|BreakF_CSVdata _returnvalue_5))))))) _displacement_randomize)) (Variables|Default|GetShuffle))))) (Math|Rotator|MakeRotator (.R_X (Utilities|Struct|BreakF_CSVdata _returnvalue_5)) (.R_Y (Utilities|Struct|BreakF_CSVdata _returnvalue_5)) (.R_Z (Utilities|Struct|BreakF_CSVdata _returnvalue_5)))) (Math|Rotator|MakeRotator (.X (Math|Vector|BreakVector (+ (+ (Math|Vector|MakeVector (Math|Random|RandomFloatinRangefromStream (* (.X (Math|Vector|BreakVector (* (Variables|Default|GetRandom%20Rotation%20[XYZ]) (Math|Conversions|ToFloat(Boolean) (!= (- (Math|Conversions|ToInteger(Boolean) (Variables|Default|GetRotation%20clamped%20to%20Displacement)) 1) (.AXIS (Utilities|Struct|BreakF_CSVdata _returnvalue_5))))))) -1.0) (.X (Math|Vector|BreakVector (* (Variables|Default|GetRandom%20Rotation%20[XYZ]) (Math|Conversions|ToFloat(Boolean) (!= (- (Math|Conversions|ToInteger(Boolean) (Variables|Default|GetRotation%20clamped%20to%20Displacement)) 1) (.AXIS (Utilities|Struct|BreakF_CSVdata _returnvalue_5))))))) _displacement_randomize) (Math|Random|RandomFloatinRangefromStream (* (.Y (Math|Vector|BreakVector (* (Variables|Default|GetRandom%20Rotation%20[XYZ]) (Math|Conversions|ToFloat(Boolean) (!= (- (Math|Conversions|ToInteger(Boolean) (Variables|Default|GetRotation%20clamped%20to%20Displacement)) 1) (.AXIS (Utilities|Struct|BreakF_CSVdata _returnvalue_5))))))) -1.0) (.Y (Math|Vector|BreakVector (* (Variables|Default|GetRandom%20Rotation%20[XYZ]) (Math|Conversions|ToFloat(Boolean) (!= (- (Math|Conversions|ToInteger(Boolean) (Variables|Default|GetRotation%20clamped%20to%20Displacement)) 1) (.AXIS (Utilities|Struct|BreakF_CSVdata _returnvalue_5))))))) _displacement_randomize) (Math|Random|RandomFloatinRangefromStream (* (.Z (Math|Vector|BreakVector (* (Variables|Default|GetRandom%20Rotation%20[XYZ]) (Math|Conversions|ToFloat(Boolean) (!= (- (Math|Conversions|ToInteger(Boolean) (Variables|Default|GetRotation%20clamped%20to%20Displacement)) 1) (.AXIS (Utilities|Struct|BreakF_CSVdata _returnvalue_5))))))) -1.0) (.Z (Math|Vector|BreakVector (* (Variables|Default|GetRandom%20Rotation%20[XYZ]) (Math|Conversions|ToFloat(Boolean) (!= (- (Math|Conversions|ToInteger(Boolean) (Variables|Default|GetRotation%20clamped%20to%20Displacement)) 1) (.AXIS (Utilities|Struct|BreakF_CSVdata _returnvalue_5))))))) _displacement_randomize)) (Variables|Default|GetShuffle)) (Math|Vector|MakeVector (.R_X (Utilities|Struct|BreakF_CSVdata _returnvalue_5)) (.R_Y (Utilities|Struct|BreakF_CSVdata _returnvalue_5)) (.R_Z (Utilities|Struct|BreakF_CSVdata _returnvalue_5)))))) (.Y (Math|Vector|BreakVector (+ (+ (Math|Vector|MakeVector (Math|Random|RandomFloatinRangefromStream (* (.X (Math|Vector|BreakVector (* (Variables|Default|GetRandom%20Rotation%20[XYZ]) (Math|Conversions|ToFloat(Boolean) (!= (- (Math|Conversions|ToInteger(Boolean) (Variables|Default|GetRotation%20clamped%20to%20Displacement)) 1) (.AXIS (Utilities|Struct|BreakF_CSVdata _returnvalue_5))))))) -1.0) (.X (Math|Vector|BreakVector (* (Variables|Default|GetRandom%20Rotation%20[XYZ]) (Math|Conversions|ToFloat(Boolean) (!= (- (Math|Conversions|ToInteger(Boolean) (Variables|Default|GetRotation%20clamped%20to%20Displacement)) 1) (.AXIS (Utilities|Struct|BreakF_CSVdata _returnvalue_5))))))) _displacement_randomize) (Math|Random|RandomFloatinRangefromStream (* (.Y (Math|Vector|BreakVector (* (Variables|Default|GetRandom%20Rotation%20[XYZ]) (Math|Conversions|ToFloat(Boolean) (!= (- (Math|Conversions|ToInteger(Boolean) (Variables|Default|GetRotation%20clamped%20to%20Displacement)) 1) (.AXIS (Utilities|Struct|BreakF_CSVdata _returnvalue_5))))))) -1.0) (.Y (Math|Vector|BreakVector (* (Variables|Default|GetRandom%20Rotation%20[XYZ]) (Math|Conversions|ToFloat(Boolean) (!= (- (Math|Conversions|ToInteger(Boolean) (Variables|Default|GetRotation%20clamped%20to%20Displacement)) 1) (.AXIS (Utilities|Struct|BreakF_CSVdata _returnvalue_5))))))) _displacement_randomize) (Math|Random|RandomFloatinRangefromStream (* (.Z (Math|Vector|BreakVector (* (Variables|Default|GetRandom%20Rotation%20[XYZ]) (Math|Conversions|ToFloat(Boolean) (!= (- (Math|Conversions|ToInteger(Boolean) (Variables|Default|GetRotation%20clamped%20to%20Displacement)) 1) (.AXIS (Utilities|Struct|BreakF_CSVdata _returnvalue_5))))))) -1.0) (.Z (Math|Vector|BreakVector (* (Variables|Default|GetRandom%20Rotation%20[XYZ]) (Math|Conversions|ToFloat(Boolean) (!= (- (Math|Conversions|ToInteger(Boolean) (Variables|Default|GetRotation%20clamped%20to%20Displacement)) 1) (.AXIS (Utilities|Struct|BreakF_CSVdata _returnvalue_5))))))) _displacement_randomize)) (Variables|Default|GetShuffle)) (Math|Vector|MakeVector (.R_X (Utilities|Struct|BreakF_CSVdata _returnvalue_5)) (.R_Y (Utilities|Struct|BreakF_CSVdata _returnvalue_5)) (.R_Z (Utilities|Struct|BreakF_CSVdata _returnvalue_5)))))) (.Z (Math|Vector|BreakVector (+ (+ (Math|Vector|MakeVector (Math|Random|RandomFloatinRangefromStream (* (.X (Math|Vector|BreakVector (* (Variables|Default|GetRandom%20Rotation%20[XYZ]) (Math|Conversions|ToFloat(Boolean) (!= (- (Math|Conversions|ToInteger(Boolean) (Variables|Default|GetRotation%20clamped%20to%20Displacement)) 1) (.AXIS (Utilities|Struct|BreakF_CSVdata _returnvalue_5))))))) -1.0) (.X (Math|Vector|BreakVector (* (Variables|Default|GetRandom%20Rotation%20[XYZ]) (Math|Conversions|ToFloat(Boolean) (!= (- (Math|Conversions|ToInteger(Boolean) (Variables|Default|GetRotation%20clamped%20to%20Displacement)) 1) (.AXIS (Utilities|Struct|BreakF_CSVdata _returnvalue_5))))))) _displacement_randomize) (Math|Random|RandomFloatinRangefromStream (* (.Y (Math|Vector|BreakVector (* (Variables|Default|GetRandom%20Rotation%20[XYZ]) (Math|Conversions|ToFloat(Boolean) (!= (- (Math|Conversions|ToInteger(Boolean) (Variables|Default|GetRotation%20clamped%20to%20Displacement)) 1) (.AXIS (Utilities|Struct|BreakF_CSVdata _returnvalue_5))))))) -1.0) (.Y (Math|Vector|BreakVector (* (Variables|Default|GetRandom%20Rotation%20[XYZ]) (Math|Conversions|ToFloat(Boolean) (!= (- (Math|Conversions|ToInteger(Boolean) (Variables|Default|GetRotation%20clamped%20to%20Displacement)) 1) (.AXIS (Utilities|Struct|BreakF_CSVdata _returnvalue_5))))))) _displacement_randomize) (Math|Random|RandomFloatinRangefromStream (* (.Z (Math|Vector|BreakVector (* (Variables|Default|GetRandom%20Rotation%20[XYZ]) (Math|Conversions|ToFloat(Boolean) (!= (- (Math|Conversions|ToInteger(Boolean) (Variables|Default|GetRotation%20clamped%20to%20Displacement)) 1) (.AXIS (Utilities|Struct|BreakF_CSVdata _returnvalue_5))))))) -1.0) (.Z (Math|Vector|BreakVector (* (Variables|Default|GetRandom%20Rotation%20[XYZ]) (Math|Conversions|ToFloat(Boolean) (!= (- (Math|Conversions|ToInteger(Boolean) (Variables|Default|GetRotation%20clamped%20to%20Displacement)) 1) (.AXIS (Utilities|Struct|BreakF_CSVdata _returnvalue_5))))))) _displacement_randomize)) (Variables|Default|GetShuffle)) (Math|Vector|MakeVector (.R_X (Utilities|Struct|BreakF_CSVdata _returnvalue_5)) (.R_Y (Utilities|Struct|BreakF_CSVdata _returnvalue_5)) (.R_Z (Utilities|Struct|BreakF_CSVdata _returnvalue_5))))))) (Math|Conversions|ToFloat(Boolean) (Variables|Default|GetRandom%20Rotation%20LOCAL/GLOBAL))) (* (Math|Vector|MakeVector (.S_X (Utilities|Struct|BreakF_CSVdata _returnvalue_5)) (.S_Y (Utilities|Struct|BreakF_CSVdata _returnvalue_5)) (.S_Z (Utilities|Struct|BreakF_CSVdata _returnvalue_5))) (Variables|Default|GetScale))) (* (Math|Vector|MakeVector (* (Math|Conversions|ToFloat(Boolean) (== (.AXIS (Utilities|Struct|BreakF_CSVdata _returnvalue_5)) 1)) _returnvalue_3) (* (Math|Conversions|ToFloat(Boolean) (== (.AXIS (Utilities|Struct|BreakF_CSVdata _returnvalue_5)) 2)) _returnvalue_3) (* (Math|Conversions|ToFloat(Boolean) (== (.AXIS (Utilities|Struct|BreakF_CSVdata _returnvalue_5)) 3)) _returnvalue_3)) (Math|Float|Clamp(Float) (+ (Math|Conversions|ToFloat(Boolean) (and (not (Class|KismetMathLibrary|IsPointinBoxwithTransform (Math|Vector|MakeVector (.T_X (Utilities|Struct|BreakF_CSVdata _returnvalue_5)) (.T_Y (Utilities|Struct|BreakF_CSVdata _returnvalue_5)) (.T_Z (Utilities|Struct|BreakF_CSVdata _returnvalue_5))) (Math|Transform|MakeTransform (Variables|Default|GetBox%20Origin%20[XYZ]) (Variables|Default|GetBox%20Rotation%20[XYZ])) (Variables|Default|GetBox%20Extent%20[XYZ]))) _boxcontrolleddisplacement)) (Variables|Default|GetBox%20Intensity)) (Math|Conversions|ToFloat(Boolean) (not _boxcontrolleddisplacement))))) (Math|Rotator|Lerp(Rotator) (Math|Rotator|CombineRotators (Math|Rotator|MakeRotator (.X (Math|Vector|BreakVector (+ (Math|Vector|MakeVector (Math|Random|RandomFloatinRangefromStream (* (.X (Math|Vector|BreakVector (* (Variables|Default|GetRandom%20Rotation%20[XYZ]) (Math|Conversions|ToFloat(Boolean) (!= (- (Math|Conversions|ToInteger(Boolean) (Variables|Default|GetRotation%20clamped%20to%20Displacement)) 1) (.AXIS (Utilities|Struct|BreakF_CSVdata _returnvalue_5))))))) -1.0) (.X (Math|Vector|BreakVector (* (Variables|Default|GetRandom%20Rotation%20[XYZ]) (Math|Conversions|ToFloat(Boolean) (!= (- (Math|Conversions|ToInteger(Boolean) (Variables|Default|GetRotation%20clamped%20to%20Displacement)) 1) (.AXIS (Utilities|Struct|BreakF_CSVdata _returnvalue_5))))))) _displacement_randomize) (Math|Random|RandomFloatinRangefromStream (* (.Y (Math|Vector|BreakVector (* (Variables|Default|GetRandom%20Rotation%20[XYZ]) (Math|Conversions|ToFloat(Boolean) (!= (- (Math|Conversions|ToInteger(Boolean) (Variables|Default|GetRotation%20clamped%20to%20Displacement)) 1) (.AXIS (Utilities|Struct|BreakF_CSVdata _returnvalue_5))))))) -1.0) (.Y (Math|Vector|BreakVector (* (Variables|Default|GetRandom%20Rotation%20[XYZ]) (Math|Conversions|ToFloat(Boolean) (!= (- (Math|Conversions|ToInteger(Boolean) (Variables|Default|GetRotation%20clamped%20to%20Displacement)) 1) (.AXIS (Utilities|Struct|BreakF_CSVdata _returnvalue_5))))))) _displacement_randomize) (Math|Random|RandomFloatinRangefromStream (* (.Z (Math|Vector|BreakVector (* (Variables|Default|GetRandom%20Rotation%20[XYZ]) (Math|Conversions|ToFloat(Boolean) (!= (- (Math|Conversions|ToInteger(Boolean) (Variables|Default|GetRotation%20clamped%20to%20Displacement)) 1) (.AXIS (Utilities|Struct|BreakF_CSVdata _returnvalue_5))))))) -1.0) (.Z (Math|Vector|BreakVector (* (Variables|Default|GetRandom%20Rotation%20[XYZ]) (Math|Conversions|ToFloat(Boolean) (!= (- (Math|Conversions|ToInteger(Boolean) (Variables|Default|GetRotation%20clamped%20to%20Displacement)) 1) (.AXIS (Utilities|Struct|BreakF_CSVdata _returnvalue_5))))))) _displacement_randomize)) (Variables|Default|GetShuffle)))) (.Y (Math|Vector|BreakVector (+ (Math|Vector|MakeVector (Math|Random|RandomFloatinRangefromStream (* (.X (Math|Vector|BreakVector (* (Variables|Default|GetRandom%20Rotation%20[XYZ]) (Math|Conversions|ToFloat(Boolean) (!= (- (Math|Conversions|ToInteger(Boolean) (Variables|Default|GetRotation%20clamped%20to%20Displacement)) 1) (.AXIS (Utilities|Struct|BreakF_CSVdata _returnvalue_5))))))) -1.0) (.X (Math|Vector|BreakVector (* (Variables|Default|GetRandom%20Rotation%20[XYZ]) (Math|Conversions|ToFloat(Boolean) (!= (- (Math|Conversions|ToInteger(Boolean) (Variables|Default|GetRotation%20clamped%20to%20Displacement)) 1) (.AXIS (Utilities|Struct|BreakF_CSVdata _returnvalue_5))))))) _displacement_randomize) (Math|Random|RandomFloatinRangefromStream (* (.Y (Math|Vector|BreakVector (* (Variables|Default|GetRandom%20Rotation%20[XYZ]) (Math|Conversions|ToFloat(Boolean) (!= (- (Math|Conversions|ToInteger(Boolean) (Variables|Default|GetRotation%20clamped%20to%20Displacement)) 1) (.AXIS (Utilities|Struct|BreakF_CSVdata _returnvalue_5))))))) -1.0) (.Y (Math|Vector|BreakVector (* (Variables|Default|GetRandom%20Rotation%20[XYZ]) (Math|Conversions|ToFloat(Boolean) (!= (- (Math|Conversions|ToInteger(Boolean) (Variables|Default|GetRotation%20clamped%20to%20Displacement)) 1) (.AXIS (Utilities|Struct|BreakF_CSVdata _returnvalue_5))))))) _displacement_randomize) (Math|Random|RandomFloatinRangefromStream (* (.Z (Math|Vector|BreakVector (* (Variables|Default|GetRandom%20Rotation%20[XYZ]) (Math|Conversions|ToFloat(Boolean) (!= (- (Math|Conversions|ToInteger(Boolean) (Variables|Default|GetRotation%20clamped%20to%20Displacement)) 1) (.AXIS (Utilities|Struct|BreakF_CSVdata _returnvalue_5))))))) -1.0) (.Z (Math|Vector|BreakVector (* (Variables|Default|GetRandom%20Rotation%20[XYZ]) (Math|Conversions|ToFloat(Boolean) (!= (- (Math|Conversions|ToInteger(Boolean) (Variables|Default|GetRotation%20clamped%20to%20Displacement)) 1) (.AXIS (Utilities|Struct|BreakF_CSVdata _returnvalue_5))))))) _displacement_randomize)) (Variables|Default|GetShuffle)))) (.Z (Math|Vector|BreakVector (+ (Math|Vector|MakeVector (Math|Random|RandomFloatinRangefromStream (* (.X (Math|Vector|BreakVector (* (Variables|Default|GetRandom%20Rotation%20[XYZ]) (Math|Conversions|ToFloat(Boolean) (!= (- (Math|Conversions|ToInteger(Boolean) (Variables|Default|GetRotation%20clamped%20to%20Displacement)) 1) (.AXIS (Utilities|Struct|BreakF_CSVdata _returnvalue_5))))))) -1.0) (.X (Math|Vector|BreakVector (* (Variables|Default|GetRandom%20Rotation%20[XYZ]) (Math|Conversions|ToFloat(Boolean) (!= (- (Math|Conversions|ToInteger(Boolean) (Variables|Default|GetRotation%20clamped%20to%20Displacement)) 1) (.AXIS (Utilities|Struct|BreakF_CSVdata _returnvalue_5))))))) _displacement_randomize) (Math|Random|RandomFloatinRangefromStream (* (.Y (Math|Vector|BreakVector (* (Variables|Default|GetRandom%20Rotation%20[XYZ]) (Math|Conversions|ToFloat(Boolean) (!= (- (Math|Conversions|ToInteger(Boolean) (Variables|Default|GetRotation%20clamped%20to%20Displacement)) 1) (.AXIS (Utilities|Struct|BreakF_CSVdata _returnvalue_5))))))) -1.0) (.Y (Math|Vector|BreakVector (* (Variables|Default|GetRandom%20Rotation%20[XYZ]) (Math|Conversions|ToFloat(Boolean) (!= (- (Math|Conversions|ToInteger(Boolean) (Variables|Default|GetRotation%20clamped%20to%20Displacement)) 1) (.AXIS (Utilities|Struct|BreakF_CSVdata _returnvalue_5))))))) _displacement_randomize) (Math|Random|RandomFloatinRangefromStream (* (.Z (Math|Vector|BreakVector (* (Variables|Default|GetRandom%20Rotation%20[XYZ]) (Math|Conversions|ToFloat(Boolean) (!= (- (Math|Conversions|ToInteger(Boolean) (Variables|Default|GetRotation%20clamped%20to%20Displacement)) 1) (.AXIS (Utilities|Struct|BreakF_CSVdata _returnvalue_5))))))) -1.0) (.Z (Math|Vector|BreakVector (* (Variables|Default|GetRandom%20Rotation%20[XYZ]) (Math|Conversions|ToFloat(Boolean) (!= (- (Math|Conversions|ToInteger(Boolean) (Variables|Default|GetRotation%20clamped%20to%20Displacement)) 1) (.AXIS (Utilities|Struct|BreakF_CSVdata _returnvalue_5))))))) _displacement_randomize)) (Variables|Default|GetShuffle))))) (Math|Rotator|MakeRotator (.R_X (Utilities|Struct|BreakF_CSVdata _returnvalue_5)) (.R_Y (Utilities|Struct|BreakF_CSVdata _returnvalue_5)) (.R_Z (Utilities|Struct|BreakF_CSVdata _returnvalue_5)))) (Math|Rotator|MakeRotator (.X (Math|Vector|BreakVector (+ (+ (Math|Vector|MakeVector (Math|Random|RandomFloatinRangefromStream (* (.X (Math|Vector|BreakVector (* (Variables|Default|GetRandom%20Rotation%20[XYZ]) (Math|Conversions|ToFloat(Boolean) (!= (- (Math|Conversions|ToInteger(Boolean) (Variables|Default|GetRotation%20clamped%20to%20Displacement)) 1) (.AXIS (Utilities|Struct|BreakF_CSVdata _returnvalue_5))))))) -1.0) (.X (Math|Vector|BreakVector (* (Variables|Default|GetRandom%20Rotation%20[XYZ]) (Math|Conversions|ToFloat(Boolean) (!= (- (Math|Conversions|ToInteger(Boolean) (Variables|Default|GetRotation%20clamped%20to%20Displacement)) 1) (.AXIS (Utilities|Struct|BreakF_CSVdata _returnvalue_5))))))) _displacement_randomize) (Math|Random|RandomFloatinRangefromStream (* (.Y (Math|Vector|BreakVector (* (Variables|Default|GetRandom%20Rotation%20[XYZ]) (Math|Conversions|ToFloat(Boolean) (!= (- (Math|Conversions|ToInteger(Boolean) (Variables|Default|GetRotation%20clamped%20to%20Displacement)) 1) (.AXIS (Utilities|Struct|BreakF_CSVdata _returnvalue_5))))))) -1.0) (.Y (Math|Vector|BreakVector (* (Variables|Default|GetRandom%20Rotation%20[XYZ]) (Math|Conversions|ToFloat(Boolean) (!= (- (Math|Conversions|ToInteger(Boolean) (Variables|Default|GetRotation%20clamped%20to%20Displacement)) 1) (.AXIS (Utilities|Struct|BreakF_CSVdata _returnvalue_5))))))) _displacement_randomize) (Math|Random|RandomFloatinRangefromStream (* (.Z (Math|Vector|BreakVector (* (Variables|Default|GetRandom%20Rotation%20[XYZ]) (Math|Conversions|ToFloat(Boolean) (!= (- (Math|Conversions|ToInteger(Boolean) (Variables|Default|GetRotation%20clamped%20to%20Displacement)) 1) (.AXIS (Utilities|Struct|BreakF_CSVdata _returnvalue_5))))))) -1.0) (.Z (Math|Vector|BreakVector (* (Variables|Default|GetRandom%20Rotation%20[XYZ]) (Math|Conversions|ToFloat(Boolean) (!= (- (Math|Conversions|ToInteger(Boolean) (Variables|Default|GetRotation%20clamped%20to%20Displacement)) 1) (.AXIS (Utilities|Struct|BreakF_CSVdata _returnvalue_5))))))) _displacement_randomize)) (Variables|Default|GetShuffle)) (Math|Vector|MakeVector (.R_X (Utilities|Struct|BreakF_CSVdata _returnvalue_5)) (.R_Y (Utilities|Struct|BreakF_CSVdata _returnvalue_5)) (.R_Z (Utilities|Struct|BreakF_CSVdata _returnvalue_5)))))) (.Y (Math|Vector|BreakVector (+ (+ (Math|Vector|MakeVector (Math|Random|RandomFloatinRangefromStream (* (.X (Math|Vector|BreakVector (* (Variables|Default|GetRandom%20Rotation%20[XYZ]) (Math|Conversions|ToFloat(Boolean) (!= (- (Math|Conversions|ToInteger(Boolean) (Variables|Default|GetRotation%20clamped%20to%20Displacement)) 1) (.AXIS (Utilities|Struct|BreakF_CSVdata _returnvalue_5))))))) -1.0) (.X (Math|Vector|BreakVector (* (Variables|Default|GetRandom%20Rotation%20[XYZ]) (Math|Conversions|ToFloat(Boolean) (!= (- (Math|Conversions|ToInteger(Boolean) (Variables|Default|GetRotation%20clamped%20to%20Displacement)) 1) (.AXIS (Utilities|Struct|BreakF_CSVdata _returnvalue_5))))))) _displacement_randomize) (Math|Random|RandomFloatinRangefromStream (* (.Y (Math|Vector|BreakVector (* (Variables|Default|GetRandom%20Rotation%20[XYZ]) (Math|Conversions|ToFloat(Boolean) (!= (- (Math|Conversions|ToInteger(Boolean) (Variables|Default|GetRotation%20clamped%20to%20Displacement)) 1) (.AXIS (Utilities|Struct|BreakF_CSVdata _returnvalue_5))))))) -1.0) (.Y (Math|Vector|BreakVector (* (Variables|Default|GetRandom%20Rotation%20[XYZ]) (Math|Conversions|ToFloat(Boolean) (!= (- (Math|Conversions|ToInteger(Boolean) (Variables|Default|GetRotation%20clamped%20to%20Displacement)) 1) (.AXIS (Utilities|Struct|BreakF_CSVdata _returnvalue_5))))))) _displacement_randomize) (Math|Random|RandomFloatinRangefromStream (* (.Z (Math|Vector|BreakVector (* (Variables|Default|GetRandom%20Rotation%20[XYZ]) (Math|Conversions|ToFloat(Boolean) (!= (- (Math|Conversions|ToInteger(Boolean) (Variables|Default|GetRotation%20clamped%20to%20Displacement)) 1) (.AXIS (Utilities|Struct|BreakF_CSVdata _returnvalue_5))))))) -1.0) (.Z (Math|Vector|BreakVector (* (Variables|Default|GetRandom%20Rotation%20[XYZ]) (Math|Conversions|ToFloat(Boolean) (!= (- (Math|Conversions|ToInteger(Boolean) (Variables|Default|GetRotation%20clamped%20to%20Displacement)) 1) (.AXIS (Utilities|Struct|BreakF_CSVdata _returnvalue_5))))))) _displacement_randomize)) (Variables|Default|GetShuffle)) (Math|Vector|MakeVector (.R_X (Utilities|Struct|BreakF_CSVdata _returnvalue_5)) (.R_Y (Utilities|Struct|BreakF_CSVdata _returnvalue_5)) (.R_Z (Utilities|Struct|BreakF_CSVdata _returnvalue_5)))))) (.Z (Math|Vector|BreakVector (+ (+ (Math|Vector|MakeVector (Math|Random|RandomFloatinRangefromStream (* (.X (Math|Vector|BreakVector (* (Variables|Default|GetRandom%20Rotation%20[XYZ]) (Math|Conversions|ToFloat(Boolean) (!= (- (Math|Conversions|ToInteger(Boolean) (Variables|Default|GetRotation%20clamped%20to%20Displacement)) 1) (.AXIS (Utilities|Struct|BreakF_CSVdata _returnvalue_5))))))) -1.0) (.X (Math|Vector|BreakVector (* (Variables|Default|GetRandom%20Rotation%20[XYZ]) (Math|Conversions|ToFloat(Boolean) (!= (- (Math|Conversions|ToInteger(Boolean) (Variables|Default|GetRotation%20clamped%20to%20Displacement)) 1) (.AXIS (Utilities|Struct|BreakF_CSVdata _returnvalue_5))))))) _displacement_randomize) (Math|Random|RandomFloatinRangefromStream (* (.Y (Math|Vector|BreakVector (* (Variables|Default|GetRandom%20Rotation%20[XYZ]) (Math|Conversions|ToFloat(Boolean) (!= (- (Math|Conversions|ToInteger(Boolean) (Variables|Default|GetRotation%20clamped%20to%20Displacement)) 1) (.AXIS (Utilities|Struct|BreakF_CSVdata _returnvalue_5))))))) -1.0) (.Y (Math|Vector|BreakVector (* (Variables|Default|GetRandom%20Rotation%20[XYZ]) (Math|Conversions|ToFloat(Boolean) (!= (- (Math|Conversions|ToInteger(Boolean) (Variables|Default|GetRotation%20clamped%20to%20Displacement)) 1) (.AXIS (Utilities|Struct|BreakF_CSVdata _returnvalue_5))))))) _displacement_randomize) (Math|Random|RandomFloatinRangefromStream (* (.Z (Math|Vector|BreakVector (* (Variables|Default|GetRandom%20Rotation%20[XYZ]) (Math|Conversions|ToFloat(Boolean) (!= (- (Math|Conversions|ToInteger(Boolean) (Variables|Default|GetRotation%20clamped%20to%20Displacement)) 1) (.AXIS (Utilities|Struct|BreakF_CSVdata _returnvalue_5))))))) -1.0) (.Z (Math|Vector|BreakVector (* (Variables|Default|GetRandom%20Rotation%20[XYZ]) (Math|Conversions|ToFloat(Boolean) (!= (- (Math|Conversions|ToInteger(Boolean) (Variables|Default|GetRotation%20clamped%20to%20Displacement)) 1) (.AXIS (Utilities|Struct|BreakF_CSVdata _returnvalue_5))))))) _displacement_randomize)) (Variables|Default|GetShuffle)) (Math|Vector|MakeVector (.R_X (Utilities|Struct|BreakF_CSVdata _returnvalue_5)) (.R_Y (Utilities|Struct|BreakF_CSVdata _returnvalue_5)) (.R_Z (Utilities|Struct|BreakF_CSVdata _returnvalue_5))))))) (Math|Conversions|ToFloat(Boolean) (Variables|Default|GetRandom%20Rotation%20LOCAL/GLOBAL))) (* (Math|Vector|MakeVector (.S_X (Utilities|Struct|BreakF_CSVdata _returnvalue_5)) (.S_Y (Utilities|Struct|BreakF_CSVdata _returnvalue_5)) (.S_Z (Utilities|Struct|BreakF_CSVdata _returnvalue_5))) (Variables|Default|GetScale))) false)))))))
                  (:7
                    (Utilities|FlowControl|Sequence :!label _label_7
                      (:then_0
                        (Utilities|FlowControl|DoOnce false
                          (:Completed
                            (bind _returnvalue_12 (AddComponent|AddHierarchicalInstancedStaticMeshComponent false))
                            (bind _output_get_7 (Variables|Default|Set07 _returnvalue_12))
                            (Rendering|Material|SetMaterial _output_get_7 0 (Variables|Default|GetStone%20Material)))))
                      (:then_1
                        (Components|InstancedStaticMesh|AddInstance (Variables|Default|Get07) (Math|Transform|MakeTransform (Math|Transform|TransformLocation (Math|Transform|MakeTransform (Math|Vector|MakeVector (.T_X (Utilities|Struct|BreakF_CSVdata _returnvalue_5)) (.T_Y (Utilities|Struct|BreakF_CSVdata _returnvalue_5)) (.T_Z (Utilities|Struct|BreakF_CSVdata _returnvalue_5))) (Math|Rotator|Lerp(Rotator) (Math|Rotator|CombineRotators (Math|Rotator|MakeRotator (.X (Math|Vector|BreakVector (+ (Math|Vector|MakeVector (Math|Random|RandomFloatinRangefromStream (* (.X (Math|Vector|BreakVector (* (Variables|Default|GetRandom%20Rotation%20[XYZ]) (Math|Conversions|ToFloat(Boolean) (!= (- (Math|Conversions|ToInteger(Boolean) (Variables|Default|GetRotation%20clamped%20to%20Displacement)) 1) (.AXIS (Utilities|Struct|BreakF_CSVdata _returnvalue_5))))))) -1.0) (.X (Math|Vector|BreakVector (* (Variables|Default|GetRandom%20Rotation%20[XYZ]) (Math|Conversions|ToFloat(Boolean) (!= (- (Math|Conversions|ToInteger(Boolean) (Variables|Default|GetRotation%20clamped%20to%20Displacement)) 1) (.AXIS (Utilities|Struct|BreakF_CSVdata _returnvalue_5))))))) _displacement_randomize) (Math|Random|RandomFloatinRangefromStream (* (.Y (Math|Vector|BreakVector (* (Variables|Default|GetRandom%20Rotation%20[XYZ]) (Math|Conversions|ToFloat(Boolean) (!= (- (Math|Conversions|ToInteger(Boolean) (Variables|Default|GetRotation%20clamped%20to%20Displacement)) 1) (.AXIS (Utilities|Struct|BreakF_CSVdata _returnvalue_5))))))) -1.0) (.Y (Math|Vector|BreakVector (* (Variables|Default|GetRandom%20Rotation%20[XYZ]) (Math|Conversions|ToFloat(Boolean) (!= (- (Math|Conversions|ToInteger(Boolean) (Variables|Default|GetRotation%20clamped%20to%20Displacement)) 1) (.AXIS (Utilities|Struct|BreakF_CSVdata _returnvalue_5))))))) _displacement_randomize) (Math|Random|RandomFloatinRangefromStream (* (.Z (Math|Vector|BreakVector (* (Variables|Default|GetRandom%20Rotation%20[XYZ]) (Math|Conversions|ToFloat(Boolean) (!= (- (Math|Conversions|ToInteger(Boolean) (Variables|Default|GetRotation%20clamped%20to%20Displacement)) 1) (.AXIS (Utilities|Struct|BreakF_CSVdata _returnvalue_5))))))) -1.0) (.Z (Math|Vector|BreakVector (* (Variables|Default|GetRandom%20Rotation%20[XYZ]) (Math|Conversions|ToFloat(Boolean) (!= (- (Math|Conversions|ToInteger(Boolean) (Variables|Default|GetRotation%20clamped%20to%20Displacement)) 1) (.AXIS (Utilities|Struct|BreakF_CSVdata _returnvalue_5))))))) _displacement_randomize)) (Variables|Default|GetShuffle)))) (.Y (Math|Vector|BreakVector (+ (Math|Vector|MakeVector (Math|Random|RandomFloatinRangefromStream (* (.X (Math|Vector|BreakVector (* (Variables|Default|GetRandom%20Rotation%20[XYZ]) (Math|Conversions|ToFloat(Boolean) (!= (- (Math|Conversions|ToInteger(Boolean) (Variables|Default|GetRotation%20clamped%20to%20Displacement)) 1) (.AXIS (Utilities|Struct|BreakF_CSVdata _returnvalue_5))))))) -1.0) (.X (Math|Vector|BreakVector (* (Variables|Default|GetRandom%20Rotation%20[XYZ]) (Math|Conversions|ToFloat(Boolean) (!= (- (Math|Conversions|ToInteger(Boolean) (Variables|Default|GetRotation%20clamped%20to%20Displacement)) 1) (.AXIS (Utilities|Struct|BreakF_CSVdata _returnvalue_5))))))) _displacement_randomize) (Math|Random|RandomFloatinRangefromStream (* (.Y (Math|Vector|BreakVector (* (Variables|Default|GetRandom%20Rotation%20[XYZ]) (Math|Conversions|ToFloat(Boolean) (!= (- (Math|Conversions|ToInteger(Boolean) (Variables|Default|GetRotation%20clamped%20to%20Displacement)) 1) (.AXIS (Utilities|Struct|BreakF_CSVdata _returnvalue_5))))))) -1.0) (.Y (Math|Vector|BreakVector (* (Variables|Default|GetRandom%20Rotation%20[XYZ]) (Math|Conversions|ToFloat(Boolean) (!= (- (Math|Conversions|ToInteger(Boolean) (Variables|Default|GetRotation%20clamped%20to%20Displacement)) 1) (.AXIS (Utilities|Struct|BreakF_CSVdata _returnvalue_5))))))) _displacement_randomize) (Math|Random|RandomFloatinRangefromStream (* (.Z (Math|Vector|BreakVector (* (Variables|Default|GetRandom%20Rotation%20[XYZ]) (Math|Conversions|ToFloat(Boolean) (!= (- (Math|Conversions|ToInteger(Boolean) (Variables|Default|GetRotation%20clamped%20to%20Displacement)) 1) (.AXIS (Utilities|Struct|BreakF_CSVdata _returnvalue_5))))))) -1.0) (.Z (Math|Vector|BreakVector (* (Variables|Default|GetRandom%20Rotation%20[XYZ]) (Math|Conversions|ToFloat(Boolean) (!= (- (Math|Conversions|ToInteger(Boolean) (Variables|Default|GetRotation%20clamped%20to%20Displacement)) 1) (.AXIS (Utilities|Struct|BreakF_CSVdata _returnvalue_5))))))) _displacement_randomize)) (Variables|Default|GetShuffle)))) (.Z (Math|Vector|BreakVector (+ (Math|Vector|MakeVector (Math|Random|RandomFloatinRangefromStream (* (.X (Math|Vector|BreakVector (* (Variables|Default|GetRandom%20Rotation%20[XYZ]) (Math|Conversions|ToFloat(Boolean) (!= (- (Math|Conversions|ToInteger(Boolean) (Variables|Default|GetRotation%20clamped%20to%20Displacement)) 1) (.AXIS (Utilities|Struct|BreakF_CSVdata _returnvalue_5))))))) -1.0) (.X (Math|Vector|BreakVector (* (Variables|Default|GetRandom%20Rotation%20[XYZ]) (Math|Conversions|ToFloat(Boolean) (!= (- (Math|Conversions|ToInteger(Boolean) (Variables|Default|GetRotation%20clamped%20to%20Displacement)) 1) (.AXIS (Utilities|Struct|BreakF_CSVdata _returnvalue_5))))))) _displacement_randomize) (Math|Random|RandomFloatinRangefromStream (* (.Y (Math|Vector|BreakVector (* (Variables|Default|GetRandom%20Rotation%20[XYZ]) (Math|Conversions|ToFloat(Boolean) (!= (- (Math|Conversions|ToInteger(Boolean) (Variables|Default|GetRotation%20clamped%20to%20Displacement)) 1) (.AXIS (Utilities|Struct|BreakF_CSVdata _returnvalue_5))))))) -1.0) (.Y (Math|Vector|BreakVector (* (Variables|Default|GetRandom%20Rotation%20[XYZ]) (Math|Conversions|ToFloat(Boolean) (!= (- (Math|Conversions|ToInteger(Boolean) (Variables|Default|GetRotation%20clamped%20to%20Displacement)) 1) (.AXIS (Utilities|Struct|BreakF_CSVdata _returnvalue_5))))))) _displacement_randomize) (Math|Random|RandomFloatinRangefromStream (* (.Z (Math|Vector|BreakVector (* (Variables|Default|GetRandom%20Rotation%20[XYZ]) (Math|Conversions|ToFloat(Boolean) (!= (- (Math|Conversions|ToInteger(Boolean) (Variables|Default|GetRotation%20clamped%20to%20Displacement)) 1) (.AXIS (Utilities|Struct|BreakF_CSVdata _returnvalue_5))))))) -1.0) (.Z (Math|Vector|BreakVector (* (Variables|Default|GetRandom%20Rotation%20[XYZ]) (Math|Conversions|ToFloat(Boolean) (!= (- (Math|Conversions|ToInteger(Boolean) (Variables|Default|GetRotation%20clamped%20to%20Displacement)) 1) (.AXIS (Utilities|Struct|BreakF_CSVdata _returnvalue_5))))))) _displacement_randomize)) (Variables|Default|GetShuffle))))) (Math|Rotator|MakeRotator (.R_X (Utilities|Struct|BreakF_CSVdata _returnvalue_5)) (.R_Y (Utilities|Struct|BreakF_CSVdata _returnvalue_5)) (.R_Z (Utilities|Struct|BreakF_CSVdata _returnvalue_5)))) (Math|Rotator|MakeRotator (.X (Math|Vector|BreakVector (+ (+ (Math|Vector|MakeVector (Math|Random|RandomFloatinRangefromStream (* (.X (Math|Vector|BreakVector (* (Variables|Default|GetRandom%20Rotation%20[XYZ]) (Math|Conversions|ToFloat(Boolean) (!= (- (Math|Conversions|ToInteger(Boolean) (Variables|Default|GetRotation%20clamped%20to%20Displacement)) 1) (.AXIS (Utilities|Struct|BreakF_CSVdata _returnvalue_5))))))) -1.0) (.X (Math|Vector|BreakVector (* (Variables|Default|GetRandom%20Rotation%20[XYZ]) (Math|Conversions|ToFloat(Boolean) (!= (- (Math|Conversions|ToInteger(Boolean) (Variables|Default|GetRotation%20clamped%20to%20Displacement)) 1) (.AXIS (Utilities|Struct|BreakF_CSVdata _returnvalue_5))))))) _displacement_randomize) (Math|Random|RandomFloatinRangefromStream (* (.Y (Math|Vector|BreakVector (* (Variables|Default|GetRandom%20Rotation%20[XYZ]) (Math|Conversions|ToFloat(Boolean) (!= (- (Math|Conversions|ToInteger(Boolean) (Variables|Default|GetRotation%20clamped%20to%20Displacement)) 1) (.AXIS (Utilities|Struct|BreakF_CSVdata _returnvalue_5))))))) -1.0) (.Y (Math|Vector|BreakVector (* (Variables|Default|GetRandom%20Rotation%20[XYZ]) (Math|Conversions|ToFloat(Boolean) (!= (- (Math|Conversions|ToInteger(Boolean) (Variables|Default|GetRotation%20clamped%20to%20Displacement)) 1) (.AXIS (Utilities|Struct|BreakF_CSVdata _returnvalue_5))))))) _displacement_randomize) (Math|Random|RandomFloatinRangefromStream (* (.Z (Math|Vector|BreakVector (* (Variables|Default|GetRandom%20Rotation%20[XYZ]) (Math|Conversions|ToFloat(Boolean) (!= (- (Math|Conversions|ToInteger(Boolean) (Variables|Default|GetRotation%20clamped%20to%20Displacement)) 1) (.AXIS (Utilities|Struct|BreakF_CSVdata _returnvalue_5))))))) -1.0) (.Z (Math|Vector|BreakVector (* (Variables|Default|GetRandom%20Rotation%20[XYZ]) (Math|Conversions|ToFloat(Boolean) (!= (- (Math|Conversions|ToInteger(Boolean) (Variables|Default|GetRotation%20clamped%20to%20Displacement)) 1) (.AXIS (Utilities|Struct|BreakF_CSVdata _returnvalue_5))))))) _displacement_randomize)) (Variables|Default|GetShuffle)) (Math|Vector|MakeVector (.R_X (Utilities|Struct|BreakF_CSVdata _returnvalue_5)) (.R_Y (Utilities|Struct|BreakF_CSVdata _returnvalue_5)) (.R_Z (Utilities|Struct|BreakF_CSVdata _returnvalue_5)))))) (.Y (Math|Vector|BreakVector (+ (+ (Math|Vector|MakeVector (Math|Random|RandomFloatinRangefromStream (* (.X (Math|Vector|BreakVector (* (Variables|Default|GetRandom%20Rotation%20[XYZ]) (Math|Conversions|ToFloat(Boolean) (!= (- (Math|Conversions|ToInteger(Boolean) (Variables|Default|GetRotation%20clamped%20to%20Displacement)) 1) (.AXIS (Utilities|Struct|BreakF_CSVdata _returnvalue_5))))))) -1.0) (.X (Math|Vector|BreakVector (* (Variables|Default|GetRandom%20Rotation%20[XYZ]) (Math|Conversions|ToFloat(Boolean) (!= (- (Math|Conversions|ToInteger(Boolean) (Variables|Default|GetRotation%20clamped%20to%20Displacement)) 1) (.AXIS (Utilities|Struct|BreakF_CSVdata _returnvalue_5))))))) _displacement_randomize) (Math|Random|RandomFloatinRangefromStream (* (.Y (Math|Vector|BreakVector (* (Variables|Default|GetRandom%20Rotation%20[XYZ]) (Math|Conversions|ToFloat(Boolean) (!= (- (Math|Conversions|ToInteger(Boolean) (Variables|Default|GetRotation%20clamped%20to%20Displacement)) 1) (.AXIS (Utilities|Struct|BreakF_CSVdata _returnvalue_5))))))) -1.0) (.Y (Math|Vector|BreakVector (* (Variables|Default|GetRandom%20Rotation%20[XYZ]) (Math|Conversions|ToFloat(Boolean) (!= (- (Math|Conversions|ToInteger(Boolean) (Variables|Default|GetRotation%20clamped%20to%20Displacement)) 1) (.AXIS (Utilities|Struct|BreakF_CSVdata _returnvalue_5))))))) _displacement_randomize) (Math|Random|RandomFloatinRangefromStream (* (.Z (Math|Vector|BreakVector (* (Variables|Default|GetRandom%20Rotation%20[XYZ]) (Math|Conversions|ToFloat(Boolean) (!= (- (Math|Conversions|ToInteger(Boolean) (Variables|Default|GetRotation%20clamped%20to%20Displacement)) 1) (.AXIS (Utilities|Struct|BreakF_CSVdata _returnvalue_5))))))) -1.0) (.Z (Math|Vector|BreakVector (* (Variables|Default|GetRandom%20Rotation%20[XYZ]) (Math|Conversions|ToFloat(Boolean) (!= (- (Math|Conversions|ToInteger(Boolean) (Variables|Default|GetRotation%20clamped%20to%20Displacement)) 1) (.AXIS (Utilities|Struct|BreakF_CSVdata _returnvalue_5))))))) _displacement_randomize)) (Variables|Default|GetShuffle)) (Math|Vector|MakeVector (.R_X (Utilities|Struct|BreakF_CSVdata _returnvalue_5)) (.R_Y (Utilities|Struct|BreakF_CSVdata _returnvalue_5)) (.R_Z (Utilities|Struct|BreakF_CSVdata _returnvalue_5)))))) (.Z (Math|Vector|BreakVector (+ (+ (Math|Vector|MakeVector (Math|Random|RandomFloatinRangefromStream (* (.X (Math|Vector|BreakVector (* (Variables|Default|GetRandom%20Rotation%20[XYZ]) (Math|Conversions|ToFloat(Boolean) (!= (- (Math|Conversions|ToInteger(Boolean) (Variables|Default|GetRotation%20clamped%20to%20Displacement)) 1) (.AXIS (Utilities|Struct|BreakF_CSVdata _returnvalue_5))))))) -1.0) (.X (Math|Vector|BreakVector (* (Variables|Default|GetRandom%20Rotation%20[XYZ]) (Math|Conversions|ToFloat(Boolean) (!= (- (Math|Conversions|ToInteger(Boolean) (Variables|Default|GetRotation%20clamped%20to%20Displacement)) 1) (.AXIS (Utilities|Struct|BreakF_CSVdata _returnvalue_5))))))) _displacement_randomize) (Math|Random|RandomFloatinRangefromStream (* (.Y (Math|Vector|BreakVector (* (Variables|Default|GetRandom%20Rotation%20[XYZ]) (Math|Conversions|ToFloat(Boolean) (!= (- (Math|Conversions|ToInteger(Boolean) (Variables|Default|GetRotation%20clamped%20to%20Displacement)) 1) (.AXIS (Utilities|Struct|BreakF_CSVdata _returnvalue_5))))))) -1.0) (.Y (Math|Vector|BreakVector (* (Variables|Default|GetRandom%20Rotation%20[XYZ]) (Math|Conversions|ToFloat(Boolean) (!= (- (Math|Conversions|ToInteger(Boolean) (Variables|Default|GetRotation%20clamped%20to%20Displacement)) 1) (.AXIS (Utilities|Struct|BreakF_CSVdata _returnvalue_5))))))) _displacement_randomize) (Math|Random|RandomFloatinRangefromStream (* (.Z (Math|Vector|BreakVector (* (Variables|Default|GetRandom%20Rotation%20[XYZ]) (Math|Conversions|ToFloat(Boolean) (!= (- (Math|Conversions|ToInteger(Boolean) (Variables|Default|GetRotation%20clamped%20to%20Displacement)) 1) (.AXIS (Utilities|Struct|BreakF_CSVdata _returnvalue_5))))))) -1.0) (.Z (Math|Vector|BreakVector (* (Variables|Default|GetRandom%20Rotation%20[XYZ]) (Math|Conversions|ToFloat(Boolean) (!= (- (Math|Conversions|ToInteger(Boolean) (Variables|Default|GetRotation%20clamped%20to%20Displacement)) 1) (.AXIS (Utilities|Struct|BreakF_CSVdata _returnvalue_5))))))) _displacement_randomize)) (Variables|Default|GetShuffle)) (Math|Vector|MakeVector (.R_X (Utilities|Struct|BreakF_CSVdata _returnvalue_5)) (.R_Y (Utilities|Struct|BreakF_CSVdata _returnvalue_5)) (.R_Z (Utilities|Struct|BreakF_CSVdata _returnvalue_5))))))) (Math|Conversions|ToFloat(Boolean) (Variables|Default|GetRandom%20Rotation%20LOCAL/GLOBAL))) (* (Math|Vector|MakeVector (.S_X (Utilities|Struct|BreakF_CSVdata _returnvalue_5)) (.S_Y (Utilities|Struct|BreakF_CSVdata _returnvalue_5)) (.S_Z (Utilities|Struct|BreakF_CSVdata _returnvalue_5))) (Variables|Default|GetScale))) (* (Math|Vector|MakeVector (* (Math|Conversions|ToFloat(Boolean) (== (.AXIS (Utilities|Struct|BreakF_CSVdata _returnvalue_5)) 1)) _returnvalue_3) (* (Math|Conversions|ToFloat(Boolean) (== (.AXIS (Utilities|Struct|BreakF_CSVdata _returnvalue_5)) 2)) _returnvalue_3) (* (Math|Conversions|ToFloat(Boolean) (== (.AXIS (Utilities|Struct|BreakF_CSVdata _returnvalue_5)) 3)) _returnvalue_3)) (Math|Float|Clamp(Float) (+ (Math|Conversions|ToFloat(Boolean) (and (not (Class|KismetMathLibrary|IsPointinBoxwithTransform (Math|Vector|MakeVector (.T_X (Utilities|Struct|BreakF_CSVdata _returnvalue_5)) (.T_Y (Utilities|Struct|BreakF_CSVdata _returnvalue_5)) (.T_Z (Utilities|Struct|BreakF_CSVdata _returnvalue_5))) (Math|Transform|MakeTransform (Variables|Default|GetBox%20Origin%20[XYZ]) (Variables|Default|GetBox%20Rotation%20[XYZ])) (Variables|Default|GetBox%20Extent%20[XYZ]))) _boxcontrolleddisplacement)) (Variables|Default|GetBox%20Intensity)) (Math|Conversions|ToFloat(Boolean) (not _boxcontrolleddisplacement))))) (Math|Rotator|Lerp(Rotator) (Math|Rotator|CombineRotators (Math|Rotator|MakeRotator (.X (Math|Vector|BreakVector (+ (Math|Vector|MakeVector (Math|Random|RandomFloatinRangefromStream (* (.X (Math|Vector|BreakVector (* (Variables|Default|GetRandom%20Rotation%20[XYZ]) (Math|Conversions|ToFloat(Boolean) (!= (- (Math|Conversions|ToInteger(Boolean) (Variables|Default|GetRotation%20clamped%20to%20Displacement)) 1) (.AXIS (Utilities|Struct|BreakF_CSVdata _returnvalue_5))))))) -1.0) (.X (Math|Vector|BreakVector (* (Variables|Default|GetRandom%20Rotation%20[XYZ]) (Math|Conversions|ToFloat(Boolean) (!= (- (Math|Conversions|ToInteger(Boolean) (Variables|Default|GetRotation%20clamped%20to%20Displacement)) 1) (.AXIS (Utilities|Struct|BreakF_CSVdata _returnvalue_5))))))) _displacement_randomize) (Math|Random|RandomFloatinRangefromStream (* (.Y (Math|Vector|BreakVector (* (Variables|Default|GetRandom%20Rotation%20[XYZ]) (Math|Conversions|ToFloat(Boolean) (!= (- (Math|Conversions|ToInteger(Boolean) (Variables|Default|GetRotation%20clamped%20to%20Displacement)) 1) (.AXIS (Utilities|Struct|BreakF_CSVdata _returnvalue_5))))))) -1.0) (.Y (Math|Vector|BreakVector (* (Variables|Default|GetRandom%20Rotation%20[XYZ]) (Math|Conversions|ToFloat(Boolean) (!= (- (Math|Conversions|ToInteger(Boolean) (Variables|Default|GetRotation%20clamped%20to%20Displacement)) 1) (.AXIS (Utilities|Struct|BreakF_CSVdata _returnvalue_5))))))) _displacement_randomize) (Math|Random|RandomFloatinRangefromStream (* (.Z (Math|Vector|BreakVector (* (Variables|Default|GetRandom%20Rotation%20[XYZ]) (Math|Conversions|ToFloat(Boolean) (!= (- (Math|Conversions|ToInteger(Boolean) (Variables|Default|GetRotation%20clamped%20to%20Displacement)) 1) (.AXIS (Utilities|Struct|BreakF_CSVdata _returnvalue_5))))))) -1.0) (.Z (Math|Vector|BreakVector (* (Variables|Default|GetRandom%20Rotation%20[XYZ]) (Math|Conversions|ToFloat(Boolean) (!= (- (Math|Conversions|ToInteger(Boolean) (Variables|Default|GetRotation%20clamped%20to%20Displacement)) 1) (.AXIS (Utilities|Struct|BreakF_CSVdata _returnvalue_5))))))) _displacement_randomize)) (Variables|Default|GetShuffle)))) (.Y (Math|Vector|BreakVector (+ (Math|Vector|MakeVector (Math|Random|RandomFloatinRangefromStream (* (.X (Math|Vector|BreakVector (* (Variables|Default|GetRandom%20Rotation%20[XYZ]) (Math|Conversions|ToFloat(Boolean) (!= (- (Math|Conversions|ToInteger(Boolean) (Variables|Default|GetRotation%20clamped%20to%20Displacement)) 1) (.AXIS (Utilities|Struct|BreakF_CSVdata _returnvalue_5))))))) -1.0) (.X (Math|Vector|BreakVector (* (Variables|Default|GetRandom%20Rotation%20[XYZ]) (Math|Conversions|ToFloat(Boolean) (!= (- (Math|Conversions|ToInteger(Boolean) (Variables|Default|GetRotation%20clamped%20to%20Displacement)) 1) (.AXIS (Utilities|Struct|BreakF_CSVdata _returnvalue_5))))))) _displacement_randomize) (Math|Random|RandomFloatinRangefromStream (* (.Y (Math|Vector|BreakVector (* (Variables|Default|GetRandom%20Rotation%20[XYZ]) (Math|Conversions|ToFloat(Boolean) (!= (- (Math|Conversions|ToInteger(Boolean) (Variables|Default|GetRotation%20clamped%20to%20Displacement)) 1) (.AXIS (Utilities|Struct|BreakF_CSVdata _returnvalue_5))))))) -1.0) (.Y (Math|Vector|BreakVector (* (Variables|Default|GetRandom%20Rotation%20[XYZ]) (Math|Conversions|ToFloat(Boolean) (!= (- (Math|Conversions|ToInteger(Boolean) (Variables|Default|GetRotation%20clamped%20to%20Displacement)) 1) (.AXIS (Utilities|Struct|BreakF_CSVdata _returnvalue_5))))))) _displacement_randomize) (Math|Random|RandomFloatinRangefromStream (* (.Z (Math|Vector|BreakVector (* (Variables|Default|GetRandom%20Rotation%20[XYZ]) (Math|Conversions|ToFloat(Boolean) (!= (- (Math|Conversions|ToInteger(Boolean) (Variables|Default|GetRotation%20clamped%20to%20Displacement)) 1) (.AXIS (Utilities|Struct|BreakF_CSVdata _returnvalue_5))))))) -1.0) (.Z (Math|Vector|BreakVector (* (Variables|Default|GetRandom%20Rotation%20[XYZ]) (Math|Conversions|ToFloat(Boolean) (!= (- (Math|Conversions|ToInteger(Boolean) (Variables|Default|GetRotation%20clamped%20to%20Displacement)) 1) (.AXIS (Utilities|Struct|BreakF_CSVdata _returnvalue_5))))))) _displacement_randomize)) (Variables|Default|GetShuffle)))) (.Z (Math|Vector|BreakVector (+ (Math|Vector|MakeVector (Math|Random|RandomFloatinRangefromStream (* (.X (Math|Vector|BreakVector (* (Variables|Default|GetRandom%20Rotation%20[XYZ]) (Math|Conversions|ToFloat(Boolean) (!= (- (Math|Conversions|ToInteger(Boolean) (Variables|Default|GetRotation%20clamped%20to%20Displacement)) 1) (.AXIS (Utilities|Struct|BreakF_CSVdata _returnvalue_5))))))) -1.0) (.X (Math|Vector|BreakVector (* (Variables|Default|GetRandom%20Rotation%20[XYZ]) (Math|Conversions|ToFloat(Boolean) (!= (- (Math|Conversions|ToInteger(Boolean) (Variables|Default|GetRotation%20clamped%20to%20Displacement)) 1) (.AXIS (Utilities|Struct|BreakF_CSVdata _returnvalue_5))))))) _displacement_randomize) (Math|Random|RandomFloatinRangefromStream (* (.Y (Math|Vector|BreakVector (* (Variables|Default|GetRandom%20Rotation%20[XYZ]) (Math|Conversions|ToFloat(Boolean) (!= (- (Math|Conversions|ToInteger(Boolean) (Variables|Default|GetRotation%20clamped%20to%20Displacement)) 1) (.AXIS (Utilities|Struct|BreakF_CSVdata _returnvalue_5))))))) -1.0) (.Y (Math|Vector|BreakVector (* (Variables|Default|GetRandom%20Rotation%20[XYZ]) (Math|Conversions|ToFloat(Boolean) (!= (- (Math|Conversions|ToInteger(Boolean) (Variables|Default|GetRotation%20clamped%20to%20Displacement)) 1) (.AXIS (Utilities|Struct|BreakF_CSVdata _returnvalue_5))))))) _displacement_randomize) (Math|Random|RandomFloatinRangefromStream (* (.Z (Math|Vector|BreakVector (* (Variables|Default|GetRandom%20Rotation%20[XYZ]) (Math|Conversions|ToFloat(Boolean) (!= (- (Math|Conversions|ToInteger(Boolean) (Variables|Default|GetRotation%20clamped%20to%20Displacement)) 1) (.AXIS (Utilities|Struct|BreakF_CSVdata _returnvalue_5))))))) -1.0) (.Z (Math|Vector|BreakVector (* (Variables|Default|GetRandom%20Rotation%20[XYZ]) (Math|Conversions|ToFloat(Boolean) (!= (- (Math|Conversions|ToInteger(Boolean) (Variables|Default|GetRotation%20clamped%20to%20Displacement)) 1) (.AXIS (Utilities|Struct|BreakF_CSVdata _returnvalue_5))))))) _displacement_randomize)) (Variables|Default|GetShuffle))))) (Math|Rotator|MakeRotator (.R_X (Utilities|Struct|BreakF_CSVdata _returnvalue_5)) (.R_Y (Utilities|Struct|BreakF_CSVdata _returnvalue_5)) (.R_Z (Utilities|Struct|BreakF_CSVdata _returnvalue_5)))) (Math|Rotator|MakeRotator (.X (Math|Vector|BreakVector (+ (+ (Math|Vector|MakeVector (Math|Random|RandomFloatinRangefromStream (* (.X (Math|Vector|BreakVector (* (Variables|Default|GetRandom%20Rotation%20[XYZ]) (Math|Conversions|ToFloat(Boolean) (!= (- (Math|Conversions|ToInteger(Boolean) (Variables|Default|GetRotation%20clamped%20to%20Displacement)) 1) (.AXIS (Utilities|Struct|BreakF_CSVdata _returnvalue_5))))))) -1.0) (.X (Math|Vector|BreakVector (* (Variables|Default|GetRandom%20Rotation%20[XYZ]) (Math|Conversions|ToFloat(Boolean) (!= (- (Math|Conversions|ToInteger(Boolean) (Variables|Default|GetRotation%20clamped%20to%20Displacement)) 1) (.AXIS (Utilities|Struct|BreakF_CSVdata _returnvalue_5))))))) _displacement_randomize) (Math|Random|RandomFloatinRangefromStream (* (.Y (Math|Vector|BreakVector (* (Variables|Default|GetRandom%20Rotation%20[XYZ]) (Math|Conversions|ToFloat(Boolean) (!= (- (Math|Conversions|ToInteger(Boolean) (Variables|Default|GetRotation%20clamped%20to%20Displacement)) 1) (.AXIS (Utilities|Struct|BreakF_CSVdata _returnvalue_5))))))) -1.0) (.Y (Math|Vector|BreakVector (* (Variables|Default|GetRandom%20Rotation%20[XYZ]) (Math|Conversions|ToFloat(Boolean) (!= (- (Math|Conversions|ToInteger(Boolean) (Variables|Default|GetRotation%20clamped%20to%20Displacement)) 1) (.AXIS (Utilities|Struct|BreakF_CSVdata _returnvalue_5))))))) _displacement_randomize) (Math|Random|RandomFloatinRangefromStream (* (.Z (Math|Vector|BreakVector (* (Variables|Default|GetRandom%20Rotation%20[XYZ]) (Math|Conversions|ToFloat(Boolean) (!= (- (Math|Conversions|ToInteger(Boolean) (Variables|Default|GetRotation%20clamped%20to%20Displacement)) 1) (.AXIS (Utilities|Struct|BreakF_CSVdata _returnvalue_5))))))) -1.0) (.Z (Math|Vector|BreakVector (* (Variables|Default|GetRandom%20Rotation%20[XYZ]) (Math|Conversions|ToFloat(Boolean) (!= (- (Math|Conversions|ToInteger(Boolean) (Variables|Default|GetRotation%20clamped%20to%20Displacement)) 1) (.AXIS (Utilities|Struct|BreakF_CSVdata _returnvalue_5))))))) _displacement_randomize)) (Variables|Default|GetShuffle)) (Math|Vector|MakeVector (.R_X (Utilities|Struct|BreakF_CSVdata _returnvalue_5)) (.R_Y (Utilities|Struct|BreakF_CSVdata _returnvalue_5)) (.R_Z (Utilities|Struct|BreakF_CSVdata _returnvalue_5)))))) (.Y (Math|Vector|BreakVector (+ (+ (Math|Vector|MakeVector (Math|Random|RandomFloatinRangefromStream (* (.X (Math|Vector|BreakVector (* (Variables|Default|GetRandom%20Rotation%20[XYZ]) (Math|Conversions|ToFloat(Boolean) (!= (- (Math|Conversions|ToInteger(Boolean) (Variables|Default|GetRotation%20clamped%20to%20Displacement)) 1) (.AXIS (Utilities|Struct|BreakF_CSVdata _returnvalue_5))))))) -1.0) (.X (Math|Vector|BreakVector (* (Variables|Default|GetRandom%20Rotation%20[XYZ]) (Math|Conversions|ToFloat(Boolean) (!= (- (Math|Conversions|ToInteger(Boolean) (Variables|Default|GetRotation%20clamped%20to%20Displacement)) 1) (.AXIS (Utilities|Struct|BreakF_CSVdata _returnvalue_5))))))) _displacement_randomize) (Math|Random|RandomFloatinRangefromStream (* (.Y (Math|Vector|BreakVector (* (Variables|Default|GetRandom%20Rotation%20[XYZ]) (Math|Conversions|ToFloat(Boolean) (!= (- (Math|Conversions|ToInteger(Boolean) (Variables|Default|GetRotation%20clamped%20to%20Displacement)) 1) (.AXIS (Utilities|Struct|BreakF_CSVdata _returnvalue_5))))))) -1.0) (.Y (Math|Vector|BreakVector (* (Variables|Default|GetRandom%20Rotation%20[XYZ]) (Math|Conversions|ToFloat(Boolean) (!= (- (Math|Conversions|ToInteger(Boolean) (Variables|Default|GetRotation%20clamped%20to%20Displacement)) 1) (.AXIS (Utilities|Struct|BreakF_CSVdata _returnvalue_5))))))) _displacement_randomize) (Math|Random|RandomFloatinRangefromStream (* (.Z (Math|Vector|BreakVector (* (Variables|Default|GetRandom%20Rotation%20[XYZ]) (Math|Conversions|ToFloat(Boolean) (!= (- (Math|Conversions|ToInteger(Boolean) (Variables|Default|GetRotation%20clamped%20to%20Displacement)) 1) (.AXIS (Utilities|Struct|BreakF_CSVdata _returnvalue_5))))))) -1.0) (.Z (Math|Vector|BreakVector (* (Variables|Default|GetRandom%20Rotation%20[XYZ]) (Math|Conversions|ToFloat(Boolean) (!= (- (Math|Conversions|ToInteger(Boolean) (Variables|Default|GetRotation%20clamped%20to%20Displacement)) 1) (.AXIS (Utilities|Struct|BreakF_CSVdata _returnvalue_5))))))) _displacement_randomize)) (Variables|Default|GetShuffle)) (Math|Vector|MakeVector (.R_X (Utilities|Struct|BreakF_CSVdata _returnvalue_5)) (.R_Y (Utilities|Struct|BreakF_CSVdata _returnvalue_5)) (.R_Z (Utilities|Struct|BreakF_CSVdata _returnvalue_5)))))) (.Z (Math|Vector|BreakVector (+ (+ (Math|Vector|MakeVector (Math|Random|RandomFloatinRangefromStream (* (.X (Math|Vector|BreakVector (* (Variables|Default|GetRandom%20Rotation%20[XYZ]) (Math|Conversions|ToFloat(Boolean) (!= (- (Math|Conversions|ToInteger(Boolean) (Variables|Default|GetRotation%20clamped%20to%20Displacement)) 1) (.AXIS (Utilities|Struct|BreakF_CSVdata _returnvalue_5))))))) -1.0) (.X (Math|Vector|BreakVector (* (Variables|Default|GetRandom%20Rotation%20[XYZ]) (Math|Conversions|ToFloat(Boolean) (!= (- (Math|Conversions|ToInteger(Boolean) (Variables|Default|GetRotation%20clamped%20to%20Displacement)) 1) (.AXIS (Utilities|Struct|BreakF_CSVdata _returnvalue_5))))))) _displacement_randomize) (Math|Random|RandomFloatinRangefromStream (* (.Y (Math|Vector|BreakVector (* (Variables|Default|GetRandom%20Rotation%20[XYZ]) (Math|Conversions|ToFloat(Boolean) (!= (- (Math|Conversions|ToInteger(Boolean) (Variables|Default|GetRotation%20clamped%20to%20Displacement)) 1) (.AXIS (Utilities|Struct|BreakF_CSVdata _returnvalue_5))))))) -1.0) (.Y (Math|Vector|BreakVector (* (Variables|Default|GetRandom%20Rotation%20[XYZ]) (Math|Conversions|ToFloat(Boolean) (!= (- (Math|Conversions|ToInteger(Boolean) (Variables|Default|GetRotation%20clamped%20to%20Displacement)) 1) (.AXIS (Utilities|Struct|BreakF_CSVdata _returnvalue_5))))))) _displacement_randomize) (Math|Random|RandomFloatinRangefromStream (* (.Z (Math|Vector|BreakVector (* (Variables|Default|GetRandom%20Rotation%20[XYZ]) (Math|Conversions|ToFloat(Boolean) (!= (- (Math|Conversions|ToInteger(Boolean) (Variables|Default|GetRotation%20clamped%20to%20Displacement)) 1) (.AXIS (Utilities|Struct|BreakF_CSVdata _returnvalue_5))))))) -1.0) (.Z (Math|Vector|BreakVector (* (Variables|Default|GetRandom%20Rotation%20[XYZ]) (Math|Conversions|ToFloat(Boolean) (!= (- (Math|Conversions|ToInteger(Boolean) (Variables|Default|GetRotation%20clamped%20to%20Displacement)) 1) (.AXIS (Utilities|Struct|BreakF_CSVdata _returnvalue_5))))))) _displacement_randomize)) (Variables|Default|GetShuffle)) (Math|Vector|MakeVector (.R_X (Utilities|Struct|BreakF_CSVdata _returnvalue_5)) (.R_Y (Utilities|Struct|BreakF_CSVdata _returnvalue_5)) (.R_Z (Utilities|Struct|BreakF_CSVdata _returnvalue_5))))))) (Math|Conversions|ToFloat(Boolean) (Variables|Default|GetRandom%20Rotation%20LOCAL/GLOBAL))) (* (Math|Vector|MakeVector (.S_X (Utilities|Struct|BreakF_CSVdata _returnvalue_5)) (.S_Y (Utilities|Struct|BreakF_CSVdata _returnvalue_5)) (.S_Z (Utilities|Struct|BreakF_CSVdata _returnvalue_5))) (Variables|Default|GetScale))) false))))
                  (:8
                    (if _undamaged_stones_3
                      (goto _label_7)
                      (elif _extrastones_2
                        (Utilities|FlowControl|MultiGate false true (Math|Integer|%(Integer) (Variables|Default|GetShuffleExtraStones) 2) :!label _label_8
                          (:Out%200
                            (Utilities|FlowControl|Sequence :!label _label_9
                              (:then_0
                                (Utilities|FlowControl|DoOnce false
                                  (:Completed
                                    (bind _returnvalue_13 (AddComponent|AddHierarchicalInstancedStaticMeshComponent false))
                                    (bind _output_get_8 (Variables|Default|Set08 _returnvalue_13))
                                    (Rendering|Material|SetMaterial _output_get_8 0 (Variables|Default|GetStone%20Material)))))
                              (:then_1
                                (Components|InstancedStaticMesh|AddInstance (Variables|Default|Get08) (Math|Transform|MakeTransform (Math|Transform|TransformLocation (Math|Transform|MakeTransform (Math|Vector|MakeVector (.T_X (Utilities|Struct|BreakF_CSVdata _returnvalue_5)) (.T_Y (Utilities|Struct|BreakF_CSVdata _returnvalue_5)) (.T_Z (Utilities|Struct|BreakF_CSVdata _returnvalue_5))) (Math|Rotator|Lerp(Rotator) (Math|Rotator|CombineRotators (Math|Rotator|MakeRotator (.X (Math|Vector|BreakVector (+ (Math|Vector|MakeVector (Math|Random|RandomFloatinRangefromStream (* (.X (Math|Vector|BreakVector (* (Variables|Default|GetRandom%20Rotation%20[XYZ]) (Math|Conversions|ToFloat(Boolean) (!= (- (Math|Conversions|ToInteger(Boolean) (Variables|Default|GetRotation%20clamped%20to%20Displacement)) 1) (.AXIS (Utilities|Struct|BreakF_CSVdata _returnvalue_5))))))) -1.0) (.X (Math|Vector|BreakVector (* (Variables|Default|GetRandom%20Rotation%20[XYZ]) (Math|Conversions|ToFloat(Boolean) (!= (- (Math|Conversions|ToInteger(Boolean) (Variables|Default|GetRotation%20clamped%20to%20Displacement)) 1) (.AXIS (Utilities|Struct|BreakF_CSVdata _returnvalue_5))))))) _displacement_randomize) (Math|Random|RandomFloatinRangefromStream (* (.Y (Math|Vector|BreakVector (* (Variables|Default|GetRandom%20Rotation%20[XYZ]) (Math|Conversions|ToFloat(Boolean) (!= (- (Math|Conversions|ToInteger(Boolean) (Variables|Default|GetRotation%20clamped%20to%20Displacement)) 1) (.AXIS (Utilities|Struct|BreakF_CSVdata _returnvalue_5))))))) -1.0) (.Y (Math|Vector|BreakVector (* (Variables|Default|GetRandom%20Rotation%20[XYZ]) (Math|Conversions|ToFloat(Boolean) (!= (- (Math|Conversions|ToInteger(Boolean) (Variables|Default|GetRotation%20clamped%20to%20Displacement)) 1) (.AXIS (Utilities|Struct|BreakF_CSVdata _returnvalue_5))))))) _displacement_randomize) (Math|Random|RandomFloatinRangefromStream (* (.Z (Math|Vector|BreakVector (* (Variables|Default|GetRandom%20Rotation%20[XYZ]) (Math|Conversions|ToFloat(Boolean) (!= (- (Math|Conversions|ToInteger(Boolean) (Variables|Default|GetRotation%20clamped%20to%20Displacement)) 1) (.AXIS (Utilities|Struct|BreakF_CSVdata _returnvalue_5))))))) -1.0) (.Z (Math|Vector|BreakVector (* (Variables|Default|GetRandom%20Rotation%20[XYZ]) (Math|Conversions|ToFloat(Boolean) (!= (- (Math|Conversions|ToInteger(Boolean) (Variables|Default|GetRotation%20clamped%20to%20Displacement)) 1) (.AXIS (Utilities|Struct|BreakF_CSVdata _returnvalue_5))))))) _displacement_randomize)) (Variables|Default|GetShuffle)))) (.Y (Math|Vector|BreakVector (+ (Math|Vector|MakeVector (Math|Random|RandomFloatinRangefromStream (* (.X (Math|Vector|BreakVector (* (Variables|Default|GetRandom%20Rotation%20[XYZ]) (Math|Conversions|ToFloat(Boolean) (!= (- (Math|Conversions|ToInteger(Boolean) (Variables|Default|GetRotation%20clamped%20to%20Displacement)) 1) (.AXIS (Utilities|Struct|BreakF_CSVdata _returnvalue_5))))))) -1.0) (.X (Math|Vector|BreakVector (* (Variables|Default|GetRandom%20Rotation%20[XYZ]) (Math|Conversions|ToFloat(Boolean) (!= (- (Math|Conversions|ToInteger(Boolean) (Variables|Default|GetRotation%20clamped%20to%20Displacement)) 1) (.AXIS (Utilities|Struct|BreakF_CSVdata _returnvalue_5))))))) _displacement_randomize) (Math|Random|RandomFloatinRangefromStream (* (.Y (Math|Vector|BreakVector (* (Variables|Default|GetRandom%20Rotation%20[XYZ]) (Math|Conversions|ToFloat(Boolean) (!= (- (Math|Conversions|ToInteger(Boolean) (Variables|Default|GetRotation%20clamped%20to%20Displacement)) 1) (.AXIS (Utilities|Struct|BreakF_CSVdata _returnvalue_5))))))) -1.0) (.Y (Math|Vector|BreakVector (* (Variables|Default|GetRandom%20Rotation%20[XYZ]) (Math|Conversions|ToFloat(Boolean) (!= (- (Math|Conversions|ToInteger(Boolean) (Variables|Default|GetRotation%20clamped%20to%20Displacement)) 1) (.AXIS (Utilities|Struct|BreakF_CSVdata _returnvalue_5))))))) _displacement_randomize) (Math|Random|RandomFloatinRangefromStream (* (.Z (Math|Vector|BreakVector (* (Variables|Default|GetRandom%20Rotation%20[XYZ]) (Math|Conversions|ToFloat(Boolean) (!= (- (Math|Conversions|ToInteger(Boolean) (Variables|Default|GetRotation%20clamped%20to%20Displacement)) 1) (.AXIS (Utilities|Struct|BreakF_CSVdata _returnvalue_5))))))) -1.0) (.Z (Math|Vector|BreakVector (* (Variables|Default|GetRandom%20Rotation%20[XYZ]) (Math|Conversions|ToFloat(Boolean) (!= (- (Math|Conversions|ToInteger(Boolean) (Variables|Default|GetRotation%20clamped%20to%20Displacement)) 1) (.AXIS (Utilities|Struct|BreakF_CSVdata _returnvalue_5))))))) _displacement_randomize)) (Variables|Default|GetShuffle)))) (.Z (Math|Vector|BreakVector (+ (Math|Vector|MakeVector (Math|Random|RandomFloatinRangefromStream (* (.X (Math|Vector|BreakVector (* (Variables|Default|GetRandom%20Rotation%20[XYZ]) (Math|Conversions|ToFloat(Boolean) (!= (- (Math|Conversions|ToInteger(Boolean) (Variables|Default|GetRotation%20clamped%20to%20Displacement)) 1) (.AXIS (Utilities|Struct|BreakF_CSVdata _returnvalue_5))))))) -1.0) (.X (Math|Vector|BreakVector (* (Variables|Default|GetRandom%20Rotation%20[XYZ]) (Math|Conversions|ToFloat(Boolean) (!= (- (Math|Conversions|ToInteger(Boolean) (Variables|Default|GetRotation%20clamped%20to%20Displacement)) 1) (.AXIS (Utilities|Struct|BreakF_CSVdata _returnvalue_5))))))) _displacement_randomize) (Math|Random|RandomFloatinRangefromStream (* (.Y (Math|Vector|BreakVector (* (Variables|Default|GetRandom%20Rotation%20[XYZ]) (Math|Conversions|ToFloat(Boolean) (!= (- (Math|Conversions|ToInteger(Boolean) (Variables|Default|GetRotation%20clamped%20to%20Displacement)) 1) (.AXIS (Utilities|Struct|BreakF_CSVdata _returnvalue_5))))))) -1.0) (.Y (Math|Vector|BreakVector (* (Variables|Default|GetRandom%20Rotation%20[XYZ]) (Math|Conversions|ToFloat(Boolean) (!= (- (Math|Conversions|ToInteger(Boolean) (Variables|Default|GetRotation%20clamped%20to%20Displacement)) 1) (.AXIS (Utilities|Struct|BreakF_CSVdata _returnvalue_5))))))) _displacement_randomize) (Math|Random|RandomFloatinRangefromStream (* (.Z (Math|Vector|BreakVector (* (Variables|Default|GetRandom%20Rotation%20[XYZ]) (Math|Conversions|ToFloat(Boolean) (!= (- (Math|Conversions|ToInteger(Boolean) (Variables|Default|GetRotation%20clamped%20to%20Displacement)) 1) (.AXIS (Utilities|Struct|BreakF_CSVdata _returnvalue_5))))))) -1.0) (.Z (Math|Vector|BreakVector (* (Variables|Default|GetRandom%20Rotation%20[XYZ]) (Math|Conversions|ToFloat(Boolean) (!= (- (Math|Conversions|ToInteger(Boolean) (Variables|Default|GetRotation%20clamped%20to%20Displacement)) 1) (.AXIS (Utilities|Struct|BreakF_CSVdata _returnvalue_5))))))) _displacement_randomize)) (Variables|Default|GetShuffle))))) (Math|Rotator|MakeRotator (.R_X (Utilities|Struct|BreakF_CSVdata _returnvalue_5)) (.R_Y (Utilities|Struct|BreakF_CSVdata _returnvalue_5)) (.R_Z (Utilities|Struct|BreakF_CSVdata _returnvalue_5)))) (Math|Rotator|MakeRotator (.X (Math|Vector|BreakVector (+ (+ (Math|Vector|MakeVector (Math|Random|RandomFloatinRangefromStream (* (.X (Math|Vector|BreakVector (* (Variables|Default|GetRandom%20Rotation%20[XYZ]) (Math|Conversions|ToFloat(Boolean) (!= (- (Math|Conversions|ToInteger(Boolean) (Variables|Default|GetRotation%20clamped%20to%20Displacement)) 1) (.AXIS (Utilities|Struct|BreakF_CSVdata _returnvalue_5))))))) -1.0) (.X (Math|Vector|BreakVector (* (Variables|Default|GetRandom%20Rotation%20[XYZ]) (Math|Conversions|ToFloat(Boolean) (!= (- (Math|Conversions|ToInteger(Boolean) (Variables|Default|GetRotation%20clamped%20to%20Displacement)) 1) (.AXIS (Utilities|Struct|BreakF_CSVdata _returnvalue_5))))))) _displacement_randomize) (Math|Random|RandomFloatinRangefromStream (* (.Y (Math|Vector|BreakVector (* (Variables|Default|GetRandom%20Rotation%20[XYZ]) (Math|Conversions|ToFloat(Boolean) (!= (- (Math|Conversions|ToInteger(Boolean) (Variables|Default|GetRotation%20clamped%20to%20Displacement)) 1) (.AXIS (Utilities|Struct|BreakF_CSVdata _returnvalue_5))))))) -1.0) (.Y (Math|Vector|BreakVector (* (Variables|Default|GetRandom%20Rotation%20[XYZ]) (Math|Conversions|ToFloat(Boolean) (!= (- (Math|Conversions|ToInteger(Boolean) (Variables|Default|GetRotation%20clamped%20to%20Displacement)) 1) (.AXIS (Utilities|Struct|BreakF_CSVdata _returnvalue_5))))))) _displacement_randomize) (Math|Random|RandomFloatinRangefromStream (* (.Z (Math|Vector|BreakVector (* (Variables|Default|GetRandom%20Rotation%20[XYZ]) (Math|Conversions|ToFloat(Boolean) (!= (- (Math|Conversions|ToInteger(Boolean) (Variables|Default|GetRotation%20clamped%20to%20Displacement)) 1) (.AXIS (Utilities|Struct|BreakF_CSVdata _returnvalue_5))))))) -1.0) (.Z (Math|Vector|BreakVector (* (Variables|Default|GetRandom%20Rotation%20[XYZ]) (Math|Conversions|ToFloat(Boolean) (!= (- (Math|Conversions|ToInteger(Boolean) (Variables|Default|GetRotation%20clamped%20to%20Displacement)) 1) (.AXIS (Utilities|Struct|BreakF_CSVdata _returnvalue_5))))))) _displacement_randomize)) (Variables|Default|GetShuffle)) (Math|Vector|MakeVector (.R_X (Utilities|Struct|BreakF_CSVdata _returnvalue_5)) (.R_Y (Utilities|Struct|BreakF_CSVdata _returnvalue_5)) (.R_Z (Utilities|Struct|BreakF_CSVdata _returnvalue_5)))))) (.Y (Math|Vector|BreakVector (+ (+ (Math|Vector|MakeVector (Math|Random|RandomFloatinRangefromStream (* (.X (Math|Vector|BreakVector (* (Variables|Default|GetRandom%20Rotation%20[XYZ]) (Math|Conversions|ToFloat(Boolean) (!= (- (Math|Conversions|ToInteger(Boolean) (Variables|Default|GetRotation%20clamped%20to%20Displacement)) 1) (.AXIS (Utilities|Struct|BreakF_CSVdata _returnvalue_5))))))) -1.0) (.X (Math|Vector|BreakVector (* (Variables|Default|GetRandom%20Rotation%20[XYZ]) (Math|Conversions|ToFloat(Boolean) (!= (- (Math|Conversions|ToInteger(Boolean) (Variables|Default|GetRotation%20clamped%20to%20Displacement)) 1) (.AXIS (Utilities|Struct|BreakF_CSVdata _returnvalue_5))))))) _displacement_randomize) (Math|Random|RandomFloatinRangefromStream (* (.Y (Math|Vector|BreakVector (* (Variables|Default|GetRandom%20Rotation%20[XYZ]) (Math|Conversions|ToFloat(Boolean) (!= (- (Math|Conversions|ToInteger(Boolean) (Variables|Default|GetRotation%20clamped%20to%20Displacement)) 1) (.AXIS (Utilities|Struct|BreakF_CSVdata _returnvalue_5))))))) -1.0) (.Y (Math|Vector|BreakVector (* (Variables|Default|GetRandom%20Rotation%20[XYZ]) (Math|Conversions|ToFloat(Boolean) (!= (- (Math|Conversions|ToInteger(Boolean) (Variables|Default|GetRotation%20clamped%20to%20Displacement)) 1) (.AXIS (Utilities|Struct|BreakF_CSVdata _returnvalue_5))))))) _displacement_randomize) (Math|Random|RandomFloatinRangefromStream (* (.Z (Math|Vector|BreakVector (* (Variables|Default|GetRandom%20Rotation%20[XYZ]) (Math|Conversions|ToFloat(Boolean) (!= (- (Math|Conversions|ToInteger(Boolean) (Variables|Default|GetRotation%20clamped%20to%20Displacement)) 1) (.AXIS (Utilities|Struct|BreakF_CSVdata _returnvalue_5))))))) -1.0) (.Z (Math|Vector|BreakVector (* (Variables|Default|GetRandom%20Rotation%20[XYZ]) (Math|Conversions|ToFloat(Boolean) (!= (- (Math|Conversions|ToInteger(Boolean) (Variables|Default|GetRotation%20clamped%20to%20Displacement)) 1) (.AXIS (Utilities|Struct|BreakF_CSVdata _returnvalue_5))))))) _displacement_randomize)) (Variables|Default|GetShuffle)) (Math|Vector|MakeVector (.R_X (Utilities|Struct|BreakF_CSVdata _returnvalue_5)) (.R_Y (Utilities|Struct|BreakF_CSVdata _returnvalue_5)) (.R_Z (Utilities|Struct|BreakF_CSVdata _returnvalue_5)))))) (.Z (Math|Vector|BreakVector (+ (+ (Math|Vector|MakeVector (Math|Random|RandomFloatinRangefromStream (* (.X (Math|Vector|BreakVector (* (Variables|Default|GetRandom%20Rotation%20[XYZ]) (Math|Conversions|ToFloat(Boolean) (!= (- (Math|Conversions|ToInteger(Boolean) (Variables|Default|GetRotation%20clamped%20to%20Displacement)) 1) (.AXIS (Utilities|Struct|BreakF_CSVdata _returnvalue_5))))))) -1.0) (.X (Math|Vector|BreakVector (* (Variables|Default|GetRandom%20Rotation%20[XYZ]) (Math|Conversions|ToFloat(Boolean) (!= (- (Math|Conversions|ToInteger(Boolean) (Variables|Default|GetRotation%20clamped%20to%20Displacement)) 1) (.AXIS (Utilities|Struct|BreakF_CSVdata _returnvalue_5))))))) _displacement_randomize) (Math|Random|RandomFloatinRangefromStream (* (.Y (Math|Vector|BreakVector (* (Variables|Default|GetRandom%20Rotation%20[XYZ]) (Math|Conversions|ToFloat(Boolean) (!= (- (Math|Conversions|ToInteger(Boolean) (Variables|Default|GetRotation%20clamped%20to%20Displacement)) 1) (.AXIS (Utilities|Struct|BreakF_CSVdata _returnvalue_5))))))) -1.0) (.Y (Math|Vector|BreakVector (* (Variables|Default|GetRandom%20Rotation%20[XYZ]) (Math|Conversions|ToFloat(Boolean) (!= (- (Math|Conversions|ToInteger(Boolean) (Variables|Default|GetRotation%20clamped%20to%20Displacement)) 1) (.AXIS (Utilities|Struct|BreakF_CSVdata _returnvalue_5))))))) _displacement_randomize) (Math|Random|RandomFloatinRangefromStream (* (.Z (Math|Vector|BreakVector (* (Variables|Default|GetRandom%20Rotation%20[XYZ]) (Math|Conversions|ToFloat(Boolean) (!= (- (Math|Conversions|ToInteger(Boolean) (Variables|Default|GetRotation%20clamped%20to%20Displacement)) 1) (.AXIS (Utilities|Struct|BreakF_CSVdata _returnvalue_5))))))) -1.0) (.Z (Math|Vector|BreakVector (* (Variables|Default|GetRandom%20Rotation%20[XYZ]) (Math|Conversions|ToFloat(Boolean) (!= (- (Math|Conversions|ToInteger(Boolean) (Variables|Default|GetRotation%20clamped%20to%20Displacement)) 1) (.AXIS (Utilities|Struct|BreakF_CSVdata _returnvalue_5))))))) _displacement_randomize)) (Variables|Default|GetShuffle)) (Math|Vector|MakeVector (.R_X (Utilities|Struct|BreakF_CSVdata _returnvalue_5)) (.R_Y (Utilities|Struct|BreakF_CSVdata _returnvalue_5)) (.R_Z (Utilities|Struct|BreakF_CSVdata _returnvalue_5))))))) (Math|Conversions|ToFloat(Boolean) (Variables|Default|GetRandom%20Rotation%20LOCAL/GLOBAL))) (* (Math|Vector|MakeVector (.S_X (Utilities|Struct|BreakF_CSVdata _returnvalue_5)) (.S_Y (Utilities|Struct|BreakF_CSVdata _returnvalue_5)) (.S_Z (Utilities|Struct|BreakF_CSVdata _returnvalue_5))) (Variables|Default|GetScale))) (* (Math|Vector|MakeVector (* (Math|Conversions|ToFloat(Boolean) (== (.AXIS (Utilities|Struct|BreakF_CSVdata _returnvalue_5)) 1)) _returnvalue_3) (* (Math|Conversions|ToFloat(Boolean) (== (.AXIS (Utilities|Struct|BreakF_CSVdata _returnvalue_5)) 2)) _returnvalue_3) (* (Math|Conversions|ToFloat(Boolean) (== (.AXIS (Utilities|Struct|BreakF_CSVdata _returnvalue_5)) 3)) _returnvalue_3)) (Math|Float|Clamp(Float) (+ (Math|Conversions|ToFloat(Boolean) (and (not (Class|KismetMathLibrary|IsPointinBoxwithTransform (Math|Vector|MakeVector (.T_X (Utilities|Struct|BreakF_CSVdata _returnvalue_5)) (.T_Y (Utilities|Struct|BreakF_CSVdata _returnvalue_5)) (.T_Z (Utilities|Struct|BreakF_CSVdata _returnvalue_5))) (Math|Transform|MakeTransform (Variables|Default|GetBox%20Origin%20[XYZ]) (Variables|Default|GetBox%20Rotation%20[XYZ])) (Variables|Default|GetBox%20Extent%20[XYZ]))) _boxcontrolleddisplacement)) (Variables|Default|GetBox%20Intensity)) (Math|Conversions|ToFloat(Boolean) (not _boxcontrolleddisplacement))))) (Math|Rotator|Lerp(Rotator) (Math|Rotator|CombineRotators (Math|Rotator|MakeRotator (.X (Math|Vector|BreakVector (+ (Math|Vector|MakeVector (Math|Random|RandomFloatinRangefromStream (* (.X (Math|Vector|BreakVector (* (Variables|Default|GetRandom%20Rotation%20[XYZ]) (Math|Conversions|ToFloat(Boolean) (!= (- (Math|Conversions|ToInteger(Boolean) (Variables|Default|GetRotation%20clamped%20to%20Displacement)) 1) (.AXIS (Utilities|Struct|BreakF_CSVdata _returnvalue_5))))))) -1.0) (.X (Math|Vector|BreakVector (* (Variables|Default|GetRandom%20Rotation%20[XYZ]) (Math|Conversions|ToFloat(Boolean) (!= (- (Math|Conversions|ToInteger(Boolean) (Variables|Default|GetRotation%20clamped%20to%20Displacement)) 1) (.AXIS (Utilities|Struct|BreakF_CSVdata _returnvalue_5))))))) _displacement_randomize) (Math|Random|RandomFloatinRangefromStream (* (.Y (Math|Vector|BreakVector (* (Variables|Default|GetRandom%20Rotation%20[XYZ]) (Math|Conversions|ToFloat(Boolean) (!= (- (Math|Conversions|ToInteger(Boolean) (Variables|Default|GetRotation%20clamped%20to%20Displacement)) 1) (.AXIS (Utilities|Struct|BreakF_CSVdata _returnvalue_5))))))) -1.0) (.Y (Math|Vector|BreakVector (* (Variables|Default|GetRandom%20Rotation%20[XYZ]) (Math|Conversions|ToFloat(Boolean) (!= (- (Math|Conversions|ToInteger(Boolean) (Variables|Default|GetRotation%20clamped%20to%20Displacement)) 1) (.AXIS (Utilities|Struct|BreakF_CSVdata _returnvalue_5))))))) _displacement_randomize) (Math|Random|RandomFloatinRangefromStream (* (.Z (Math|Vector|BreakVector (* (Variables|Default|GetRandom%20Rotation%20[XYZ]) (Math|Conversions|ToFloat(Boolean) (!= (- (Math|Conversions|ToInteger(Boolean) (Variables|Default|GetRotation%20clamped%20to%20Displacement)) 1) (.AXIS (Utilities|Struct|BreakF_CSVdata _returnvalue_5))))))) -1.0) (.Z (Math|Vector|BreakVector (* (Variables|Default|GetRandom%20Rotation%20[XYZ]) (Math|Conversions|ToFloat(Boolean) (!= (- (Math|Conversions|ToInteger(Boolean) (Variables|Default|GetRotation%20clamped%20to%20Displacement)) 1) (.AXIS (Utilities|Struct|BreakF_CSVdata _returnvalue_5))))))) _displacement_randomize)) (Variables|Default|GetShuffle)))) (.Y (Math|Vector|BreakVector (+ (Math|Vector|MakeVector (Math|Random|RandomFloatinRangefromStream (* (.X (Math|Vector|BreakVector (* (Variables|Default|GetRandom%20Rotation%20[XYZ]) (Math|Conversions|ToFloat(Boolean) (!= (- (Math|Conversions|ToInteger(Boolean) (Variables|Default|GetRotation%20clamped%20to%20Displacement)) 1) (.AXIS (Utilities|Struct|BreakF_CSVdata _returnvalue_5))))))) -1.0) (.X (Math|Vector|BreakVector (* (Variables|Default|GetRandom%20Rotation%20[XYZ]) (Math|Conversions|ToFloat(Boolean) (!= (- (Math|Conversions|ToInteger(Boolean) (Variables|Default|GetRotation%20clamped%20to%20Displacement)) 1) (.AXIS (Utilities|Struct|BreakF_CSVdata _returnvalue_5))))))) _displacement_randomize) (Math|Random|RandomFloatinRangefromStream (* (.Y (Math|Vector|BreakVector (* (Variables|Default|GetRandom%20Rotation%20[XYZ]) (Math|Conversions|ToFloat(Boolean) (!= (- (Math|Conversions|ToInteger(Boolean) (Variables|Default|GetRotation%20clamped%20to%20Displacement)) 1) (.AXIS (Utilities|Struct|BreakF_CSVdata _returnvalue_5))))))) -1.0) (.Y (Math|Vector|BreakVector (* (Variables|Default|GetRandom%20Rotation%20[XYZ]) (Math|Conversions|ToFloat(Boolean) (!= (- (Math|Conversions|ToInteger(Boolean) (Variables|Default|GetRotation%20clamped%20to%20Displacement)) 1) (.AXIS (Utilities|Struct|BreakF_CSVdata _returnvalue_5))))))) _displacement_randomize) (Math|Random|RandomFloatinRangefromStream (* (.Z (Math|Vector|BreakVector (* (Variables|Default|GetRandom%20Rotation%20[XYZ]) (Math|Conversions|ToFloat(Boolean) (!= (- (Math|Conversions|ToInteger(Boolean) (Variables|Default|GetRotation%20clamped%20to%20Displacement)) 1) (.AXIS (Utilities|Struct|BreakF_CSVdata _returnvalue_5))))))) -1.0) (.Z (Math|Vector|BreakVector (* (Variables|Default|GetRandom%20Rotation%20[XYZ]) (Math|Conversions|ToFloat(Boolean) (!= (- (Math|Conversions|ToInteger(Boolean) (Variables|Default|GetRotation%20clamped%20to%20Displacement)) 1) (.AXIS (Utilities|Struct|BreakF_CSVdata _returnvalue_5))))))) _displacement_randomize)) (Variables|Default|GetShuffle)))) (.Z (Math|Vector|BreakVector (+ (Math|Vector|MakeVector (Math|Random|RandomFloatinRangefromStream (* (.X (Math|Vector|BreakVector (* (Variables|Default|GetRandom%20Rotation%20[XYZ]) (Math|Conversions|ToFloat(Boolean) (!= (- (Math|Conversions|ToInteger(Boolean) (Variables|Default|GetRotation%20clamped%20to%20Displacement)) 1) (.AXIS (Utilities|Struct|BreakF_CSVdata _returnvalue_5))))))) -1.0) (.X (Math|Vector|BreakVector (* (Variables|Default|GetRandom%20Rotation%20[XYZ]) (Math|Conversions|ToFloat(Boolean) (!= (- (Math|Conversions|ToInteger(Boolean) (Variables|Default|GetRotation%20clamped%20to%20Displacement)) 1) (.AXIS (Utilities|Struct|BreakF_CSVdata _returnvalue_5))))))) _displacement_randomize) (Math|Random|RandomFloatinRangefromStream (* (.Y (Math|Vector|BreakVector (* (Variables|Default|GetRandom%20Rotation%20[XYZ]) (Math|Conversions|ToFloat(Boolean) (!= (- (Math|Conversions|ToInteger(Boolean) (Variables|Default|GetRotation%20clamped%20to%20Displacement)) 1) (.AXIS (Utilities|Struct|BreakF_CSVdata _returnvalue_5))))))) -1.0) (.Y (Math|Vector|BreakVector (* (Variables|Default|GetRandom%20Rotation%20[XYZ]) (Math|Conversions|ToFloat(Boolean) (!= (- (Math|Conversions|ToInteger(Boolean) (Variables|Default|GetRotation%20clamped%20to%20Displacement)) 1) (.AXIS (Utilities|Struct|BreakF_CSVdata _returnvalue_5))))))) _displacement_randomize) (Math|Random|RandomFloatinRangefromStream (* (.Z (Math|Vector|BreakVector (* (Variables|Default|GetRandom%20Rotation%20[XYZ]) (Math|Conversions|ToFloat(Boolean) (!= (- (Math|Conversions|ToInteger(Boolean) (Variables|Default|GetRotation%20clamped%20to%20Displacement)) 1) (.AXIS (Utilities|Struct|BreakF_CSVdata _returnvalue_5))))))) -1.0) (.Z (Math|Vector|BreakVector (* (Variables|Default|GetRandom%20Rotation%20[XYZ]) (Math|Conversions|ToFloat(Boolean) (!= (- (Math|Conversions|ToInteger(Boolean) (Variables|Default|GetRotation%20clamped%20to%20Displacement)) 1) (.AXIS (Utilities|Struct|BreakF_CSVdata _returnvalue_5))))))) _displacement_randomize)) (Variables|Default|GetShuffle))))) (Math|Rotator|MakeRotator (.R_X (Utilities|Struct|BreakF_CSVdata _returnvalue_5)) (.R_Y (Utilities|Struct|BreakF_CSVdata _returnvalue_5)) (.R_Z (Utilities|Struct|BreakF_CSVdata _returnvalue_5)))) (Math|Rotator|MakeRotator (.X (Math|Vector|BreakVector (+ (+ (Math|Vector|MakeVector (Math|Random|RandomFloatinRangefromStream (* (.X (Math|Vector|BreakVector (* (Variables|Default|GetRandom%20Rotation%20[XYZ]) (Math|Conversions|ToFloat(Boolean) (!= (- (Math|Conversions|ToInteger(Boolean) (Variables|Default|GetRotation%20clamped%20to%20Displacement)) 1) (.AXIS (Utilities|Struct|BreakF_CSVdata _returnvalue_5))))))) -1.0) (.X (Math|Vector|BreakVector (* (Variables|Default|GetRandom%20Rotation%20[XYZ]) (Math|Conversions|ToFloat(Boolean) (!= (- (Math|Conversions|ToInteger(Boolean) (Variables|Default|GetRotation%20clamped%20to%20Displacement)) 1) (.AXIS (Utilities|Struct|BreakF_CSVdata _returnvalue_5))))))) _displacement_randomize) (Math|Random|RandomFloatinRangefromStream (* (.Y (Math|Vector|BreakVector (* (Variables|Default|GetRandom%20Rotation%20[XYZ]) (Math|Conversions|ToFloat(Boolean) (!= (- (Math|Conversions|ToInteger(Boolean) (Variables|Default|GetRotation%20clamped%20to%20Displacement)) 1) (.AXIS (Utilities|Struct|BreakF_CSVdata _returnvalue_5))))))) -1.0) (.Y (Math|Vector|BreakVector (* (Variables|Default|GetRandom%20Rotation%20[XYZ]) (Math|Conversions|ToFloat(Boolean) (!= (- (Math|Conversions|ToInteger(Boolean) (Variables|Default|GetRotation%20clamped%20to%20Displacement)) 1) (.AXIS (Utilities|Struct|BreakF_CSVdata _returnvalue_5))))))) _displacement_randomize) (Math|Random|RandomFloatinRangefromStream (* (.Z (Math|Vector|BreakVector (* (Variables|Default|GetRandom%20Rotation%20[XYZ]) (Math|Conversions|ToFloat(Boolean) (!= (- (Math|Conversions|ToInteger(Boolean) (Variables|Default|GetRotation%20clamped%20to%20Displacement)) 1) (.AXIS (Utilities|Struct|BreakF_CSVdata _returnvalue_5))))))) -1.0) (.Z (Math|Vector|BreakVector (* (Variables|Default|GetRandom%20Rotation%20[XYZ]) (Math|Conversions|ToFloat(Boolean) (!= (- (Math|Conversions|ToInteger(Boolean) (Variables|Default|GetRotation%20clamped%20to%20Displacement)) 1) (.AXIS (Utilities|Struct|BreakF_CSVdata _returnvalue_5))))))) _displacement_randomize)) (Variables|Default|GetShuffle)) (Math|Vector|MakeVector (.R_X (Utilities|Struct|BreakF_CSVdata _returnvalue_5)) (.R_Y (Utilities|Struct|BreakF_CSVdata _returnvalue_5)) (.R_Z (Utilities|Struct|BreakF_CSVdata _returnvalue_5)))))) (.Y (Math|Vector|BreakVector (+ (+ (Math|Vector|MakeVector (Math|Random|RandomFloatinRangefromStream (* (.X (Math|Vector|BreakVector (* (Variables|Default|GetRandom%20Rotation%20[XYZ]) (Math|Conversions|ToFloat(Boolean) (!= (- (Math|Conversions|ToInteger(Boolean) (Variables|Default|GetRotation%20clamped%20to%20Displacement)) 1) (.AXIS (Utilities|Struct|BreakF_CSVdata _returnvalue_5))))))) -1.0) (.X (Math|Vector|BreakVector (* (Variables|Default|GetRandom%20Rotation%20[XYZ]) (Math|Conversions|ToFloat(Boolean) (!= (- (Math|Conversions|ToInteger(Boolean) (Variables|Default|GetRotation%20clamped%20to%20Displacement)) 1) (.AXIS (Utilities|Struct|BreakF_CSVdata _returnvalue_5))))))) _displacement_randomize) (Math|Random|RandomFloatinRangefromStream (* (.Y (Math|Vector|BreakVector (* (Variables|Default|GetRandom%20Rotation%20[XYZ]) (Math|Conversions|ToFloat(Boolean) (!= (- (Math|Conversions|ToInteger(Boolean) (Variables|Default|GetRotation%20clamped%20to%20Displacement)) 1) (.AXIS (Utilities|Struct|BreakF_CSVdata _returnvalue_5))))))) -1.0) (.Y (Math|Vector|BreakVector (* (Variables|Default|GetRandom%20Rotation%20[XYZ]) (Math|Conversions|ToFloat(Boolean) (!= (- (Math|Conversions|ToInteger(Boolean) (Variables|Default|GetRotation%20clamped%20to%20Displacement)) 1) (.AXIS (Utilities|Struct|BreakF_CSVdata _returnvalue_5))))))) _displacement_randomize) (Math|Random|RandomFloatinRangefromStream (* (.Z (Math|Vector|BreakVector (* (Variables|Default|GetRandom%20Rotation%20[XYZ]) (Math|Conversions|ToFloat(Boolean) (!= (- (Math|Conversions|ToInteger(Boolean) (Variables|Default|GetRotation%20clamped%20to%20Displacement)) 1) (.AXIS (Utilities|Struct|BreakF_CSVdata _returnvalue_5))))))) -1.0) (.Z (Math|Vector|BreakVector (* (Variables|Default|GetRandom%20Rotation%20[XYZ]) (Math|Conversions|ToFloat(Boolean) (!= (- (Math|Conversions|ToInteger(Boolean) (Variables|Default|GetRotation%20clamped%20to%20Displacement)) 1) (.AXIS (Utilities|Struct|BreakF_CSVdata _returnvalue_5))))))) _displacement_randomize)) (Variables|Default|GetShuffle)) (Math|Vector|MakeVector (.R_X (Utilities|Struct|BreakF_CSVdata _returnvalue_5)) (.R_Y (Utilities|Struct|BreakF_CSVdata _returnvalue_5)) (.R_Z (Utilities|Struct|BreakF_CSVdata _returnvalue_5)))))) (.Z (Math|Vector|BreakVector (+ (+ (Math|Vector|MakeVector (Math|Random|RandomFloatinRangefromStream (* (.X (Math|Vector|BreakVector (* (Variables|Default|GetRandom%20Rotation%20[XYZ]) (Math|Conversions|ToFloat(Boolean) (!= (- (Math|Conversions|ToInteger(Boolean) (Variables|Default|GetRotation%20clamped%20to%20Displacement)) 1) (.AXIS (Utilities|Struct|BreakF_CSVdata _returnvalue_5))))))) -1.0) (.X (Math|Vector|BreakVector (* (Variables|Default|GetRandom%20Rotation%20[XYZ]) (Math|Conversions|ToFloat(Boolean) (!= (- (Math|Conversions|ToInteger(Boolean) (Variables|Default|GetRotation%20clamped%20to%20Displacement)) 1) (.AXIS (Utilities|Struct|BreakF_CSVdata _returnvalue_5))))))) _displacement_randomize) (Math|Random|RandomFloatinRangefromStream (* (.Y (Math|Vector|BreakVector (* (Variables|Default|GetRandom%20Rotation%20[XYZ]) (Math|Conversions|ToFloat(Boolean) (!= (- (Math|Conversions|ToInteger(Boolean) (Variables|Default|GetRotation%20clamped%20to%20Displacement)) 1) (.AXIS (Utilities|Struct|BreakF_CSVdata _returnvalue_5))))))) -1.0) (.Y (Math|Vector|BreakVector (* (Variables|Default|GetRandom%20Rotation%20[XYZ]) (Math|Conversions|ToFloat(Boolean) (!= (- (Math|Conversions|ToInteger(Boolean) (Variables|Default|GetRotation%20clamped%20to%20Displacement)) 1) (.AXIS (Utilities|Struct|BreakF_CSVdata _returnvalue_5))))))) _displacement_randomize) (Math|Random|RandomFloatinRangefromStream (* (.Z (Math|Vector|BreakVector (* (Variables|Default|GetRandom%20Rotation%20[XYZ]) (Math|Conversions|ToFloat(Boolean) (!= (- (Math|Conversions|ToInteger(Boolean) (Variables|Default|GetRotation%20clamped%20to%20Displacement)) 1) (.AXIS (Utilities|Struct|BreakF_CSVdata _returnvalue_5))))))) -1.0) (.Z (Math|Vector|BreakVector (* (Variables|Default|GetRandom%20Rotation%20[XYZ]) (Math|Conversions|ToFloat(Boolean) (!= (- (Math|Conversions|ToInteger(Boolean) (Variables|Default|GetRotation%20clamped%20to%20Displacement)) 1) (.AXIS (Utilities|Struct|BreakF_CSVdata _returnvalue_5))))))) _displacement_randomize)) (Variables|Default|GetShuffle)) (Math|Vector|MakeVector (.R_X (Utilities|Struct|BreakF_CSVdata _returnvalue_5)) (.R_Y (Utilities|Struct|BreakF_CSVdata _returnvalue_5)) (.R_Z (Utilities|Struct|BreakF_CSVdata _returnvalue_5))))))) (Math|Conversions|ToFloat(Boolean) (Variables|Default|GetRandom%20Rotation%20LOCAL/GLOBAL))) (* (Math|Vector|MakeVector (.S_X (Utilities|Struct|BreakF_CSVdata _returnvalue_5)) (.S_Y (Utilities|Struct|BreakF_CSVdata _returnvalue_5)) (.S_Z (Utilities|Struct|BreakF_CSVdata _returnvalue_5))) (Variables|Default|GetScale))) false))))
                          (:Out%201
                            (Utilities|FlowControl|Sequence :!label _label_10
                              (:then_0
                                (Utilities|FlowControl|DoOnce false
                                  (:Completed
                                    (bind _returnvalue_14 (AddComponent|AddHierarchicalInstancedStaticMeshComponent false))
                                    (bind _output_get_9 (Variables|Default|Set09 _returnvalue_14))
                                    (Rendering|Material|SetMaterial _output_get_9 0 (Variables|Default|GetStone%20Material)))))
                              (:then_1
                                (Components|InstancedStaticMesh|AddInstance (Variables|Default|Get09) (Math|Transform|MakeTransform (Math|Transform|TransformLocation (Math|Transform|MakeTransform (Math|Vector|MakeVector (.T_X (Utilities|Struct|BreakF_CSVdata _returnvalue_5)) (.T_Y (Utilities|Struct|BreakF_CSVdata _returnvalue_5)) (.T_Z (Utilities|Struct|BreakF_CSVdata _returnvalue_5))) (Math|Rotator|Lerp(Rotator) (Math|Rotator|CombineRotators (Math|Rotator|MakeRotator (.X (Math|Vector|BreakVector (+ (Math|Vector|MakeVector (Math|Random|RandomFloatinRangefromStream (* (.X (Math|Vector|BreakVector (* (Variables|Default|GetRandom%20Rotation%20[XYZ]) (Math|Conversions|ToFloat(Boolean) (!= (- (Math|Conversions|ToInteger(Boolean) (Variables|Default|GetRotation%20clamped%20to%20Displacement)) 1) (.AXIS (Utilities|Struct|BreakF_CSVdata _returnvalue_5))))))) -1.0) (.X (Math|Vector|BreakVector (* (Variables|Default|GetRandom%20Rotation%20[XYZ]) (Math|Conversions|ToFloat(Boolean) (!= (- (Math|Conversions|ToInteger(Boolean) (Variables|Default|GetRotation%20clamped%20to%20Displacement)) 1) (.AXIS (Utilities|Struct|BreakF_CSVdata _returnvalue_5))))))) _displacement_randomize) (Math|Random|RandomFloatinRangefromStream (* (.Y (Math|Vector|BreakVector (* (Variables|Default|GetRandom%20Rotation%20[XYZ]) (Math|Conversions|ToFloat(Boolean) (!= (- (Math|Conversions|ToInteger(Boolean) (Variables|Default|GetRotation%20clamped%20to%20Displacement)) 1) (.AXIS (Utilities|Struct|BreakF_CSVdata _returnvalue_5))))))) -1.0) (.Y (Math|Vector|BreakVector (* (Variables|Default|GetRandom%20Rotation%20[XYZ]) (Math|Conversions|ToFloat(Boolean) (!= (- (Math|Conversions|ToInteger(Boolean) (Variables|Default|GetRotation%20clamped%20to%20Displacement)) 1) (.AXIS (Utilities|Struct|BreakF_CSVdata _returnvalue_5))))))) _displacement_randomize) (Math|Random|RandomFloatinRangefromStream (* (.Z (Math|Vector|BreakVector (* (Variables|Default|GetRandom%20Rotation%20[XYZ]) (Math|Conversions|ToFloat(Boolean) (!= (- (Math|Conversions|ToInteger(Boolean) (Variables|Default|GetRotation%20clamped%20to%20Displacement)) 1) (.AXIS (Utilities|Struct|BreakF_CSVdata _returnvalue_5))))))) -1.0) (.Z (Math|Vector|BreakVector (* (Variables|Default|GetRandom%20Rotation%20[XYZ]) (Math|Conversions|ToFloat(Boolean) (!= (- (Math|Conversions|ToInteger(Boolean) (Variables|Default|GetRotation%20clamped%20to%20Displacement)) 1) (.AXIS (Utilities|Struct|BreakF_CSVdata _returnvalue_5))))))) _displacement_randomize)) (Variables|Default|GetShuffle)))) (.Y (Math|Vector|BreakVector (+ (Math|Vector|MakeVector (Math|Random|RandomFloatinRangefromStream (* (.X (Math|Vector|BreakVector (* (Variables|Default|GetRandom%20Rotation%20[XYZ]) (Math|Conversions|ToFloat(Boolean) (!= (- (Math|Conversions|ToInteger(Boolean) (Variables|Default|GetRotation%20clamped%20to%20Displacement)) 1) (.AXIS (Utilities|Struct|BreakF_CSVdata _returnvalue_5))))))) -1.0) (.X (Math|Vector|BreakVector (* (Variables|Default|GetRandom%20Rotation%20[XYZ]) (Math|Conversions|ToFloat(Boolean) (!= (- (Math|Conversions|ToInteger(Boolean) (Variables|Default|GetRotation%20clamped%20to%20Displacement)) 1) (.AXIS (Utilities|Struct|BreakF_CSVdata _returnvalue_5))))))) _displacement_randomize) (Math|Random|RandomFloatinRangefromStream (* (.Y (Math|Vector|BreakVector (* (Variables|Default|GetRandom%20Rotation%20[XYZ]) (Math|Conversions|ToFloat(Boolean) (!= (- (Math|Conversions|ToInteger(Boolean) (Variables|Default|GetRotation%20clamped%20to%20Displacement)) 1) (.AXIS (Utilities|Struct|BreakF_CSVdata _returnvalue_5))))))) -1.0) (.Y (Math|Vector|BreakVector (* (Variables|Default|GetRandom%20Rotation%20[XYZ]) (Math|Conversions|ToFloat(Boolean) (!= (- (Math|Conversions|ToInteger(Boolean) (Variables|Default|GetRotation%20clamped%20to%20Displacement)) 1) (.AXIS (Utilities|Struct|BreakF_CSVdata _returnvalue_5))))))) _displacement_randomize) (Math|Random|RandomFloatinRangefromStream (* (.Z (Math|Vector|BreakVector (* (Variables|Default|GetRandom%20Rotation%20[XYZ]) (Math|Conversions|ToFloat(Boolean) (!= (- (Math|Conversions|ToInteger(Boolean) (Variables|Default|GetRotation%20clamped%20to%20Displacement)) 1) (.AXIS (Utilities|Struct|BreakF_CSVdata _returnvalue_5))))))) -1.0) (.Z (Math|Vector|BreakVector (* (Variables|Default|GetRandom%20Rotation%20[XYZ]) (Math|Conversions|ToFloat(Boolean) (!= (- (Math|Conversions|ToInteger(Boolean) (Variables|Default|GetRotation%20clamped%20to%20Displacement)) 1) (.AXIS (Utilities|Struct|BreakF_CSVdata _returnvalue_5))))))) _displacement_randomize)) (Variables|Default|GetShuffle)))) (.Z (Math|Vector|BreakVector (+ (Math|Vector|MakeVector (Math|Random|RandomFloatinRangefromStream (* (.X (Math|Vector|BreakVector (* (Variables|Default|GetRandom%20Rotation%20[XYZ]) (Math|Conversions|ToFloat(Boolean) (!= (- (Math|Conversions|ToInteger(Boolean) (Variables|Default|GetRotation%20clamped%20to%20Displacement)) 1) (.AXIS (Utilities|Struct|BreakF_CSVdata _returnvalue_5))))))) -1.0) (.X (Math|Vector|BreakVector (* (Variables|Default|GetRandom%20Rotation%20[XYZ]) (Math|Conversions|ToFloat(Boolean) (!= (- (Math|Conversions|ToInteger(Boolean) (Variables|Default|GetRotation%20clamped%20to%20Displacement)) 1) (.AXIS (Utilities|Struct|BreakF_CSVdata _returnvalue_5))))))) _displacement_randomize) (Math|Random|RandomFloatinRangefromStream (* (.Y (Math|Vector|BreakVector (* (Variables|Default|GetRandom%20Rotation%20[XYZ]) (Math|Conversions|ToFloat(Boolean) (!= (- (Math|Conversions|ToInteger(Boolean) (Variables|Default|GetRotation%20clamped%20to%20Displacement)) 1) (.AXIS (Utilities|Struct|BreakF_CSVdata _returnvalue_5))))))) -1.0) (.Y (Math|Vector|BreakVector (* (Variables|Default|GetRandom%20Rotation%20[XYZ]) (Math|Conversions|ToFloat(Boolean) (!= (- (Math|Conversions|ToInteger(Boolean) (Variables|Default|GetRotation%20clamped%20to%20Displacement)) 1) (.AXIS (Utilities|Struct|BreakF_CSVdata _returnvalue_5))))))) _displacement_randomize) (Math|Random|RandomFloatinRangefromStream (* (.Z (Math|Vector|BreakVector (* (Variables|Default|GetRandom%20Rotation%20[XYZ]) (Math|Conversions|ToFloat(Boolean) (!= (- (Math|Conversions|ToInteger(Boolean) (Variables|Default|GetRotation%20clamped%20to%20Displacement)) 1) (.AXIS (Utilities|Struct|BreakF_CSVdata _returnvalue_5))))))) -1.0) (.Z (Math|Vector|BreakVector (* (Variables|Default|GetRandom%20Rotation%20[XYZ]) (Math|Conversions|ToFloat(Boolean) (!= (- (Math|Conversions|ToInteger(Boolean) (Variables|Default|GetRotation%20clamped%20to%20Displacement)) 1) (.AXIS (Utilities|Struct|BreakF_CSVdata _returnvalue_5))))))) _displacement_randomize)) (Variables|Default|GetShuffle))))) (Math|Rotator|MakeRotator (.R_X (Utilities|Struct|BreakF_CSVdata _returnvalue_5)) (.R_Y (Utilities|Struct|BreakF_CSVdata _returnvalue_5)) (.R_Z (Utilities|Struct|BreakF_CSVdata _returnvalue_5)))) (Math|Rotator|MakeRotator (.X (Math|Vector|BreakVector (+ (+ (Math|Vector|MakeVector (Math|Random|RandomFloatinRangefromStream (* (.X (Math|Vector|BreakVector (* (Variables|Default|GetRandom%20Rotation%20[XYZ]) (Math|Conversions|ToFloat(Boolean) (!= (- (Math|Conversions|ToInteger(Boolean) (Variables|Default|GetRotation%20clamped%20to%20Displacement)) 1) (.AXIS (Utilities|Struct|BreakF_CSVdata _returnvalue_5))))))) -1.0) (.X (Math|Vector|BreakVector (* (Variables|Default|GetRandom%20Rotation%20[XYZ]) (Math|Conversions|ToFloat(Boolean) (!= (- (Math|Conversions|ToInteger(Boolean) (Variables|Default|GetRotation%20clamped%20to%20Displacement)) 1) (.AXIS (Utilities|Struct|BreakF_CSVdata _returnvalue_5))))))) _displacement_randomize) (Math|Random|RandomFloatinRangefromStream (* (.Y (Math|Vector|BreakVector (* (Variables|Default|GetRandom%20Rotation%20[XYZ]) (Math|Conversions|ToFloat(Boolean) (!= (- (Math|Conversions|ToInteger(Boolean) (Variables|Default|GetRotation%20clamped%20to%20Displacement)) 1) (.AXIS (Utilities|Struct|BreakF_CSVdata _returnvalue_5))))))) -1.0) (.Y (Math|Vector|BreakVector (* (Variables|Default|GetRandom%20Rotation%20[XYZ]) (Math|Conversions|ToFloat(Boolean) (!= (- (Math|Conversions|ToInteger(Boolean) (Variables|Default|GetRotation%20clamped%20to%20Displacement)) 1) (.AXIS (Utilities|Struct|BreakF_CSVdata _returnvalue_5))))))) _displacement_randomize) (Math|Random|RandomFloatinRangefromStream (* (.Z (Math|Vector|BreakVector (* (Variables|Default|GetRandom%20Rotation%20[XYZ]) (Math|Conversions|ToFloat(Boolean) (!= (- (Math|Conversions|ToInteger(Boolean) (Variables|Default|GetRotation%20clamped%20to%20Displacement)) 1) (.AXIS (Utilities|Struct|BreakF_CSVdata _returnvalue_5))))))) -1.0) (.Z (Math|Vector|BreakVector (* (Variables|Default|GetRandom%20Rotation%20[XYZ]) (Math|Conversions|ToFloat(Boolean) (!= (- (Math|Conversions|ToInteger(Boolean) (Variables|Default|GetRotation%20clamped%20to%20Displacement)) 1) (.AXIS (Utilities|Struct|BreakF_CSVdata _returnvalue_5))))))) _displacement_randomize)) (Variables|Default|GetShuffle)) (Math|Vector|MakeVector (.R_X (Utilities|Struct|BreakF_CSVdata _returnvalue_5)) (.R_Y (Utilities|Struct|BreakF_CSVdata _returnvalue_5)) (.R_Z (Utilities|Struct|BreakF_CSVdata _returnvalue_5)))))) (.Y (Math|Vector|BreakVector (+ (+ (Math|Vector|MakeVector (Math|Random|RandomFloatinRangefromStream (* (.X (Math|Vector|BreakVector (* (Variables|Default|GetRandom%20Rotation%20[XYZ]) (Math|Conversions|ToFloat(Boolean) (!= (- (Math|Conversions|ToInteger(Boolean) (Variables|Default|GetRotation%20clamped%20to%20Displacement)) 1) (.AXIS (Utilities|Struct|BreakF_CSVdata _returnvalue_5))))))) -1.0) (.X (Math|Vector|BreakVector (* (Variables|Default|GetRandom%20Rotation%20[XYZ]) (Math|Conversions|ToFloat(Boolean) (!= (- (Math|Conversions|ToInteger(Boolean) (Variables|Default|GetRotation%20clamped%20to%20Displacement)) 1) (.AXIS (Utilities|Struct|BreakF_CSVdata _returnvalue_5))))))) _displacement_randomize) (Math|Random|RandomFloatinRangefromStream (* (.Y (Math|Vector|BreakVector (* (Variables|Default|GetRandom%20Rotation%20[XYZ]) (Math|Conversions|ToFloat(Boolean) (!= (- (Math|Conversions|ToInteger(Boolean) (Variables|Default|GetRotation%20clamped%20to%20Displacement)) 1) (.AXIS (Utilities|Struct|BreakF_CSVdata _returnvalue_5))))))) -1.0) (.Y (Math|Vector|BreakVector (* (Variables|Default|GetRandom%20Rotation%20[XYZ]) (Math|Conversions|ToFloat(Boolean) (!= (- (Math|Conversions|ToInteger(Boolean) (Variables|Default|GetRotation%20clamped%20to%20Displacement)) 1) (.AXIS (Utilities|Struct|BreakF_CSVdata _returnvalue_5))))))) _displacement_randomize) (Math|Random|RandomFloatinRangefromStream (* (.Z (Math|Vector|BreakVector (* (Variables|Default|GetRandom%20Rotation%20[XYZ]) (Math|Conversions|ToFloat(Boolean) (!= (- (Math|Conversions|ToInteger(Boolean) (Variables|Default|GetRotation%20clamped%20to%20Displacement)) 1) (.AXIS (Utilities|Struct|BreakF_CSVdata _returnvalue_5))))))) -1.0) (.Z (Math|Vector|BreakVector (* (Variables|Default|GetRandom%20Rotation%20[XYZ]) (Math|Conversions|ToFloat(Boolean) (!= (- (Math|Conversions|ToInteger(Boolean) (Variables|Default|GetRotation%20clamped%20to%20Displacement)) 1) (.AXIS (Utilities|Struct|BreakF_CSVdata _returnvalue_5))))))) _displacement_randomize)) (Variables|Default|GetShuffle)) (Math|Vector|MakeVector (.R_X (Utilities|Struct|BreakF_CSVdata _returnvalue_5)) (.R_Y (Utilities|Struct|BreakF_CSVdata _returnvalue_5)) (.R_Z (Utilities|Struct|BreakF_CSVdata _returnvalue_5)))))) (.Z (Math|Vector|BreakVector (+ (+ (Math|Vector|MakeVector (Math|Random|RandomFloatinRangefromStream (* (.X (Math|Vector|BreakVector (* (Variables|Default|GetRandom%20Rotation%20[XYZ]) (Math|Conversions|ToFloat(Boolean) (!= (- (Math|Conversions|ToInteger(Boolean) (Variables|Default|GetRotation%20clamped%20to%20Displacement)) 1) (.AXIS (Utilities|Struct|BreakF_CSVdata _returnvalue_5))))))) -1.0) (.X (Math|Vector|BreakVector (* (Variables|Default|GetRandom%20Rotation%20[XYZ]) (Math|Conversions|ToFloat(Boolean) (!= (- (Math|Conversions|ToInteger(Boolean) (Variables|Default|GetRotation%20clamped%20to%20Displacement)) 1) (.AXIS (Utilities|Struct|BreakF_CSVdata _returnvalue_5))))))) _displacement_randomize) (Math|Random|RandomFloatinRangefromStream (* (.Y (Math|Vector|BreakVector (* (Variables|Default|GetRandom%20Rotation%20[XYZ]) (Math|Conversions|ToFloat(Boolean) (!= (- (Math|Conversions|ToInteger(Boolean) (Variables|Default|GetRotation%20clamped%20to%20Displacement)) 1) (.AXIS (Utilities|Struct|BreakF_CSVdata _returnvalue_5))))))) -1.0) (.Y (Math|Vector|BreakVector (* (Variables|Default|GetRandom%20Rotation%20[XYZ]) (Math|Conversions|ToFloat(Boolean) (!= (- (Math|Conversions|ToInteger(Boolean) (Variables|Default|GetRotation%20clamped%20to%20Displacement)) 1) (.AXIS (Utilities|Struct|BreakF_CSVdata _returnvalue_5))))))) _displacement_randomize) (Math|Random|RandomFloatinRangefromStream (* (.Z (Math|Vector|BreakVector (* (Variables|Default|GetRandom%20Rotation%20[XYZ]) (Math|Conversions|ToFloat(Boolean) (!= (- (Math|Conversions|ToInteger(Boolean) (Variables|Default|GetRotation%20clamped%20to%20Displacement)) 1) (.AXIS (Utilities|Struct|BreakF_CSVdata _returnvalue_5))))))) -1.0) (.Z (Math|Vector|BreakVector (* (Variables|Default|GetRandom%20Rotation%20[XYZ]) (Math|Conversions|ToFloat(Boolean) (!= (- (Math|Conversions|ToInteger(Boolean) (Variables|Default|GetRotation%20clamped%20to%20Displacement)) 1) (.AXIS (Utilities|Struct|BreakF_CSVdata _returnvalue_5))))))) _displacement_randomize)) (Variables|Default|GetShuffle)) (Math|Vector|MakeVector (.R_X (Utilities|Struct|BreakF_CSVdata _returnvalue_5)) (.R_Y (Utilities|Struct|BreakF_CSVdata _returnvalue_5)) (.R_Z (Utilities|Struct|BreakF_CSVdata _returnvalue_5))))))) (Math|Conversions|ToFloat(Boolean) (Variables|Default|GetRandom%20Rotation%20LOCAL/GLOBAL))) (* (Math|Vector|MakeVector (.S_X (Utilities|Struct|BreakF_CSVdata _returnvalue_5)) (.S_Y (Utilities|Struct|BreakF_CSVdata _returnvalue_5)) (.S_Z (Utilities|Struct|BreakF_CSVdata _returnvalue_5))) (Variables|Default|GetScale))) (* (Math|Vector|MakeVector (* (Math|Conversions|ToFloat(Boolean) (== (.AXIS (Utilities|Struct|BreakF_CSVdata _returnvalue_5)) 1)) _returnvalue_3) (* (Math|Conversions|ToFloat(Boolean) (== (.AXIS (Utilities|Struct|BreakF_CSVdata _returnvalue_5)) 2)) _returnvalue_3) (* (Math|Conversions|ToFloat(Boolean) (== (.AXIS (Utilities|Struct|BreakF_CSVdata _returnvalue_5)) 3)) _returnvalue_3)) (Math|Float|Clamp(Float) (+ (Math|Conversions|ToFloat(Boolean) (and (not (Class|KismetMathLibrary|IsPointinBoxwithTransform (Math|Vector|MakeVector (.T_X (Utilities|Struct|BreakF_CSVdata _returnvalue_5)) (.T_Y (Utilities|Struct|BreakF_CSVdata _returnvalue_5)) (.T_Z (Utilities|Struct|BreakF_CSVdata _returnvalue_5))) (Math|Transform|MakeTransform (Variables|Default|GetBox%20Origin%20[XYZ]) (Variables|Default|GetBox%20Rotation%20[XYZ])) (Variables|Default|GetBox%20Extent%20[XYZ]))) _boxcontrolleddisplacement)) (Variables|Default|GetBox%20Intensity)) (Math|Conversions|ToFloat(Boolean) (not _boxcontrolleddisplacement))))) (Math|Rotator|Lerp(Rotator) (Math|Rotator|CombineRotators (Math|Rotator|MakeRotator (.X (Math|Vector|BreakVector (+ (Math|Vector|MakeVector (Math|Random|RandomFloatinRangefromStream (* (.X (Math|Vector|BreakVector (* (Variables|Default|GetRandom%20Rotation%20[XYZ]) (Math|Conversions|ToFloat(Boolean) (!= (- (Math|Conversions|ToInteger(Boolean) (Variables|Default|GetRotation%20clamped%20to%20Displacement)) 1) (.AXIS (Utilities|Struct|BreakF_CSVdata _returnvalue_5))))))) -1.0) (.X (Math|Vector|BreakVector (* (Variables|Default|GetRandom%20Rotation%20[XYZ]) (Math|Conversions|ToFloat(Boolean) (!= (- (Math|Conversions|ToInteger(Boolean) (Variables|Default|GetRotation%20clamped%20to%20Displacement)) 1) (.AXIS (Utilities|Struct|BreakF_CSVdata _returnvalue_5))))))) _displacement_randomize) (Math|Random|RandomFloatinRangefromStream (* (.Y (Math|Vector|BreakVector (* (Variables|Default|GetRandom%20Rotation%20[XYZ]) (Math|Conversions|ToFloat(Boolean) (!= (- (Math|Conversions|ToInteger(Boolean) (Variables|Default|GetRotation%20clamped%20to%20Displacement)) 1) (.AXIS (Utilities|Struct|BreakF_CSVdata _returnvalue_5))))))) -1.0) (.Y (Math|Vector|BreakVector (* (Variables|Default|GetRandom%20Rotation%20[XYZ]) (Math|Conversions|ToFloat(Boolean) (!= (- (Math|Conversions|ToInteger(Boolean) (Variables|Default|GetRotation%20clamped%20to%20Displacement)) 1) (.AXIS (Utilities|Struct|BreakF_CSVdata _returnvalue_5))))))) _displacement_randomize) (Math|Random|RandomFloatinRangefromStream (* (.Z (Math|Vector|BreakVector (* (Variables|Default|GetRandom%20Rotation%20[XYZ]) (Math|Conversions|ToFloat(Boolean) (!= (- (Math|Conversions|ToInteger(Boolean) (Variables|Default|GetRotation%20clamped%20to%20Displacement)) 1) (.AXIS (Utilities|Struct|BreakF_CSVdata _returnvalue_5))))))) -1.0) (.Z (Math|Vector|BreakVector (* (Variables|Default|GetRandom%20Rotation%20[XYZ]) (Math|Conversions|ToFloat(Boolean) (!= (- (Math|Conversions|ToInteger(Boolean) (Variables|Default|GetRotation%20clamped%20to%20Displacement)) 1) (.AXIS (Utilities|Struct|BreakF_CSVdata _returnvalue_5))))))) _displacement_randomize)) (Variables|Default|GetShuffle)))) (.Y (Math|Vector|BreakVector (+ (Math|Vector|MakeVector (Math|Random|RandomFloatinRangefromStream (* (.X (Math|Vector|BreakVector (* (Variables|Default|GetRandom%20Rotation%20[XYZ]) (Math|Conversions|ToFloat(Boolean) (!= (- (Math|Conversions|ToInteger(Boolean) (Variables|Default|GetRotation%20clamped%20to%20Displacement)) 1) (.AXIS (Utilities|Struct|BreakF_CSVdata _returnvalue_5))))))) -1.0) (.X (Math|Vector|BreakVector (* (Variables|Default|GetRandom%20Rotation%20[XYZ]) (Math|Conversions|ToFloat(Boolean) (!= (- (Math|Conversions|ToInteger(Boolean) (Variables|Default|GetRotation%20clamped%20to%20Displacement)) 1) (.AXIS (Utilities|Struct|BreakF_CSVdata _returnvalue_5))))))) _displacement_randomize) (Math|Random|RandomFloatinRangefromStream (* (.Y (Math|Vector|BreakVector (* (Variables|Default|GetRandom%20Rotation%20[XYZ]) (Math|Conversions|ToFloat(Boolean) (!= (- (Math|Conversions|ToInteger(Boolean) (Variables|Default|GetRotation%20clamped%20to%20Displacement)) 1) (.AXIS (Utilities|Struct|BreakF_CSVdata _returnvalue_5))))))) -1.0) (.Y (Math|Vector|BreakVector (* (Variables|Default|GetRandom%20Rotation%20[XYZ]) (Math|Conversions|ToFloat(Boolean) (!= (- (Math|Conversions|ToInteger(Boolean) (Variables|Default|GetRotation%20clamped%20to%20Displacement)) 1) (.AXIS (Utilities|Struct|BreakF_CSVdata _returnvalue_5))))))) _displacement_randomize) (Math|Random|RandomFloatinRangefromStream (* (.Z (Math|Vector|BreakVector (* (Variables|Default|GetRandom%20Rotation%20[XYZ]) (Math|Conversions|ToFloat(Boolean) (!= (- (Math|Conversions|ToInteger(Boolean) (Variables|Default|GetRotation%20clamped%20to%20Displacement)) 1) (.AXIS (Utilities|Struct|BreakF_CSVdata _returnvalue_5))))))) -1.0) (.Z (Math|Vector|BreakVector (* (Variables|Default|GetRandom%20Rotation%20[XYZ]) (Math|Conversions|ToFloat(Boolean) (!= (- (Math|Conversions|ToInteger(Boolean) (Variables|Default|GetRotation%20clamped%20to%20Displacement)) 1) (.AXIS (Utilities|Struct|BreakF_CSVdata _returnvalue_5))))))) _displacement_randomize)) (Variables|Default|GetShuffle)))) (.Z (Math|Vector|BreakVector (+ (Math|Vector|MakeVector (Math|Random|RandomFloatinRangefromStream (* (.X (Math|Vector|BreakVector (* (Variables|Default|GetRandom%20Rotation%20[XYZ]) (Math|Conversions|ToFloat(Boolean) (!= (- (Math|Conversions|ToInteger(Boolean) (Variables|Default|GetRotation%20clamped%20to%20Displacement)) 1) (.AXIS (Utilities|Struct|BreakF_CSVdata _returnvalue_5))))))) -1.0) (.X (Math|Vector|BreakVector (* (Variables|Default|GetRandom%20Rotation%20[XYZ]) (Math|Conversions|ToFloat(Boolean) (!= (- (Math|Conversions|ToInteger(Boolean) (Variables|Default|GetRotation%20clamped%20to%20Displacement)) 1) (.AXIS (Utilities|Struct|BreakF_CSVdata _returnvalue_5))))))) _displacement_randomize) (Math|Random|RandomFloatinRangefromStream (* (.Y (Math|Vector|BreakVector (* (Variables|Default|GetRandom%20Rotation%20[XYZ]) (Math|Conversions|ToFloat(Boolean) (!= (- (Math|Conversions|ToInteger(Boolean) (Variables|Default|GetRotation%20clamped%20to%20Displacement)) 1) (.AXIS (Utilities|Struct|BreakF_CSVdata _returnvalue_5))))))) -1.0) (.Y (Math|Vector|BreakVector (* (Variables|Default|GetRandom%20Rotation%20[XYZ]) (Math|Conversions|ToFloat(Boolean) (!= (- (Math|Conversions|ToInteger(Boolean) (Variables|Default|GetRotation%20clamped%20to%20Displacement)) 1) (.AXIS (Utilities|Struct|BreakF_CSVdata _returnvalue_5))))))) _displacement_randomize) (Math|Random|RandomFloatinRangefromStream (* (.Z (Math|Vector|BreakVector (* (Variables|Default|GetRandom%20Rotation%20[XYZ]) (Math|Conversions|ToFloat(Boolean) (!= (- (Math|Conversions|ToInteger(Boolean) (Variables|Default|GetRotation%20clamped%20to%20Displacement)) 1) (.AXIS (Utilities|Struct|BreakF_CSVdata _returnvalue_5))))))) -1.0) (.Z (Math|Vector|BreakVector (* (Variables|Default|GetRandom%20Rotation%20[XYZ]) (Math|Conversions|ToFloat(Boolean) (!= (- (Math|Conversions|ToInteger(Boolean) (Variables|Default|GetRotation%20clamped%20to%20Displacement)) 1) (.AXIS (Utilities|Struct|BreakF_CSVdata _returnvalue_5))))))) _displacement_randomize)) (Variables|Default|GetShuffle))))) (Math|Rotator|MakeRotator (.R_X (Utilities|Struct|BreakF_CSVdata _returnvalue_5)) (.R_Y (Utilities|Struct|BreakF_CSVdata _returnvalue_5)) (.R_Z (Utilities|Struct|BreakF_CSVdata _returnvalue_5)))) (Math|Rotator|MakeRotator (.X (Math|Vector|BreakVector (+ (+ (Math|Vector|MakeVector (Math|Random|RandomFloatinRangefromStream (* (.X (Math|Vector|BreakVector (* (Variables|Default|GetRandom%20Rotation%20[XYZ]) (Math|Conversions|ToFloat(Boolean) (!= (- (Math|Conversions|ToInteger(Boolean) (Variables|Default|GetRotation%20clamped%20to%20Displacement)) 1) (.AXIS (Utilities|Struct|BreakF_CSVdata _returnvalue_5))))))) -1.0) (.X (Math|Vector|BreakVector (* (Variables|Default|GetRandom%20Rotation%20[XYZ]) (Math|Conversions|ToFloat(Boolean) (!= (- (Math|Conversions|ToInteger(Boolean) (Variables|Default|GetRotation%20clamped%20to%20Displacement)) 1) (.AXIS (Utilities|Struct|BreakF_CSVdata _returnvalue_5))))))) _displacement_randomize) (Math|Random|RandomFloatinRangefromStream (* (.Y (Math|Vector|BreakVector (* (Variables|Default|GetRandom%20Rotation%20[XYZ]) (Math|Conversions|ToFloat(Boolean) (!= (- (Math|Conversions|ToInteger(Boolean) (Variables|Default|GetRotation%20clamped%20to%20Displacement)) 1) (.AXIS (Utilities|Struct|BreakF_CSVdata _returnvalue_5))))))) -1.0) (.Y (Math|Vector|BreakVector (* (Variables|Default|GetRandom%20Rotation%20[XYZ]) (Math|Conversions|ToFloat(Boolean) (!= (- (Math|Conversions|ToInteger(Boolean) (Variables|Default|GetRotation%20clamped%20to%20Displacement)) 1) (.AXIS (Utilities|Struct|BreakF_CSVdata _returnvalue_5))))))) _displacement_randomize) (Math|Random|RandomFloatinRangefromStream (* (.Z (Math|Vector|BreakVector (* (Variables|Default|GetRandom%20Rotation%20[XYZ]) (Math|Conversions|ToFloat(Boolean) (!= (- (Math|Conversions|ToInteger(Boolean) (Variables|Default|GetRotation%20clamped%20to%20Displacement)) 1) (.AXIS (Utilities|Struct|BreakF_CSVdata _returnvalue_5))))))) -1.0) (.Z (Math|Vector|BreakVector (* (Variables|Default|GetRandom%20Rotation%20[XYZ]) (Math|Conversions|ToFloat(Boolean) (!= (- (Math|Conversions|ToInteger(Boolean) (Variables|Default|GetRotation%20clamped%20to%20Displacement)) 1) (.AXIS (Utilities|Struct|BreakF_CSVdata _returnvalue_5))))))) _displacement_randomize)) (Variables|Default|GetShuffle)) (Math|Vector|MakeVector (.R_X (Utilities|Struct|BreakF_CSVdata _returnvalue_5)) (.R_Y (Utilities|Struct|BreakF_CSVdata _returnvalue_5)) (.R_Z (Utilities|Struct|BreakF_CSVdata _returnvalue_5)))))) (.Y (Math|Vector|BreakVector (+ (+ (Math|Vector|MakeVector (Math|Random|RandomFloatinRangefromStream (* (.X (Math|Vector|BreakVector (* (Variables|Default|GetRandom%20Rotation%20[XYZ]) (Math|Conversions|ToFloat(Boolean) (!= (- (Math|Conversions|ToInteger(Boolean) (Variables|Default|GetRotation%20clamped%20to%20Displacement)) 1) (.AXIS (Utilities|Struct|BreakF_CSVdata _returnvalue_5))))))) -1.0) (.X (Math|Vector|BreakVector (* (Variables|Default|GetRandom%20Rotation%20[XYZ]) (Math|Conversions|ToFloat(Boolean) (!= (- (Math|Conversions|ToInteger(Boolean) (Variables|Default|GetRotation%20clamped%20to%20Displacement)) 1) (.AXIS (Utilities|Struct|BreakF_CSVdata _returnvalue_5))))))) _displacement_randomize) (Math|Random|RandomFloatinRangefromStream (* (.Y (Math|Vector|BreakVector (* (Variables|Default|GetRandom%20Rotation%20[XYZ]) (Math|Conversions|ToFloat(Boolean) (!= (- (Math|Conversions|ToInteger(Boolean) (Variables|Default|GetRotation%20clamped%20to%20Displacement)) 1) (.AXIS (Utilities|Struct|BreakF_CSVdata _returnvalue_5))))))) -1.0) (.Y (Math|Vector|BreakVector (* (Variables|Default|GetRandom%20Rotation%20[XYZ]) (Math|Conversions|ToFloat(Boolean) (!= (- (Math|Conversions|ToInteger(Boolean) (Variables|Default|GetRotation%20clamped%20to%20Displacement)) 1) (.AXIS (Utilities|Struct|BreakF_CSVdata _returnvalue_5))))))) _displacement_randomize) (Math|Random|RandomFloatinRangefromStream (* (.Z (Math|Vector|BreakVector (* (Variables|Default|GetRandom%20Rotation%20[XYZ]) (Math|Conversions|ToFloat(Boolean) (!= (- (Math|Conversions|ToInteger(Boolean) (Variables|Default|GetRotation%20clamped%20to%20Displacement)) 1) (.AXIS (Utilities|Struct|BreakF_CSVdata _returnvalue_5))))))) -1.0) (.Z (Math|Vector|BreakVector (* (Variables|Default|GetRandom%20Rotation%20[XYZ]) (Math|Conversions|ToFloat(Boolean) (!= (- (Math|Conversions|ToInteger(Boolean) (Variables|Default|GetRotation%20clamped%20to%20Displacement)) 1) (.AXIS (Utilities|Struct|BreakF_CSVdata _returnvalue_5))))))) _displacement_randomize)) (Variables|Default|GetShuffle)) (Math|Vector|MakeVector (.R_X (Utilities|Struct|BreakF_CSVdata _returnvalue_5)) (.R_Y (Utilities|Struct|BreakF_CSVdata _returnvalue_5)) (.R_Z (Utilities|Struct|BreakF_CSVdata _returnvalue_5)))))) (.Z (Math|Vector|BreakVector (+ (+ (Math|Vector|MakeVector (Math|Random|RandomFloatinRangefromStream (* (.X (Math|Vector|BreakVector (* (Variables|Default|GetRandom%20Rotation%20[XYZ]) (Math|Conversions|ToFloat(Boolean) (!= (- (Math|Conversions|ToInteger(Boolean) (Variables|Default|GetRotation%20clamped%20to%20Displacement)) 1) (.AXIS (Utilities|Struct|BreakF_CSVdata _returnvalue_5))))))) -1.0) (.X (Math|Vector|BreakVector (* (Variables|Default|GetRandom%20Rotation%20[XYZ]) (Math|Conversions|ToFloat(Boolean) (!= (- (Math|Conversions|ToInteger(Boolean) (Variables|Default|GetRotation%20clamped%20to%20Displacement)) 1) (.AXIS (Utilities|Struct|BreakF_CSVdata _returnvalue_5))))))) _displacement_randomize) (Math|Random|RandomFloatinRangefromStream (* (.Y (Math|Vector|BreakVector (* (Variables|Default|GetRandom%20Rotation%20[XYZ]) (Math|Conversions|ToFloat(Boolean) (!= (- (Math|Conversions|ToInteger(Boolean) (Variables|Default|GetRotation%20clamped%20to%20Displacement)) 1) (.AXIS (Utilities|Struct|BreakF_CSVdata _returnvalue_5))))))) -1.0) (.Y (Math|Vector|BreakVector (* (Variables|Default|GetRandom%20Rotation%20[XYZ]) (Math|Conversions|ToFloat(Boolean) (!= (- (Math|Conversions|ToInteger(Boolean) (Variables|Default|GetRotation%20clamped%20to%20Displacement)) 1) (.AXIS (Utilities|Struct|BreakF_CSVdata _returnvalue_5))))))) _displacement_randomize) (Math|Random|RandomFloatinRangefromStream (* (.Z (Math|Vector|BreakVector (* (Variables|Default|GetRandom%20Rotation%20[XYZ]) (Math|Conversions|ToFloat(Boolean) (!= (- (Math|Conversions|ToInteger(Boolean) (Variables|Default|GetRotation%20clamped%20to%20Displacement)) 1) (.AXIS (Utilities|Struct|BreakF_CSVdata _returnvalue_5))))))) -1.0) (.Z (Math|Vector|BreakVector (* (Variables|Default|GetRandom%20Rotation%20[XYZ]) (Math|Conversions|ToFloat(Boolean) (!= (- (Math|Conversions|ToInteger(Boolean) (Variables|Default|GetRotation%20clamped%20to%20Displacement)) 1) (.AXIS (Utilities|Struct|BreakF_CSVdata _returnvalue_5))))))) _displacement_randomize)) (Variables|Default|GetShuffle)) (Math|Vector|MakeVector (.R_X (Utilities|Struct|BreakF_CSVdata _returnvalue_5)) (.R_Y (Utilities|Struct|BreakF_CSVdata _returnvalue_5)) (.R_Z (Utilities|Struct|BreakF_CSVdata _returnvalue_5))))))) (Math|Conversions|ToFloat(Boolean) (Variables|Default|GetRandom%20Rotation%20LOCAL/GLOBAL))) (* (Math|Vector|MakeVector (.S_X (Utilities|Struct|BreakF_CSVdata _returnvalue_5)) (.S_Y (Utilities|Struct|BreakF_CSVdata _returnvalue_5)) (.S_Z (Utilities|Struct|BreakF_CSVdata _returnvalue_5))) (Variables|Default|GetScale))) false)))))
                        (else
                          (goto _label_9)))))
                  (:9
                    (if _undamaged_stones_3
                      (goto _label_7)
                      (elif _extrastones_2
                        (goto _label_8)
                        (else
                          (goto _label_10)))))
                  (:10
                    (Utilities|FlowControl|Sequence :!label _label_11
                      (:then_0
                        (Utilities|FlowControl|DoOnce false
                          (:Completed
                            (bind _returnvalue_15 (AddComponent|AddHierarchicalInstancedStaticMeshComponent false))
                            (bind _output_get_10 (Variables|Default|Set10 _returnvalue_15))
                            (Rendering|Material|SetMaterial _output_get_10 0 (Variables|Default|GetStone%20Material)))))
                      (:then_1
                        (Components|InstancedStaticMesh|AddInstance (Variables|Default|Get10) (Math|Transform|MakeTransform (Math|Transform|TransformLocation (Math|Transform|MakeTransform (Math|Vector|MakeVector (.T_X (Utilities|Struct|BreakF_CSVdata _returnvalue_5)) (.T_Y (Utilities|Struct|BreakF_CSVdata _returnvalue_5)) (.T_Z (Utilities|Struct|BreakF_CSVdata _returnvalue_5))) (Math|Rotator|Lerp(Rotator) (Math|Rotator|CombineRotators (Math|Rotator|MakeRotator (.X (Math|Vector|BreakVector (+ (Math|Vector|MakeVector (Math|Random|RandomFloatinRangefromStream (* (.X (Math|Vector|BreakVector (* (Variables|Default|GetRandom%20Rotation%20[XYZ]) (Math|Conversions|ToFloat(Boolean) (!= (- (Math|Conversions|ToInteger(Boolean) (Variables|Default|GetRotation%20clamped%20to%20Displacement)) 1) (.AXIS (Utilities|Struct|BreakF_CSVdata _returnvalue_5))))))) -1.0) (.X (Math|Vector|BreakVector (* (Variables|Default|GetRandom%20Rotation%20[XYZ]) (Math|Conversions|ToFloat(Boolean) (!= (- (Math|Conversions|ToInteger(Boolean) (Variables|Default|GetRotation%20clamped%20to%20Displacement)) 1) (.AXIS (Utilities|Struct|BreakF_CSVdata _returnvalue_5))))))) _displacement_randomize) (Math|Random|RandomFloatinRangefromStream (* (.Y (Math|Vector|BreakVector (* (Variables|Default|GetRandom%20Rotation%20[XYZ]) (Math|Conversions|ToFloat(Boolean) (!= (- (Math|Conversions|ToInteger(Boolean) (Variables|Default|GetRotation%20clamped%20to%20Displacement)) 1) (.AXIS (Utilities|Struct|BreakF_CSVdata _returnvalue_5))))))) -1.0) (.Y (Math|Vector|BreakVector (* (Variables|Default|GetRandom%20Rotation%20[XYZ]) (Math|Conversions|ToFloat(Boolean) (!= (- (Math|Conversions|ToInteger(Boolean) (Variables|Default|GetRotation%20clamped%20to%20Displacement)) 1) (.AXIS (Utilities|Struct|BreakF_CSVdata _returnvalue_5))))))) _displacement_randomize) (Math|Random|RandomFloatinRangefromStream (* (.Z (Math|Vector|BreakVector (* (Variables|Default|GetRandom%20Rotation%20[XYZ]) (Math|Conversions|ToFloat(Boolean) (!= (- (Math|Conversions|ToInteger(Boolean) (Variables|Default|GetRotation%20clamped%20to%20Displacement)) 1) (.AXIS (Utilities|Struct|BreakF_CSVdata _returnvalue_5))))))) -1.0) (.Z (Math|Vector|BreakVector (* (Variables|Default|GetRandom%20Rotation%20[XYZ]) (Math|Conversions|ToFloat(Boolean) (!= (- (Math|Conversions|ToInteger(Boolean) (Variables|Default|GetRotation%20clamped%20to%20Displacement)) 1) (.AXIS (Utilities|Struct|BreakF_CSVdata _returnvalue_5))))))) _displacement_randomize)) (Variables|Default|GetShuffle)))) (.Y (Math|Vector|BreakVector (+ (Math|Vector|MakeVector (Math|Random|RandomFloatinRangefromStream (* (.X (Math|Vector|BreakVector (* (Variables|Default|GetRandom%20Rotation%20[XYZ]) (Math|Conversions|ToFloat(Boolean) (!= (- (Math|Conversions|ToInteger(Boolean) (Variables|Default|GetRotation%20clamped%20to%20Displacement)) 1) (.AXIS (Utilities|Struct|BreakF_CSVdata _returnvalue_5))))))) -1.0) (.X (Math|Vector|BreakVector (* (Variables|Default|GetRandom%20Rotation%20[XYZ]) (Math|Conversions|ToFloat(Boolean) (!= (- (Math|Conversions|ToInteger(Boolean) (Variables|Default|GetRotation%20clamped%20to%20Displacement)) 1) (.AXIS (Utilities|Struct|BreakF_CSVdata _returnvalue_5))))))) _displacement_randomize) (Math|Random|RandomFloatinRangefromStream (* (.Y (Math|Vector|BreakVector (* (Variables|Default|GetRandom%20Rotation%20[XYZ]) (Math|Conversions|ToFloat(Boolean) (!= (- (Math|Conversions|ToInteger(Boolean) (Variables|Default|GetRotation%20clamped%20to%20Displacement)) 1) (.AXIS (Utilities|Struct|BreakF_CSVdata _returnvalue_5))))))) -1.0) (.Y (Math|Vector|BreakVector (* (Variables|Default|GetRandom%20Rotation%20[XYZ]) (Math|Conversions|ToFloat(Boolean) (!= (- (Math|Conversions|ToInteger(Boolean) (Variables|Default|GetRotation%20clamped%20to%20Displacement)) 1) (.AXIS (Utilities|Struct|BreakF_CSVdata _returnvalue_5))))))) _displacement_randomize) (Math|Random|RandomFloatinRangefromStream (* (.Z (Math|Vector|BreakVector (* (Variables|Default|GetRandom%20Rotation%20[XYZ]) (Math|Conversions|ToFloat(Boolean) (!= (- (Math|Conversions|ToInteger(Boolean) (Variables|Default|GetRotation%20clamped%20to%20Displacement)) 1) (.AXIS (Utilities|Struct|BreakF_CSVdata _returnvalue_5))))))) -1.0) (.Z (Math|Vector|BreakVector (* (Variables|Default|GetRandom%20Rotation%20[XYZ]) (Math|Conversions|ToFloat(Boolean) (!= (- (Math|Conversions|ToInteger(Boolean) (Variables|Default|GetRotation%20clamped%20to%20Displacement)) 1) (.AXIS (Utilities|Struct|BreakF_CSVdata _returnvalue_5))))))) _displacement_randomize)) (Variables|Default|GetShuffle)))) (.Z (Math|Vector|BreakVector (+ (Math|Vector|MakeVector (Math|Random|RandomFloatinRangefromStream (* (.X (Math|Vector|BreakVector (* (Variables|Default|GetRandom%20Rotation%20[XYZ]) (Math|Conversions|ToFloat(Boolean) (!= (- (Math|Conversions|ToInteger(Boolean) (Variables|Default|GetRotation%20clamped%20to%20Displacement)) 1) (.AXIS (Utilities|Struct|BreakF_CSVdata _returnvalue_5))))))) -1.0) (.X (Math|Vector|BreakVector (* (Variables|Default|GetRandom%20Rotation%20[XYZ]) (Math|Conversions|ToFloat(Boolean) (!= (- (Math|Conversions|ToInteger(Boolean) (Variables|Default|GetRotation%20clamped%20to%20Displacement)) 1) (.AXIS (Utilities|Struct|BreakF_CSVdata _returnvalue_5))))))) _displacement_randomize) (Math|Random|RandomFloatinRangefromStream (* (.Y (Math|Vector|BreakVector (* (Variables|Default|GetRandom%20Rotation%20[XYZ]) (Math|Conversions|ToFloat(Boolean) (!= (- (Math|Conversions|ToInteger(Boolean) (Variables|Default|GetRotation%20clamped%20to%20Displacement)) 1) (.AXIS (Utilities|Struct|BreakF_CSVdata _returnvalue_5))))))) -1.0) (.Y (Math|Vector|BreakVector (* (Variables|Default|GetRandom%20Rotation%20[XYZ]) (Math|Conversions|ToFloat(Boolean) (!= (- (Math|Conversions|ToInteger(Boolean) (Variables|Default|GetRotation%20clamped%20to%20Displacement)) 1) (.AXIS (Utilities|Struct|BreakF_CSVdata _returnvalue_5))))))) _displacement_randomize) (Math|Random|RandomFloatinRangefromStream (* (.Z (Math|Vector|BreakVector (* (Variables|Default|GetRandom%20Rotation%20[XYZ]) (Math|Conversions|ToFloat(Boolean) (!= (- (Math|Conversions|ToInteger(Boolean) (Variables|Default|GetRotation%20clamped%20to%20Displacement)) 1) (.AXIS (Utilities|Struct|BreakF_CSVdata _returnvalue_5))))))) -1.0) (.Z (Math|Vector|BreakVector (* (Variables|Default|GetRandom%20Rotation%20[XYZ]) (Math|Conversions|ToFloat(Boolean) (!= (- (Math|Conversions|ToInteger(Boolean) (Variables|Default|GetRotation%20clamped%20to%20Displacement)) 1) (.AXIS (Utilities|Struct|BreakF_CSVdata _returnvalue_5))))))) _displacement_randomize)) (Variables|Default|GetShuffle))))) (Math|Rotator|MakeRotator (.R_X (Utilities|Struct|BreakF_CSVdata _returnvalue_5)) (.R_Y (Utilities|Struct|BreakF_CSVdata _returnvalue_5)) (.R_Z (Utilities|Struct|BreakF_CSVdata _returnvalue_5)))) (Math|Rotator|MakeRotator (.X (Math|Vector|BreakVector (+ (+ (Math|Vector|MakeVector (Math|Random|RandomFloatinRangefromStream (* (.X (Math|Vector|BreakVector (* (Variables|Default|GetRandom%20Rotation%20[XYZ]) (Math|Conversions|ToFloat(Boolean) (!= (- (Math|Conversions|ToInteger(Boolean) (Variables|Default|GetRotation%20clamped%20to%20Displacement)) 1) (.AXIS (Utilities|Struct|BreakF_CSVdata _returnvalue_5))))))) -1.0) (.X (Math|Vector|BreakVector (* (Variables|Default|GetRandom%20Rotation%20[XYZ]) (Math|Conversions|ToFloat(Boolean) (!= (- (Math|Conversions|ToInteger(Boolean) (Variables|Default|GetRotation%20clamped%20to%20Displacement)) 1) (.AXIS (Utilities|Struct|BreakF_CSVdata _returnvalue_5))))))) _displacement_randomize) (Math|Random|RandomFloatinRangefromStream (* (.Y (Math|Vector|BreakVector (* (Variables|Default|GetRandom%20Rotation%20[XYZ]) (Math|Conversions|ToFloat(Boolean) (!= (- (Math|Conversions|ToInteger(Boolean) (Variables|Default|GetRotation%20clamped%20to%20Displacement)) 1) (.AXIS (Utilities|Struct|BreakF_CSVdata _returnvalue_5))))))) -1.0) (.Y (Math|Vector|BreakVector (* (Variables|Default|GetRandom%20Rotation%20[XYZ]) (Math|Conversions|ToFloat(Boolean) (!= (- (Math|Conversions|ToInteger(Boolean) (Variables|Default|GetRotation%20clamped%20to%20Displacement)) 1) (.AXIS (Utilities|Struct|BreakF_CSVdata _returnvalue_5))))))) _displacement_randomize) (Math|Random|RandomFloatinRangefromStream (* (.Z (Math|Vector|BreakVector (* (Variables|Default|GetRandom%20Rotation%20[XYZ]) (Math|Conversions|ToFloat(Boolean) (!= (- (Math|Conversions|ToInteger(Boolean) (Variables|Default|GetRotation%20clamped%20to%20Displacement)) 1) (.AXIS (Utilities|Struct|BreakF_CSVdata _returnvalue_5))))))) -1.0) (.Z (Math|Vector|BreakVector (* (Variables|Default|GetRandom%20Rotation%20[XYZ]) (Math|Conversions|ToFloat(Boolean) (!= (- (Math|Conversions|ToInteger(Boolean) (Variables|Default|GetRotation%20clamped%20to%20Displacement)) 1) (.AXIS (Utilities|Struct|BreakF_CSVdata _returnvalue_5))))))) _displacement_randomize)) (Variables|Default|GetShuffle)) (Math|Vector|MakeVector (.R_X (Utilities|Struct|BreakF_CSVdata _returnvalue_5)) (.R_Y (Utilities|Struct|BreakF_CSVdata _returnvalue_5)) (.R_Z (Utilities|Struct|BreakF_CSVdata _returnvalue_5)))))) (.Y (Math|Vector|BreakVector (+ (+ (Math|Vector|MakeVector (Math|Random|RandomFloatinRangefromStream (* (.X (Math|Vector|BreakVector (* (Variables|Default|GetRandom%20Rotation%20[XYZ]) (Math|Conversions|ToFloat(Boolean) (!= (- (Math|Conversions|ToInteger(Boolean) (Variables|Default|GetRotation%20clamped%20to%20Displacement)) 1) (.AXIS (Utilities|Struct|BreakF_CSVdata _returnvalue_5))))))) -1.0) (.X (Math|Vector|BreakVector (* (Variables|Default|GetRandom%20Rotation%20[XYZ]) (Math|Conversions|ToFloat(Boolean) (!= (- (Math|Conversions|ToInteger(Boolean) (Variables|Default|GetRotation%20clamped%20to%20Displacement)) 1) (.AXIS (Utilities|Struct|BreakF_CSVdata _returnvalue_5))))))) _displacement_randomize) (Math|Random|RandomFloatinRangefromStream (* (.Y (Math|Vector|BreakVector (* (Variables|Default|GetRandom%20Rotation%20[XYZ]) (Math|Conversions|ToFloat(Boolean) (!= (- (Math|Conversions|ToInteger(Boolean) (Variables|Default|GetRotation%20clamped%20to%20Displacement)) 1) (.AXIS (Utilities|Struct|BreakF_CSVdata _returnvalue_5))))))) -1.0) (.Y (Math|Vector|BreakVector (* (Variables|Default|GetRandom%20Rotation%20[XYZ]) (Math|Conversions|ToFloat(Boolean) (!= (- (Math|Conversions|ToInteger(Boolean) (Variables|Default|GetRotation%20clamped%20to%20Displacement)) 1) (.AXIS (Utilities|Struct|BreakF_CSVdata _returnvalue_5))))))) _displacement_randomize) (Math|Random|RandomFloatinRangefromStream (* (.Z (Math|Vector|BreakVector (* (Variables|Default|GetRandom%20Rotation%20[XYZ]) (Math|Conversions|ToFloat(Boolean) (!= (- (Math|Conversions|ToInteger(Boolean) (Variables|Default|GetRotation%20clamped%20to%20Displacement)) 1) (.AXIS (Utilities|Struct|BreakF_CSVdata _returnvalue_5))))))) -1.0) (.Z (Math|Vector|BreakVector (* (Variables|Default|GetRandom%20Rotation%20[XYZ]) (Math|Conversions|ToFloat(Boolean) (!= (- (Math|Conversions|ToInteger(Boolean) (Variables|Default|GetRotation%20clamped%20to%20Displacement)) 1) (.AXIS (Utilities|Struct|BreakF_CSVdata _returnvalue_5))))))) _displacement_randomize)) (Variables|Default|GetShuffle)) (Math|Vector|MakeVector (.R_X (Utilities|Struct|BreakF_CSVdata _returnvalue_5)) (.R_Y (Utilities|Struct|BreakF_CSVdata _returnvalue_5)) (.R_Z (Utilities|Struct|BreakF_CSVdata _returnvalue_5)))))) (.Z (Math|Vector|BreakVector (+ (+ (Math|Vector|MakeVector (Math|Random|RandomFloatinRangefromStream (* (.X (Math|Vector|BreakVector (* (Variables|Default|GetRandom%20Rotation%20[XYZ]) (Math|Conversions|ToFloat(Boolean) (!= (- (Math|Conversions|ToInteger(Boolean) (Variables|Default|GetRotation%20clamped%20to%20Displacement)) 1) (.AXIS (Utilities|Struct|BreakF_CSVdata _returnvalue_5))))))) -1.0) (.X (Math|Vector|BreakVector (* (Variables|Default|GetRandom%20Rotation%20[XYZ]) (Math|Conversions|ToFloat(Boolean) (!= (- (Math|Conversions|ToInteger(Boolean) (Variables|Default|GetRotation%20clamped%20to%20Displacement)) 1) (.AXIS (Utilities|Struct|BreakF_CSVdata _returnvalue_5))))))) _displacement_randomize) (Math|Random|RandomFloatinRangefromStream (* (.Y (Math|Vector|BreakVector (* (Variables|Default|GetRandom%20Rotation%20[XYZ]) (Math|Conversions|ToFloat(Boolean) (!= (- (Math|Conversions|ToInteger(Boolean) (Variables|Default|GetRotation%20clamped%20to%20Displacement)) 1) (.AXIS (Utilities|Struct|BreakF_CSVdata _returnvalue_5))))))) -1.0) (.Y (Math|Vector|BreakVector (* (Variables|Default|GetRandom%20Rotation%20[XYZ]) (Math|Conversions|ToFloat(Boolean) (!= (- (Math|Conversions|ToInteger(Boolean) (Variables|Default|GetRotation%20clamped%20to%20Displacement)) 1) (.AXIS (Utilities|Struct|BreakF_CSVdata _returnvalue_5))))))) _displacement_randomize) (Math|Random|RandomFloatinRangefromStream (* (.Z (Math|Vector|BreakVector (* (Variables|Default|GetRandom%20Rotation%20[XYZ]) (Math|Conversions|ToFloat(Boolean) (!= (- (Math|Conversions|ToInteger(Boolean) (Variables|Default|GetRotation%20clamped%20to%20Displacement)) 1) (.AXIS (Utilities|Struct|BreakF_CSVdata _returnvalue_5))))))) -1.0) (.Z (Math|Vector|BreakVector (* (Variables|Default|GetRandom%20Rotation%20[XYZ]) (Math|Conversions|ToFloat(Boolean) (!= (- (Math|Conversions|ToInteger(Boolean) (Variables|Default|GetRotation%20clamped%20to%20Displacement)) 1) (.AXIS (Utilities|Struct|BreakF_CSVdata _returnvalue_5))))))) _displacement_randomize)) (Variables|Default|GetShuffle)) (Math|Vector|MakeVector (.R_X (Utilities|Struct|BreakF_CSVdata _returnvalue_5)) (.R_Y (Utilities|Struct|BreakF_CSVdata _returnvalue_5)) (.R_Z (Utilities|Struct|BreakF_CSVdata _returnvalue_5))))))) (Math|Conversions|ToFloat(Boolean) (Variables|Default|GetRandom%20Rotation%20LOCAL/GLOBAL))) (* (Math|Vector|MakeVector (.S_X (Utilities|Struct|BreakF_CSVdata _returnvalue_5)) (.S_Y (Utilities|Struct|BreakF_CSVdata _returnvalue_5)) (.S_Z (Utilities|Struct|BreakF_CSVdata _returnvalue_5))) (Variables|Default|GetScale))) (* (Math|Vector|MakeVector (* (Math|Conversions|ToFloat(Boolean) (== (.AXIS (Utilities|Struct|BreakF_CSVdata _returnvalue_5)) 1)) _returnvalue_3) (* (Math|Conversions|ToFloat(Boolean) (== (.AXIS (Utilities|Struct|BreakF_CSVdata _returnvalue_5)) 2)) _returnvalue_3) (* (Math|Conversions|ToFloat(Boolean) (== (.AXIS (Utilities|Struct|BreakF_CSVdata _returnvalue_5)) 3)) _returnvalue_3)) (Math|Float|Clamp(Float) (+ (Math|Conversions|ToFloat(Boolean) (and (not (Class|KismetMathLibrary|IsPointinBoxwithTransform (Math|Vector|MakeVector (.T_X (Utilities|Struct|BreakF_CSVdata _returnvalue_5)) (.T_Y (Utilities|Struct|BreakF_CSVdata _returnvalue_5)) (.T_Z (Utilities|Struct|BreakF_CSVdata _returnvalue_5))) (Math|Transform|MakeTransform (Variables|Default|GetBox%20Origin%20[XYZ]) (Variables|Default|GetBox%20Rotation%20[XYZ])) (Variables|Default|GetBox%20Extent%20[XYZ]))) _boxcontrolleddisplacement)) (Variables|Default|GetBox%20Intensity)) (Math|Conversions|ToFloat(Boolean) (not _boxcontrolleddisplacement))))) (Math|Rotator|Lerp(Rotator) (Math|Rotator|CombineRotators (Math|Rotator|MakeRotator (.X (Math|Vector|BreakVector (+ (Math|Vector|MakeVector (Math|Random|RandomFloatinRangefromStream (* (.X (Math|Vector|BreakVector (* (Variables|Default|GetRandom%20Rotation%20[XYZ]) (Math|Conversions|ToFloat(Boolean) (!= (- (Math|Conversions|ToInteger(Boolean) (Variables|Default|GetRotation%20clamped%20to%20Displacement)) 1) (.AXIS (Utilities|Struct|BreakF_CSVdata _returnvalue_5))))))) -1.0) (.X (Math|Vector|BreakVector (* (Variables|Default|GetRandom%20Rotation%20[XYZ]) (Math|Conversions|ToFloat(Boolean) (!= (- (Math|Conversions|ToInteger(Boolean) (Variables|Default|GetRotation%20clamped%20to%20Displacement)) 1) (.AXIS (Utilities|Struct|BreakF_CSVdata _returnvalue_5))))))) _displacement_randomize) (Math|Random|RandomFloatinRangefromStream (* (.Y (Math|Vector|BreakVector (* (Variables|Default|GetRandom%20Rotation%20[XYZ]) (Math|Conversions|ToFloat(Boolean) (!= (- (Math|Conversions|ToInteger(Boolean) (Variables|Default|GetRotation%20clamped%20to%20Displacement)) 1) (.AXIS (Utilities|Struct|BreakF_CSVdata _returnvalue_5))))))) -1.0) (.Y (Math|Vector|BreakVector (* (Variables|Default|GetRandom%20Rotation%20[XYZ]) (Math|Conversions|ToFloat(Boolean) (!= (- (Math|Conversions|ToInteger(Boolean) (Variables|Default|GetRotation%20clamped%20to%20Displacement)) 1) (.AXIS (Utilities|Struct|BreakF_CSVdata _returnvalue_5))))))) _displacement_randomize) (Math|Random|RandomFloatinRangefromStream (* (.Z (Math|Vector|BreakVector (* (Variables|Default|GetRandom%20Rotation%20[XYZ]) (Math|Conversions|ToFloat(Boolean) (!= (- (Math|Conversions|ToInteger(Boolean) (Variables|Default|GetRotation%20clamped%20to%20Displacement)) 1) (.AXIS (Utilities|Struct|BreakF_CSVdata _returnvalue_5))))))) -1.0) (.Z (Math|Vector|BreakVector (* (Variables|Default|GetRandom%20Rotation%20[XYZ]) (Math|Conversions|ToFloat(Boolean) (!= (- (Math|Conversions|ToInteger(Boolean) (Variables|Default|GetRotation%20clamped%20to%20Displacement)) 1) (.AXIS (Utilities|Struct|BreakF_CSVdata _returnvalue_5))))))) _displacement_randomize)) (Variables|Default|GetShuffle)))) (.Y (Math|Vector|BreakVector (+ (Math|Vector|MakeVector (Math|Random|RandomFloatinRangefromStream (* (.X (Math|Vector|BreakVector (* (Variables|Default|GetRandom%20Rotation%20[XYZ]) (Math|Conversions|ToFloat(Boolean) (!= (- (Math|Conversions|ToInteger(Boolean) (Variables|Default|GetRotation%20clamped%20to%20Displacement)) 1) (.AXIS (Utilities|Struct|BreakF_CSVdata _returnvalue_5))))))) -1.0) (.X (Math|Vector|BreakVector (* (Variables|Default|GetRandom%20Rotation%20[XYZ]) (Math|Conversions|ToFloat(Boolean) (!= (- (Math|Conversions|ToInteger(Boolean) (Variables|Default|GetRotation%20clamped%20to%20Displacement)) 1) (.AXIS (Utilities|Struct|BreakF_CSVdata _returnvalue_5))))))) _displacement_randomize) (Math|Random|RandomFloatinRangefromStream (* (.Y (Math|Vector|BreakVector (* (Variables|Default|GetRandom%20Rotation%20[XYZ]) (Math|Conversions|ToFloat(Boolean) (!= (- (Math|Conversions|ToInteger(Boolean) (Variables|Default|GetRotation%20clamped%20to%20Displacement)) 1) (.AXIS (Utilities|Struct|BreakF_CSVdata _returnvalue_5))))))) -1.0) (.Y (Math|Vector|BreakVector (* (Variables|Default|GetRandom%20Rotation%20[XYZ]) (Math|Conversions|ToFloat(Boolean) (!= (- (Math|Conversions|ToInteger(Boolean) (Variables|Default|GetRotation%20clamped%20to%20Displacement)) 1) (.AXIS (Utilities|Struct|BreakF_CSVdata _returnvalue_5))))))) _displacement_randomize) (Math|Random|RandomFloatinRangefromStream (* (.Z (Math|Vector|BreakVector (* (Variables|Default|GetRandom%20Rotation%20[XYZ]) (Math|Conversions|ToFloat(Boolean) (!= (- (Math|Conversions|ToInteger(Boolean) (Variables|Default|GetRotation%20clamped%20to%20Displacement)) 1) (.AXIS (Utilities|Struct|BreakF_CSVdata _returnvalue_5))))))) -1.0) (.Z (Math|Vector|BreakVector (* (Variables|Default|GetRandom%20Rotation%20[XYZ]) (Math|Conversions|ToFloat(Boolean) (!= (- (Math|Conversions|ToInteger(Boolean) (Variables|Default|GetRotation%20clamped%20to%20Displacement)) 1) (.AXIS (Utilities|Struct|BreakF_CSVdata _returnvalue_5))))))) _displacement_randomize)) (Variables|Default|GetShuffle)))) (.Z (Math|Vector|BreakVector (+ (Math|Vector|MakeVector (Math|Random|RandomFloatinRangefromStream (* (.X (Math|Vector|BreakVector (* (Variables|Default|GetRandom%20Rotation%20[XYZ]) (Math|Conversions|ToFloat(Boolean) (!= (- (Math|Conversions|ToInteger(Boolean) (Variables|Default|GetRotation%20clamped%20to%20Displacement)) 1) (.AXIS (Utilities|Struct|BreakF_CSVdata _returnvalue_5))))))) -1.0) (.X (Math|Vector|BreakVector (* (Variables|Default|GetRandom%20Rotation%20[XYZ]) (Math|Conversions|ToFloat(Boolean) (!= (- (Math|Conversions|ToInteger(Boolean) (Variables|Default|GetRotation%20clamped%20to%20Displacement)) 1) (.AXIS (Utilities|Struct|BreakF_CSVdata _returnvalue_5))))))) _displacement_randomize) (Math|Random|RandomFloatinRangefromStream (* (.Y (Math|Vector|BreakVector (* (Variables|Default|GetRandom%20Rotation%20[XYZ]) (Math|Conversions|ToFloat(Boolean) (!= (- (Math|Conversions|ToInteger(Boolean) (Variables|Default|GetRotation%20clamped%20to%20Displacement)) 1) (.AXIS (Utilities|Struct|BreakF_CSVdata _returnvalue_5))))))) -1.0) (.Y (Math|Vector|BreakVector (* (Variables|Default|GetRandom%20Rotation%20[XYZ]) (Math|Conversions|ToFloat(Boolean) (!= (- (Math|Conversions|ToInteger(Boolean) (Variables|Default|GetRotation%20clamped%20to%20Displacement)) 1) (.AXIS (Utilities|Struct|BreakF_CSVdata _returnvalue_5))))))) _displacement_randomize) (Math|Random|RandomFloatinRangefromStream (* (.Z (Math|Vector|BreakVector (* (Variables|Default|GetRandom%20Rotation%20[XYZ]) (Math|Conversions|ToFloat(Boolean) (!= (- (Math|Conversions|ToInteger(Boolean) (Variables|Default|GetRotation%20clamped%20to%20Displacement)) 1) (.AXIS (Utilities|Struct|BreakF_CSVdata _returnvalue_5))))))) -1.0) (.Z (Math|Vector|BreakVector (* (Variables|Default|GetRandom%20Rotation%20[XYZ]) (Math|Conversions|ToFloat(Boolean) (!= (- (Math|Conversions|ToInteger(Boolean) (Variables|Default|GetRotation%20clamped%20to%20Displacement)) 1) (.AXIS (Utilities|Struct|BreakF_CSVdata _returnvalue_5))))))) _displacement_randomize)) (Variables|Default|GetShuffle))))) (Math|Rotator|MakeRotator (.R_X (Utilities|Struct|BreakF_CSVdata _returnvalue_5)) (.R_Y (Utilities|Struct|BreakF_CSVdata _returnvalue_5)) (.R_Z (Utilities|Struct|BreakF_CSVdata _returnvalue_5)))) (Math|Rotator|MakeRotator (.X (Math|Vector|BreakVector (+ (+ (Math|Vector|MakeVector (Math|Random|RandomFloatinRangefromStream (* (.X (Math|Vector|BreakVector (* (Variables|Default|GetRandom%20Rotation%20[XYZ]) (Math|Conversions|ToFloat(Boolean) (!= (- (Math|Conversions|ToInteger(Boolean) (Variables|Default|GetRotation%20clamped%20to%20Displacement)) 1) (.AXIS (Utilities|Struct|BreakF_CSVdata _returnvalue_5))))))) -1.0) (.X (Math|Vector|BreakVector (* (Variables|Default|GetRandom%20Rotation%20[XYZ]) (Math|Conversions|ToFloat(Boolean) (!= (- (Math|Conversions|ToInteger(Boolean) (Variables|Default|GetRotation%20clamped%20to%20Displacement)) 1) (.AXIS (Utilities|Struct|BreakF_CSVdata _returnvalue_5))))))) _displacement_randomize) (Math|Random|RandomFloatinRangefromStream (* (.Y (Math|Vector|BreakVector (* (Variables|Default|GetRandom%20Rotation%20[XYZ]) (Math|Conversions|ToFloat(Boolean) (!= (- (Math|Conversions|ToInteger(Boolean) (Variables|Default|GetRotation%20clamped%20to%20Displacement)) 1) (.AXIS (Utilities|Struct|BreakF_CSVdata _returnvalue_5))))))) -1.0) (.Y (Math|Vector|BreakVector (* (Variables|Default|GetRandom%20Rotation%20[XYZ]) (Math|Conversions|ToFloat(Boolean) (!= (- (Math|Conversions|ToInteger(Boolean) (Variables|Default|GetRotation%20clamped%20to%20Displacement)) 1) (.AXIS (Utilities|Struct|BreakF_CSVdata _returnvalue_5))))))) _displacement_randomize) (Math|Random|RandomFloatinRangefromStream (* (.Z (Math|Vector|BreakVector (* (Variables|Default|GetRandom%20Rotation%20[XYZ]) (Math|Conversions|ToFloat(Boolean) (!= (- (Math|Conversions|ToInteger(Boolean) (Variables|Default|GetRotation%20clamped%20to%20Displacement)) 1) (.AXIS (Utilities|Struct|BreakF_CSVdata _returnvalue_5))))))) -1.0) (.Z (Math|Vector|BreakVector (* (Variables|Default|GetRandom%20Rotation%20[XYZ]) (Math|Conversions|ToFloat(Boolean) (!= (- (Math|Conversions|ToInteger(Boolean) (Variables|Default|GetRotation%20clamped%20to%20Displacement)) 1) (.AXIS (Utilities|Struct|BreakF_CSVdata _returnvalue_5))))))) _displacement_randomize)) (Variables|Default|GetShuffle)) (Math|Vector|MakeVector (.R_X (Utilities|Struct|BreakF_CSVdata _returnvalue_5)) (.R_Y (Utilities|Struct|BreakF_CSVdata _returnvalue_5)) (.R_Z (Utilities|Struct|BreakF_CSVdata _returnvalue_5)))))) (.Y (Math|Vector|BreakVector (+ (+ (Math|Vector|MakeVector (Math|Random|RandomFloatinRangefromStream (* (.X (Math|Vector|BreakVector (* (Variables|Default|GetRandom%20Rotation%20[XYZ]) (Math|Conversions|ToFloat(Boolean) (!= (- (Math|Conversions|ToInteger(Boolean) (Variables|Default|GetRotation%20clamped%20to%20Displacement)) 1) (.AXIS (Utilities|Struct|BreakF_CSVdata _returnvalue_5))))))) -1.0) (.X (Math|Vector|BreakVector (* (Variables|Default|GetRandom%20Rotation%20[XYZ]) (Math|Conversions|ToFloat(Boolean) (!= (- (Math|Conversions|ToInteger(Boolean) (Variables|Default|GetRotation%20clamped%20to%20Displacement)) 1) (.AXIS (Utilities|Struct|BreakF_CSVdata _returnvalue_5))))))) _displacement_randomize) (Math|Random|RandomFloatinRangefromStream (* (.Y (Math|Vector|BreakVector (* (Variables|Default|GetRandom%20Rotation%20[XYZ]) (Math|Conversions|ToFloat(Boolean) (!= (- (Math|Conversions|ToInteger(Boolean) (Variables|Default|GetRotation%20clamped%20to%20Displacement)) 1) (.AXIS (Utilities|Struct|BreakF_CSVdata _returnvalue_5))))))) -1.0) (.Y (Math|Vector|BreakVector (* (Variables|Default|GetRandom%20Rotation%20[XYZ]) (Math|Conversions|ToFloat(Boolean) (!= (- (Math|Conversions|ToInteger(Boolean) (Variables|Default|GetRotation%20clamped%20to%20Displacement)) 1) (.AXIS (Utilities|Struct|BreakF_CSVdata _returnvalue_5))))))) _displacement_randomize) (Math|Random|RandomFloatinRangefromStream (* (.Z (Math|Vector|BreakVector (* (Variables|Default|GetRandom%20Rotation%20[XYZ]) (Math|Conversions|ToFloat(Boolean) (!= (- (Math|Conversions|ToInteger(Boolean) (Variables|Default|GetRotation%20clamped%20to%20Displacement)) 1) (.AXIS (Utilities|Struct|BreakF_CSVdata _returnvalue_5))))))) -1.0) (.Z (Math|Vector|BreakVector (* (Variables|Default|GetRandom%20Rotation%20[XYZ]) (Math|Conversions|ToFloat(Boolean) (!= (- (Math|Conversions|ToInteger(Boolean) (Variables|Default|GetRotation%20clamped%20to%20Displacement)) 1) (.AXIS (Utilities|Struct|BreakF_CSVdata _returnvalue_5))))))) _displacement_randomize)) (Variables|Default|GetShuffle)) (Math|Vector|MakeVector (.R_X (Utilities|Struct|BreakF_CSVdata _returnvalue_5)) (.R_Y (Utilities|Struct|BreakF_CSVdata _returnvalue_5)) (.R_Z (Utilities|Struct|BreakF_CSVdata _returnvalue_5)))))) (.Z (Math|Vector|BreakVector (+ (+ (Math|Vector|MakeVector (Math|Random|RandomFloatinRangefromStream (* (.X (Math|Vector|BreakVector (* (Variables|Default|GetRandom%20Rotation%20[XYZ]) (Math|Conversions|ToFloat(Boolean) (!= (- (Math|Conversions|ToInteger(Boolean) (Variables|Default|GetRotation%20clamped%20to%20Displacement)) 1) (.AXIS (Utilities|Struct|BreakF_CSVdata _returnvalue_5))))))) -1.0) (.X (Math|Vector|BreakVector (* (Variables|Default|GetRandom%20Rotation%20[XYZ]) (Math|Conversions|ToFloat(Boolean) (!= (- (Math|Conversions|ToInteger(Boolean) (Variables|Default|GetRotation%20clamped%20to%20Displacement)) 1) (.AXIS (Utilities|Struct|BreakF_CSVdata _returnvalue_5))))))) _displacement_randomize) (Math|Random|RandomFloatinRangefromStream (* (.Y (Math|Vector|BreakVector (* (Variables|Default|GetRandom%20Rotation%20[XYZ]) (Math|Conversions|ToFloat(Boolean) (!= (- (Math|Conversions|ToInteger(Boolean) (Variables|Default|GetRotation%20clamped%20to%20Displacement)) 1) (.AXIS (Utilities|Struct|BreakF_CSVdata _returnvalue_5))))))) -1.0) (.Y (Math|Vector|BreakVector (* (Variables|Default|GetRandom%20Rotation%20[XYZ]) (Math|Conversions|ToFloat(Boolean) (!= (- (Math|Conversions|ToInteger(Boolean) (Variables|Default|GetRotation%20clamped%20to%20Displacement)) 1) (.AXIS (Utilities|Struct|BreakF_CSVdata _returnvalue_5))))))) _displacement_randomize) (Math|Random|RandomFloatinRangefromStream (* (.Z (Math|Vector|BreakVector (* (Variables|Default|GetRandom%20Rotation%20[XYZ]) (Math|Conversions|ToFloat(Boolean) (!= (- (Math|Conversions|ToInteger(Boolean) (Variables|Default|GetRotation%20clamped%20to%20Displacement)) 1) (.AXIS (Utilities|Struct|BreakF_CSVdata _returnvalue_5))))))) -1.0) (.Z (Math|Vector|BreakVector (* (Variables|Default|GetRandom%20Rotation%20[XYZ]) (Math|Conversions|ToFloat(Boolean) (!= (- (Math|Conversions|ToInteger(Boolean) (Variables|Default|GetRotation%20clamped%20to%20Displacement)) 1) (.AXIS (Utilities|Struct|BreakF_CSVdata _returnvalue_5))))))) _displacement_randomize)) (Variables|Default|GetShuffle)) (Math|Vector|MakeVector (.R_X (Utilities|Struct|BreakF_CSVdata _returnvalue_5)) (.R_Y (Utilities|Struct|BreakF_CSVdata _returnvalue_5)) (.R_Z (Utilities|Struct|BreakF_CSVdata _returnvalue_5))))))) (Math|Conversions|ToFloat(Boolean) (Variables|Default|GetRandom%20Rotation%20LOCAL/GLOBAL))) (* (Math|Vector|MakeVector (.S_X (Utilities|Struct|BreakF_CSVdata _returnvalue_5)) (.S_Y (Utilities|Struct|BreakF_CSVdata _returnvalue_5)) (.S_Z (Utilities|Struct|BreakF_CSVdata _returnvalue_5))) (Variables|Default|GetScale))) false))))
                  (:11
                    (if _undamaged_stones_2
                      (goto _label_11)
                      (elif _extrastones_3
                        (Utilities|FlowControl|MultiGate false true (Math|Integer|%(Integer) (Variables|Default|GetShuffleExtraStones) 2) :!label _label_12
                          (:Out%200
                            (Utilities|FlowControl|Sequence :!label _label_13
                              (:then_0
                                (Utilities|FlowControl|DoOnce false
                                  (:Completed
                                    (bind _returnvalue_16 (AddComponent|AddHierarchicalInstancedStaticMeshComponent false))
                                    (bind _output_get_11 (Variables|Default|Set11 _returnvalue_16))
                                    (Rendering|Material|SetMaterial _output_get_11 0 (Variables|Default|GetStone%20Material)))))
                              (:then_1
                                (Components|InstancedStaticMesh|AddInstance (Variables|Default|Get11) (Math|Transform|MakeTransform (Math|Transform|TransformLocation (Math|Transform|MakeTransform (Math|Vector|MakeVector (.T_X (Utilities|Struct|BreakF_CSVdata _returnvalue_5)) (.T_Y (Utilities|Struct|BreakF_CSVdata _returnvalue_5)) (.T_Z (Utilities|Struct|BreakF_CSVdata _returnvalue_5))) (Math|Rotator|Lerp(Rotator) (Math|Rotator|CombineRotators (Math|Rotator|MakeRotator (.X (Math|Vector|BreakVector (+ (Math|Vector|MakeVector (Math|Random|RandomFloatinRangefromStream (* (.X (Math|Vector|BreakVector (* (Variables|Default|GetRandom%20Rotation%20[XYZ]) (Math|Conversions|ToFloat(Boolean) (!= (- (Math|Conversions|ToInteger(Boolean) (Variables|Default|GetRotation%20clamped%20to%20Displacement)) 1) (.AXIS (Utilities|Struct|BreakF_CSVdata _returnvalue_5))))))) -1.0) (.X (Math|Vector|BreakVector (* (Variables|Default|GetRandom%20Rotation%20[XYZ]) (Math|Conversions|ToFloat(Boolean) (!= (- (Math|Conversions|ToInteger(Boolean) (Variables|Default|GetRotation%20clamped%20to%20Displacement)) 1) (.AXIS (Utilities|Struct|BreakF_CSVdata _returnvalue_5))))))) _displacement_randomize) (Math|Random|RandomFloatinRangefromStream (* (.Y (Math|Vector|BreakVector (* (Variables|Default|GetRandom%20Rotation%20[XYZ]) (Math|Conversions|ToFloat(Boolean) (!= (- (Math|Conversions|ToInteger(Boolean) (Variables|Default|GetRotation%20clamped%20to%20Displacement)) 1) (.AXIS (Utilities|Struct|BreakF_CSVdata _returnvalue_5))))))) -1.0) (.Y (Math|Vector|BreakVector (* (Variables|Default|GetRandom%20Rotation%20[XYZ]) (Math|Conversions|ToFloat(Boolean) (!= (- (Math|Conversions|ToInteger(Boolean) (Variables|Default|GetRotation%20clamped%20to%20Displacement)) 1) (.AXIS (Utilities|Struct|BreakF_CSVdata _returnvalue_5))))))) _displacement_randomize) (Math|Random|RandomFloatinRangefromStream (* (.Z (Math|Vector|BreakVector (* (Variables|Default|GetRandom%20Rotation%20[XYZ]) (Math|Conversions|ToFloat(Boolean) (!= (- (Math|Conversions|ToInteger(Boolean) (Variables|Default|GetRotation%20clamped%20to%20Displacement)) 1) (.AXIS (Utilities|Struct|BreakF_CSVdata _returnvalue_5))))))) -1.0) (.Z (Math|Vector|BreakVector (* (Variables|Default|GetRandom%20Rotation%20[XYZ]) (Math|Conversions|ToFloat(Boolean) (!= (- (Math|Conversions|ToInteger(Boolean) (Variables|Default|GetRotation%20clamped%20to%20Displacement)) 1) (.AXIS (Utilities|Struct|BreakF_CSVdata _returnvalue_5))))))) _displacement_randomize)) (Variables|Default|GetShuffle)))) (.Y (Math|Vector|BreakVector (+ (Math|Vector|MakeVector (Math|Random|RandomFloatinRangefromStream (* (.X (Math|Vector|BreakVector (* (Variables|Default|GetRandom%20Rotation%20[XYZ]) (Math|Conversions|ToFloat(Boolean) (!= (- (Math|Conversions|ToInteger(Boolean) (Variables|Default|GetRotation%20clamped%20to%20Displacement)) 1) (.AXIS (Utilities|Struct|BreakF_CSVdata _returnvalue_5))))))) -1.0) (.X (Math|Vector|BreakVector (* (Variables|Default|GetRandom%20Rotation%20[XYZ]) (Math|Conversions|ToFloat(Boolean) (!= (- (Math|Conversions|ToInteger(Boolean) (Variables|Default|GetRotation%20clamped%20to%20Displacement)) 1) (.AXIS (Utilities|Struct|BreakF_CSVdata _returnvalue_5))))))) _displacement_randomize) (Math|Random|RandomFloatinRangefromStream (* (.Y (Math|Vector|BreakVector (* (Variables|Default|GetRandom%20Rotation%20[XYZ]) (Math|Conversions|ToFloat(Boolean) (!= (- (Math|Conversions|ToInteger(Boolean) (Variables|Default|GetRotation%20clamped%20to%20Displacement)) 1) (.AXIS (Utilities|Struct|BreakF_CSVdata _returnvalue_5))))))) -1.0) (.Y (Math|Vector|BreakVector (* (Variables|Default|GetRandom%20Rotation%20[XYZ]) (Math|Conversions|ToFloat(Boolean) (!= (- (Math|Conversions|ToInteger(Boolean) (Variables|Default|GetRotation%20clamped%20to%20Displacement)) 1) (.AXIS (Utilities|Struct|BreakF_CSVdata _returnvalue_5))))))) _displacement_randomize) (Math|Random|RandomFloatinRangefromStream (* (.Z (Math|Vector|BreakVector (* (Variables|Default|GetRandom%20Rotation%20[XYZ]) (Math|Conversions|ToFloat(Boolean) (!= (- (Math|Conversions|ToInteger(Boolean) (Variables|Default|GetRotation%20clamped%20to%20Displacement)) 1) (.AXIS (Utilities|Struct|BreakF_CSVdata _returnvalue_5))))))) -1.0) (.Z (Math|Vector|BreakVector (* (Variables|Default|GetRandom%20Rotation%20[XYZ]) (Math|Conversions|ToFloat(Boolean) (!= (- (Math|Conversions|ToInteger(Boolean) (Variables|Default|GetRotation%20clamped%20to%20Displacement)) 1) (.AXIS (Utilities|Struct|BreakF_CSVdata _returnvalue_5))))))) _displacement_randomize)) (Variables|Default|GetShuffle)))) (.Z (Math|Vector|BreakVector (+ (Math|Vector|MakeVector (Math|Random|RandomFloatinRangefromStream (* (.X (Math|Vector|BreakVector (* (Variables|Default|GetRandom%20Rotation%20[XYZ]) (Math|Conversions|ToFloat(Boolean) (!= (- (Math|Conversions|ToInteger(Boolean) (Variables|Default|GetRotation%20clamped%20to%20Displacement)) 1) (.AXIS (Utilities|Struct|BreakF_CSVdata _returnvalue_5))))))) -1.0) (.X (Math|Vector|BreakVector (* (Variables|Default|GetRandom%20Rotation%20[XYZ]) (Math|Conversions|ToFloat(Boolean) (!= (- (Math|Conversions|ToInteger(Boolean) (Variables|Default|GetRotation%20clamped%20to%20Displacement)) 1) (.AXIS (Utilities|Struct|BreakF_CSVdata _returnvalue_5))))))) _displacement_randomize) (Math|Random|RandomFloatinRangefromStream (* (.Y (Math|Vector|BreakVector (* (Variables|Default|GetRandom%20Rotation%20[XYZ]) (Math|Conversions|ToFloat(Boolean) (!= (- (Math|Conversions|ToInteger(Boolean) (Variables|Default|GetRotation%20clamped%20to%20Displacement)) 1) (.AXIS (Utilities|Struct|BreakF_CSVdata _returnvalue_5))))))) -1.0) (.Y (Math|Vector|BreakVector (* (Variables|Default|GetRandom%20Rotation%20[XYZ]) (Math|Conversions|ToFloat(Boolean) (!= (- (Math|Conversions|ToInteger(Boolean) (Variables|Default|GetRotation%20clamped%20to%20Displacement)) 1) (.AXIS (Utilities|Struct|BreakF_CSVdata _returnvalue_5))))))) _displacement_randomize) (Math|Random|RandomFloatinRangefromStream (* (.Z (Math|Vector|BreakVector (* (Variables|Default|GetRandom%20Rotation%20[XYZ]) (Math|Conversions|ToFloat(Boolean) (!= (- (Math|Conversions|ToInteger(Boolean) (Variables|Default|GetRotation%20clamped%20to%20Displacement)) 1) (.AXIS (Utilities|Struct|BreakF_CSVdata _returnvalue_5))))))) -1.0) (.Z (Math|Vector|BreakVector (* (Variables|Default|GetRandom%20Rotation%20[XYZ]) (Math|Conversions|ToFloat(Boolean) (!= (- (Math|Conversions|ToInteger(Boolean) (Variables|Default|GetRotation%20clamped%20to%20Displacement)) 1) (.AXIS (Utilities|Struct|BreakF_CSVdata _returnvalue_5))))))) _displacement_randomize)) (Variables|Default|GetShuffle))))) (Math|Rotator|MakeRotator (.R_X (Utilities|Struct|BreakF_CSVdata _returnvalue_5)) (.R_Y (Utilities|Struct|BreakF_CSVdata _returnvalue_5)) (.R_Z (Utilities|Struct|BreakF_CSVdata _returnvalue_5)))) (Math|Rotator|MakeRotator (.X (Math|Vector|BreakVector (+ (+ (Math|Vector|MakeVector (Math|Random|RandomFloatinRangefromStream (* (.X (Math|Vector|BreakVector (* (Variables|Default|GetRandom%20Rotation%20[XYZ]) (Math|Conversions|ToFloat(Boolean) (!= (- (Math|Conversions|ToInteger(Boolean) (Variables|Default|GetRotation%20clamped%20to%20Displacement)) 1) (.AXIS (Utilities|Struct|BreakF_CSVdata _returnvalue_5))))))) -1.0) (.X (Math|Vector|BreakVector (* (Variables|Default|GetRandom%20Rotation%20[XYZ]) (Math|Conversions|ToFloat(Boolean) (!= (- (Math|Conversions|ToInteger(Boolean) (Variables|Default|GetRotation%20clamped%20to%20Displacement)) 1) (.AXIS (Utilities|Struct|BreakF_CSVdata _returnvalue_5))))))) _displacement_randomize) (Math|Random|RandomFloatinRangefromStream (* (.Y (Math|Vector|BreakVector (* (Variables|Default|GetRandom%20Rotation%20[XYZ]) (Math|Conversions|ToFloat(Boolean) (!= (- (Math|Conversions|ToInteger(Boolean) (Variables|Default|GetRotation%20clamped%20to%20Displacement)) 1) (.AXIS (Utilities|Struct|BreakF_CSVdata _returnvalue_5))))))) -1.0) (.Y (Math|Vector|BreakVector (* (Variables|Default|GetRandom%20Rotation%20[XYZ]) (Math|Conversions|ToFloat(Boolean) (!= (- (Math|Conversions|ToInteger(Boolean) (Variables|Default|GetRotation%20clamped%20to%20Displacement)) 1) (.AXIS (Utilities|Struct|BreakF_CSVdata _returnvalue_5))))))) _displacement_randomize) (Math|Random|RandomFloatinRangefromStream (* (.Z (Math|Vector|BreakVector (* (Variables|Default|GetRandom%20Rotation%20[XYZ]) (Math|Conversions|ToFloat(Boolean) (!= (- (Math|Conversions|ToInteger(Boolean) (Variables|Default|GetRotation%20clamped%20to%20Displacement)) 1) (.AXIS (Utilities|Struct|BreakF_CSVdata _returnvalue_5))))))) -1.0) (.Z (Math|Vector|BreakVector (* (Variables|Default|GetRandom%20Rotation%20[XYZ]) (Math|Conversions|ToFloat(Boolean) (!= (- (Math|Conversions|ToInteger(Boolean) (Variables|Default|GetRotation%20clamped%20to%20Displacement)) 1) (.AXIS (Utilities|Struct|BreakF_CSVdata _returnvalue_5))))))) _displacement_randomize)) (Variables|Default|GetShuffle)) (Math|Vector|MakeVector (.R_X (Utilities|Struct|BreakF_CSVdata _returnvalue_5)) (.R_Y (Utilities|Struct|BreakF_CSVdata _returnvalue_5)) (.R_Z (Utilities|Struct|BreakF_CSVdata _returnvalue_5)))))) (.Y (Math|Vector|BreakVector (+ (+ (Math|Vector|MakeVector (Math|Random|RandomFloatinRangefromStream (* (.X (Math|Vector|BreakVector (* (Variables|Default|GetRandom%20Rotation%20[XYZ]) (Math|Conversions|ToFloat(Boolean) (!= (- (Math|Conversions|ToInteger(Boolean) (Variables|Default|GetRotation%20clamped%20to%20Displacement)) 1) (.AXIS (Utilities|Struct|BreakF_CSVdata _returnvalue_5))))))) -1.0) (.X (Math|Vector|BreakVector (* (Variables|Default|GetRandom%20Rotation%20[XYZ]) (Math|Conversions|ToFloat(Boolean) (!= (- (Math|Conversions|ToInteger(Boolean) (Variables|Default|GetRotation%20clamped%20to%20Displacement)) 1) (.AXIS (Utilities|Struct|BreakF_CSVdata _returnvalue_5))))))) _displacement_randomize) (Math|Random|RandomFloatinRangefromStream (* (.Y (Math|Vector|BreakVector (* (Variables|Default|GetRandom%20Rotation%20[XYZ]) (Math|Conversions|ToFloat(Boolean) (!= (- (Math|Conversions|ToInteger(Boolean) (Variables|Default|GetRotation%20clamped%20to%20Displacement)) 1) (.AXIS (Utilities|Struct|BreakF_CSVdata _returnvalue_5))))))) -1.0) (.Y (Math|Vector|BreakVector (* (Variables|Default|GetRandom%20Rotation%20[XYZ]) (Math|Conversions|ToFloat(Boolean) (!= (- (Math|Conversions|ToInteger(Boolean) (Variables|Default|GetRotation%20clamped%20to%20Displacement)) 1) (.AXIS (Utilities|Struct|BreakF_CSVdata _returnvalue_5))))))) _displacement_randomize) (Math|Random|RandomFloatinRangefromStream (* (.Z (Math|Vector|BreakVector (* (Variables|Default|GetRandom%20Rotation%20[XYZ]) (Math|Conversions|ToFloat(Boolean) (!= (- (Math|Conversions|ToInteger(Boolean) (Variables|Default|GetRotation%20clamped%20to%20Displacement)) 1) (.AXIS (Utilities|Struct|BreakF_CSVdata _returnvalue_5))))))) -1.0) (.Z (Math|Vector|BreakVector (* (Variables|Default|GetRandom%20Rotation%20[XYZ]) (Math|Conversions|ToFloat(Boolean) (!= (- (Math|Conversions|ToInteger(Boolean) (Variables|Default|GetRotation%20clamped%20to%20Displacement)) 1) (.AXIS (Utilities|Struct|BreakF_CSVdata _returnvalue_5))))))) _displacement_randomize)) (Variables|Default|GetShuffle)) (Math|Vector|MakeVector (.R_X (Utilities|Struct|BreakF_CSVdata _returnvalue_5)) (.R_Y (Utilities|Struct|BreakF_CSVdata _returnvalue_5)) (.R_Z (Utilities|Struct|BreakF_CSVdata _returnvalue_5)))))) (.Z (Math|Vector|BreakVector (+ (+ (Math|Vector|MakeVector (Math|Random|RandomFloatinRangefromStream (* (.X (Math|Vector|BreakVector (* (Variables|Default|GetRandom%20Rotation%20[XYZ]) (Math|Conversions|ToFloat(Boolean) (!= (- (Math|Conversions|ToInteger(Boolean) (Variables|Default|GetRotation%20clamped%20to%20Displacement)) 1) (.AXIS (Utilities|Struct|BreakF_CSVdata _returnvalue_5))))))) -1.0) (.X (Math|Vector|BreakVector (* (Variables|Default|GetRandom%20Rotation%20[XYZ]) (Math|Conversions|ToFloat(Boolean) (!= (- (Math|Conversions|ToInteger(Boolean) (Variables|Default|GetRotation%20clamped%20to%20Displacement)) 1) (.AXIS (Utilities|Struct|BreakF_CSVdata _returnvalue_5))))))) _displacement_randomize) (Math|Random|RandomFloatinRangefromStream (* (.Y (Math|Vector|BreakVector (* (Variables|Default|GetRandom%20Rotation%20[XYZ]) (Math|Conversions|ToFloat(Boolean) (!= (- (Math|Conversions|ToInteger(Boolean) (Variables|Default|GetRotation%20clamped%20to%20Displacement)) 1) (.AXIS (Utilities|Struct|BreakF_CSVdata _returnvalue_5))))))) -1.0) (.Y (Math|Vector|BreakVector (* (Variables|Default|GetRandom%20Rotation%20[XYZ]) (Math|Conversions|ToFloat(Boolean) (!= (- (Math|Conversions|ToInteger(Boolean) (Variables|Default|GetRotation%20clamped%20to%20Displacement)) 1) (.AXIS (Utilities|Struct|BreakF_CSVdata _returnvalue_5))))))) _displacement_randomize) (Math|Random|RandomFloatinRangefromStream (* (.Z (Math|Vector|BreakVector (* (Variables|Default|GetRandom%20Rotation%20[XYZ]) (Math|Conversions|ToFloat(Boolean) (!= (- (Math|Conversions|ToInteger(Boolean) (Variables|Default|GetRotation%20clamped%20to%20Displacement)) 1) (.AXIS (Utilities|Struct|BreakF_CSVdata _returnvalue_5))))))) -1.0) (.Z (Math|Vector|BreakVector (* (Variables|Default|GetRandom%20Rotation%20[XYZ]) (Math|Conversions|ToFloat(Boolean) (!= (- (Math|Conversions|ToInteger(Boolean) (Variables|Default|GetRotation%20clamped%20to%20Displacement)) 1) (.AXIS (Utilities|Struct|BreakF_CSVdata _returnvalue_5))))))) _displacement_randomize)) (Variables|Default|GetShuffle)) (Math|Vector|MakeVector (.R_X (Utilities|Struct|BreakF_CSVdata _returnvalue_5)) (.R_Y (Utilities|Struct|BreakF_CSVdata _returnvalue_5)) (.R_Z (Utilities|Struct|BreakF_CSVdata _returnvalue_5))))))) (Math|Conversions|ToFloat(Boolean) (Variables|Default|GetRandom%20Rotation%20LOCAL/GLOBAL))) (* (Math|Vector|MakeVector (.S_X (Utilities|Struct|BreakF_CSVdata _returnvalue_5)) (.S_Y (Utilities|Struct|BreakF_CSVdata _returnvalue_5)) (.S_Z (Utilities|Struct|BreakF_CSVdata _returnvalue_5))) (Variables|Default|GetScale))) (* (Math|Vector|MakeVector (* (Math|Conversions|ToFloat(Boolean) (== (.AXIS (Utilities|Struct|BreakF_CSVdata _returnvalue_5)) 1)) _returnvalue_3) (* (Math|Conversions|ToFloat(Boolean) (== (.AXIS (Utilities|Struct|BreakF_CSVdata _returnvalue_5)) 2)) _returnvalue_3) (* (Math|Conversions|ToFloat(Boolean) (== (.AXIS (Utilities|Struct|BreakF_CSVdata _returnvalue_5)) 3)) _returnvalue_3)) (Math|Float|Clamp(Float) (+ (Math|Conversions|ToFloat(Boolean) (and (not (Class|KismetMathLibrary|IsPointinBoxwithTransform (Math|Vector|MakeVector (.T_X (Utilities|Struct|BreakF_CSVdata _returnvalue_5)) (.T_Y (Utilities|Struct|BreakF_CSVdata _returnvalue_5)) (.T_Z (Utilities|Struct|BreakF_CSVdata _returnvalue_5))) (Math|Transform|MakeTransform (Variables|Default|GetBox%20Origin%20[XYZ]) (Variables|Default|GetBox%20Rotation%20[XYZ])) (Variables|Default|GetBox%20Extent%20[XYZ]))) _boxcontrolleddisplacement)) (Variables|Default|GetBox%20Intensity)) (Math|Conversions|ToFloat(Boolean) (not _boxcontrolleddisplacement))))) (Math|Rotator|Lerp(Rotator) (Math|Rotator|CombineRotators (Math|Rotator|MakeRotator (.X (Math|Vector|BreakVector (+ (Math|Vector|MakeVector (Math|Random|RandomFloatinRangefromStream (* (.X (Math|Vector|BreakVector (* (Variables|Default|GetRandom%20Rotation%20[XYZ]) (Math|Conversions|ToFloat(Boolean) (!= (- (Math|Conversions|ToInteger(Boolean) (Variables|Default|GetRotation%20clamped%20to%20Displacement)) 1) (.AXIS (Utilities|Struct|BreakF_CSVdata _returnvalue_5))))))) -1.0) (.X (Math|Vector|BreakVector (* (Variables|Default|GetRandom%20Rotation%20[XYZ]) (Math|Conversions|ToFloat(Boolean) (!= (- (Math|Conversions|ToInteger(Boolean) (Variables|Default|GetRotation%20clamped%20to%20Displacement)) 1) (.AXIS (Utilities|Struct|BreakF_CSVdata _returnvalue_5))))))) _displacement_randomize) (Math|Random|RandomFloatinRangefromStream (* (.Y (Math|Vector|BreakVector (* (Variables|Default|GetRandom%20Rotation%20[XYZ]) (Math|Conversions|ToFloat(Boolean) (!= (- (Math|Conversions|ToInteger(Boolean) (Variables|Default|GetRotation%20clamped%20to%20Displacement)) 1) (.AXIS (Utilities|Struct|BreakF_CSVdata _returnvalue_5))))))) -1.0) (.Y (Math|Vector|BreakVector (* (Variables|Default|GetRandom%20Rotation%20[XYZ]) (Math|Conversions|ToFloat(Boolean) (!= (- (Math|Conversions|ToInteger(Boolean) (Variables|Default|GetRotation%20clamped%20to%20Displacement)) 1) (.AXIS (Utilities|Struct|BreakF_CSVdata _returnvalue_5))))))) _displacement_randomize) (Math|Random|RandomFloatinRangefromStream (* (.Z (Math|Vector|BreakVector (* (Variables|Default|GetRandom%20Rotation%20[XYZ]) (Math|Conversions|ToFloat(Boolean) (!= (- (Math|Conversions|ToInteger(Boolean) (Variables|Default|GetRotation%20clamped%20to%20Displacement)) 1) (.AXIS (Utilities|Struct|BreakF_CSVdata _returnvalue_5))))))) -1.0) (.Z (Math|Vector|BreakVector (* (Variables|Default|GetRandom%20Rotation%20[XYZ]) (Math|Conversions|ToFloat(Boolean) (!= (- (Math|Conversions|ToInteger(Boolean) (Variables|Default|GetRotation%20clamped%20to%20Displacement)) 1) (.AXIS (Utilities|Struct|BreakF_CSVdata _returnvalue_5))))))) _displacement_randomize)) (Variables|Default|GetShuffle)))) (.Y (Math|Vector|BreakVector (+ (Math|Vector|MakeVector (Math|Random|RandomFloatinRangefromStream (* (.X (Math|Vector|BreakVector (* (Variables|Default|GetRandom%20Rotation%20[XYZ]) (Math|Conversions|ToFloat(Boolean) (!= (- (Math|Conversions|ToInteger(Boolean) (Variables|Default|GetRotation%20clamped%20to%20Displacement)) 1) (.AXIS (Utilities|Struct|BreakF_CSVdata _returnvalue_5))))))) -1.0) (.X (Math|Vector|BreakVector (* (Variables|Default|GetRandom%20Rotation%20[XYZ]) (Math|Conversions|ToFloat(Boolean) (!= (- (Math|Conversions|ToInteger(Boolean) (Variables|Default|GetRotation%20clamped%20to%20Displacement)) 1) (.AXIS (Utilities|Struct|BreakF_CSVdata _returnvalue_5))))))) _displacement_randomize) (Math|Random|RandomFloatinRangefromStream (* (.Y (Math|Vector|BreakVector (* (Variables|Default|GetRandom%20Rotation%20[XYZ]) (Math|Conversions|ToFloat(Boolean) (!= (- (Math|Conversions|ToInteger(Boolean) (Variables|Default|GetRotation%20clamped%20to%20Displacement)) 1) (.AXIS (Utilities|Struct|BreakF_CSVdata _returnvalue_5))))))) -1.0) (.Y (Math|Vector|BreakVector (* (Variables|Default|GetRandom%20Rotation%20[XYZ]) (Math|Conversions|ToFloat(Boolean) (!= (- (Math|Conversions|ToInteger(Boolean) (Variables|Default|GetRotation%20clamped%20to%20Displacement)) 1) (.AXIS (Utilities|Struct|BreakF_CSVdata _returnvalue_5))))))) _displacement_randomize) (Math|Random|RandomFloatinRangefromStream (* (.Z (Math|Vector|BreakVector (* (Variables|Default|GetRandom%20Rotation%20[XYZ]) (Math|Conversions|ToFloat(Boolean) (!= (- (Math|Conversions|ToInteger(Boolean) (Variables|Default|GetRotation%20clamped%20to%20Displacement)) 1) (.AXIS (Utilities|Struct|BreakF_CSVdata _returnvalue_5))))))) -1.0) (.Z (Math|Vector|BreakVector (* (Variables|Default|GetRandom%20Rotation%20[XYZ]) (Math|Conversions|ToFloat(Boolean) (!= (- (Math|Conversions|ToInteger(Boolean) (Variables|Default|GetRotation%20clamped%20to%20Displacement)) 1) (.AXIS (Utilities|Struct|BreakF_CSVdata _returnvalue_5))))))) _displacement_randomize)) (Variables|Default|GetShuffle)))) (.Z (Math|Vector|BreakVector (+ (Math|Vector|MakeVector (Math|Random|RandomFloatinRangefromStream (* (.X (Math|Vector|BreakVector (* (Variables|Default|GetRandom%20Rotation%20[XYZ]) (Math|Conversions|ToFloat(Boolean) (!= (- (Math|Conversions|ToInteger(Boolean) (Variables|Default|GetRotation%20clamped%20to%20Displacement)) 1) (.AXIS (Utilities|Struct|BreakF_CSVdata _returnvalue_5))))))) -1.0) (.X (Math|Vector|BreakVector (* (Variables|Default|GetRandom%20Rotation%20[XYZ]) (Math|Conversions|ToFloat(Boolean) (!= (- (Math|Conversions|ToInteger(Boolean) (Variables|Default|GetRotation%20clamped%20to%20Displacement)) 1) (.AXIS (Utilities|Struct|BreakF_CSVdata _returnvalue_5))))))) _displacement_randomize) (Math|Random|RandomFloatinRangefromStream (* (.Y (Math|Vector|BreakVector (* (Variables|Default|GetRandom%20Rotation%20[XYZ]) (Math|Conversions|ToFloat(Boolean) (!= (- (Math|Conversions|ToInteger(Boolean) (Variables|Default|GetRotation%20clamped%20to%20Displacement)) 1) (.AXIS (Utilities|Struct|BreakF_CSVdata _returnvalue_5))))))) -1.0) (.Y (Math|Vector|BreakVector (* (Variables|Default|GetRandom%20Rotation%20[XYZ]) (Math|Conversions|ToFloat(Boolean) (!= (- (Math|Conversions|ToInteger(Boolean) (Variables|Default|GetRotation%20clamped%20to%20Displacement)) 1) (.AXIS (Utilities|Struct|BreakF_CSVdata _returnvalue_5))))))) _displacement_randomize) (Math|Random|RandomFloatinRangefromStream (* (.Z (Math|Vector|BreakVector (* (Variables|Default|GetRandom%20Rotation%20[XYZ]) (Math|Conversions|ToFloat(Boolean) (!= (- (Math|Conversions|ToInteger(Boolean) (Variables|Default|GetRotation%20clamped%20to%20Displacement)) 1) (.AXIS (Utilities|Struct|BreakF_CSVdata _returnvalue_5))))))) -1.0) (.Z (Math|Vector|BreakVector (* (Variables|Default|GetRandom%20Rotation%20[XYZ]) (Math|Conversions|ToFloat(Boolean) (!= (- (Math|Conversions|ToInteger(Boolean) (Variables|Default|GetRotation%20clamped%20to%20Displacement)) 1) (.AXIS (Utilities|Struct|BreakF_CSVdata _returnvalue_5))))))) _displacement_randomize)) (Variables|Default|GetShuffle))))) (Math|Rotator|MakeRotator (.R_X (Utilities|Struct|BreakF_CSVdata _returnvalue_5)) (.R_Y (Utilities|Struct|BreakF_CSVdata _returnvalue_5)) (.R_Z (Utilities|Struct|BreakF_CSVdata _returnvalue_5)))) (Math|Rotator|MakeRotator (.X (Math|Vector|BreakVector (+ (+ (Math|Vector|MakeVector (Math|Random|RandomFloatinRangefromStream (* (.X (Math|Vector|BreakVector (* (Variables|Default|GetRandom%20Rotation%20[XYZ]) (Math|Conversions|ToFloat(Boolean) (!= (- (Math|Conversions|ToInteger(Boolean) (Variables|Default|GetRotation%20clamped%20to%20Displacement)) 1) (.AXIS (Utilities|Struct|BreakF_CSVdata _returnvalue_5))))))) -1.0) (.X (Math|Vector|BreakVector (* (Variables|Default|GetRandom%20Rotation%20[XYZ]) (Math|Conversions|ToFloat(Boolean) (!= (- (Math|Conversions|ToInteger(Boolean) (Variables|Default|GetRotation%20clamped%20to%20Displacement)) 1) (.AXIS (Utilities|Struct|BreakF_CSVdata _returnvalue_5))))))) _displacement_randomize) (Math|Random|RandomFloatinRangefromStream (* (.Y (Math|Vector|BreakVector (* (Variables|Default|GetRandom%20Rotation%20[XYZ]) (Math|Conversions|ToFloat(Boolean) (!= (- (Math|Conversions|ToInteger(Boolean) (Variables|Default|GetRotation%20clamped%20to%20Displacement)) 1) (.AXIS (Utilities|Struct|BreakF_CSVdata _returnvalue_5))))))) -1.0) (.Y (Math|Vector|BreakVector (* (Variables|Default|GetRandom%20Rotation%20[XYZ]) (Math|Conversions|ToFloat(Boolean) (!= (- (Math|Conversions|ToInteger(Boolean) (Variables|Default|GetRotation%20clamped%20to%20Displacement)) 1) (.AXIS (Utilities|Struct|BreakF_CSVdata _returnvalue_5))))))) _displacement_randomize) (Math|Random|RandomFloatinRangefromStream (* (.Z (Math|Vector|BreakVector (* (Variables|Default|GetRandom%20Rotation%20[XYZ]) (Math|Conversions|ToFloat(Boolean) (!= (- (Math|Conversions|ToInteger(Boolean) (Variables|Default|GetRotation%20clamped%20to%20Displacement)) 1) (.AXIS (Utilities|Struct|BreakF_CSVdata _returnvalue_5))))))) -1.0) (.Z (Math|Vector|BreakVector (* (Variables|Default|GetRandom%20Rotation%20[XYZ]) (Math|Conversions|ToFloat(Boolean) (!= (- (Math|Conversions|ToInteger(Boolean) (Variables|Default|GetRotation%20clamped%20to%20Displacement)) 1) (.AXIS (Utilities|Struct|BreakF_CSVdata _returnvalue_5))))))) _displacement_randomize)) (Variables|Default|GetShuffle)) (Math|Vector|MakeVector (.R_X (Utilities|Struct|BreakF_CSVdata _returnvalue_5)) (.R_Y (Utilities|Struct|BreakF_CSVdata _returnvalue_5)) (.R_Z (Utilities|Struct|BreakF_CSVdata _returnvalue_5)))))) (.Y (Math|Vector|BreakVector (+ (+ (Math|Vector|MakeVector (Math|Random|RandomFloatinRangefromStream (* (.X (Math|Vector|BreakVector (* (Variables|Default|GetRandom%20Rotation%20[XYZ]) (Math|Conversions|ToFloat(Boolean) (!= (- (Math|Conversions|ToInteger(Boolean) (Variables|Default|GetRotation%20clamped%20to%20Displacement)) 1) (.AXIS (Utilities|Struct|BreakF_CSVdata _returnvalue_5))))))) -1.0) (.X (Math|Vector|BreakVector (* (Variables|Default|GetRandom%20Rotation%20[XYZ]) (Math|Conversions|ToFloat(Boolean) (!= (- (Math|Conversions|ToInteger(Boolean) (Variables|Default|GetRotation%20clamped%20to%20Displacement)) 1) (.AXIS (Utilities|Struct|BreakF_CSVdata _returnvalue_5))))))) _displacement_randomize) (Math|Random|RandomFloatinRangefromStream (* (.Y (Math|Vector|BreakVector (* (Variables|Default|GetRandom%20Rotation%20[XYZ]) (Math|Conversions|ToFloat(Boolean) (!= (- (Math|Conversions|ToInteger(Boolean) (Variables|Default|GetRotation%20clamped%20to%20Displacement)) 1) (.AXIS (Utilities|Struct|BreakF_CSVdata _returnvalue_5))))))) -1.0) (.Y (Math|Vector|BreakVector (* (Variables|Default|GetRandom%20Rotation%20[XYZ]) (Math|Conversions|ToFloat(Boolean) (!= (- (Math|Conversions|ToInteger(Boolean) (Variables|Default|GetRotation%20clamped%20to%20Displacement)) 1) (.AXIS (Utilities|Struct|BreakF_CSVdata _returnvalue_5))))))) _displacement_randomize) (Math|Random|RandomFloatinRangefromStream (* (.Z (Math|Vector|BreakVector (* (Variables|Default|GetRandom%20Rotation%20[XYZ]) (Math|Conversions|ToFloat(Boolean) (!= (- (Math|Conversions|ToInteger(Boolean) (Variables|Default|GetRotation%20clamped%20to%20Displacement)) 1) (.AXIS (Utilities|Struct|BreakF_CSVdata _returnvalue_5))))))) -1.0) (.Z (Math|Vector|BreakVector (* (Variables|Default|GetRandom%20Rotation%20[XYZ]) (Math|Conversions|ToFloat(Boolean) (!= (- (Math|Conversions|ToInteger(Boolean) (Variables|Default|GetRotation%20clamped%20to%20Displacement)) 1) (.AXIS (Utilities|Struct|BreakF_CSVdata _returnvalue_5))))))) _displacement_randomize)) (Variables|Default|GetShuffle)) (Math|Vector|MakeVector (.R_X (Utilities|Struct|BreakF_CSVdata _returnvalue_5)) (.R_Y (Utilities|Struct|BreakF_CSVdata _returnvalue_5)) (.R_Z (Utilities|Struct|BreakF_CSVdata _returnvalue_5)))))) (.Z (Math|Vector|BreakVector (+ (+ (Math|Vector|MakeVector (Math|Random|RandomFloatinRangefromStream (* (.X (Math|Vector|BreakVector (* (Variables|Default|GetRandom%20Rotation%20[XYZ]) (Math|Conversions|ToFloat(Boolean) (!= (- (Math|Conversions|ToInteger(Boolean) (Variables|Default|GetRotation%20clamped%20to%20Displacement)) 1) (.AXIS (Utilities|Struct|BreakF_CSVdata _returnvalue_5))))))) -1.0) (.X (Math|Vector|BreakVector (* (Variables|Default|GetRandom%20Rotation%20[XYZ]) (Math|Conversions|ToFloat(Boolean) (!= (- (Math|Conversions|ToInteger(Boolean) (Variables|Default|GetRotation%20clamped%20to%20Displacement)) 1) (.AXIS (Utilities|Struct|BreakF_CSVdata _returnvalue_5))))))) _displacement_randomize) (Math|Random|RandomFloatinRangefromStream (* (.Y (Math|Vector|BreakVector (* (Variables|Default|GetRandom%20Rotation%20[XYZ]) (Math|Conversions|ToFloat(Boolean) (!= (- (Math|Conversions|ToInteger(Boolean) (Variables|Default|GetRotation%20clamped%20to%20Displacement)) 1) (.AXIS (Utilities|Struct|BreakF_CSVdata _returnvalue_5))))))) -1.0) (.Y (Math|Vector|BreakVector (* (Variables|Default|GetRandom%20Rotation%20[XYZ]) (Math|Conversions|ToFloat(Boolean) (!= (- (Math|Conversions|ToInteger(Boolean) (Variables|Default|GetRotation%20clamped%20to%20Displacement)) 1) (.AXIS (Utilities|Struct|BreakF_CSVdata _returnvalue_5))))))) _displacement_randomize) (Math|Random|RandomFloatinRangefromStream (* (.Z (Math|Vector|BreakVector (* (Variables|Default|GetRandom%20Rotation%20[XYZ]) (Math|Conversions|ToFloat(Boolean) (!= (- (Math|Conversions|ToInteger(Boolean) (Variables|Default|GetRotation%20clamped%20to%20Displacement)) 1) (.AXIS (Utilities|Struct|BreakF_CSVdata _returnvalue_5))))))) -1.0) (.Z (Math|Vector|BreakVector (* (Variables|Default|GetRandom%20Rotation%20[XYZ]) (Math|Conversions|ToFloat(Boolean) (!= (- (Math|Conversions|ToInteger(Boolean) (Variables|Default|GetRotation%20clamped%20to%20Displacement)) 1) (.AXIS (Utilities|Struct|BreakF_CSVdata _returnvalue_5))))))) _displacement_randomize)) (Variables|Default|GetShuffle)) (Math|Vector|MakeVector (.R_X (Utilities|Struct|BreakF_CSVdata _returnvalue_5)) (.R_Y (Utilities|Struct|BreakF_CSVdata _returnvalue_5)) (.R_Z (Utilities|Struct|BreakF_CSVdata _returnvalue_5))))))) (Math|Conversions|ToFloat(Boolean) (Variables|Default|GetRandom%20Rotation%20LOCAL/GLOBAL))) (* (Math|Vector|MakeVector (.S_X (Utilities|Struct|BreakF_CSVdata _returnvalue_5)) (.S_Y (Utilities|Struct|BreakF_CSVdata _returnvalue_5)) (.S_Z (Utilities|Struct|BreakF_CSVdata _returnvalue_5))) (Variables|Default|GetScale))) false))))
                          (:Out%201
                            (Utilities|FlowControl|Sequence :!label _label_14
                              (:then_0
                                (Utilities|FlowControl|DoOnce false
                                  (:Completed
                                    (bind _returnvalue_17 (AddComponent|AddHierarchicalInstancedStaticMeshComponent false))
                                    (bind _output_get_12 (Variables|Default|Set12 _returnvalue_17))
                                    (Rendering|Material|SetMaterial _output_get_12 0 (Variables|Default|GetStone%20Material)))))
                              (:then_1
                                (Components|InstancedStaticMesh|AddInstance (Variables|Default|Get12) (Math|Transform|MakeTransform (Math|Transform|TransformLocation (Math|Transform|MakeTransform (Math|Vector|MakeVector (.T_X (Utilities|Struct|BreakF_CSVdata _returnvalue_5)) (.T_Y (Utilities|Struct|BreakF_CSVdata _returnvalue_5)) (.T_Z (Utilities|Struct|BreakF_CSVdata _returnvalue_5))) (Math|Rotator|Lerp(Rotator) (Math|Rotator|CombineRotators (Math|Rotator|MakeRotator (.X (Math|Vector|BreakVector (+ (Math|Vector|MakeVector (Math|Random|RandomFloatinRangefromStream (* (.X (Math|Vector|BreakVector (* (Variables|Default|GetRandom%20Rotation%20[XYZ]) (Math|Conversions|ToFloat(Boolean) (!= (- (Math|Conversions|ToInteger(Boolean) (Variables|Default|GetRotation%20clamped%20to%20Displacement)) 1) (.AXIS (Utilities|Struct|BreakF_CSVdata _returnvalue_5))))))) -1.0) (.X (Math|Vector|BreakVector (* (Variables|Default|GetRandom%20Rotation%20[XYZ]) (Math|Conversions|ToFloat(Boolean) (!= (- (Math|Conversions|ToInteger(Boolean) (Variables|Default|GetRotation%20clamped%20to%20Displacement)) 1) (.AXIS (Utilities|Struct|BreakF_CSVdata _returnvalue_5))))))) _displacement_randomize) (Math|Random|RandomFloatinRangefromStream (* (.Y (Math|Vector|BreakVector (* (Variables|Default|GetRandom%20Rotation%20[XYZ]) (Math|Conversions|ToFloat(Boolean) (!= (- (Math|Conversions|ToInteger(Boolean) (Variables|Default|GetRotation%20clamped%20to%20Displacement)) 1) (.AXIS (Utilities|Struct|BreakF_CSVdata _returnvalue_5))))))) -1.0) (.Y (Math|Vector|BreakVector (* (Variables|Default|GetRandom%20Rotation%20[XYZ]) (Math|Conversions|ToFloat(Boolean) (!= (- (Math|Conversions|ToInteger(Boolean) (Variables|Default|GetRotation%20clamped%20to%20Displacement)) 1) (.AXIS (Utilities|Struct|BreakF_CSVdata _returnvalue_5))))))) _displacement_randomize) (Math|Random|RandomFloatinRangefromStream (* (.Z (Math|Vector|BreakVector (* (Variables|Default|GetRandom%20Rotation%20[XYZ]) (Math|Conversions|ToFloat(Boolean) (!= (- (Math|Conversions|ToInteger(Boolean) (Variables|Default|GetRotation%20clamped%20to%20Displacement)) 1) (.AXIS (Utilities|Struct|BreakF_CSVdata _returnvalue_5))))))) -1.0) (.Z (Math|Vector|BreakVector (* (Variables|Default|GetRandom%20Rotation%20[XYZ]) (Math|Conversions|ToFloat(Boolean) (!= (- (Math|Conversions|ToInteger(Boolean) (Variables|Default|GetRotation%20clamped%20to%20Displacement)) 1) (.AXIS (Utilities|Struct|BreakF_CSVdata _returnvalue_5))))))) _displacement_randomize)) (Variables|Default|GetShuffle)))) (.Y (Math|Vector|BreakVector (+ (Math|Vector|MakeVector (Math|Random|RandomFloatinRangefromStream (* (.X (Math|Vector|BreakVector (* (Variables|Default|GetRandom%20Rotation%20[XYZ]) (Math|Conversions|ToFloat(Boolean) (!= (- (Math|Conversions|ToInteger(Boolean) (Variables|Default|GetRotation%20clamped%20to%20Displacement)) 1) (.AXIS (Utilities|Struct|BreakF_CSVdata _returnvalue_5))))))) -1.0) (.X (Math|Vector|BreakVector (* (Variables|Default|GetRandom%20Rotation%20[XYZ]) (Math|Conversions|ToFloat(Boolean) (!= (- (Math|Conversions|ToInteger(Boolean) (Variables|Default|GetRotation%20clamped%20to%20Displacement)) 1) (.AXIS (Utilities|Struct|BreakF_CSVdata _returnvalue_5))))))) _displacement_randomize) (Math|Random|RandomFloatinRangefromStream (* (.Y (Math|Vector|BreakVector (* (Variables|Default|GetRandom%20Rotation%20[XYZ]) (Math|Conversions|ToFloat(Boolean) (!= (- (Math|Conversions|ToInteger(Boolean) (Variables|Default|GetRotation%20clamped%20to%20Displacement)) 1) (.AXIS (Utilities|Struct|BreakF_CSVdata _returnvalue_5))))))) -1.0) (.Y (Math|Vector|BreakVector (* (Variables|Default|GetRandom%20Rotation%20[XYZ]) (Math|Conversions|ToFloat(Boolean) (!= (- (Math|Conversions|ToInteger(Boolean) (Variables|Default|GetRotation%20clamped%20to%20Displacement)) 1) (.AXIS (Utilities|Struct|BreakF_CSVdata _returnvalue_5))))))) _displacement_randomize) (Math|Random|RandomFloatinRangefromStream (* (.Z (Math|Vector|BreakVector (* (Variables|Default|GetRandom%20Rotation%20[XYZ]) (Math|Conversions|ToFloat(Boolean) (!= (- (Math|Conversions|ToInteger(Boolean) (Variables|Default|GetRotation%20clamped%20to%20Displacement)) 1) (.AXIS (Utilities|Struct|BreakF_CSVdata _returnvalue_5))))))) -1.0) (.Z (Math|Vector|BreakVector (* (Variables|Default|GetRandom%20Rotation%20[XYZ]) (Math|Conversions|ToFloat(Boolean) (!= (- (Math|Conversions|ToInteger(Boolean) (Variables|Default|GetRotation%20clamped%20to%20Displacement)) 1) (.AXIS (Utilities|Struct|BreakF_CSVdata _returnvalue_5))))))) _displacement_randomize)) (Variables|Default|GetShuffle)))) (.Z (Math|Vector|BreakVector (+ (Math|Vector|MakeVector (Math|Random|RandomFloatinRangefromStream (* (.X (Math|Vector|BreakVector (* (Variables|Default|GetRandom%20Rotation%20[XYZ]) (Math|Conversions|ToFloat(Boolean) (!= (- (Math|Conversions|ToInteger(Boolean) (Variables|Default|GetRotation%20clamped%20to%20Displacement)) 1) (.AXIS (Utilities|Struct|BreakF_CSVdata _returnvalue_5))))))) -1.0) (.X (Math|Vector|BreakVector (* (Variables|Default|GetRandom%20Rotation%20[XYZ]) (Math|Conversions|ToFloat(Boolean) (!= (- (Math|Conversions|ToInteger(Boolean) (Variables|Default|GetRotation%20clamped%20to%20Displacement)) 1) (.AXIS (Utilities|Struct|BreakF_CSVdata _returnvalue_5))))))) _displacement_randomize) (Math|Random|RandomFloatinRangefromStream (* (.Y (Math|Vector|BreakVector (* (Variables|Default|GetRandom%20Rotation%20[XYZ]) (Math|Conversions|ToFloat(Boolean) (!= (- (Math|Conversions|ToInteger(Boolean) (Variables|Default|GetRotation%20clamped%20to%20Displacement)) 1) (.AXIS (Utilities|Struct|BreakF_CSVdata _returnvalue_5))))))) -1.0) (.Y (Math|Vector|BreakVector (* (Variables|Default|GetRandom%20Rotation%20[XYZ]) (Math|Conversions|ToFloat(Boolean) (!= (- (Math|Conversions|ToInteger(Boolean) (Variables|Default|GetRotation%20clamped%20to%20Displacement)) 1) (.AXIS (Utilities|Struct|BreakF_CSVdata _returnvalue_5))))))) _displacement_randomize) (Math|Random|RandomFloatinRangefromStream (* (.Z (Math|Vector|BreakVector (* (Variables|Default|GetRandom%20Rotation%20[XYZ]) (Math|Conversions|ToFloat(Boolean) (!= (- (Math|Conversions|ToInteger(Boolean) (Variables|Default|GetRotation%20clamped%20to%20Displacement)) 1) (.AXIS (Utilities|Struct|BreakF_CSVdata _returnvalue_5))))))) -1.0) (.Z (Math|Vector|BreakVector (* (Variables|Default|GetRandom%20Rotation%20[XYZ]) (Math|Conversions|ToFloat(Boolean) (!= (- (Math|Conversions|ToInteger(Boolean) (Variables|Default|GetRotation%20clamped%20to%20Displacement)) 1) (.AXIS (Utilities|Struct|BreakF_CSVdata _returnvalue_5))))))) _displacement_randomize)) (Variables|Default|GetShuffle))))) (Math|Rotator|MakeRotator (.R_X (Utilities|Struct|BreakF_CSVdata _returnvalue_5)) (.R_Y (Utilities|Struct|BreakF_CSVdata _returnvalue_5)) (.R_Z (Utilities|Struct|BreakF_CSVdata _returnvalue_5)))) (Math|Rotator|MakeRotator (.X (Math|Vector|BreakVector (+ (+ (Math|Vector|MakeVector (Math|Random|RandomFloatinRangefromStream (* (.X (Math|Vector|BreakVector (* (Variables|Default|GetRandom%20Rotation%20[XYZ]) (Math|Conversions|ToFloat(Boolean) (!= (- (Math|Conversions|ToInteger(Boolean) (Variables|Default|GetRotation%20clamped%20to%20Displacement)) 1) (.AXIS (Utilities|Struct|BreakF_CSVdata _returnvalue_5))))))) -1.0) (.X (Math|Vector|BreakVector (* (Variables|Default|GetRandom%20Rotation%20[XYZ]) (Math|Conversions|ToFloat(Boolean) (!= (- (Math|Conversions|ToInteger(Boolean) (Variables|Default|GetRotation%20clamped%20to%20Displacement)) 1) (.AXIS (Utilities|Struct|BreakF_CSVdata _returnvalue_5))))))) _displacement_randomize) (Math|Random|RandomFloatinRangefromStream (* (.Y (Math|Vector|BreakVector (* (Variables|Default|GetRandom%20Rotation%20[XYZ]) (Math|Conversions|ToFloat(Boolean) (!= (- (Math|Conversions|ToInteger(Boolean) (Variables|Default|GetRotation%20clamped%20to%20Displacement)) 1) (.AXIS (Utilities|Struct|BreakF_CSVdata _returnvalue_5))))))) -1.0) (.Y (Math|Vector|BreakVector (* (Variables|Default|GetRandom%20Rotation%20[XYZ]) (Math|Conversions|ToFloat(Boolean) (!= (- (Math|Conversions|ToInteger(Boolean) (Variables|Default|GetRotation%20clamped%20to%20Displacement)) 1) (.AXIS (Utilities|Struct|BreakF_CSVdata _returnvalue_5))))))) _displacement_randomize) (Math|Random|RandomFloatinRangefromStream (* (.Z (Math|Vector|BreakVector (* (Variables|Default|GetRandom%20Rotation%20[XYZ]) (Math|Conversions|ToFloat(Boolean) (!= (- (Math|Conversions|ToInteger(Boolean) (Variables|Default|GetRotation%20clamped%20to%20Displacement)) 1) (.AXIS (Utilities|Struct|BreakF_CSVdata _returnvalue_5))))))) -1.0) (.Z (Math|Vector|BreakVector (* (Variables|Default|GetRandom%20Rotation%20[XYZ]) (Math|Conversions|ToFloat(Boolean) (!= (- (Math|Conversions|ToInteger(Boolean) (Variables|Default|GetRotation%20clamped%20to%20Displacement)) 1) (.AXIS (Utilities|Struct|BreakF_CSVdata _returnvalue_5))))))) _displacement_randomize)) (Variables|Default|GetShuffle)) (Math|Vector|MakeVector (.R_X (Utilities|Struct|BreakF_CSVdata _returnvalue_5)) (.R_Y (Utilities|Struct|BreakF_CSVdata _returnvalue_5)) (.R_Z (Utilities|Struct|BreakF_CSVdata _returnvalue_5)))))) (.Y (Math|Vector|BreakVector (+ (+ (Math|Vector|MakeVector (Math|Random|RandomFloatinRangefromStream (* (.X (Math|Vector|BreakVector (* (Variables|Default|GetRandom%20Rotation%20[XYZ]) (Math|Conversions|ToFloat(Boolean) (!= (- (Math|Conversions|ToInteger(Boolean) (Variables|Default|GetRotation%20clamped%20to%20Displacement)) 1) (.AXIS (Utilities|Struct|BreakF_CSVdata _returnvalue_5))))))) -1.0) (.X (Math|Vector|BreakVector (* (Variables|Default|GetRandom%20Rotation%20[XYZ]) (Math|Conversions|ToFloat(Boolean) (!= (- (Math|Conversions|ToInteger(Boolean) (Variables|Default|GetRotation%20clamped%20to%20Displacement)) 1) (.AXIS (Utilities|Struct|BreakF_CSVdata _returnvalue_5))))))) _displacement_randomize) (Math|Random|RandomFloatinRangefromStream (* (.Y (Math|Vector|BreakVector (* (Variables|Default|GetRandom%20Rotation%20[XYZ]) (Math|Conversions|ToFloat(Boolean) (!= (- (Math|Conversions|ToInteger(Boolean) (Variables|Default|GetRotation%20clamped%20to%20Displacement)) 1) (.AXIS (Utilities|Struct|BreakF_CSVdata _returnvalue_5))))))) -1.0) (.Y (Math|Vector|BreakVector (* (Variables|Default|GetRandom%20Rotation%20[XYZ]) (Math|Conversions|ToFloat(Boolean) (!= (- (Math|Conversions|ToInteger(Boolean) (Variables|Default|GetRotation%20clamped%20to%20Displacement)) 1) (.AXIS (Utilities|Struct|BreakF_CSVdata _returnvalue_5))))))) _displacement_randomize) (Math|Random|RandomFloatinRangefromStream (* (.Z (Math|Vector|BreakVector (* (Variables|Default|GetRandom%20Rotation%20[XYZ]) (Math|Conversions|ToFloat(Boolean) (!= (- (Math|Conversions|ToInteger(Boolean) (Variables|Default|GetRotation%20clamped%20to%20Displacement)) 1) (.AXIS (Utilities|Struct|BreakF_CSVdata _returnvalue_5))))))) -1.0) (.Z (Math|Vector|BreakVector (* (Variables|Default|GetRandom%20Rotation%20[XYZ]) (Math|Conversions|ToFloat(Boolean) (!= (- (Math|Conversions|ToInteger(Boolean) (Variables|Default|GetRotation%20clamped%20to%20Displacement)) 1) (.AXIS (Utilities|Struct|BreakF_CSVdata _returnvalue_5))))))) _displacement_randomize)) (Variables|Default|GetShuffle)) (Math|Vector|MakeVector (.R_X (Utilities|Struct|BreakF_CSVdata _returnvalue_5)) (.R_Y (Utilities|Struct|BreakF_CSVdata _returnvalue_5)) (.R_Z (Utilities|Struct|BreakF_CSVdata _returnvalue_5)))))) (.Z (Math|Vector|BreakVector (+ (+ (Math|Vector|MakeVector (Math|Random|RandomFloatinRangefromStream (* (.X (Math|Vector|BreakVector (* (Variables|Default|GetRandom%20Rotation%20[XYZ]) (Math|Conversions|ToFloat(Boolean) (!= (- (Math|Conversions|ToInteger(Boolean) (Variables|Default|GetRotation%20clamped%20to%20Displacement)) 1) (.AXIS (Utilities|Struct|BreakF_CSVdata _returnvalue_5))))))) -1.0) (.X (Math|Vector|BreakVector (* (Variables|Default|GetRandom%20Rotation%20[XYZ]) (Math|Conversions|ToFloat(Boolean) (!= (- (Math|Conversions|ToInteger(Boolean) (Variables|Default|GetRotation%20clamped%20to%20Displacement)) 1) (.AXIS (Utilities|Struct|BreakF_CSVdata _returnvalue_5))))))) _displacement_randomize) (Math|Random|RandomFloatinRangefromStream (* (.Y (Math|Vector|BreakVector (* (Variables|Default|GetRandom%20Rotation%20[XYZ]) (Math|Conversions|ToFloat(Boolean) (!= (- (Math|Conversions|ToInteger(Boolean) (Variables|Default|GetRotation%20clamped%20to%20Displacement)) 1) (.AXIS (Utilities|Struct|BreakF_CSVdata _returnvalue_5))))))) -1.0) (.Y (Math|Vector|BreakVector (* (Variables|Default|GetRandom%20Rotation%20[XYZ]) (Math|Conversions|ToFloat(Boolean) (!= (- (Math|Conversions|ToInteger(Boolean) (Variables|Default|GetRotation%20clamped%20to%20Displacement)) 1) (.AXIS (Utilities|Struct|BreakF_CSVdata _returnvalue_5))))))) _displacement_randomize) (Math|Random|RandomFloatinRangefromStream (* (.Z (Math|Vector|BreakVector (* (Variables|Default|GetRandom%20Rotation%20[XYZ]) (Math|Conversions|ToFloat(Boolean) (!= (- (Math|Conversions|ToInteger(Boolean) (Variables|Default|GetRotation%20clamped%20to%20Displacement)) 1) (.AXIS (Utilities|Struct|BreakF_CSVdata _returnvalue_5))))))) -1.0) (.Z (Math|Vector|BreakVector (* (Variables|Default|GetRandom%20Rotation%20[XYZ]) (Math|Conversions|ToFloat(Boolean) (!= (- (Math|Conversions|ToInteger(Boolean) (Variables|Default|GetRotation%20clamped%20to%20Displacement)) 1) (.AXIS (Utilities|Struct|BreakF_CSVdata _returnvalue_5))))))) _displacement_randomize)) (Variables|Default|GetShuffle)) (Math|Vector|MakeVector (.R_X (Utilities|Struct|BreakF_CSVdata _returnvalue_5)) (.R_Y (Utilities|Struct|BreakF_CSVdata _returnvalue_5)) (.R_Z (Utilities|Struct|BreakF_CSVdata _returnvalue_5))))))) (Math|Conversions|ToFloat(Boolean) (Variables|Default|GetRandom%20Rotation%20LOCAL/GLOBAL))) (* (Math|Vector|MakeVector (.S_X (Utilities|Struct|BreakF_CSVdata _returnvalue_5)) (.S_Y (Utilities|Struct|BreakF_CSVdata _returnvalue_5)) (.S_Z (Utilities|Struct|BreakF_CSVdata _returnvalue_5))) (Variables|Default|GetScale))) (* (Math|Vector|MakeVector (* (Math|Conversions|ToFloat(Boolean) (== (.AXIS (Utilities|Struct|BreakF_CSVdata _returnvalue_5)) 1)) _returnvalue_3) (* (Math|Conversions|ToFloat(Boolean) (== (.AXIS (Utilities|Struct|BreakF_CSVdata _returnvalue_5)) 2)) _returnvalue_3) (* (Math|Conversions|ToFloat(Boolean) (== (.AXIS (Utilities|Struct|BreakF_CSVdata _returnvalue_5)) 3)) _returnvalue_3)) (Math|Float|Clamp(Float) (+ (Math|Conversions|ToFloat(Boolean) (and (not (Class|KismetMathLibrary|IsPointinBoxwithTransform (Math|Vector|MakeVector (.T_X (Utilities|Struct|BreakF_CSVdata _returnvalue_5)) (.T_Y (Utilities|Struct|BreakF_CSVdata _returnvalue_5)) (.T_Z (Utilities|Struct|BreakF_CSVdata _returnvalue_5))) (Math|Transform|MakeTransform (Variables|Default|GetBox%20Origin%20[XYZ]) (Variables|Default|GetBox%20Rotation%20[XYZ])) (Variables|Default|GetBox%20Extent%20[XYZ]))) _boxcontrolleddisplacement)) (Variables|Default|GetBox%20Intensity)) (Math|Conversions|ToFloat(Boolean) (not _boxcontrolleddisplacement))))) (Math|Rotator|Lerp(Rotator) (Math|Rotator|CombineRotators (Math|Rotator|MakeRotator (.X (Math|Vector|BreakVector (+ (Math|Vector|MakeVector (Math|Random|RandomFloatinRangefromStream (* (.X (Math|Vector|BreakVector (* (Variables|Default|GetRandom%20Rotation%20[XYZ]) (Math|Conversions|ToFloat(Boolean) (!= (- (Math|Conversions|ToInteger(Boolean) (Variables|Default|GetRotation%20clamped%20to%20Displacement)) 1) (.AXIS (Utilities|Struct|BreakF_CSVdata _returnvalue_5))))))) -1.0) (.X (Math|Vector|BreakVector (* (Variables|Default|GetRandom%20Rotation%20[XYZ]) (Math|Conversions|ToFloat(Boolean) (!= (- (Math|Conversions|ToInteger(Boolean) (Variables|Default|GetRotation%20clamped%20to%20Displacement)) 1) (.AXIS (Utilities|Struct|BreakF_CSVdata _returnvalue_5))))))) _displacement_randomize) (Math|Random|RandomFloatinRangefromStream (* (.Y (Math|Vector|BreakVector (* (Variables|Default|GetRandom%20Rotation%20[XYZ]) (Math|Conversions|ToFloat(Boolean) (!= (- (Math|Conversions|ToInteger(Boolean) (Variables|Default|GetRotation%20clamped%20to%20Displacement)) 1) (.AXIS (Utilities|Struct|BreakF_CSVdata _returnvalue_5))))))) -1.0) (.Y (Math|Vector|BreakVector (* (Variables|Default|GetRandom%20Rotation%20[XYZ]) (Math|Conversions|ToFloat(Boolean) (!= (- (Math|Conversions|ToInteger(Boolean) (Variables|Default|GetRotation%20clamped%20to%20Displacement)) 1) (.AXIS (Utilities|Struct|BreakF_CSVdata _returnvalue_5))))))) _displacement_randomize) (Math|Random|RandomFloatinRangefromStream (* (.Z (Math|Vector|BreakVector (* (Variables|Default|GetRandom%20Rotation%20[XYZ]) (Math|Conversions|ToFloat(Boolean) (!= (- (Math|Conversions|ToInteger(Boolean) (Variables|Default|GetRotation%20clamped%20to%20Displacement)) 1) (.AXIS (Utilities|Struct|BreakF_CSVdata _returnvalue_5))))))) -1.0) (.Z (Math|Vector|BreakVector (* (Variables|Default|GetRandom%20Rotation%20[XYZ]) (Math|Conversions|ToFloat(Boolean) (!= (- (Math|Conversions|ToInteger(Boolean) (Variables|Default|GetRotation%20clamped%20to%20Displacement)) 1) (.AXIS (Utilities|Struct|BreakF_CSVdata _returnvalue_5))))))) _displacement_randomize)) (Variables|Default|GetShuffle)))) (.Y (Math|Vector|BreakVector (+ (Math|Vector|MakeVector (Math|Random|RandomFloatinRangefromStream (* (.X (Math|Vector|BreakVector (* (Variables|Default|GetRandom%20Rotation%20[XYZ]) (Math|Conversions|ToFloat(Boolean) (!= (- (Math|Conversions|ToInteger(Boolean) (Variables|Default|GetRotation%20clamped%20to%20Displacement)) 1) (.AXIS (Utilities|Struct|BreakF_CSVdata _returnvalue_5))))))) -1.0) (.X (Math|Vector|BreakVector (* (Variables|Default|GetRandom%20Rotation%20[XYZ]) (Math|Conversions|ToFloat(Boolean) (!= (- (Math|Conversions|ToInteger(Boolean) (Variables|Default|GetRotation%20clamped%20to%20Displacement)) 1) (.AXIS (Utilities|Struct|BreakF_CSVdata _returnvalue_5))))))) _displacement_randomize) (Math|Random|RandomFloatinRangefromStream (* (.Y (Math|Vector|BreakVector (* (Variables|Default|GetRandom%20Rotation%20[XYZ]) (Math|Conversions|ToFloat(Boolean) (!= (- (Math|Conversions|ToInteger(Boolean) (Variables|Default|GetRotation%20clamped%20to%20Displacement)) 1) (.AXIS (Utilities|Struct|BreakF_CSVdata _returnvalue_5))))))) -1.0) (.Y (Math|Vector|BreakVector (* (Variables|Default|GetRandom%20Rotation%20[XYZ]) (Math|Conversions|ToFloat(Boolean) (!= (- (Math|Conversions|ToInteger(Boolean) (Variables|Default|GetRotation%20clamped%20to%20Displacement)) 1) (.AXIS (Utilities|Struct|BreakF_CSVdata _returnvalue_5))))))) _displacement_randomize) (Math|Random|RandomFloatinRangefromStream (* (.Z (Math|Vector|BreakVector (* (Variables|Default|GetRandom%20Rotation%20[XYZ]) (Math|Conversions|ToFloat(Boolean) (!= (- (Math|Conversions|ToInteger(Boolean) (Variables|Default|GetRotation%20clamped%20to%20Displacement)) 1) (.AXIS (Utilities|Struct|BreakF_CSVdata _returnvalue_5))))))) -1.0) (.Z (Math|Vector|BreakVector (* (Variables|Default|GetRandom%20Rotation%20[XYZ]) (Math|Conversions|ToFloat(Boolean) (!= (- (Math|Conversions|ToInteger(Boolean) (Variables|Default|GetRotation%20clamped%20to%20Displacement)) 1) (.AXIS (Utilities|Struct|BreakF_CSVdata _returnvalue_5))))))) _displacement_randomize)) (Variables|Default|GetShuffle)))) (.Z (Math|Vector|BreakVector (+ (Math|Vector|MakeVector (Math|Random|RandomFloatinRangefromStream (* (.X (Math|Vector|BreakVector (* (Variables|Default|GetRandom%20Rotation%20[XYZ]) (Math|Conversions|ToFloat(Boolean) (!= (- (Math|Conversions|ToInteger(Boolean) (Variables|Default|GetRotation%20clamped%20to%20Displacement)) 1) (.AXIS (Utilities|Struct|BreakF_CSVdata _returnvalue_5))))))) -1.0) (.X (Math|Vector|BreakVector (* (Variables|Default|GetRandom%20Rotation%20[XYZ]) (Math|Conversions|ToFloat(Boolean) (!= (- (Math|Conversions|ToInteger(Boolean) (Variables|Default|GetRotation%20clamped%20to%20Displacement)) 1) (.AXIS (Utilities|Struct|BreakF_CSVdata _returnvalue_5))))))) _displacement_randomize) (Math|Random|RandomFloatinRangefromStream (* (.Y (Math|Vector|BreakVector (* (Variables|Default|GetRandom%20Rotation%20[XYZ]) (Math|Conversions|ToFloat(Boolean) (!= (- (Math|Conversions|ToInteger(Boolean) (Variables|Default|GetRotation%20clamped%20to%20Displacement)) 1) (.AXIS (Utilities|Struct|BreakF_CSVdata _returnvalue_5))))))) -1.0) (.Y (Math|Vector|BreakVector (* (Variables|Default|GetRandom%20Rotation%20[XYZ]) (Math|Conversions|ToFloat(Boolean) (!= (- (Math|Conversions|ToInteger(Boolean) (Variables|Default|GetRotation%20clamped%20to%20Displacement)) 1) (.AXIS (Utilities|Struct|BreakF_CSVdata _returnvalue_5))))))) _displacement_randomize) (Math|Random|RandomFloatinRangefromStream (* (.Z (Math|Vector|BreakVector (* (Variables|Default|GetRandom%20Rotation%20[XYZ]) (Math|Conversions|ToFloat(Boolean) (!= (- (Math|Conversions|ToInteger(Boolean) (Variables|Default|GetRotation%20clamped%20to%20Displacement)) 1) (.AXIS (Utilities|Struct|BreakF_CSVdata _returnvalue_5))))))) -1.0) (.Z (Math|Vector|BreakVector (* (Variables|Default|GetRandom%20Rotation%20[XYZ]) (Math|Conversions|ToFloat(Boolean) (!= (- (Math|Conversions|ToInteger(Boolean) (Variables|Default|GetRotation%20clamped%20to%20Displacement)) 1) (.AXIS (Utilities|Struct|BreakF_CSVdata _returnvalue_5))))))) _displacement_randomize)) (Variables|Default|GetShuffle))))) (Math|Rotator|MakeRotator (.R_X (Utilities|Struct|BreakF_CSVdata _returnvalue_5)) (.R_Y (Utilities|Struct|BreakF_CSVdata _returnvalue_5)) (.R_Z (Utilities|Struct|BreakF_CSVdata _returnvalue_5)))) (Math|Rotator|MakeRotator (.X (Math|Vector|BreakVector (+ (+ (Math|Vector|MakeVector (Math|Random|RandomFloatinRangefromStream (* (.X (Math|Vector|BreakVector (* (Variables|Default|GetRandom%20Rotation%20[XYZ]) (Math|Conversions|ToFloat(Boolean) (!= (- (Math|Conversions|ToInteger(Boolean) (Variables|Default|GetRotation%20clamped%20to%20Displacement)) 1) (.AXIS (Utilities|Struct|BreakF_CSVdata _returnvalue_5))))))) -1.0) (.X (Math|Vector|BreakVector (* (Variables|Default|GetRandom%20Rotation%20[XYZ]) (Math|Conversions|ToFloat(Boolean) (!= (- (Math|Conversions|ToInteger(Boolean) (Variables|Default|GetRotation%20clamped%20to%20Displacement)) 1) (.AXIS (Utilities|Struct|BreakF_CSVdata _returnvalue_5))))))) _displacement_randomize) (Math|Random|RandomFloatinRangefromStream (* (.Y (Math|Vector|BreakVector (* (Variables|Default|GetRandom%20Rotation%20[XYZ]) (Math|Conversions|ToFloat(Boolean) (!= (- (Math|Conversions|ToInteger(Boolean) (Variables|Default|GetRotation%20clamped%20to%20Displacement)) 1) (.AXIS (Utilities|Struct|BreakF_CSVdata _returnvalue_5))))))) -1.0) (.Y (Math|Vector|BreakVector (* (Variables|Default|GetRandom%20Rotation%20[XYZ]) (Math|Conversions|ToFloat(Boolean) (!= (- (Math|Conversions|ToInteger(Boolean) (Variables|Default|GetRotation%20clamped%20to%20Displacement)) 1) (.AXIS (Utilities|Struct|BreakF_CSVdata _returnvalue_5))))))) _displacement_randomize) (Math|Random|RandomFloatinRangefromStream (* (.Z (Math|Vector|BreakVector (* (Variables|Default|GetRandom%20Rotation%20[XYZ]) (Math|Conversions|ToFloat(Boolean) (!= (- (Math|Conversions|ToInteger(Boolean) (Variables|Default|GetRotation%20clamped%20to%20Displacement)) 1) (.AXIS (Utilities|Struct|BreakF_CSVdata _returnvalue_5))))))) -1.0) (.Z (Math|Vector|BreakVector (* (Variables|Default|GetRandom%20Rotation%20[XYZ]) (Math|Conversions|ToFloat(Boolean) (!= (- (Math|Conversions|ToInteger(Boolean) (Variables|Default|GetRotation%20clamped%20to%20Displacement)) 1) (.AXIS (Utilities|Struct|BreakF_CSVdata _returnvalue_5))))))) _displacement_randomize)) (Variables|Default|GetShuffle)) (Math|Vector|MakeVector (.R_X (Utilities|Struct|BreakF_CSVdata _returnvalue_5)) (.R_Y (Utilities|Struct|BreakF_CSVdata _returnvalue_5)) (.R_Z (Utilities|Struct|BreakF_CSVdata _returnvalue_5)))))) (.Y (Math|Vector|BreakVector (+ (+ (Math|Vector|MakeVector (Math|Random|RandomFloatinRangefromStream (* (.X (Math|Vector|BreakVector (* (Variables|Default|GetRandom%20Rotation%20[XYZ]) (Math|Conversions|ToFloat(Boolean) (!= (- (Math|Conversions|ToInteger(Boolean) (Variables|Default|GetRotation%20clamped%20to%20Displacement)) 1) (.AXIS (Utilities|Struct|BreakF_CSVdata _returnvalue_5))))))) -1.0) (.X (Math|Vector|BreakVector (* (Variables|Default|GetRandom%20Rotation%20[XYZ]) (Math|Conversions|ToFloat(Boolean) (!= (- (Math|Conversions|ToInteger(Boolean) (Variables|Default|GetRotation%20clamped%20to%20Displacement)) 1) (.AXIS (Utilities|Struct|BreakF_CSVdata _returnvalue_5))))))) _displacement_randomize) (Math|Random|RandomFloatinRangefromStream (* (.Y (Math|Vector|BreakVector (* (Variables|Default|GetRandom%20Rotation%20[XYZ]) (Math|Conversions|ToFloat(Boolean) (!= (- (Math|Conversions|ToInteger(Boolean) (Variables|Default|GetRotation%20clamped%20to%20Displacement)) 1) (.AXIS (Utilities|Struct|BreakF_CSVdata _returnvalue_5))))))) -1.0) (.Y (Math|Vector|BreakVector (* (Variables|Default|GetRandom%20Rotation%20[XYZ]) (Math|Conversions|ToFloat(Boolean) (!= (- (Math|Conversions|ToInteger(Boolean) (Variables|Default|GetRotation%20clamped%20to%20Displacement)) 1) (.AXIS (Utilities|Struct|BreakF_CSVdata _returnvalue_5))))))) _displacement_randomize) (Math|Random|RandomFloatinRangefromStream (* (.Z (Math|Vector|BreakVector (* (Variables|Default|GetRandom%20Rotation%20[XYZ]) (Math|Conversions|ToFloat(Boolean) (!= (- (Math|Conversions|ToInteger(Boolean) (Variables|Default|GetRotation%20clamped%20to%20Displacement)) 1) (.AXIS (Utilities|Struct|BreakF_CSVdata _returnvalue_5))))))) -1.0) (.Z (Math|Vector|BreakVector (* (Variables|Default|GetRandom%20Rotation%20[XYZ]) (Math|Conversions|ToFloat(Boolean) (!= (- (Math|Conversions|ToInteger(Boolean) (Variables|Default|GetRotation%20clamped%20to%20Displacement)) 1) (.AXIS (Utilities|Struct|BreakF_CSVdata _returnvalue_5))))))) _displacement_randomize)) (Variables|Default|GetShuffle)) (Math|Vector|MakeVector (.R_X (Utilities|Struct|BreakF_CSVdata _returnvalue_5)) (.R_Y (Utilities|Struct|BreakF_CSVdata _returnvalue_5)) (.R_Z (Utilities|Struct|BreakF_CSVdata _returnvalue_5)))))) (.Z (Math|Vector|BreakVector (+ (+ (Math|Vector|MakeVector (Math|Random|RandomFloatinRangefromStream (* (.X (Math|Vector|BreakVector (* (Variables|Default|GetRandom%20Rotation%20[XYZ]) (Math|Conversions|ToFloat(Boolean) (!= (- (Math|Conversions|ToInteger(Boolean) (Variables|Default|GetRotation%20clamped%20to%20Displacement)) 1) (.AXIS (Utilities|Struct|BreakF_CSVdata _returnvalue_5))))))) -1.0) (.X (Math|Vector|BreakVector (* (Variables|Default|GetRandom%20Rotation%20[XYZ]) (Math|Conversions|ToFloat(Boolean) (!= (- (Math|Conversions|ToInteger(Boolean) (Variables|Default|GetRotation%20clamped%20to%20Displacement)) 1) (.AXIS (Utilities|Struct|BreakF_CSVdata _returnvalue_5))))))) _displacement_randomize) (Math|Random|RandomFloatinRangefromStream (* (.Y (Math|Vector|BreakVector (* (Variables|Default|GetRandom%20Rotation%20[XYZ]) (Math|Conversions|ToFloat(Boolean) (!= (- (Math|Conversions|ToInteger(Boolean) (Variables|Default|GetRotation%20clamped%20to%20Displacement)) 1) (.AXIS (Utilities|Struct|BreakF_CSVdata _returnvalue_5))))))) -1.0) (.Y (Math|Vector|BreakVector (* (Variables|Default|GetRandom%20Rotation%20[XYZ]) (Math|Conversions|ToFloat(Boolean) (!= (- (Math|Conversions|ToInteger(Boolean) (Variables|Default|GetRotation%20clamped%20to%20Displacement)) 1) (.AXIS (Utilities|Struct|BreakF_CSVdata _returnvalue_5))))))) _displacement_randomize) (Math|Random|RandomFloatinRangefromStream (* (.Z (Math|Vector|BreakVector (* (Variables|Default|GetRandom%20Rotation%20[XYZ]) (Math|Conversions|ToFloat(Boolean) (!= (- (Math|Conversions|ToInteger(Boolean) (Variables|Default|GetRotation%20clamped%20to%20Displacement)) 1) (.AXIS (Utilities|Struct|BreakF_CSVdata _returnvalue_5))))))) -1.0) (.Z (Math|Vector|BreakVector (* (Variables|Default|GetRandom%20Rotation%20[XYZ]) (Math|Conversions|ToFloat(Boolean) (!= (- (Math|Conversions|ToInteger(Boolean) (Variables|Default|GetRotation%20clamped%20to%20Displacement)) 1) (.AXIS (Utilities|Struct|BreakF_CSVdata _returnvalue_5))))))) _displacement_randomize)) (Variables|Default|GetShuffle)) (Math|Vector|MakeVector (.R_X (Utilities|Struct|BreakF_CSVdata _returnvalue_5)) (.R_Y (Utilities|Struct|BreakF_CSVdata _returnvalue_5)) (.R_Z (Utilities|Struct|BreakF_CSVdata _returnvalue_5))))))) (Math|Conversions|ToFloat(Boolean) (Variables|Default|GetRandom%20Rotation%20LOCAL/GLOBAL))) (* (Math|Vector|MakeVector (.S_X (Utilities|Struct|BreakF_CSVdata _returnvalue_5)) (.S_Y (Utilities|Struct|BreakF_CSVdata _returnvalue_5)) (.S_Z (Utilities|Struct|BreakF_CSVdata _returnvalue_5))) (Variables|Default|GetScale))) false)))))
                        (else
                          (goto _label_13)))))
                  (:12
                    (if _undamaged_stones_2
                      (goto _label_11)
                      (elif _extrastones_3
                        (goto _label_12)
                        (else
                          (goto _label_14)))))
                  (:13
                    (Utilities|FlowControl|Sequence :!label _label_15
                      (:then_0
                        (Utilities|FlowControl|DoOnce false
                          (:Completed
                            (bind _returnvalue_18 (AddComponent|AddHierarchicalInstancedStaticMeshComponent false))
                            (bind _output_get_13 (Variables|Default|Set13 _returnvalue_18))
                            (Rendering|Material|SetMaterial _output_get_13 0 (Variables|Default|GetStone%20Material)))))
                      (:then_1
                        (Components|InstancedStaticMesh|AddInstance (Variables|Default|Get13) (Math|Transform|MakeTransform (Math|Transform|TransformLocation (Math|Transform|MakeTransform (Math|Vector|MakeVector (.T_X (Utilities|Struct|BreakF_CSVdata _returnvalue_5)) (.T_Y (Utilities|Struct|BreakF_CSVdata _returnvalue_5)) (.T_Z (Utilities|Struct|BreakF_CSVdata _returnvalue_5))) (Math|Rotator|Lerp(Rotator) (Math|Rotator|CombineRotators (Math|Rotator|MakeRotator (.X (Math|Vector|BreakVector (+ (Math|Vector|MakeVector (Math|Random|RandomFloatinRangefromStream (* (.X (Math|Vector|BreakVector (* (Variables|Default|GetRandom%20Rotation%20[XYZ]) (Math|Conversions|ToFloat(Boolean) (!= (- (Math|Conversions|ToInteger(Boolean) (Variables|Default|GetRotation%20clamped%20to%20Displacement)) 1) (.AXIS (Utilities|Struct|BreakF_CSVdata _returnvalue_5))))))) -1.0) (.X (Math|Vector|BreakVector (* (Variables|Default|GetRandom%20Rotation%20[XYZ]) (Math|Conversions|ToFloat(Boolean) (!= (- (Math|Conversions|ToInteger(Boolean) (Variables|Default|GetRotation%20clamped%20to%20Displacement)) 1) (.AXIS (Utilities|Struct|BreakF_CSVdata _returnvalue_5))))))) _displacement_randomize) (Math|Random|RandomFloatinRangefromStream (* (.Y (Math|Vector|BreakVector (* (Variables|Default|GetRandom%20Rotation%20[XYZ]) (Math|Conversions|ToFloat(Boolean) (!= (- (Math|Conversions|ToInteger(Boolean) (Variables|Default|GetRotation%20clamped%20to%20Displacement)) 1) (.AXIS (Utilities|Struct|BreakF_CSVdata _returnvalue_5))))))) -1.0) (.Y (Math|Vector|BreakVector (* (Variables|Default|GetRandom%20Rotation%20[XYZ]) (Math|Conversions|ToFloat(Boolean) (!= (- (Math|Conversions|ToInteger(Boolean) (Variables|Default|GetRotation%20clamped%20to%20Displacement)) 1) (.AXIS (Utilities|Struct|BreakF_CSVdata _returnvalue_5))))))) _displacement_randomize) (Math|Random|RandomFloatinRangefromStream (* (.Z (Math|Vector|BreakVector (* (Variables|Default|GetRandom%20Rotation%20[XYZ]) (Math|Conversions|ToFloat(Boolean) (!= (- (Math|Conversions|ToInteger(Boolean) (Variables|Default|GetRotation%20clamped%20to%20Displacement)) 1) (.AXIS (Utilities|Struct|BreakF_CSVdata _returnvalue_5))))))) -1.0) (.Z (Math|Vector|BreakVector (* (Variables|Default|GetRandom%20Rotation%20[XYZ]) (Math|Conversions|ToFloat(Boolean) (!= (- (Math|Conversions|ToInteger(Boolean) (Variables|Default|GetRotation%20clamped%20to%20Displacement)) 1) (.AXIS (Utilities|Struct|BreakF_CSVdata _returnvalue_5))))))) _displacement_randomize)) (Variables|Default|GetShuffle)))) (.Y (Math|Vector|BreakVector (+ (Math|Vector|MakeVector (Math|Random|RandomFloatinRangefromStream (* (.X (Math|Vector|BreakVector (* (Variables|Default|GetRandom%20Rotation%20[XYZ]) (Math|Conversions|ToFloat(Boolean) (!= (- (Math|Conversions|ToInteger(Boolean) (Variables|Default|GetRotation%20clamped%20to%20Displacement)) 1) (.AXIS (Utilities|Struct|BreakF_CSVdata _returnvalue_5))))))) -1.0) (.X (Math|Vector|BreakVector (* (Variables|Default|GetRandom%20Rotation%20[XYZ]) (Math|Conversions|ToFloat(Boolean) (!= (- (Math|Conversions|ToInteger(Boolean) (Variables|Default|GetRotation%20clamped%20to%20Displacement)) 1) (.AXIS (Utilities|Struct|BreakF_CSVdata _returnvalue_5))))))) _displacement_randomize) (Math|Random|RandomFloatinRangefromStream (* (.Y (Math|Vector|BreakVector (* (Variables|Default|GetRandom%20Rotation%20[XYZ]) (Math|Conversions|ToFloat(Boolean) (!= (- (Math|Conversions|ToInteger(Boolean) (Variables|Default|GetRotation%20clamped%20to%20Displacement)) 1) (.AXIS (Utilities|Struct|BreakF_CSVdata _returnvalue_5))))))) -1.0) (.Y (Math|Vector|BreakVector (* (Variables|Default|GetRandom%20Rotation%20[XYZ]) (Math|Conversions|ToFloat(Boolean) (!= (- (Math|Conversions|ToInteger(Boolean) (Variables|Default|GetRotation%20clamped%20to%20Displacement)) 1) (.AXIS (Utilities|Struct|BreakF_CSVdata _returnvalue_5))))))) _displacement_randomize) (Math|Random|RandomFloatinRangefromStream (* (.Z (Math|Vector|BreakVector (* (Variables|Default|GetRandom%20Rotation%20[XYZ]) (Math|Conversions|ToFloat(Boolean) (!= (- (Math|Conversions|ToInteger(Boolean) (Variables|Default|GetRotation%20clamped%20to%20Displacement)) 1) (.AXIS (Utilities|Struct|BreakF_CSVdata _returnvalue_5))))))) -1.0) (.Z (Math|Vector|BreakVector (* (Variables|Default|GetRandom%20Rotation%20[XYZ]) (Math|Conversions|ToFloat(Boolean) (!= (- (Math|Conversions|ToInteger(Boolean) (Variables|Default|GetRotation%20clamped%20to%20Displacement)) 1) (.AXIS (Utilities|Struct|BreakF_CSVdata _returnvalue_5))))))) _displacement_randomize)) (Variables|Default|GetShuffle)))) (.Z (Math|Vector|BreakVector (+ (Math|Vector|MakeVector (Math|Random|RandomFloatinRangefromStream (* (.X (Math|Vector|BreakVector (* (Variables|Default|GetRandom%20Rotation%20[XYZ]) (Math|Conversions|ToFloat(Boolean) (!= (- (Math|Conversions|ToInteger(Boolean) (Variables|Default|GetRotation%20clamped%20to%20Displacement)) 1) (.AXIS (Utilities|Struct|BreakF_CSVdata _returnvalue_5))))))) -1.0) (.X (Math|Vector|BreakVector (* (Variables|Default|GetRandom%20Rotation%20[XYZ]) (Math|Conversions|ToFloat(Boolean) (!= (- (Math|Conversions|ToInteger(Boolean) (Variables|Default|GetRotation%20clamped%20to%20Displacement)) 1) (.AXIS (Utilities|Struct|BreakF_CSVdata _returnvalue_5))))))) _displacement_randomize) (Math|Random|RandomFloatinRangefromStream (* (.Y (Math|Vector|BreakVector (* (Variables|Default|GetRandom%20Rotation%20[XYZ]) (Math|Conversions|ToFloat(Boolean) (!= (- (Math|Conversions|ToInteger(Boolean) (Variables|Default|GetRotation%20clamped%20to%20Displacement)) 1) (.AXIS (Utilities|Struct|BreakF_CSVdata _returnvalue_5))))))) -1.0) (.Y (Math|Vector|BreakVector (* (Variables|Default|GetRandom%20Rotation%20[XYZ]) (Math|Conversions|ToFloat(Boolean) (!= (- (Math|Conversions|ToInteger(Boolean) (Variables|Default|GetRotation%20clamped%20to%20Displacement)) 1) (.AXIS (Utilities|Struct|BreakF_CSVdata _returnvalue_5))))))) _displacement_randomize) (Math|Random|RandomFloatinRangefromStream (* (.Z (Math|Vector|BreakVector (* (Variables|Default|GetRandom%20Rotation%20[XYZ]) (Math|Conversions|ToFloat(Boolean) (!= (- (Math|Conversions|ToInteger(Boolean) (Variables|Default|GetRotation%20clamped%20to%20Displacement)) 1) (.AXIS (Utilities|Struct|BreakF_CSVdata _returnvalue_5))))))) -1.0) (.Z (Math|Vector|BreakVector (* (Variables|Default|GetRandom%20Rotation%20[XYZ]) (Math|Conversions|ToFloat(Boolean) (!= (- (Math|Conversions|ToInteger(Boolean) (Variables|Default|GetRotation%20clamped%20to%20Displacement)) 1) (.AXIS (Utilities|Struct|BreakF_CSVdata _returnvalue_5))))))) _displacement_randomize)) (Variables|Default|GetShuffle))))) (Math|Rotator|MakeRotator (.R_X (Utilities|Struct|BreakF_CSVdata _returnvalue_5)) (.R_Y (Utilities|Struct|BreakF_CSVdata _returnvalue_5)) (.R_Z (Utilities|Struct|BreakF_CSVdata _returnvalue_5)))) (Math|Rotator|MakeRotator (.X (Math|Vector|BreakVector (+ (+ (Math|Vector|MakeVector (Math|Random|RandomFloatinRangefromStream (* (.X (Math|Vector|BreakVector (* (Variables|Default|GetRandom%20Rotation%20[XYZ]) (Math|Conversions|ToFloat(Boolean) (!= (- (Math|Conversions|ToInteger(Boolean) (Variables|Default|GetRotation%20clamped%20to%20Displacement)) 1) (.AXIS (Utilities|Struct|BreakF_CSVdata _returnvalue_5))))))) -1.0) (.X (Math|Vector|BreakVector (* (Variables|Default|GetRandom%20Rotation%20[XYZ]) (Math|Conversions|ToFloat(Boolean) (!= (- (Math|Conversions|ToInteger(Boolean) (Variables|Default|GetRotation%20clamped%20to%20Displacement)) 1) (.AXIS (Utilities|Struct|BreakF_CSVdata _returnvalue_5))))))) _displacement_randomize) (Math|Random|RandomFloatinRangefromStream (* (.Y (Math|Vector|BreakVector (* (Variables|Default|GetRandom%20Rotation%20[XYZ]) (Math|Conversions|ToFloat(Boolean) (!= (- (Math|Conversions|ToInteger(Boolean) (Variables|Default|GetRotation%20clamped%20to%20Displacement)) 1) (.AXIS (Utilities|Struct|BreakF_CSVdata _returnvalue_5))))))) -1.0) (.Y (Math|Vector|BreakVector (* (Variables|Default|GetRandom%20Rotation%20[XYZ]) (Math|Conversions|ToFloat(Boolean) (!= (- (Math|Conversions|ToInteger(Boolean) (Variables|Default|GetRotation%20clamped%20to%20Displacement)) 1) (.AXIS (Utilities|Struct|BreakF_CSVdata _returnvalue_5))))))) _displacement_randomize) (Math|Random|RandomFloatinRangefromStream (* (.Z (Math|Vector|BreakVector (* (Variables|Default|GetRandom%20Rotation%20[XYZ]) (Math|Conversions|ToFloat(Boolean) (!= (- (Math|Conversions|ToInteger(Boolean) (Variables|Default|GetRotation%20clamped%20to%20Displacement)) 1) (.AXIS (Utilities|Struct|BreakF_CSVdata _returnvalue_5))))))) -1.0) (.Z (Math|Vector|BreakVector (* (Variables|Default|GetRandom%20Rotation%20[XYZ]) (Math|Conversions|ToFloat(Boolean) (!= (- (Math|Conversions|ToInteger(Boolean) (Variables|Default|GetRotation%20clamped%20to%20Displacement)) 1) (.AXIS (Utilities|Struct|BreakF_CSVdata _returnvalue_5))))))) _displacement_randomize)) (Variables|Default|GetShuffle)) (Math|Vector|MakeVector (.R_X (Utilities|Struct|BreakF_CSVdata _returnvalue_5)) (.R_Y (Utilities|Struct|BreakF_CSVdata _returnvalue_5)) (.R_Z (Utilities|Struct|BreakF_CSVdata _returnvalue_5)))))) (.Y (Math|Vector|BreakVector (+ (+ (Math|Vector|MakeVector (Math|Random|RandomFloatinRangefromStream (* (.X (Math|Vector|BreakVector (* (Variables|Default|GetRandom%20Rotation%20[XYZ]) (Math|Conversions|ToFloat(Boolean) (!= (- (Math|Conversions|ToInteger(Boolean) (Variables|Default|GetRotation%20clamped%20to%20Displacement)) 1) (.AXIS (Utilities|Struct|BreakF_CSVdata _returnvalue_5))))))) -1.0) (.X (Math|Vector|BreakVector (* (Variables|Default|GetRandom%20Rotation%20[XYZ]) (Math|Conversions|ToFloat(Boolean) (!= (- (Math|Conversions|ToInteger(Boolean) (Variables|Default|GetRotation%20clamped%20to%20Displacement)) 1) (.AXIS (Utilities|Struct|BreakF_CSVdata _returnvalue_5))))))) _displacement_randomize) (Math|Random|RandomFloatinRangefromStream (* (.Y (Math|Vector|BreakVector (* (Variables|Default|GetRandom%20Rotation%20[XYZ]) (Math|Conversions|ToFloat(Boolean) (!= (- (Math|Conversions|ToInteger(Boolean) (Variables|Default|GetRotation%20clamped%20to%20Displacement)) 1) (.AXIS (Utilities|Struct|BreakF_CSVdata _returnvalue_5))))))) -1.0) (.Y (Math|Vector|BreakVector (* (Variables|Default|GetRandom%20Rotation%20[XYZ]) (Math|Conversions|ToFloat(Boolean) (!= (- (Math|Conversions|ToInteger(Boolean) (Variables|Default|GetRotation%20clamped%20to%20Displacement)) 1) (.AXIS (Utilities|Struct|BreakF_CSVdata _returnvalue_5))))))) _displacement_randomize) (Math|Random|RandomFloatinRangefromStream (* (.Z (Math|Vector|BreakVector (* (Variables|Default|GetRandom%20Rotation%20[XYZ]) (Math|Conversions|ToFloat(Boolean) (!= (- (Math|Conversions|ToInteger(Boolean) (Variables|Default|GetRotation%20clamped%20to%20Displacement)) 1) (.AXIS (Utilities|Struct|BreakF_CSVdata _returnvalue_5))))))) -1.0) (.Z (Math|Vector|BreakVector (* (Variables|Default|GetRandom%20Rotation%20[XYZ]) (Math|Conversions|ToFloat(Boolean) (!= (- (Math|Conversions|ToInteger(Boolean) (Variables|Default|GetRotation%20clamped%20to%20Displacement)) 1) (.AXIS (Utilities|Struct|BreakF_CSVdata _returnvalue_5))))))) _displacement_randomize)) (Variables|Default|GetShuffle)) (Math|Vector|MakeVector (.R_X (Utilities|Struct|BreakF_CSVdata _returnvalue_5)) (.R_Y (Utilities|Struct|BreakF_CSVdata _returnvalue_5)) (.R_Z (Utilities|Struct|BreakF_CSVdata _returnvalue_5)))))) (.Z (Math|Vector|BreakVector (+ (+ (Math|Vector|MakeVector (Math|Random|RandomFloatinRangefromStream (* (.X (Math|Vector|BreakVector (* (Variables|Default|GetRandom%20Rotation%20[XYZ]) (Math|Conversions|ToFloat(Boolean) (!= (- (Math|Conversions|ToInteger(Boolean) (Variables|Default|GetRotation%20clamped%20to%20Displacement)) 1) (.AXIS (Utilities|Struct|BreakF_CSVdata _returnvalue_5))))))) -1.0) (.X (Math|Vector|BreakVector (* (Variables|Default|GetRandom%20Rotation%20[XYZ]) (Math|Conversions|ToFloat(Boolean) (!= (- (Math|Conversions|ToInteger(Boolean) (Variables|Default|GetRotation%20clamped%20to%20Displacement)) 1) (.AXIS (Utilities|Struct|BreakF_CSVdata _returnvalue_5))))))) _displacement_randomize) (Math|Random|RandomFloatinRangefromStream (* (.Y (Math|Vector|BreakVector (* (Variables|Default|GetRandom%20Rotation%20[XYZ]) (Math|Conversions|ToFloat(Boolean) (!= (- (Math|Conversions|ToInteger(Boolean) (Variables|Default|GetRotation%20clamped%20to%20Displacement)) 1) (.AXIS (Utilities|Struct|BreakF_CSVdata _returnvalue_5))))))) -1.0) (.Y (Math|Vector|BreakVector (* (Variables|Default|GetRandom%20Rotation%20[XYZ]) (Math|Conversions|ToFloat(Boolean) (!= (- (Math|Conversions|ToInteger(Boolean) (Variables|Default|GetRotation%20clamped%20to%20Displacement)) 1) (.AXIS (Utilities|Struct|BreakF_CSVdata _returnvalue_5))))))) _displacement_randomize) (Math|Random|RandomFloatinRangefromStream (* (.Z (Math|Vector|BreakVector (* (Variables|Default|GetRandom%20Rotation%20[XYZ]) (Math|Conversions|ToFloat(Boolean) (!= (- (Math|Conversions|ToInteger(Boolean) (Variables|Default|GetRotation%20clamped%20to%20Displacement)) 1) (.AXIS (Utilities|Struct|BreakF_CSVdata _returnvalue_5))))))) -1.0) (.Z (Math|Vector|BreakVector (* (Variables|Default|GetRandom%20Rotation%20[XYZ]) (Math|Conversions|ToFloat(Boolean) (!= (- (Math|Conversions|ToInteger(Boolean) (Variables|Default|GetRotation%20clamped%20to%20Displacement)) 1) (.AXIS (Utilities|Struct|BreakF_CSVdata _returnvalue_5))))))) _displacement_randomize)) (Variables|Default|GetShuffle)) (Math|Vector|MakeVector (.R_X (Utilities|Struct|BreakF_CSVdata _returnvalue_5)) (.R_Y (Utilities|Struct|BreakF_CSVdata _returnvalue_5)) (.R_Z (Utilities|Struct|BreakF_CSVdata _returnvalue_5))))))) (Math|Conversions|ToFloat(Boolean) (Variables|Default|GetRandom%20Rotation%20LOCAL/GLOBAL))) (* (Math|Vector|MakeVector (.S_X (Utilities|Struct|BreakF_CSVdata _returnvalue_5)) (.S_Y (Utilities|Struct|BreakF_CSVdata _returnvalue_5)) (.S_Z (Utilities|Struct|BreakF_CSVdata _returnvalue_5))) (Variables|Default|GetScale))) (* (Math|Vector|MakeVector (* (Math|Conversions|ToFloat(Boolean) (== (.AXIS (Utilities|Struct|BreakF_CSVdata _returnvalue_5)) 1)) _returnvalue_3) (* (Math|Conversions|ToFloat(Boolean) (== (.AXIS (Utilities|Struct|BreakF_CSVdata _returnvalue_5)) 2)) _returnvalue_3) (* (Math|Conversions|ToFloat(Boolean) (== (.AXIS (Utilities|Struct|BreakF_CSVdata _returnvalue_5)) 3)) _returnvalue_3)) (Math|Float|Clamp(Float) (+ (Math|Conversions|ToFloat(Boolean) (and (not (Class|KismetMathLibrary|IsPointinBoxwithTransform (Math|Vector|MakeVector (.T_X (Utilities|Struct|BreakF_CSVdata _returnvalue_5)) (.T_Y (Utilities|Struct|BreakF_CSVdata _returnvalue_5)) (.T_Z (Utilities|Struct|BreakF_CSVdata _returnvalue_5))) (Math|Transform|MakeTransform (Variables|Default|GetBox%20Origin%20[XYZ]) (Variables|Default|GetBox%20Rotation%20[XYZ])) (Variables|Default|GetBox%20Extent%20[XYZ]))) _boxcontrolleddisplacement)) (Variables|Default|GetBox%20Intensity)) (Math|Conversions|ToFloat(Boolean) (not _boxcontrolleddisplacement))))) (Math|Rotator|Lerp(Rotator) (Math|Rotator|CombineRotators (Math|Rotator|MakeRotator (.X (Math|Vector|BreakVector (+ (Math|Vector|MakeVector (Math|Random|RandomFloatinRangefromStream (* (.X (Math|Vector|BreakVector (* (Variables|Default|GetRandom%20Rotation%20[XYZ]) (Math|Conversions|ToFloat(Boolean) (!= (- (Math|Conversions|ToInteger(Boolean) (Variables|Default|GetRotation%20clamped%20to%20Displacement)) 1) (.AXIS (Utilities|Struct|BreakF_CSVdata _returnvalue_5))))))) -1.0) (.X (Math|Vector|BreakVector (* (Variables|Default|GetRandom%20Rotation%20[XYZ]) (Math|Conversions|ToFloat(Boolean) (!= (- (Math|Conversions|ToInteger(Boolean) (Variables|Default|GetRotation%20clamped%20to%20Displacement)) 1) (.AXIS (Utilities|Struct|BreakF_CSVdata _returnvalue_5))))))) _displacement_randomize) (Math|Random|RandomFloatinRangefromStream (* (.Y (Math|Vector|BreakVector (* (Variables|Default|GetRandom%20Rotation%20[XYZ]) (Math|Conversions|ToFloat(Boolean) (!= (- (Math|Conversions|ToInteger(Boolean) (Variables|Default|GetRotation%20clamped%20to%20Displacement)) 1) (.AXIS (Utilities|Struct|BreakF_CSVdata _returnvalue_5))))))) -1.0) (.Y (Math|Vector|BreakVector (* (Variables|Default|GetRandom%20Rotation%20[XYZ]) (Math|Conversions|ToFloat(Boolean) (!= (- (Math|Conversions|ToInteger(Boolean) (Variables|Default|GetRotation%20clamped%20to%20Displacement)) 1) (.AXIS (Utilities|Struct|BreakF_CSVdata _returnvalue_5))))))) _displacement_randomize) (Math|Random|RandomFloatinRangefromStream (* (.Z (Math|Vector|BreakVector (* (Variables|Default|GetRandom%20Rotation%20[XYZ]) (Math|Conversions|ToFloat(Boolean) (!= (- (Math|Conversions|ToInteger(Boolean) (Variables|Default|GetRotation%20clamped%20to%20Displacement)) 1) (.AXIS (Utilities|Struct|BreakF_CSVdata _returnvalue_5))))))) -1.0) (.Z (Math|Vector|BreakVector (* (Variables|Default|GetRandom%20Rotation%20[XYZ]) (Math|Conversions|ToFloat(Boolean) (!= (- (Math|Conversions|ToInteger(Boolean) (Variables|Default|GetRotation%20clamped%20to%20Displacement)) 1) (.AXIS (Utilities|Struct|BreakF_CSVdata _returnvalue_5))))))) _displacement_randomize)) (Variables|Default|GetShuffle)))) (.Y (Math|Vector|BreakVector (+ (Math|Vector|MakeVector (Math|Random|RandomFloatinRangefromStream (* (.X (Math|Vector|BreakVector (* (Variables|Default|GetRandom%20Rotation%20[XYZ]) (Math|Conversions|ToFloat(Boolean) (!= (- (Math|Conversions|ToInteger(Boolean) (Variables|Default|GetRotation%20clamped%20to%20Displacement)) 1) (.AXIS (Utilities|Struct|BreakF_CSVdata _returnvalue_5))))))) -1.0) (.X (Math|Vector|BreakVector (* (Variables|Default|GetRandom%20Rotation%20[XYZ]) (Math|Conversions|ToFloat(Boolean) (!= (- (Math|Conversions|ToInteger(Boolean) (Variables|Default|GetRotation%20clamped%20to%20Displacement)) 1) (.AXIS (Utilities|Struct|BreakF_CSVdata _returnvalue_5))))))) _displacement_randomize) (Math|Random|RandomFloatinRangefromStream (* (.Y (Math|Vector|BreakVector (* (Variables|Default|GetRandom%20Rotation%20[XYZ]) (Math|Conversions|ToFloat(Boolean) (!= (- (Math|Conversions|ToInteger(Boolean) (Variables|Default|GetRotation%20clamped%20to%20Displacement)) 1) (.AXIS (Utilities|Struct|BreakF_CSVdata _returnvalue_5))))))) -1.0) (.Y (Math|Vector|BreakVector (* (Variables|Default|GetRandom%20Rotation%20[XYZ]) (Math|Conversions|ToFloat(Boolean) (!= (- (Math|Conversions|ToInteger(Boolean) (Variables|Default|GetRotation%20clamped%20to%20Displacement)) 1) (.AXIS (Utilities|Struct|BreakF_CSVdata _returnvalue_5))))))) _displacement_randomize) (Math|Random|RandomFloatinRangefromStream (* (.Z (Math|Vector|BreakVector (* (Variables|Default|GetRandom%20Rotation%20[XYZ]) (Math|Conversions|ToFloat(Boolean) (!= (- (Math|Conversions|ToInteger(Boolean) (Variables|Default|GetRotation%20clamped%20to%20Displacement)) 1) (.AXIS (Utilities|Struct|BreakF_CSVdata _returnvalue_5))))))) -1.0) (.Z (Math|Vector|BreakVector (* (Variables|Default|GetRandom%20Rotation%20[XYZ]) (Math|Conversions|ToFloat(Boolean) (!= (- (Math|Conversions|ToInteger(Boolean) (Variables|Default|GetRotation%20clamped%20to%20Displacement)) 1) (.AXIS (Utilities|Struct|BreakF_CSVdata _returnvalue_5))))))) _displacement_randomize)) (Variables|Default|GetShuffle)))) (.Z (Math|Vector|BreakVector (+ (Math|Vector|MakeVector (Math|Random|RandomFloatinRangefromStream (* (.X (Math|Vector|BreakVector (* (Variables|Default|GetRandom%20Rotation%20[XYZ]) (Math|Conversions|ToFloat(Boolean) (!= (- (Math|Conversions|ToInteger(Boolean) (Variables|Default|GetRotation%20clamped%20to%20Displacement)) 1) (.AXIS (Utilities|Struct|BreakF_CSVdata _returnvalue_5))))))) -1.0) (.X (Math|Vector|BreakVector (* (Variables|Default|GetRandom%20Rotation%20[XYZ]) (Math|Conversions|ToFloat(Boolean) (!= (- (Math|Conversions|ToInteger(Boolean) (Variables|Default|GetRotation%20clamped%20to%20Displacement)) 1) (.AXIS (Utilities|Struct|BreakF_CSVdata _returnvalue_5))))))) _displacement_randomize) (Math|Random|RandomFloatinRangefromStream (* (.Y (Math|Vector|BreakVector (* (Variables|Default|GetRandom%20Rotation%20[XYZ]) (Math|Conversions|ToFloat(Boolean) (!= (- (Math|Conversions|ToInteger(Boolean) (Variables|Default|GetRotation%20clamped%20to%20Displacement)) 1) (.AXIS (Utilities|Struct|BreakF_CSVdata _returnvalue_5))))))) -1.0) (.Y (Math|Vector|BreakVector (* (Variables|Default|GetRandom%20Rotation%20[XYZ]) (Math|Conversions|ToFloat(Boolean) (!= (- (Math|Conversions|ToInteger(Boolean) (Variables|Default|GetRotation%20clamped%20to%20Displacement)) 1) (.AXIS (Utilities|Struct|BreakF_CSVdata _returnvalue_5))))))) _displacement_randomize) (Math|Random|RandomFloatinRangefromStream (* (.Z (Math|Vector|BreakVector (* (Variables|Default|GetRandom%20Rotation%20[XYZ]) (Math|Conversions|ToFloat(Boolean) (!= (- (Math|Conversions|ToInteger(Boolean) (Variables|Default|GetRotation%20clamped%20to%20Displacement)) 1) (.AXIS (Utilities|Struct|BreakF_CSVdata _returnvalue_5))))))) -1.0) (.Z (Math|Vector|BreakVector (* (Variables|Default|GetRandom%20Rotation%20[XYZ]) (Math|Conversions|ToFloat(Boolean) (!= (- (Math|Conversions|ToInteger(Boolean) (Variables|Default|GetRotation%20clamped%20to%20Displacement)) 1) (.AXIS (Utilities|Struct|BreakF_CSVdata _returnvalue_5))))))) _displacement_randomize)) (Variables|Default|GetShuffle))))) (Math|Rotator|MakeRotator (.R_X (Utilities|Struct|BreakF_CSVdata _returnvalue_5)) (.R_Y (Utilities|Struct|BreakF_CSVdata _returnvalue_5)) (.R_Z (Utilities|Struct|BreakF_CSVdata _returnvalue_5)))) (Math|Rotator|MakeRotator (.X (Math|Vector|BreakVector (+ (+ (Math|Vector|MakeVector (Math|Random|RandomFloatinRangefromStream (* (.X (Math|Vector|BreakVector (* (Variables|Default|GetRandom%20Rotation%20[XYZ]) (Math|Conversions|ToFloat(Boolean) (!= (- (Math|Conversions|ToInteger(Boolean) (Variables|Default|GetRotation%20clamped%20to%20Displacement)) 1) (.AXIS (Utilities|Struct|BreakF_CSVdata _returnvalue_5))))))) -1.0) (.X (Math|Vector|BreakVector (* (Variables|Default|GetRandom%20Rotation%20[XYZ]) (Math|Conversions|ToFloat(Boolean) (!= (- (Math|Conversions|ToInteger(Boolean) (Variables|Default|GetRotation%20clamped%20to%20Displacement)) 1) (.AXIS (Utilities|Struct|BreakF_CSVdata _returnvalue_5))))))) _displacement_randomize) (Math|Random|RandomFloatinRangefromStream (* (.Y (Math|Vector|BreakVector (* (Variables|Default|GetRandom%20Rotation%20[XYZ]) (Math|Conversions|ToFloat(Boolean) (!= (- (Math|Conversions|ToInteger(Boolean) (Variables|Default|GetRotation%20clamped%20to%20Displacement)) 1) (.AXIS (Utilities|Struct|BreakF_CSVdata _returnvalue_5))))))) -1.0) (.Y (Math|Vector|BreakVector (* (Variables|Default|GetRandom%20Rotation%20[XYZ]) (Math|Conversions|ToFloat(Boolean) (!= (- (Math|Conversions|ToInteger(Boolean) (Variables|Default|GetRotation%20clamped%20to%20Displacement)) 1) (.AXIS (Utilities|Struct|BreakF_CSVdata _returnvalue_5))))))) _displacement_randomize) (Math|Random|RandomFloatinRangefromStream (* (.Z (Math|Vector|BreakVector (* (Variables|Default|GetRandom%20Rotation%20[XYZ]) (Math|Conversions|ToFloat(Boolean) (!= (- (Math|Conversions|ToInteger(Boolean) (Variables|Default|GetRotation%20clamped%20to%20Displacement)) 1) (.AXIS (Utilities|Struct|BreakF_CSVdata _returnvalue_5))))))) -1.0) (.Z (Math|Vector|BreakVector (* (Variables|Default|GetRandom%20Rotation%20[XYZ]) (Math|Conversions|ToFloat(Boolean) (!= (- (Math|Conversions|ToInteger(Boolean) (Variables|Default|GetRotation%20clamped%20to%20Displacement)) 1) (.AXIS (Utilities|Struct|BreakF_CSVdata _returnvalue_5))))))) _displacement_randomize)) (Variables|Default|GetShuffle)) (Math|Vector|MakeVector (.R_X (Utilities|Struct|BreakF_CSVdata _returnvalue_5)) (.R_Y (Utilities|Struct|BreakF_CSVdata _returnvalue_5)) (.R_Z (Utilities|Struct|BreakF_CSVdata _returnvalue_5)))))) (.Y (Math|Vector|BreakVector (+ (+ (Math|Vector|MakeVector (Math|Random|RandomFloatinRangefromStream (* (.X (Math|Vector|BreakVector (* (Variables|Default|GetRandom%20Rotation%20[XYZ]) (Math|Conversions|ToFloat(Boolean) (!= (- (Math|Conversions|ToInteger(Boolean) (Variables|Default|GetRotation%20clamped%20to%20Displacement)) 1) (.AXIS (Utilities|Struct|BreakF_CSVdata _returnvalue_5))))))) -1.0) (.X (Math|Vector|BreakVector (* (Variables|Default|GetRandom%20Rotation%20[XYZ]) (Math|Conversions|ToFloat(Boolean) (!= (- (Math|Conversions|ToInteger(Boolean) (Variables|Default|GetRotation%20clamped%20to%20Displacement)) 1) (.AXIS (Utilities|Struct|BreakF_CSVdata _returnvalue_5))))))) _displacement_randomize) (Math|Random|RandomFloatinRangefromStream (* (.Y (Math|Vector|BreakVector (* (Variables|Default|GetRandom%20Rotation%20[XYZ]) (Math|Conversions|ToFloat(Boolean) (!= (- (Math|Conversions|ToInteger(Boolean) (Variables|Default|GetRotation%20clamped%20to%20Displacement)) 1) (.AXIS (Utilities|Struct|BreakF_CSVdata _returnvalue_5))))))) -1.0) (.Y (Math|Vector|BreakVector (* (Variables|Default|GetRandom%20Rotation%20[XYZ]) (Math|Conversions|ToFloat(Boolean) (!= (- (Math|Conversions|ToInteger(Boolean) (Variables|Default|GetRotation%20clamped%20to%20Displacement)) 1) (.AXIS (Utilities|Struct|BreakF_CSVdata _returnvalue_5))))))) _displacement_randomize) (Math|Random|RandomFloatinRangefromStream (* (.Z (Math|Vector|BreakVector (* (Variables|Default|GetRandom%20Rotation%20[XYZ]) (Math|Conversions|ToFloat(Boolean) (!= (- (Math|Conversions|ToInteger(Boolean) (Variables|Default|GetRotation%20clamped%20to%20Displacement)) 1) (.AXIS (Utilities|Struct|BreakF_CSVdata _returnvalue_5))))))) -1.0) (.Z (Math|Vector|BreakVector (* (Variables|Default|GetRandom%20Rotation%20[XYZ]) (Math|Conversions|ToFloat(Boolean) (!= (- (Math|Conversions|ToInteger(Boolean) (Variables|Default|GetRotation%20clamped%20to%20Displacement)) 1) (.AXIS (Utilities|Struct|BreakF_CSVdata _returnvalue_5))))))) _displacement_randomize)) (Variables|Default|GetShuffle)) (Math|Vector|MakeVector (.R_X (Utilities|Struct|BreakF_CSVdata _returnvalue_5)) (.R_Y (Utilities|Struct|BreakF_CSVdata _returnvalue_5)) (.R_Z (Utilities|Struct|BreakF_CSVdata _returnvalue_5)))))) (.Z (Math|Vector|BreakVector (+ (+ (Math|Vector|MakeVector (Math|Random|RandomFloatinRangefromStream (* (.X (Math|Vector|BreakVector (* (Variables|Default|GetRandom%20Rotation%20[XYZ]) (Math|Conversions|ToFloat(Boolean) (!= (- (Math|Conversions|ToInteger(Boolean) (Variables|Default|GetRotation%20clamped%20to%20Displacement)) 1) (.AXIS (Utilities|Struct|BreakF_CSVdata _returnvalue_5))))))) -1.0) (.X (Math|Vector|BreakVector (* (Variables|Default|GetRandom%20Rotation%20[XYZ]) (Math|Conversions|ToFloat(Boolean) (!= (- (Math|Conversions|ToInteger(Boolean) (Variables|Default|GetRotation%20clamped%20to%20Displacement)) 1) (.AXIS (Utilities|Struct|BreakF_CSVdata _returnvalue_5))))))) _displacement_randomize) (Math|Random|RandomFloatinRangefromStream (* (.Y (Math|Vector|BreakVector (* (Variables|Default|GetRandom%20Rotation%20[XYZ]) (Math|Conversions|ToFloat(Boolean) (!= (- (Math|Conversions|ToInteger(Boolean) (Variables|Default|GetRotation%20clamped%20to%20Displacement)) 1) (.AXIS (Utilities|Struct|BreakF_CSVdata _returnvalue_5))))))) -1.0) (.Y (Math|Vector|BreakVector (* (Variables|Default|GetRandom%20Rotation%20[XYZ]) (Math|Conversions|ToFloat(Boolean) (!= (- (Math|Conversions|ToInteger(Boolean) (Variables|Default|GetRotation%20clamped%20to%20Displacement)) 1) (.AXIS (Utilities|Struct|BreakF_CSVdata _returnvalue_5))))))) _displacement_randomize) (Math|Random|RandomFloatinRangefromStream (* (.Z (Math|Vector|BreakVector (* (Variables|Default|GetRandom%20Rotation%20[XYZ]) (Math|Conversions|ToFloat(Boolean) (!= (- (Math|Conversions|ToInteger(Boolean) (Variables|Default|GetRotation%20clamped%20to%20Displacement)) 1) (.AXIS (Utilities|Struct|BreakF_CSVdata _returnvalue_5))))))) -1.0) (.Z (Math|Vector|BreakVector (* (Variables|Default|GetRandom%20Rotation%20[XYZ]) (Math|Conversions|ToFloat(Boolean) (!= (- (Math|Conversions|ToInteger(Boolean) (Variables|Default|GetRotation%20clamped%20to%20Displacement)) 1) (.AXIS (Utilities|Struct|BreakF_CSVdata _returnvalue_5))))))) _displacement_randomize)) (Variables|Default|GetShuffle)) (Math|Vector|MakeVector (.R_X (Utilities|Struct|BreakF_CSVdata _returnvalue_5)) (.R_Y (Utilities|Struct|BreakF_CSVdata _returnvalue_5)) (.R_Z (Utilities|Struct|BreakF_CSVdata _returnvalue_5))))))) (Math|Conversions|ToFloat(Boolean) (Variables|Default|GetRandom%20Rotation%20LOCAL/GLOBAL))) (* (Math|Vector|MakeVector (.S_X (Utilities|Struct|BreakF_CSVdata _returnvalue_5)) (.S_Y (Utilities|Struct|BreakF_CSVdata _returnvalue_5)) (.S_Z (Utilities|Struct|BreakF_CSVdata _returnvalue_5))) (Variables|Default|GetScale))) false))))
                  (:14
                    (if _undamaged_stones_2
                      (goto _label_15)
                      (else
                        (Utilities|FlowControl|Sequence
                          (:then_0
                            (Utilities|FlowControl|DoOnce false
                              (:Completed
                                (bind _returnvalue_19 (AddComponent|AddHierarchicalInstancedStaticMeshComponent false))
                                (bind _output_get_14 (Variables|Default|Set14 _returnvalue_19))
                                (Rendering|Material|SetMaterial _output_get_14 0 (Variables|Default|GetStone%20Material)))))
                          (:then_1
                            (Components|InstancedStaticMesh|AddInstance (Variables|Default|Get14) (Math|Transform|MakeTransform (Math|Transform|TransformLocation (Math|Transform|MakeTransform (Math|Vector|MakeVector (.T_X (Utilities|Struct|BreakF_CSVdata _returnvalue_5)) (.T_Y (Utilities|Struct|BreakF_CSVdata _returnvalue_5)) (.T_Z (Utilities|Struct|BreakF_CSVdata _returnvalue_5))) (Math|Rotator|Lerp(Rotator) (Math|Rotator|CombineRotators (Math|Rotator|MakeRotator (.X (Math|Vector|BreakVector (+ (Math|Vector|MakeVector (Math|Random|RandomFloatinRangefromStream (* (.X (Math|Vector|BreakVector (* (Variables|Default|GetRandom%20Rotation%20[XYZ]) (Math|Conversions|ToFloat(Boolean) (!= (- (Math|Conversions|ToInteger(Boolean) (Variables|Default|GetRotation%20clamped%20to%20Displacement)) 1) (.AXIS (Utilities|Struct|BreakF_CSVdata _returnvalue_5))))))) -1.0) (.X (Math|Vector|BreakVector (* (Variables|Default|GetRandom%20Rotation%20[XYZ]) (Math|Conversions|ToFloat(Boolean) (!= (- (Math|Conversions|ToInteger(Boolean) (Variables|Default|GetRotation%20clamped%20to%20Displacement)) 1) (.AXIS (Utilities|Struct|BreakF_CSVdata _returnvalue_5))))))) _displacement_randomize) (Math|Random|RandomFloatinRangefromStream (* (.Y (Math|Vector|BreakVector (* (Variables|Default|GetRandom%20Rotation%20[XYZ]) (Math|Conversions|ToFloat(Boolean) (!= (- (Math|Conversions|ToInteger(Boolean) (Variables|Default|GetRotation%20clamped%20to%20Displacement)) 1) (.AXIS (Utilities|Struct|BreakF_CSVdata _returnvalue_5))))))) -1.0) (.Y (Math|Vector|BreakVector (* (Variables|Default|GetRandom%20Rotation%20[XYZ]) (Math|Conversions|ToFloat(Boolean) (!= (- (Math|Conversions|ToInteger(Boolean) (Variables|Default|GetRotation%20clamped%20to%20Displacement)) 1) (.AXIS (Utilities|Struct|BreakF_CSVdata _returnvalue_5))))))) _displacement_randomize) (Math|Random|RandomFloatinRangefromStream (* (.Z (Math|Vector|BreakVector (* (Variables|Default|GetRandom%20Rotation%20[XYZ]) (Math|Conversions|ToFloat(Boolean) (!= (- (Math|Conversions|ToInteger(Boolean) (Variables|Default|GetRotation%20clamped%20to%20Displacement)) 1) (.AXIS (Utilities|Struct|BreakF_CSVdata _returnvalue_5))))))) -1.0) (.Z (Math|Vector|BreakVector (* (Variables|Default|GetRandom%20Rotation%20[XYZ]) (Math|Conversions|ToFloat(Boolean) (!= (- (Math|Conversions|ToInteger(Boolean) (Variables|Default|GetRotation%20clamped%20to%20Displacement)) 1) (.AXIS (Utilities|Struct|BreakF_CSVdata _returnvalue_5))))))) _displacement_randomize)) (Variables|Default|GetShuffle)))) (.Y (Math|Vector|BreakVector (+ (Math|Vector|MakeVector (Math|Random|RandomFloatinRangefromStream (* (.X (Math|Vector|BreakVector (* (Variables|Default|GetRandom%20Rotation%20[XYZ]) (Math|Conversions|ToFloat(Boolean) (!= (- (Math|Conversions|ToInteger(Boolean) (Variables|Default|GetRotation%20clamped%20to%20Displacement)) 1) (.AXIS (Utilities|Struct|BreakF_CSVdata _returnvalue_5))))))) -1.0) (.X (Math|Vector|BreakVector (* (Variables|Default|GetRandom%20Rotation%20[XYZ]) (Math|Conversions|ToFloat(Boolean) (!= (- (Math|Conversions|ToInteger(Boolean) (Variables|Default|GetRotation%20clamped%20to%20Displacement)) 1) (.AXIS (Utilities|Struct|BreakF_CSVdata _returnvalue_5))))))) _displacement_randomize) (Math|Random|RandomFloatinRangefromStream (* (.Y (Math|Vector|BreakVector (* (Variables|Default|GetRandom%20Rotation%20[XYZ]) (Math|Conversions|ToFloat(Boolean) (!= (- (Math|Conversions|ToInteger(Boolean) (Variables|Default|GetRotation%20clamped%20to%20Displacement)) 1) (.AXIS (Utilities|Struct|BreakF_CSVdata _returnvalue_5))))))) -1.0) (.Y (Math|Vector|BreakVector (* (Variables|Default|GetRandom%20Rotation%20[XYZ]) (Math|Conversions|ToFloat(Boolean) (!= (- (Math|Conversions|ToInteger(Boolean) (Variables|Default|GetRotation%20clamped%20to%20Displacement)) 1) (.AXIS (Utilities|Struct|BreakF_CSVdata _returnvalue_5))))))) _displacement_randomize) (Math|Random|RandomFloatinRangefromStream (* (.Z (Math|Vector|BreakVector (* (Variables|Default|GetRandom%20Rotation%20[XYZ]) (Math|Conversions|ToFloat(Boolean) (!= (- (Math|Conversions|ToInteger(Boolean) (Variables|Default|GetRotation%20clamped%20to%20Displacement)) 1) (.AXIS (Utilities|Struct|BreakF_CSVdata _returnvalue_5))))))) -1.0) (.Z (Math|Vector|BreakVector (* (Variables|Default|GetRandom%20Rotation%20[XYZ]) (Math|Conversions|ToFloat(Boolean) (!= (- (Math|Conversions|ToInteger(Boolean) (Variables|Default|GetRotation%20clamped%20to%20Displacement)) 1) (.AXIS (Utilities|Struct|BreakF_CSVdata _returnvalue_5))))))) _displacement_randomize)) (Variables|Default|GetShuffle)))) (.Z (Math|Vector|BreakVector (+ (Math|Vector|MakeVector (Math|Random|RandomFloatinRangefromStream (* (.X (Math|Vector|BreakVector (* (Variables|Default|GetRandom%20Rotation%20[XYZ]) (Math|Conversions|ToFloat(Boolean) (!= (- (Math|Conversions|ToInteger(Boolean) (Variables|Default|GetRotation%20clamped%20to%20Displacement)) 1) (.AXIS (Utilities|Struct|BreakF_CSVdata _returnvalue_5))))))) -1.0) (.X (Math|Vector|BreakVector (* (Variables|Default|GetRandom%20Rotation%20[XYZ]) (Math|Conversions|ToFloat(Boolean) (!= (- (Math|Conversions|ToInteger(Boolean) (Variables|Default|GetRotation%20clamped%20to%20Displacement)) 1) (.AXIS (Utilities|Struct|BreakF_CSVdata _returnvalue_5))))))) _displacement_randomize) (Math|Random|RandomFloatinRangefromStream (* (.Y (Math|Vector|BreakVector (* (Variables|Default|GetRandom%20Rotation%20[XYZ]) (Math|Conversions|ToFloat(Boolean) (!= (- (Math|Conversions|ToInteger(Boolean) (Variables|Default|GetRotation%20clamped%20to%20Displacement)) 1) (.AXIS (Utilities|Struct|BreakF_CSVdata _returnvalue_5))))))) -1.0) (.Y (Math|Vector|BreakVector (* (Variables|Default|GetRandom%20Rotation%20[XYZ]) (Math|Conversions|ToFloat(Boolean) (!= (- (Math|Conversions|ToInteger(Boolean) (Variables|Default|GetRotation%20clamped%20to%20Displacement)) 1) (.AXIS (Utilities|Struct|BreakF_CSVdata _returnvalue_5))))))) _displacement_randomize) (Math|Random|RandomFloatinRangefromStream (* (.Z (Math|Vector|BreakVector (* (Variables|Default|GetRandom%20Rotation%20[XYZ]) (Math|Conversions|ToFloat(Boolean) (!= (- (Math|Conversions|ToInteger(Boolean) (Variables|Default|GetRotation%20clamped%20to%20Displacement)) 1) (.AXIS (Utilities|Struct|BreakF_CSVdata _returnvalue_5))))))) -1.0) (.Z (Math|Vector|BreakVector (* (Variables|Default|GetRandom%20Rotation%20[XYZ]) (Math|Conversions|ToFloat(Boolean) (!= (- (Math|Conversions|ToInteger(Boolean) (Variables|Default|GetRotation%20clamped%20to%20Displacement)) 1) (.AXIS (Utilities|Struct|BreakF_CSVdata _returnvalue_5))))))) _displacement_randomize)) (Variables|Default|GetShuffle))))) (Math|Rotator|MakeRotator (.R_X (Utilities|Struct|BreakF_CSVdata _returnvalue_5)) (.R_Y (Utilities|Struct|BreakF_CSVdata _returnvalue_5)) (.R_Z (Utilities|Struct|BreakF_CSVdata _returnvalue_5)))) (Math|Rotator|MakeRotator (.X (Math|Vector|BreakVector (+ (+ (Math|Vector|MakeVector (Math|Random|RandomFloatinRangefromStream (* (.X (Math|Vector|BreakVector (* (Variables|Default|GetRandom%20Rotation%20[XYZ]) (Math|Conversions|ToFloat(Boolean) (!= (- (Math|Conversions|ToInteger(Boolean) (Variables|Default|GetRotation%20clamped%20to%20Displacement)) 1) (.AXIS (Utilities|Struct|BreakF_CSVdata _returnvalue_5))))))) -1.0) (.X (Math|Vector|BreakVector (* (Variables|Default|GetRandom%20Rotation%20[XYZ]) (Math|Conversions|ToFloat(Boolean) (!= (- (Math|Conversions|ToInteger(Boolean) (Variables|Default|GetRotation%20clamped%20to%20Displacement)) 1) (.AXIS (Utilities|Struct|BreakF_CSVdata _returnvalue_5))))))) _displacement_randomize) (Math|Random|RandomFloatinRangefromStream (* (.Y (Math|Vector|BreakVector (* (Variables|Default|GetRandom%20Rotation%20[XYZ]) (Math|Conversions|ToFloat(Boolean) (!= (- (Math|Conversions|ToInteger(Boolean) (Variables|Default|GetRotation%20clamped%20to%20Displacement)) 1) (.AXIS (Utilities|Struct|BreakF_CSVdata _returnvalue_5))))))) -1.0) (.Y (Math|Vector|BreakVector (* (Variables|Default|GetRandom%20Rotation%20[XYZ]) (Math|Conversions|ToFloat(Boolean) (!= (- (Math|Conversions|ToInteger(Boolean) (Variables|Default|GetRotation%20clamped%20to%20Displacement)) 1) (.AXIS (Utilities|Struct|BreakF_CSVdata _returnvalue_5))))))) _displacement_randomize) (Math|Random|RandomFloatinRangefromStream (* (.Z (Math|Vector|BreakVector (* (Variables|Default|GetRandom%20Rotation%20[XYZ]) (Math|Conversions|ToFloat(Boolean) (!= (- (Math|Conversions|ToInteger(Boolean) (Variables|Default|GetRotation%20clamped%20to%20Displacement)) 1) (.AXIS (Utilities|Struct|BreakF_CSVdata _returnvalue_5))))))) -1.0) (.Z (Math|Vector|BreakVector (* (Variables|Default|GetRandom%20Rotation%20[XYZ]) (Math|Conversions|ToFloat(Boolean) (!= (- (Math|Conversions|ToInteger(Boolean) (Variables|Default|GetRotation%20clamped%20to%20Displacement)) 1) (.AXIS (Utilities|Struct|BreakF_CSVdata _returnvalue_5))))))) _displacement_randomize)) (Variables|Default|GetShuffle)) (Math|Vector|MakeVector (.R_X (Utilities|Struct|BreakF_CSVdata _returnvalue_5)) (.R_Y (Utilities|Struct|BreakF_CSVdata _returnvalue_5)) (.R_Z (Utilities|Struct|BreakF_CSVdata _returnvalue_5)))))) (.Y (Math|Vector|BreakVector (+ (+ (Math|Vector|MakeVector (Math|Random|RandomFloatinRangefromStream (* (.X (Math|Vector|BreakVector (* (Variables|Default|GetRandom%20Rotation%20[XYZ]) (Math|Conversions|ToFloat(Boolean) (!= (- (Math|Conversions|ToInteger(Boolean) (Variables|Default|GetRotation%20clamped%20to%20Displacement)) 1) (.AXIS (Utilities|Struct|BreakF_CSVdata _returnvalue_5))))))) -1.0) (.X (Math|Vector|BreakVector (* (Variables|Default|GetRandom%20Rotation%20[XYZ]) (Math|Conversions|ToFloat(Boolean) (!= (- (Math|Conversions|ToInteger(Boolean) (Variables|Default|GetRotation%20clamped%20to%20Displacement)) 1) (.AXIS (Utilities|Struct|BreakF_CSVdata _returnvalue_5))))))) _displacement_randomize) (Math|Random|RandomFloatinRangefromStream (* (.Y (Math|Vector|BreakVector (* (Variables|Default|GetRandom%20Rotation%20[XYZ]) (Math|Conversions|ToFloat(Boolean) (!= (- (Math|Conversions|ToInteger(Boolean) (Variables|Default|GetRotation%20clamped%20to%20Displacement)) 1) (.AXIS (Utilities|Struct|BreakF_CSVdata _returnvalue_5))))))) -1.0) (.Y (Math|Vector|BreakVector (* (Variables|Default|GetRandom%20Rotation%20[XYZ]) (Math|Conversions|ToFloat(Boolean) (!= (- (Math|Conversions|ToInteger(Boolean) (Variables|Default|GetRotation%20clamped%20to%20Displacement)) 1) (.AXIS (Utilities|Struct|BreakF_CSVdata _returnvalue_5))))))) _displacement_randomize) (Math|Random|RandomFloatinRangefromStream (* (.Z (Math|Vector|BreakVector (* (Variables|Default|GetRandom%20Rotation%20[XYZ]) (Math|Conversions|ToFloat(Boolean) (!= (- (Math|Conversions|ToInteger(Boolean) (Variables|Default|GetRotation%20clamped%20to%20Displacement)) 1) (.AXIS (Utilities|Struct|BreakF_CSVdata _returnvalue_5))))))) -1.0) (.Z (Math|Vector|BreakVector (* (Variables|Default|GetRandom%20Rotation%20[XYZ]) (Math|Conversions|ToFloat(Boolean) (!= (- (Math|Conversions|ToInteger(Boolean) (Variables|Default|GetRotation%20clamped%20to%20Displacement)) 1) (.AXIS (Utilities|Struct|BreakF_CSVdata _returnvalue_5))))))) _displacement_randomize)) (Variables|Default|GetShuffle)) (Math|Vector|MakeVector (.R_X (Utilities|Struct|BreakF_CSVdata _returnvalue_5)) (.R_Y (Utilities|Struct|BreakF_CSVdata _returnvalue_5)) (.R_Z (Utilities|Struct|BreakF_CSVdata _returnvalue_5)))))) (.Z (Math|Vector|BreakVector (+ (+ (Math|Vector|MakeVector (Math|Random|RandomFloatinRangefromStream (* (.X (Math|Vector|BreakVector (* (Variables|Default|GetRandom%20Rotation%20[XYZ]) (Math|Conversions|ToFloat(Boolean) (!= (- (Math|Conversions|ToInteger(Boolean) (Variables|Default|GetRotation%20clamped%20to%20Displacement)) 1) (.AXIS (Utilities|Struct|BreakF_CSVdata _returnvalue_5))))))) -1.0) (.X (Math|Vector|BreakVector (* (Variables|Default|GetRandom%20Rotation%20[XYZ]) (Math|Conversions|ToFloat(Boolean) (!= (- (Math|Conversions|ToInteger(Boolean) (Variables|Default|GetRotation%20clamped%20to%20Displacement)) 1) (.AXIS (Utilities|Struct|BreakF_CSVdata _returnvalue_5))))))) _displacement_randomize) (Math|Random|RandomFloatinRangefromStream (* (.Y (Math|Vector|BreakVector (* (Variables|Default|GetRandom%20Rotation%20[XYZ]) (Math|Conversions|ToFloat(Boolean) (!= (- (Math|Conversions|ToInteger(Boolean) (Variables|Default|GetRotation%20clamped%20to%20Displacement)) 1) (.AXIS (Utilities|Struct|BreakF_CSVdata _returnvalue_5))))))) -1.0) (.Y (Math|Vector|BreakVector (* (Variables|Default|GetRandom%20Rotation%20[XYZ]) (Math|Conversions|ToFloat(Boolean) (!= (- (Math|Conversions|ToInteger(Boolean) (Variables|Default|GetRotation%20clamped%20to%20Displacement)) 1) (.AXIS (Utilities|Struct|BreakF_CSVdata _returnvalue_5))))))) _displacement_randomize) (Math|Random|RandomFloatinRangefromStream (* (.Z (Math|Vector|BreakVector (* (Variables|Default|GetRandom%20Rotation%20[XYZ]) (Math|Conversions|ToFloat(Boolean) (!= (- (Math|Conversions|ToInteger(Boolean) (Variables|Default|GetRotation%20clamped%20to%20Displacement)) 1) (.AXIS (Utilities|Struct|BreakF_CSVdata _returnvalue_5))))))) -1.0) (.Z (Math|Vector|BreakVector (* (Variables|Default|GetRandom%20Rotation%20[XYZ]) (Math|Conversions|ToFloat(Boolean) (!= (- (Math|Conversions|ToInteger(Boolean) (Variables|Default|GetRotation%20clamped%20to%20Displacement)) 1) (.AXIS (Utilities|Struct|BreakF_CSVdata _returnvalue_5))))))) _displacement_randomize)) (Variables|Default|GetShuffle)) (Math|Vector|MakeVector (.R_X (Utilities|Struct|BreakF_CSVdata _returnvalue_5)) (.R_Y (Utilities|Struct|BreakF_CSVdata _returnvalue_5)) (.R_Z (Utilities|Struct|BreakF_CSVdata _returnvalue_5))))))) (Math|Conversions|ToFloat(Boolean) (Variables|Default|GetRandom%20Rotation%20LOCAL/GLOBAL))) (* (Math|Vector|MakeVector (.S_X (Utilities|Struct|BreakF_CSVdata _returnvalue_5)) (.S_Y (Utilities|Struct|BreakF_CSVdata _returnvalue_5)) (.S_Z (Utilities|Struct|BreakF_CSVdata _returnvalue_5))) (Variables|Default|GetScale))) (* (Math|Vector|MakeVector (* (Math|Conversions|ToFloat(Boolean) (== (.AXIS (Utilities|Struct|BreakF_CSVdata _returnvalue_5)) 1)) _returnvalue_3) (* (Math|Conversions|ToFloat(Boolean) (== (.AXIS (Utilities|Struct|BreakF_CSVdata _returnvalue_5)) 2)) _returnvalue_3) (* (Math|Conversions|ToFloat(Boolean) (== (.AXIS (Utilities|Struct|BreakF_CSVdata _returnvalue_5)) 3)) _returnvalue_3)) (Math|Float|Clamp(Float) (+ (Math|Conversions|ToFloat(Boolean) (and (not (Class|KismetMathLibrary|IsPointinBoxwithTransform (Math|Vector|MakeVector (.T_X (Utilities|Struct|BreakF_CSVdata _returnvalue_5)) (.T_Y (Utilities|Struct|BreakF_CSVdata _returnvalue_5)) (.T_Z (Utilities|Struct|BreakF_CSVdata _returnvalue_5))) (Math|Transform|MakeTransform (Variables|Default|GetBox%20Origin%20[XYZ]) (Variables|Default|GetBox%20Rotation%20[XYZ])) (Variables|Default|GetBox%20Extent%20[XYZ]))) _boxcontrolleddisplacement)) (Variables|Default|GetBox%20Intensity)) (Math|Conversions|ToFloat(Boolean) (not _boxcontrolleddisplacement))))) (Math|Rotator|Lerp(Rotator) (Math|Rotator|CombineRotators (Math|Rotator|MakeRotator (.X (Math|Vector|BreakVector (+ (Math|Vector|MakeVector (Math|Random|RandomFloatinRangefromStream (* (.X (Math|Vector|BreakVector (* (Variables|Default|GetRandom%20Rotation%20[XYZ]) (Math|Conversions|ToFloat(Boolean) (!= (- (Math|Conversions|ToInteger(Boolean) (Variables|Default|GetRotation%20clamped%20to%20Displacement)) 1) (.AXIS (Utilities|Struct|BreakF_CSVdata _returnvalue_5))))))) -1.0) (.X (Math|Vector|BreakVector (* (Variables|Default|GetRandom%20Rotation%20[XYZ]) (Math|Conversions|ToFloat(Boolean) (!= (- (Math|Conversions|ToInteger(Boolean) (Variables|Default|GetRotation%20clamped%20to%20Displacement)) 1) (.AXIS (Utilities|Struct|BreakF_CSVdata _returnvalue_5))))))) _displacement_randomize) (Math|Random|RandomFloatinRangefromStream (* (.Y (Math|Vector|BreakVector (* (Variables|Default|GetRandom%20Rotation%20[XYZ]) (Math|Conversions|ToFloat(Boolean) (!= (- (Math|Conversions|ToInteger(Boolean) (Variables|Default|GetRotation%20clamped%20to%20Displacement)) 1) (.AXIS (Utilities|Struct|BreakF_CSVdata _returnvalue_5))))))) -1.0) (.Y (Math|Vector|BreakVector (* (Variables|Default|GetRandom%20Rotation%20[XYZ]) (Math|Conversions|ToFloat(Boolean) (!= (- (Math|Conversions|ToInteger(Boolean) (Variables|Default|GetRotation%20clamped%20to%20Displacement)) 1) (.AXIS (Utilities|Struct|BreakF_CSVdata _returnvalue_5))))))) _displacement_randomize) (Math|Random|RandomFloatinRangefromStream (* (.Z (Math|Vector|BreakVector (* (Variables|Default|GetRandom%20Rotation%20[XYZ]) (Math|Conversions|ToFloat(Boolean) (!= (- (Math|Conversions|ToInteger(Boolean) (Variables|Default|GetRotation%20clamped%20to%20Displacement)) 1) (.AXIS (Utilities|Struct|BreakF_CSVdata _returnvalue_5))))))) -1.0) (.Z (Math|Vector|BreakVector (* (Variables|Default|GetRandom%20Rotation%20[XYZ]) (Math|Conversions|ToFloat(Boolean) (!= (- (Math|Conversions|ToInteger(Boolean) (Variables|Default|GetRotation%20clamped%20to%20Displacement)) 1) (.AXIS (Utilities|Struct|BreakF_CSVdata _returnvalue_5))))))) _displacement_randomize)) (Variables|Default|GetShuffle)))) (.Y (Math|Vector|BreakVector (+ (Math|Vector|MakeVector (Math|Random|RandomFloatinRangefromStream (* (.X (Math|Vector|BreakVector (* (Variables|Default|GetRandom%20Rotation%20[XYZ]) (Math|Conversions|ToFloat(Boolean) (!= (- (Math|Conversions|ToInteger(Boolean) (Variables|Default|GetRotation%20clamped%20to%20Displacement)) 1) (.AXIS (Utilities|Struct|BreakF_CSVdata _returnvalue_5))))))) -1.0) (.X (Math|Vector|BreakVector (* (Variables|Default|GetRandom%20Rotation%20[XYZ]) (Math|Conversions|ToFloat(Boolean) (!= (- (Math|Conversions|ToInteger(Boolean) (Variables|Default|GetRotation%20clamped%20to%20Displacement)) 1) (.AXIS (Utilities|Struct|BreakF_CSVdata _returnvalue_5))))))) _displacement_randomize) (Math|Random|RandomFloatinRangefromStream (* (.Y (Math|Vector|BreakVector (* (Variables|Default|GetRandom%20Rotation%20[XYZ]) (Math|Conversions|ToFloat(Boolean) (!= (- (Math|Conversions|ToInteger(Boolean) (Variables|Default|GetRotation%20clamped%20to%20Displacement)) 1) (.AXIS (Utilities|Struct|BreakF_CSVdata _returnvalue_5))))))) -1.0) (.Y (Math|Vector|BreakVector (* (Variables|Default|GetRandom%20Rotation%20[XYZ]) (Math|Conversions|ToFloat(Boolean) (!= (- (Math|Conversions|ToInteger(Boolean) (Variables|Default|GetRotation%20clamped%20to%20Displacement)) 1) (.AXIS (Utilities|Struct|BreakF_CSVdata _returnvalue_5))))))) _displacement_randomize) (Math|Random|RandomFloatinRangefromStream (* (.Z (Math|Vector|BreakVector (* (Variables|Default|GetRandom%20Rotation%20[XYZ]) (Math|Conversions|ToFloat(Boolean) (!= (- (Math|Conversions|ToInteger(Boolean) (Variables|Default|GetRotation%20clamped%20to%20Displacement)) 1) (.AXIS (Utilities|Struct|BreakF_CSVdata _returnvalue_5))))))) -1.0) (.Z (Math|Vector|BreakVector (* (Variables|Default|GetRandom%20Rotation%20[XYZ]) (Math|Conversions|ToFloat(Boolean) (!= (- (Math|Conversions|ToInteger(Boolean) (Variables|Default|GetRotation%20clamped%20to%20Displacement)) 1) (.AXIS (Utilities|Struct|BreakF_CSVdata _returnvalue_5))))))) _displacement_randomize)) (Variables|Default|GetShuffle)))) (.Z (Math|Vector|BreakVector (+ (Math|Vector|MakeVector (Math|Random|RandomFloatinRangefromStream (* (.X (Math|Vector|BreakVector (* (Variables|Default|GetRandom%20Rotation%20[XYZ]) (Math|Conversions|ToFloat(Boolean) (!= (- (Math|Conversions|ToInteger(Boolean) (Variables|Default|GetRotation%20clamped%20to%20Displacement)) 1) (.AXIS (Utilities|Struct|BreakF_CSVdata _returnvalue_5))))))) -1.0) (.X (Math|Vector|BreakVector (* (Variables|Default|GetRandom%20Rotation%20[XYZ]) (Math|Conversions|ToFloat(Boolean) (!= (- (Math|Conversions|ToInteger(Boolean) (Variables|Default|GetRotation%20clamped%20to%20Displacement)) 1) (.AXIS (Utilities|Struct|BreakF_CSVdata _returnvalue_5))))))) _displacement_randomize) (Math|Random|RandomFloatinRangefromStream (* (.Y (Math|Vector|BreakVector (* (Variables|Default|GetRandom%20Rotation%20[XYZ]) (Math|Conversions|ToFloat(Boolean) (!= (- (Math|Conversions|ToInteger(Boolean) (Variables|Default|GetRotation%20clamped%20to%20Displacement)) 1) (.AXIS (Utilities|Struct|BreakF_CSVdata _returnvalue_5))))))) -1.0) (.Y (Math|Vector|BreakVector (* (Variables|Default|GetRandom%20Rotation%20[XYZ]) (Math|Conversions|ToFloat(Boolean) (!= (- (Math|Conversions|ToInteger(Boolean) (Variables|Default|GetRotation%20clamped%20to%20Displacement)) 1) (.AXIS (Utilities|Struct|BreakF_CSVdata _returnvalue_5))))))) _displacement_randomize) (Math|Random|RandomFloatinRangefromStream (* (.Z (Math|Vector|BreakVector (* (Variables|Default|GetRandom%20Rotation%20[XYZ]) (Math|Conversions|ToFloat(Boolean) (!= (- (Math|Conversions|ToInteger(Boolean) (Variables|Default|GetRotation%20clamped%20to%20Displacement)) 1) (.AXIS (Utilities|Struct|BreakF_CSVdata _returnvalue_5))))))) -1.0) (.Z (Math|Vector|BreakVector (* (Variables|Default|GetRandom%20Rotation%20[XYZ]) (Math|Conversions|ToFloat(Boolean) (!= (- (Math|Conversions|ToInteger(Boolean) (Variables|Default|GetRotation%20clamped%20to%20Displacement)) 1) (.AXIS (Utilities|Struct|BreakF_CSVdata _returnvalue_5))))))) _displacement_randomize)) (Variables|Default|GetShuffle))))) (Math|Rotator|MakeRotator (.R_X (Utilities|Struct|BreakF_CSVdata _returnvalue_5)) (.R_Y (Utilities|Struct|BreakF_CSVdata _returnvalue_5)) (.R_Z (Utilities|Struct|BreakF_CSVdata _returnvalue_5)))) (Math|Rotator|MakeRotator (.X (Math|Vector|BreakVector (+ (+ (Math|Vector|MakeVector (Math|Random|RandomFloatinRangefromStream (* (.X (Math|Vector|BreakVector (* (Variables|Default|GetRandom%20Rotation%20[XYZ]) (Math|Conversions|ToFloat(Boolean) (!= (- (Math|Conversions|ToInteger(Boolean) (Variables|Default|GetRotation%20clamped%20to%20Displacement)) 1) (.AXIS (Utilities|Struct|BreakF_CSVdata _returnvalue_5))))))) -1.0) (.X (Math|Vector|BreakVector (* (Variables|Default|GetRandom%20Rotation%20[XYZ]) (Math|Conversions|ToFloat(Boolean) (!= (- (Math|Conversions|ToInteger(Boolean) (Variables|Default|GetRotation%20clamped%20to%20Displacement)) 1) (.AXIS (Utilities|Struct|BreakF_CSVdata _returnvalue_5))))))) _displacement_randomize) (Math|Random|RandomFloatinRangefromStream (* (.Y (Math|Vector|BreakVector (* (Variables|Default|GetRandom%20Rotation%20[XYZ]) (Math|Conversions|ToFloat(Boolean) (!= (- (Math|Conversions|ToInteger(Boolean) (Variables|Default|GetRotation%20clamped%20to%20Displacement)) 1) (.AXIS (Utilities|Struct|BreakF_CSVdata _returnvalue_5))))))) -1.0) (.Y (Math|Vector|BreakVector (* (Variables|Default|GetRandom%20Rotation%20[XYZ]) (Math|Conversions|ToFloat(Boolean) (!= (- (Math|Conversions|ToInteger(Boolean) (Variables|Default|GetRotation%20clamped%20to%20Displacement)) 1) (.AXIS (Utilities|Struct|BreakF_CSVdata _returnvalue_5))))))) _displacement_randomize) (Math|Random|RandomFloatinRangefromStream (* (.Z (Math|Vector|BreakVector (* (Variables|Default|GetRandom%20Rotation%20[XYZ]) (Math|Conversions|ToFloat(Boolean) (!= (- (Math|Conversions|ToInteger(Boolean) (Variables|Default|GetRotation%20clamped%20to%20Displacement)) 1) (.AXIS (Utilities|Struct|BreakF_CSVdata _returnvalue_5))))))) -1.0) (.Z (Math|Vector|BreakVector (* (Variables|Default|GetRandom%20Rotation%20[XYZ]) (Math|Conversions|ToFloat(Boolean) (!= (- (Math|Conversions|ToInteger(Boolean) (Variables|Default|GetRotation%20clamped%20to%20Displacement)) 1) (.AXIS (Utilities|Struct|BreakF_CSVdata _returnvalue_5))))))) _displacement_randomize)) (Variables|Default|GetShuffle)) (Math|Vector|MakeVector (.R_X (Utilities|Struct|BreakF_CSVdata _returnvalue_5)) (.R_Y (Utilities|Struct|BreakF_CSVdata _returnvalue_5)) (.R_Z (Utilities|Struct|BreakF_CSVdata _returnvalue_5)))))) (.Y (Math|Vector|BreakVector (+ (+ (Math|Vector|MakeVector (Math|Random|RandomFloatinRangefromStream (* (.X (Math|Vector|BreakVector (* (Variables|Default|GetRandom%20Rotation%20[XYZ]) (Math|Conversions|ToFloat(Boolean) (!= (- (Math|Conversions|ToInteger(Boolean) (Variables|Default|GetRotation%20clamped%20to%20Displacement)) 1) (.AXIS (Utilities|Struct|BreakF_CSVdata _returnvalue_5))))))) -1.0) (.X (Math|Vector|BreakVector (* (Variables|Default|GetRandom%20Rotation%20[XYZ]) (Math|Conversions|ToFloat(Boolean) (!= (- (Math|Conversions|ToInteger(Boolean) (Variables|Default|GetRotation%20clamped%20to%20Displacement)) 1) (.AXIS (Utilities|Struct|BreakF_CSVdata _returnvalue_5))))))) _displacement_randomize) (Math|Random|RandomFloatinRangefromStream (* (.Y (Math|Vector|BreakVector (* (Variables|Default|GetRandom%20Rotation%20[XYZ]) (Math|Conversions|ToFloat(Boolean) (!= (- (Math|Conversions|ToInteger(Boolean) (Variables|Default|GetRotation%20clamped%20to%20Displacement)) 1) (.AXIS (Utilities|Struct|BreakF_CSVdata _returnvalue_5))))))) -1.0) (.Y (Math|Vector|BreakVector (* (Variables|Default|GetRandom%20Rotation%20[XYZ]) (Math|Conversions|ToFloat(Boolean) (!= (- (Math|Conversions|ToInteger(Boolean) (Variables|Default|GetRotation%20clamped%20to%20Displacement)) 1) (.AXIS (Utilities|Struct|BreakF_CSVdata _returnvalue_5))))))) _displacement_randomize) (Math|Random|RandomFloatinRangefromStream (* (.Z (Math|Vector|BreakVector (* (Variables|Default|GetRandom%20Rotation%20[XYZ]) (Math|Conversions|ToFloat(Boolean) (!= (- (Math|Conversions|ToInteger(Boolean) (Variables|Default|GetRotation%20clamped%20to%20Displacement)) 1) (.AXIS (Utilities|Struct|BreakF_CSVdata _returnvalue_5))))))) -1.0) (.Z (Math|Vector|BreakVector (* (Variables|Default|GetRandom%20Rotation%20[XYZ]) (Math|Conversions|ToFloat(Boolean) (!= (- (Math|Conversions|ToInteger(Boolean) (Variables|Default|GetRotation%20clamped%20to%20Displacement)) 1) (.AXIS (Utilities|Struct|BreakF_CSVdata _returnvalue_5))))))) _displacement_randomize)) (Variables|Default|GetShuffle)) (Math|Vector|MakeVector (.R_X (Utilities|Struct|BreakF_CSVdata _returnvalue_5)) (.R_Y (Utilities|Struct|BreakF_CSVdata _returnvalue_5)) (.R_Z (Utilities|Struct|BreakF_CSVdata _returnvalue_5)))))) (.Z (Math|Vector|BreakVector (+ (+ (Math|Vector|MakeVector (Math|Random|RandomFloatinRangefromStream (* (.X (Math|Vector|BreakVector (* (Variables|Default|GetRandom%20Rotation%20[XYZ]) (Math|Conversions|ToFloat(Boolean) (!= (- (Math|Conversions|ToInteger(Boolean) (Variables|Default|GetRotation%20clamped%20to%20Displacement)) 1) (.AXIS (Utilities|Struct|BreakF_CSVdata _returnvalue_5))))))) -1.0) (.X (Math|Vector|BreakVector (* (Variables|Default|GetRandom%20Rotation%20[XYZ]) (Math|Conversions|ToFloat(Boolean) (!= (- (Math|Conversions|ToInteger(Boolean) (Variables|Default|GetRotation%20clamped%20to%20Displacement)) 1) (.AXIS (Utilities|Struct|BreakF_CSVdata _returnvalue_5))))))) _displacement_randomize) (Math|Random|RandomFloatinRangefromStream (* (.Y (Math|Vector|BreakVector (* (Variables|Default|GetRandom%20Rotation%20[XYZ]) (Math|Conversions|ToFloat(Boolean) (!= (- (Math|Conversions|ToInteger(Boolean) (Variables|Default|GetRotation%20clamped%20to%20Displacement)) 1) (.AXIS (Utilities|Struct|BreakF_CSVdata _returnvalue_5))))))) -1.0) (.Y (Math|Vector|BreakVector (* (Variables|Default|GetRandom%20Rotation%20[XYZ]) (Math|Conversions|ToFloat(Boolean) (!= (- (Math|Conversions|ToInteger(Boolean) (Variables|Default|GetRotation%20clamped%20to%20Displacement)) 1) (.AXIS (Utilities|Struct|BreakF_CSVdata _returnvalue_5))))))) _displacement_randomize) (Math|Random|RandomFloatinRangefromStream (* (.Z (Math|Vector|BreakVector (* (Variables|Default|GetRandom%20Rotation%20[XYZ]) (Math|Conversions|ToFloat(Boolean) (!= (- (Math|Conversions|ToInteger(Boolean) (Variables|Default|GetRotation%20clamped%20to%20Displacement)) 1) (.AXIS (Utilities|Struct|BreakF_CSVdata _returnvalue_5))))))) -1.0) (.Z (Math|Vector|BreakVector (* (Variables|Default|GetRandom%20Rotation%20[XYZ]) (Math|Conversions|ToFloat(Boolean) (!= (- (Math|Conversions|ToInteger(Boolean) (Variables|Default|GetRotation%20clamped%20to%20Displacement)) 1) (.AXIS (Utilities|Struct|BreakF_CSVdata _returnvalue_5))))))) _displacement_randomize)) (Variables|Default|GetShuffle)) (Math|Vector|MakeVector (.R_X (Utilities|Struct|BreakF_CSVdata _returnvalue_5)) (.R_Y (Utilities|Struct|BreakF_CSVdata _returnvalue_5)) (.R_Z (Utilities|Struct|BreakF_CSVdata _returnvalue_5))))))) (Math|Conversions|ToFloat(Boolean) (Variables|Default|GetRandom%20Rotation%20LOCAL/GLOBAL))) (* (Math|Vector|MakeVector (.S_X (Utilities|Struct|BreakF_CSVdata _returnvalue_5)) (.S_Y (Utilities|Struct|BreakF_CSVdata _returnvalue_5)) (.S_Z (Utilities|Struct|BreakF_CSVdata _returnvalue_5))) (Variables|Default|GetScale))) false)))))))))))))))