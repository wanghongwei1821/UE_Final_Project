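; Stone bridge actor that assembles itself in the construction script from modular stone meshes laid out in a data table.
; It creates an invisible extra-collision mesh and seventeen hierarchical instanced static mesh components sharing one stone material.
; Each row of ObjectDAT selects a component and mesh by ID and adds a local-space instance from its stored location, rotation and scale, using instancing for the repeated pieces.
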(fn ConstructionScript
  (bind _object_dat (Variables|Default|GetObject%20DAT))
  (bind _returnvalue (AddComponent|AddStaticMeshComponent false))
  (Components|StaticMesh|SetStaticMesh _returnvalue (Variables|Default|GetExtra%20Collision))
  (Rendering|SetVisibility _returnvalue false false)
  (bind _returnvalue_2 (AddComponent|AddHierarchicalInstancedStaticMeshComponent false))
  (bind _output_get (Variables|Default|Set01 _returnvalue_2))
  (Rendering|Material|SetMaterial _output_get 0 (Variables|Default|GetStoneMaterial))
  (bind _returnvalue_3 (AddComponent|AddHierarchicalInstancedStaticMeshComponent false))
  (bind _output_get_2 (Variables|Default|Set02 _returnvalue_3))
  (Rendering|Material|SetMaterial _output_get_2 0 (Variables|Default|GetStoneMaterial))
  (bind _returnvalue_4 (AddComponent|AddHierarchicalInstancedStaticMeshComponent false))
  (bind _output_get_3 (Variables|Default|Set03 _returnvalue_4))
  (Rendering|Material|SetMaterial _output_get_3 0 (Variables|Default|GetStoneMaterial))
  (bind _returnvalue_5 (AddComponent|AddHierarchicalInstancedStaticMeshComponent false))
  (bind _output_get_4 (Variables|Default|Set04 _returnvalue_5))
  (Rendering|Material|SetMaterial _output_get_4 0 (Variables|Default|GetStoneMaterial))
  (bind _returnvalue_6 (AddComponent|AddHierarchicalInstancedStaticMeshComponent false))
  (bind _output_get_5 (Variables|Default|Set05 _returnvalue_6))
  (Rendering|Material|SetMaterial _output_get_5 0 (Variables|Default|GetStoneMaterial))
  (bind _returnvalue_7 (AddComponent|AddHierarchicalInstancedStaticMeshComponent false))
  (bind _output_get_6 (Variables|Default|Set06 _returnvalue_7))
  (Rendering|Material|SetMaterial _output_get_6 0 (Variables|Default|GetStoneMaterial))
  (bind _returnvalue_8 (AddComponent|AddHierarchicalInstancedStaticMeshComponent false))
  (bind _output_get_7 (Variables|Default|Set07 _returnvalue_8))
  (Rendering|Material|SetMaterial _output_get_7 0 (Variables|Default|GetStoneMaterial))
  (bind _returnvalue_9 (AddComponent|AddHierarchicalInstancedStaticMeshComponent false))
  (bind _output_get_8 (Variables|Default|Set08 _returnvalue_9))
  (Rendering|Material|SetMaterial _output_get_8 0 (Variables|Default|GetStoneMaterial))
  (bind _returnvalue_10 (AddComponent|AddHierarchicalInstancedStaticMeshComponent false))
  (bind _output_get_9 (Variables|Default|Set09 _returnvalue_10))
  (Rendering|Material|SetMaterial _output_get_9 0 (Variables|Default|GetStoneMaterial))
  (bind _returnvalue_11 (AddComponent|AddHierarchicalInstancedStaticMeshComponent false))
  (bind _output_get_10 (Variables|Default|Set10 _returnvalue_11))
  (Rendering|Material|SetMaterial _output_get_10 0 (Variables|Default|GetStoneMaterial))
  (bind _returnvalue_12 (AddComponent|AddHierarchicalInstancedStaticMeshComponent false))
  (bind _output_get_11 (Variables|Default|Set11 _returnvalue_12))
  (Rendering|Material|SetMaterial _output_get_11 0 (Variables|Default|GetStoneMaterial))
  (bind _returnvalue_13 (AddComponent|AddHierarchicalInstancedStaticMeshComponent false))
  (bind _output_get_12 (Variables|Default|Set12 _returnvalue_13))
  (Rendering|Material|SetMaterial _output_get_12 0 (Variables|Default|GetStoneMaterial))
  (bind _returnvalue_14 (AddComponent|AddHierarchicalInstancedStaticMeshComponent false))
  (bind _output_get_13 (Variables|Default|Set13 _returnvalue_14))
  (Rendering|Material|SetMaterial _output_get_13 0 (Variables|Default|GetStoneMaterial))
  (bind _returnvalue_15 (AddComponent|AddHierarchicalInstancedStaticMeshComponent false))
  (bind _output_get_14 (Variables|Default|Set14 _returnvalue_15))
  (Rendering|Material|SetMaterial _output_get_14 0 (Variables|Default|GetStoneMaterial))
  (bind _returnvalue_16 (AddComponent|AddHierarchicalInstancedStaticMeshComponent false))
  (bind _output_get_15 (Variables|Default|Set15 _returnvalue_16))
  (Rendering|Material|SetMaterial _output_get_15 0 (Variables|Default|GetStoneMaterial))
  (bind _returnvalue_17 (AddComponent|AddHierarchicalInstancedStaticMeshComponent false))
  (bind _output_get_16 (Variables|Default|Set16 _returnvalue_17))
  (Rendering|Material|SetMaterial _output_get_16 0 (Variables|Default|GetStoneMaterial))
  (bind _returnvalue_18 (AddComponent|AddHierarchicalInstancedStaticMeshComponent false))
  (bind _output_get_17 (Variables|Default|Set17 _returnvalue_18))
  (Rendering|Material|SetMaterial _output_get_17 0 (Variables|Default|GetStoneMaterial))
  (bind _outrownames (DataTable|GetDataTableRowNames _object_dat))
  (for _array_element _outrownames
    (bind _returnvalue_19 (Utilities|GetDataTableRow _object_dat _array_element)
      (:then
        (if (== (.ID (Utilities|Struct|BreakF_CSVdata _returnvalue_19)) 1)
          (Components|StaticMesh|SetStaticMesh (Variables|Default|Get01) (Variables|Default|GetMesh_01))
          (Components|InstancedStaticMesh|AddInstance (Variables|Default|Get01) (Math|Transform|MakeTransform (Math|Vector|MakeVector (.T_X (Utilities|Struct|BreakF_CSVdata _returnvalue_19)) (.T_Y (Utilities|Struct|BreakF_CSVdata _returnvalue_19)) (.T_Z (Utilities|Struct|BreakF_CSVdata _returnvalue_19))) (Math|Rotator|MakeRotator (.R_X (Utilities|Struct|BreakF_CSVdata _returnvalue_19)) (.R_Y (Utilities|Struct|BreakF_CSVdata _returnvalue_19)) (.R_Z (Utilities|Struct|BreakF_CSVdata _returnvalue_19))) (Math|Vector|MakeVector (.S_X (Utilities|Struct|BreakF_CSVdata _returnvalue_19)) (.S_Y (Utilities|Struct|BreakF_CSVdata _returnvalue_19)) (.S_Z (Utilities|Struct|BreakF_CSVdata _returnvalue_19)))) false)
          (elif (== (.ID (Utilities|Struct|BreakF_CSVdata _returnvalue_19)) 2)
            (Components|StaticMesh|SetStaticMesh (Variables|Default|Get02) (Variables|Default|GetMesh_02))
            (Components|InstancedStaticMesh|AddInstance (Variables|Default|Get02) (Math|Transform|MakeTransform (Math|Vector|MakeVector (.T_X (Utilities|Struct|BreakF_CSVdata _returnvalue_19)) (.T_Y (Utilities|Struct|BreakF_CSVdata _returnvalue_19)) (.T_Z (Utilities|Struct|BreakF_CSVdata _returnvalue_19))) (Math|Rotator|MakeRotator (.R_X (Utilities|Struct|BreakF_CSVdata _returnvalue_19)) (.R_Y (Utilities|Struct|BreakF_CSVdata _returnvalue_19)) (.R_Z (Utilities|Struct|BreakF_CSVdata _returnvalue_19))) (Math|Vector|MakeVector (.S_X (Utilities|Struct|BreakF_CSVdata _returnvalue_19)) (.S_Y (Utilities|Struct|BreakF_CSVdata _returnvalue_19)) (.S_Z (Utilities|Struct|BreakF_CSVdata _returnvalue_19)))) false)
            (elif (== (.ID (Utilities|Struct|BreakF_CSVdata _returnvalue_19)) 3)
              (Components|StaticMesh|SetStaticMesh (Variables|Default|Get03) (Variables|Default|GetMesh_03))
              (Components|InstancedStaticMesh|AddInstance (Variables|Default|Get03) (Math|Transform|MakeTransform (Math|Vector|MakeVector (.T_X (Utilities|Struct|BreakF_CSVdata _returnvalue_19)) (.T_Y (Utilities|Struct|BreakF_CSVdata _returnvalue_19)) (.T_Z (Utilities|Struct|BreakF_CSVdata _returnvalue_19))) (Math|Rotator|MakeRotator (.R_X (Utilities|Struct|BreakF_CSVdata _returnvalue_19)) (.R_Y (Utilities|Struct|BreakF_CSVdata _returnvalue_19)) (.R_Z (Utilities|Struct|BreakF_CSVdata _returnvalue_19))) (Math|Vector|MakeVector (.S_X (Utilities|Struct|BreakF_CSVdata _returnvalue_19)) (.S_Y (Utilities|Struct|BreakF_CSVdata _returnvalue_19)) (.S_Z (Utilities|Struct|BreakF_CSVdata _returnvalue_19)))) false)
              (elif (== (.ID (Utilities|Struct|BreakF_CSVdata _returnvalue_19)) 4)
                (Components|StaticMesh|SetStaticMesh (Variables|Default|Get04) (Variables|Default|GetMesh_04))
                (Components|InstancedStaticMesh|AddInstance (Variables|Default|Get04) (Math|Transform|MakeTransform (Math|Vector|MakeVector (.T_X (Utilities|Struct|BreakF_CSVdata _returnvalue_19)) (.T_Y (Utilities|Struct|BreakF_CSVdata _returnvalue_19)) (.T_Z (Utilities|Struct|BreakF_CSVdata _returnvalue_19))) (Math|Rotator|MakeRotator (.R_X (Utilities|Struct|BreakF_CSVdata _returnvalue_19)) (.R_Y (Utilities|Struct|BreakF_CSVdata _returnvalue_19)) (.R_Z (Utilities|Struct|BreakF_CSVdata _returnvalue_19))) (Math|Vector|MakeVector (.S_X (Utilities|Struct|BreakF_CSVdata _returnvalue_19)) (.S_Y (Utilities|Struct|BreakF_CSVdata _returnvalue_19)) (.S_Z (Utilities|Struct|BreakF_CSVdata _returnvalue_19)))) false)
                (elif (== (.ID (Utilities|Struct|BreakF_CSVdata _returnvalue_19)) 5)
                  (Components|StaticMesh|SetStaticMesh (Variables|Default|Get05) (Variables|Default|GetMesh_05))
                  (Components|InstancedStaticMesh|AddInstance (Variables|Default|Get05) (Math|Transform|MakeTransform (Math|Vector|MakeVector (.T_X (Utilities|Struct|BreakF_CSVdata _returnvalue_19)) (.T_Y (Utilities|Struct|BreakF_CSVdata _returnvalue_19)) (.T_Z (Utilities|Struct|BreakF_CSVdata _returnvalue_19))) (Math|Rotator|MakeRotator (.R_X (Utilities|Struct|BreakF_CSVdata _returnvalue_19)) (.R_Y (Utilities|Struct|BreakF_CSVdata _returnvalue_19)) (.R_Z (Utilities|Struct|BreakF_CSVdata _returnvalue_19))) (Math|Vector|MakeVector (.S_X (Utilities|Struct|BreakF_CSVdata _returnvalue_19)) (.S_Y (Utilities|Struct|BreakF_CSVdata _returnvalue_19)) (.S_Z (Utilities|Struct|BreakF_CSVdata _returnvalue_19)))) false)
                  (elif (== (.ID (Utilities|Struct|BreakF_CSVdata _returnvalue_19)) 6)
                    (Components|StaticMesh|SetStaticMesh (Variables|Default|Get06) (Variables|Default|GetMesh_06))
                    (Components|InstancedStaticMesh|AddInstance (Variables|Default|Get06) (Math|Transform|MakeTransform (Math|Vector|MakeVector (.T_X (Utilities|Struct|BreakF_CSVdata _returnvalue_19)) (.T_Y (Utilities|Struct|BreakF_CSVdata _returnvalue_19)) (.T_Z (Utilities|Struct|BreakF_CSVdata _returnvalue_19))) (Math|Rotator|MakeRotator (.R_X (Utilities|Struct|BreakF_CSVdata _returnvalue_19)) (.R_Y (Utilities|Struct|BreakF_CSVdata _returnvalue_19)) (.R_Z (Utilities|Struct|BreakF_CSVdata _returnvalue_19))) (Math|Vector|MakeVector (.S_X (Utilities|Struct|BreakF_CSVdata _returnvalue_19)) (.S_Y (Utilities|Struct|BreakF_CSVdata _returnvalue_19)) (.S_Z (Utilities|Struct|BreakF_CSVdata _returnvalue_19)))) false)
                    (elif (== (.ID (Utilities|Struct|BreakF_CSVdata _returnvalue_19)) 7)
                      (Components|StaticMesh|SetStaticMesh (Variables|Default|Get07) (Variables|Default|GetMesh_07))
                      (Components|InstancedStaticMesh|AddInstance (Variables|Default|Get07) (Math|Transform|MakeTransform (Math|Vector|MakeVector (.T_X (Utilities|Struct|BreakF_CSVdata _returnvalue_19)) (.T_Y (Utilities|Struct|BreakF_CSVdata _returnvalue_19)) (.T_Z (Utilities|Struct|BreakF_CSVdata _returnvalue_19))) (Math|Rotator|MakeRotator (.R_X (Utilities|Struct|BreakF_CSVdata _returnvalue_19)) (.R_Y (Utilities|Struct|BreakF_CSVdata _returnvalue_19)) (.R_Z (Utilities|Struct|BreakF_CSVdata _returnvalue_19))) (Math|Vector|MakeVector (.S_X (Utilities|Struct|BreakF_CSVdata _returnvalue_19)) (.S_Y (Utilities|Struct|BreakF_CSVdata _returnvalue_19)) (.S_Z (Utilities|Struct|BreakF_CSVdata _returnvalue_19)))) false)
                      (elif (== (.ID (Utilities|Struct|BreakF_CSVdata _returnvalue_19)) 8)
                        (Components|StaticMesh|SetStaticMesh (Variables|Default|Get08) (Variables|Default|GetMesh_08))
                        (Components|InstancedStaticMesh|AddInstance (Variables|Default|Get08) (Math|Transform|MakeTransform (Math|Vector|MakeVector (.T_X (Utilities|Struct|BreakF_CSVdata _returnvalue_19)) (.T_Y (Utilities|Struct|BreakF_CSVdata _returnvalue_19)) (.T_Z (Utilities|Struct|BreakF_CSVdata _returnvalue_19))) (Math|Rotator|MakeRotator (.R_X (Utilities|Struct|BreakF_CSVdata _returnvalue_19)) (.R_Y (Utilities|Struct|BreakF_CSVdata _returnvalue_19)) (.R_Z (Utilities|Struct|BreakF_CSVdata _returnvalue_19))) (Math|Vector|MakeVector (.S_X (Utilities|Struct|BreakF_CSVdata _returnvalue_19)) (.S_Y (Utilities|Struct|BreakF_CSVdata _returnvalue_19)) (.S_Z (Utilities|Struct|BreakF_CSVdata _returnvalue_19)))) false)
                        (elif (== (.ID (Utilities|Struct|BreakF_CSVdata _returnvalue_19)) 9)
                          (Components|StaticMesh|SetStaticMesh (Variables|Default|Get09) (Variables|Default|GetMesh_09))
                          (Components|InstancedStaticMesh|AddInstance (Variables|Default|Get09) (Math|Transform|MakeTransform (Math|Vector|MakeVector (.T_X (Utilities|Struct|BreakF_CSVdata _returnvalue_19)) (.T_Y (Utilities|Struct|BreakF_CSVdata _returnvalue_19)) (.T_Z (Utilities|Struct|BreakF_CSVdata _returnvalue_19))) (Math|Rotator|MakeRotator (.R_X (Utilities|Struct|BreakF_CSVdata _returnvalue_19)) (.R_Y (Utilities|Struct|BreakF_CSVdata _returnvalue_19)) (.R_Z (Utilities|Struct|BreakF_CSVdata _returnvalue_19))) (Math|Vector|MakeVector (.S_X (Utilities|Struct|BreakF_CSVdata _returnvalue_19)) (.S_Y (Utilities|Struct|BreakF_CSVdata _returnvalue_19)) (.S_Z (Utilities|Struct|BreakF_CSVdata _returnvalue_19)))) false)
                          (elif (== (.ID (Utilities|Struct|BreakF_CSVdata _returnvalue_19)) 10)
                            (Components|StaticMesh|SetStaticMesh (Variables|Default|Get10) (Variables|Default|GetMesh_10))
                            (Components|InstancedStaticMesh|AddInstance (Variables|Default|Get10) (Math|Transform|MakeTransform (Math|Vector|MakeVector (.T_X (Utilities|Struct|BreakF_CSVdata _returnvalue_19)) (.T_Y (Utilities|Struct|BreakF_CSVdata _returnvalue_19)) (.T_Z (Utilities|Struct|BreakF_CSVdata _returnvalue_19))) (Math|Rotator|MakeRotator (.R_X (Utilities|Struct|BreakF_CSVdata _returnvalue_19)) (.R_Y (Utilities|Struct|BreakF_CSVdata _returnvalue_19)) (.R_Z (Utilities|Struct|BreakF_CSVdata _returnvalue_19))) (Math|Vector|MakeVector (.S_X (Utilities|Struct|BreakF_CSVdata _returnvalue_19)) (.S_Y (Utilities|Struct|BreakF_CSVdata _returnvalue_19)) (.S_Z (Utilities|Struct|BreakF_CSVdata _returnvalue_19)))) false)
                            (elif (== (.ID (Utilities|Struct|BreakF_CSVdata _returnvalue_19)) 11)
                              (Components|StaticMesh|SetStaticMesh (Variables|Default|Get11) (Variables|Default|GetMesh_11))
                              (Components|InstancedStaticMesh|AddInstance (Variables|Default|Get11) (Math|Transform|MakeTransform (Math|Vector|MakeVector (.T_X (Utilities|Struct|BreakF_CSVdata _returnvalue_19)) (.T_Y (Utilities|Struct|BreakF_CSVdata _returnvalue_19)) (.T_Z (Utilities|Struct|BreakF_CSVdata _returnvalue_19))) (Math|Rotator|MakeRotator (.R_X (Utilities|Struct|BreakF_CSVdata _returnvalue_19)) (.R_Y (Utilities|Struct|BreakF_CSVdata _returnvalue_19)) (.R_Z (Utilities|Struct|BreakF_CSVdata _returnvalue_19))) (Math|Vector|MakeVector (.S_X (Utilities|Struct|BreakF_CSVdata _returnvalue_19)) (.S_Y (Utilities|Struct|BreakF_CSVdata _returnvalue_19)) (.S_Z (Utilities|Struct|BreakF_CSVdata _returnvalue_19)))) false)
                              (elif (== (.ID (Utilities|Struct|BreakF_CSVdata _returnvalue_19)) 12)
                                (Components|StaticMesh|SetStaticMesh (Variables|Default|Get12) (Variables|Default|GetMesh_12))
                                (Components|InstancedStaticMesh|AddInstance (Variables|Default|Get12) (Math|Transform|MakeTransform (Math|Vector|MakeVector (.T_X (Utilities|Struct|BreakF_CSVdata _returnvalue_19)) (.T_Y (Utilities|Struct|BreakF_CSVdata _returnvalue_19)) (.T_Z (Utilities|Struct|BreakF_CSVdata _returnvalue_19))) (Math|Rotator|MakeRotator (.R_X (Utilities|Struct|BreakF_CSVdata _returnvalue_19)) (.R_Y (Utilities|Struct|BreakF_CSVdata _returnvalue_19)) (.R_Z (Utilities|Struct|BreakF_CSVdata _returnvalue_19))) (Math|Vector|MakeVector (.S_X (Utilities|Struct|BreakF_CSVdata _returnvalue_19)) (.S_Y (Utilities|Struct|BreakF_CSVdata _returnvalue_19)) (.S_Z (Utilities|Struct|BreakF_CSVdata _returnvalue_19)))) false)
                                (elif (== (.ID (Utilities|Struct|BreakF_CSVdata _returnvalue_19)) 13)
                                  (Components|StaticMesh|SetStaticMesh (Variables|Default|Get13) (Variables|Default|GetMesh_13))
                                  (Components|InstancedStaticMesh|AddInstance (Variables|Default|Get13) (Math|Transform|MakeTransform (Math|Vector|MakeVector (.T_X (Utilities|Struct|BreakF_CSVdata _returnvalue_19)) (.T_Y (Utilities|Struct|BreakF_CSVdata _returnvalue_19)) (.T_Z (Utilities|Struct|BreakF_CSVdata _returnvalue_19))) (Math|Rotator|MakeRotator (.R_X (Utilities|Struct|BreakF_CSVdata _returnvalue_19)) (.R_Y (Utilities|Struct|BreakF_CSVdata _returnvalue_19)) (.R_Z (Utilities|Struct|BreakF_CSVdata _returnvalue_19))) (Math|Vector|MakeVector (.S_X (Utilities|Struct|BreakF_CSVdata _returnvalue_19)) (.S_Y (Utilities|Struct|BreakF_CSVdata _returnvalue_19)) (.S_Z (Utilities|Struct|BreakF_CSVdata _returnvalue_19)))) false)
                                  (elif (== (.ID (Utilities|Struct|BreakF_CSVdata _returnvalue_19)) 14)
                                    (Components|StaticMesh|SetStaticMesh (Variables|Default|Get14) (Variables|Default|GetMesh_14))
                                    (Components|InstancedStaticMesh|AddInstance (Variables|Default|Get14) (Math|Transform|MakeTransform (Math|Vector|MakeVector (.T_X (Utilities|Struct|BreakF_CSVdata _returnvalue_19)) (.T_Y (Utilities|Struct|BreakF_CSVdata _returnvalue_19)) (.T_Z (Utilities|Struct|BreakF_CSVdata _returnvalue_19))) (Math|Rotator|MakeRotator (.R_X (Utilities|Struct|BreakF_CSVdata _returnvalue_19)) (.R_Y (Utilities|Struct|BreakF_CSVdata _returnvalue_19)) (.R_Z (Utilities|Struct|BreakF_CSVdata _returnvalue_19))) (Math|Vector|MakeVector (.S_X (Utilities|Struct|BreakF_CSVdata _returnvalue_19)) (.S_Y (Utilities|Struct|BreakF_CSVdata _returnvalue_19)) (.S_Z (Utilities|Struct|BreakF_CSVdata _returnvalue_19)))) false)
                                    (elif (== (.ID (Utilities|Struct|BreakF_CSVdata _returnvalue_19)) 15)
                                      (Components|StaticMesh|SetStaticMesh (Variables|Default|Get15) (Variables|Default|GetMesh_15))
                                      (Components|InstancedStaticMesh|AddInstance (Variables|Default|Get15) (Math|Transform|MakeTransform (Math|Vector|MakeVector (.T_X (Utilities|Struct|BreakF_CSVdata _returnvalue_19)) (.T_Y (Utilities|Struct|BreakF_CSVdata _returnvalue_19)) (.T_Z (Utilities|Struct|BreakF_CSVdata _returnvalue_19))) (Math|Rotator|MakeRotator (.R_X (Utilities|Struct|BreakF_CSVdata _returnvalue_19)) (.R_Y (Utilities|Struct|BreakF_CSVdata _returnvalue_19)) (.R_Z (Utilities|Struct|BreakF_CSVdata _returnvalue_19))) (Math|Vector|MakeVector (.S_X (Utilities|Struct|BreakF_CSVdata _returnvalue_19)) (.S_Y (Utilities|Struct|BreakF_CSVdata _returnvalue_19)) (.S_Z (Utilities|Struct|BreakF_CSVdata _returnvalue_19)))) false)
                                      (elif (== (.ID (Utilities|Struct|BreakF_CSVdata _returnvalue_19)) 16)
                                        (Components|StaticMesh|SetStaticMesh (Variables|Default|Get16) (Variables|Default|GetMesh_16))
                                        (Components|InstancedStaticMesh|AddInstance (Variables|Default|Get16) (Math|Transform|MakeTransform (Math|Vector|MakeVector (.T_X (Utilities|Struct|BreakF_CSVdata _returnvalue_19)) (.T_Y (Utilities|Struct|BreakF_CSVdata _returnvalue_19)) (.T_Z (Utilities|Struct|BreakF_CSVdata _returnvalue_19))) (Math|Rotator|MakeRotator (.R_X (Utilities|Struct|BreakF_CSVdata _returnvalue_19)) (.R_Y (Utilities|Struct|BreakF_CSVdata _returnvalue_19)) (.R_Z (Utilities|Struct|BreakF_CSVdata _returnvalue_19))) (Math|Vector|MakeVector (.S_X (Utilities|Struct|BreakF_CSVdata _returnvalue_19)) (.S_Y (Utilities|Struct|BreakF_CSVdata _returnvalue_19)) (.S_Z (Utilities|Struct|BreakF_CSVdata _returnvalue_19)))) false)
                                        (elif (== (.ID (Utilities|Struct|BreakF_CSVdata _returnvalue_19)) 17)
                                          (Components|StaticMesh|SetStaticMesh (Variables|Default|Get17) (Variables|Default|GetMesh_17))
                                          (Components|InstancedStaticMesh|AddInstance (Variables|Default|Get17) (Math|Transform|MakeTransform (Math|Vector|MakeVector (.T_X (Utilities|Struct|BreakF_CSVdata _returnvalue_19)) (.T_Y (Utilities|Struct|BreakF_CSVdata _returnvalue_19)) (.T_Z (Utilities|Struct|BreakF_CSVdata _returnvalue_19))) (Math|Rotator|MakeRotator (.R_X (Utilities|Struct|BreakF_CSVdata _returnvalue_19)) (.R_Y (Utilities|Struct|BreakF_CSVdata _returnvalue_19)) (.R_Z (Utilities|Struct|BreakF_CSVdata _returnvalue_19))) (Math|Vector|MakeVector (.S_X (Utilities|Struct|BreakF_CSVdata _returnvalue_19)) (.S_Y (Utilities|Struct|BreakF_CSVdata _returnvalue_19)) (.S_Z (Utilities|Struct|BreakF_CSVdata _returnvalue_19)))) false))))))))))))))))))))))