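; Cloud Forge actor that renders a selectable VDB cloud as a heterogeneous volume, with tunable shading and noise-driven movement.
; The construction script sets up the viewport volume and applies billboard visibility plus console commands for indirect lighting and trace distance.
; BeginPlay applies the same setup to a separate render volume and hides the viewport one.
; Both feed a dynamic material the sparse volume texture, parameters and inverted directional light forward vector for self-shadowing.
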(event EventBeginPlay
  (Cloud_Forge|CloudForgeRender)
  (Rendering|SetVisibility (Variables|Default|GetHeterogeneousVolume_Viewport) false false))

(fn ConstructionScript
  (Cloud_Forge|CloudForgeViewport)
  (VDB_Settings|Settings))

(fn Settings
  (Utilities|FlowControl|Sequence
    (:then_0
      ;[1 0 0] Indirect Lighting
      (if (Variables|CloudSetup|GetbIndirect_Lighting)
        (Development|ExecuteConsoleCommand "r.HeterogeneousVolumes.IndirectLighting 1" 0)
        (else
          (Development|ExecuteConsoleCommand "r.HeterogeneousVolumes.IndirectLighting 0" 0))))
    (:then_1
      ;[1 0 0] Billboard
      (Rendering|SetVisibility (Variables|Default|GetBillboard) (Variables|CloudSetup|GetbBillboard_Visible) false))
    (:then_2
      ;[1 0 0] Trace Distance
      (if (Variables|CloudSetup|GetbSet_Trace_Distance)
        (Development|ExecuteConsoleCommand (Utilities|String|Append (Utilities|String|MakeLiteralString "r.HeterogeneousVolumes.MaxTraceDistance ") (Utilities|String|ToString(Float) (Variables|CloudSetup|GetTrace_Distance))) 0)
        (else
          (Development|ExecuteConsoleCommand "r.HeterogeneousVolumes.MaxTraceDistance 100000" 0))))))

(fn CloudForgeViewport
  (bind _sparse_texture (Variables|CloudSetup|GetSparse_Texture))
  (bind _vdb_array_selector (Variables|CloudSetup|GetVDB_Array_Selector))
  (bind _output (Utilities|Array|Get(acopy) _sparse_texture _vdb_array_selector))
  (Utilities|FlowControl|Sequence
    (:then_0
      ;[0 0.1291 1] Material
      (bind _returnvalue (Rendering|Material|CreateDynamicMaterialInstance (Variables|Default|GetHeterogeneousVolume_Viewport) 0 (Variables|Components|GetSource_Material) "None" :!class /Script/Engine.PrimitiveComponent))
      (Variables|Components|SetCF_MID _returnvalue))
    (:then_1
      ;[0 1 0.9975] VDB Texture
      (Variables|Performance|SetDisplay (Utilities|String|ToString(Text) (Utilities|Text|ToText(Object) _output)))
      (Class|MaterialInstanceDynamic|SetSparseVolumeTextureParameterValue (Variables|Components|GetCF_MID) "VDB_Texture" _output))
    (:then_2
      ;[0 1 0.03871] Material
      (Rendering|Material|SetScalarParameterValue (Variables|Components|GetCF_MID) "Density_Multiplier" (Variables|Color&Density|GetDensity_Multiplier) :!class /Script/Engine.MaterialInstanceDynamic)
      (Rendering|Material|SetVectorParameterValue (Variables|Components|GetCF_MID) "Scattering_Color" (Variables|Color&Density|GetScattering_Color) :!class /Script/Engine.MaterialInstanceDynamic)
      (Rendering|Material|SetScalarParameterValue (Variables|Components|GetCF_MID) "Remap_InputHigh" (Variables|Color&Density|GetRemap_InputHigh) :!class /Script/Engine.MaterialInstanceDynamic)
      (Rendering|Material|SetScalarParameterValue (Variables|Components|GetCF_MID) "Remap_InputLow" (Variables|Color&Density|GetRemap_InputLow) :!class /Script/Engine.MaterialInstanceDynamic)
      (Rendering|Material|SetScalarParameterValue (Variables|Components|GetCF_MID) "Remap_TargetHigh" (Variables|Color&Density|GetRemap_TargetHigh) :!class /Script/Engine.MaterialInstanceDynamic)
      (Rendering|Material|SetScalarParameterValue (Variables|Components|GetCF_MID) "Remap_TargetLow" (Variables|Color&Density|GetRemap_TargetLow) :!class /Script/Engine.MaterialInstanceDynamic)
      (Rendering|Material|SetScalarParameterValue (Variables|Components|GetCF_MID) "Cloud_Self_Shadow" (Variables|DirectionalShadow|GetCloud_Self_Shadow) :!class /Script/Engine.MaterialInstanceDynamic)
      (Rendering|Material|SetScalarParameterValue (Variables|Components|GetCF_MID) "Desaturation" (Variables|Color&Density|GetDesaturation) :!class /Script/Engine.MaterialInstanceDynamic)
      (Rendering|Material|SetVectorParameterValue (Variables|Components|GetCF_MID) "Sub Scattering Control" (Variables|Color&Density|GetSub%20Scattering%20Control) :!class /Script/Engine.MaterialInstanceDynamic)
      (Rendering|Material|SetScalarParameterValue (Variables|Components|GetCF_MID) "Invert_Shadow?" (Math|Conversions|ToFloat(Boolean) (Variables|DirectionalShadow|GetbInvert_Self_Shadow_Direction)) :!class /Script/Engine.MaterialInstanceDynamic)
      (if (Variables|DirectionalShadow|GetbRefresh)
        _
        (else
          _))
      (Rendering|Material|SetVectorParameterValue (Variables|Components|GetCF_MID) "Directional_Light" (Math|Conversions|ToLinearColor(Vector) (* (Math|Rotator|GetRotationXVector (Transformation|GetActorRotation (Variables|DirectionalShadow|GetDirectional_Light))) "-1.000000,-1.000000,-1.000000")) :!class /Script/Engine.MaterialInstanceDynamic))
    (:then_3
      ;[1 0.9128 0] Animation
      (Rendering|Material|SetScalarParameterValue (Variables|Components|GetCF_MID) "Cloud_Movement?" (Math|Conversions|ToFloat(Boolean) (Variables|Animation|GetbCloud_Movement)) :!class /Script/Engine.MaterialInstanceDynamic)
      (Rendering|Material|SetScalarParameterValue (Variables|Components|GetCF_MID) "Large_Noise_Scale" (Variables|Animation|GetLarge_Noise_Scale) :!class /Script/Engine.MaterialInstanceDynamic)
      (Rendering|Material|SetScalarParameterValue (Variables|Components|GetCF_MID) "Small_Noise_Scale" (Variables|Animation|GetSmall_Noise_Scale) :!class /Script/Engine.MaterialInstanceDynamic)
      (Rendering|Material|SetVectorParameterValue (Variables|Components|GetCF_MID) "NoisePan" (Variables|Animation|GetCloud_Flow_Direction) :!class /Script/Engine.MaterialInstanceDynamic))))

(fn CloudForgeRender
  (bind _sparse_texture (Variables|CloudSetup|GetSparse_Texture))
  (bind _vdb_array_selector (Variables|CloudSetup|GetVDB_Array_Selector))
  (bind _output (Utilities|Array|Get(acopy) _sparse_texture _vdb_array_selector))
  (Utilities|FlowControl|Sequence
    (:then_0
      ;[0 0.1291 1] Material
      (bind _returnvalue (Rendering|Material|CreateDynamicMaterialInstance (Variables|Default|GetHeterogeneousVolume_Render) 0 (Variables|Components|GetSource_Material) "None" :!class /Script/Engine.PrimitiveComponent))
      (Variables|Components|SetCF_MID _returnvalue))
    (:then_1
      ;[0 1 0.9975] VDB Texture
      (Variables|Performance|SetDisplay (Utilities|String|ToString(Text) (Utilities|Text|ToText(Object) _output)))
      (Class|MaterialInstanceDynamic|SetSparseVolumeTextureParameterValue (Variables|Components|GetCF_MID) "VDB_Texture" _output))
    (:then_2
      ;[0 1 0.03871] Material
      (Rendering|Material|SetScalarParameterValue (Variables|Components|GetCF_MID) "Density_Multiplier" (Variables|Color&Density|GetDensity_Multiplier) :!class /Script/Engine.MaterialInstanceDynamic)
      (Rendering|Material|SetVectorParameterValue (Variables|Components|GetCF_MID) "Scattering_Color" (Variables|Color&Density|GetScattering_Color) :!class /Script/Engine.MaterialInstanceDynamic)
      (Rendering|Material|SetScalarParameterValue (Variables|Components|GetCF_MID) "Remap_InputHigh" (Variables|Color&Density|GetRemap_InputHigh) :!class /Script/Engine.MaterialInstanceDynamic)
      (Rendering|Material|SetScalarParameterValue (Variables|Components|GetCF_MID) "Remap_InputLow" (Variables|Color&Density|GetRemap_InputLow) :!class /Script/Engine.MaterialInstanceDynamic)
      (Rendering|Material|SetScalarParameterValue (Variables|Components|GetCF_MID) "Remap_TargetHigh" (Variables|Color&Density|GetRemap_TargetHigh) :!class /Script/Engine.MaterialInstanceDynamic)
      (Rendering|Material|SetScalarParameterValue (Variables|Components|GetCF_MID) "Remap_TargetLow" (Variables|Color&Density|GetRemap_TargetLow) :!class /Script/Engine.MaterialInstanceDynamic)
      (Rendering|Material|SetScalarParameterValue (Variables|Components|GetCF_MID) "Cloud_Self_Shadow" (Variables|DirectionalShadow|GetCloud_Self_Shadow) :!class /Script/Engine.MaterialInstanceDynamic)
      (Rendering|Material|SetScalarParameterValue (Variables|Components|GetCF_MID) "Desaturation" (Variables|Color&Density|GetDesaturation) :!class /Script/Engine.MaterialInstanceDynamic)
      (Rendering|Material|SetVectorParameterValue (Variables|Components|GetCF_MID) "Sub Scattering Control" (Variables|Color&Density|GetSub%20Scattering%20Control) :!class /Script/Engine.MaterialInstanceDynamic)
      (Rendering|Material|SetScalarParameterValue (Variables|Components|GetCF_MID) "Invert_Shadow?" (Math|Conversions|ToFloat(Boolean) (Variables|DirectionalShadow|GetbInvert_Self_Shadow_Direction)) :!class /Script/Engine.MaterialInstanceDynamic)
      (if (Variables|DirectionalShadow|GetbRefresh)
        _
        (else
          _))
      (Rendering|Material|SetVectorParameterValue (Variables|Components|GetCF_MID) "Directional_Light" (Math|Conversions|ToLinearColor(Vector) (* (Math|Rotator|GetRotationXVector (Transformation|GetActorRotation (Variables|DirectionalShadow|GetDirectional_Light))) "-1.000000,-1.000000,-1.000000")) :!class /Script/Engine.MaterialInstanceDynamic))
    (:then_3
      ;[1 0.9128 0] Animation
      (Rendering|Material|SetScalarParameterValue (Variables|Components|GetCF_MID) "Cloud_Movement?" (Math|Conversions|ToFloat(Boolean) (Variables|Animation|GetbCloud_Movement)) :!class /Script/Engine.MaterialInstanceDynamic)
      (Rendering|Material|SetScalarParameterValue (Variables|Components|GetCF_MID) "Large_Noise_Scale" (Variables|Animation|GetLarge_Noise_Scale) :!class /Script/Engine.MaterialInstanceDynamic)
      (Rendering|Material|SetScalarParameterValue (Variables|Components|GetCF_MID) "Small_Noise_Scale" (Variables|Animation|GetSmall_Noise_Scale) :!class /Script/Engine.MaterialInstanceDynamic)
      (Rendering|Material|SetVectorParameterValue (Variables|Components|GetCF_MID) "NoisePan" (Variables|Animation|GetCloud_Flow_Direction) :!class /Script/Engine.MaterialInstanceDynamic))))