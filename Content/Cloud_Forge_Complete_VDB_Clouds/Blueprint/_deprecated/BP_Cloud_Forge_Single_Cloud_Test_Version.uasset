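; Deprecated test Blueprint for a single VDB cloud, rendered through a Heterogeneous Volume component.
; The Construction Script and BeginPlay both run VDB_Material_Functions, which adds the component at runtime or construction with a dynamic instance of MI_VDB_Cloud_Single.
; That function feeds the sparse volume texture and exposed density, color, remap, shadow, noise and movement variables into the material.
; A separate Apply VDB Settings function, uncalled here, toggles indirect lighting and trace distance via console commands.
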(event EventBeginPlay
  ;[0.7465 0.159 1] Ref custom event
  (VDBSettings|VDBMaterialFunctions))

(fn ConstructionScript
  ;[1 1 1] Ref Custom Event
  (VDBSettings|VDBMaterialFunctions))

(fn ApplyVDBSettings
  ;[1 1 1] Cloud_Quality
  (Utilities|FlowControl|Sequence
    (:then_0
      (if (Variables|Default|GetIndirect_Lighting?)
        (Development|ExecuteConsoleCommand "r.HeterogeneousVolumes.IndirectLighting 1" 0)
        (else
          (Development|ExecuteConsoleCommand "r.HeterogeneousVolumes.IndirectLighting 0" 0))))
    (:then_1
      (if (Variables|Default|GetInfinite_Trace?)
        (Development|ExecuteConsoleCommand "r.HeterogeneousVolumes.MaxTraceDistance 100000000" 0)
        (else
          (Development|ExecuteConsoleCommand "r.HeterogeneousVolumes.MaxTraceDistance 1" 0))))))

(fn VDBMaterialFunctions
  (bind _returnvalue (AddComponent|AddHeterogeneousVolumeComponent false))
  ;[1 1 1] Cloud_Material_Setup
  (bind _returnvalue_2 (Rendering|Material|CreateDynamicMaterialInstance _returnvalue 0 "/Game/Cloud_Forge_Complete_VDB_Clouds/Materials/VDB_Single_Material/MI_VDB_Cloud_Single.MI_VDB_Cloud_Single" "" :!class /Script/Engine.PrimitiveComponent))
  (Class|MaterialInstanceDynamic|SetSparseVolumeTextureParameterValue _returnvalue_2 "VDB_Texture" (Variables|Default|GetVDB_Texture))
  (Rendering|Material|SetScalarParameterValueonMaterials _returnvalue "Density_Multiplier" (Variables|Default|GetDensity_Multiplier))
  (Rendering|Material|SetVectorParameterValueonMaterials _returnvalue "Scattering_Color" (Math|Conversions|ToVector(LinearColor) (Variables|Default|GetScattering_Color)))
  (Class|MaterialInstanceDynamic|SetSparseVolumeTextureParameterValue _returnvalue_2 "VDB_Texture" (Variables|Default|GetVDB_Texture))
  (Rendering|Material|SetScalarParameterValueonMaterials _returnvalue "Remap_InputHigh" (Variables|Default|GetRemap_InputHigh))
  (Rendering|Material|SetScalarParameterValueonMaterials _returnvalue "Remap_InputLow" (Variables|Default|GetRemap_InputLow))
  (Rendering|Material|SetScalarParameterValueonMaterials _returnvalue "Remap_TargetHigh" (Variables|Default|GetRemap_TargetHigh))
  (Rendering|Material|SetScalarParameterValueonMaterials _returnvalue "Remap_TargetLow" (Variables|Default|GetRemap_TargetLow))
  (Rendering|Material|SetScalarParameterValueonMaterials _returnvalue "Cloud_Self_Shadow" (Variables|Default|GetCloud_Self_Shadow))
  (Rendering|Material|SetScalarParameterValueonMaterials _returnvalue "Desaturation" (Variables|Default|GetDesaturation))
  (Rendering|Material|SetVectorParameterValueonMaterials _returnvalue "Sub Scattering Control" (Math|Conversions|ToVector(LinearColor) (Variables|Default|GetSub%20Scattering%20Control)))
  (Rendering|Material|SetScalarParameterValueonMaterials _returnvalue "Large_Noise_Scale" (Variables|Default|GetLarge_Noise_Scale))
  (Rendering|Material|SetScalarParameterValueonMaterials _returnvalue "Small_Noise_Scale" (Variables|Default|GetSmall_Noise_Scale))
  (Rendering|Material|SetVectorParameterValueonMaterials _returnvalue "NoisePan" (Math|Conversions|ToVector(LinearColor) (Variables|Default|GetCloud_Flow_Direction)))
  (if (Variables|Default|GetCloud_Movement?)
    (Rendering|Material|SetScalarParameterValueonMaterials _returnvalue "Cloud_Movement?" (Variables|Default|GetCloud_Movement_ON))
    (else
      (Rendering|Material|SetScalarParameterValueonMaterials _returnvalue "Cloud_Movement?" (Variables|Default|GetCloud_Movement_OFF)))))